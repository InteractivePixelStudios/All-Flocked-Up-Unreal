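; BP_HumanThrower is a human thrower AI that detects the player and shows an alert when the pigeon character comes near.
; PawnSensing sets the CanSeePlayer blackboard key for BT_HumanThrower, currently testing against DefaultPawn as a placeholder for the pigeon, with debug prints.
; Separately, a sphere overlap with BP_PigeonCharacter_AB spawns a notification object just above the actor, plays a 2D sound and destroys the object after a short delay.
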(event OnSeePawn(PawnSensing)
  (params (Pawn :type Pawn%20Object%20Reference))
  ;[1 1 1] Sets CanSeePlayer to true for use in BT_HumanThrower
  ;;[1 0.1771 0.1771 1 20] CHANGE THIS TO THE PIGEON CONTROLLER
  (Utilities|Casting|CastToDefaultPawn Pawn
    (:then
      ;;[1 0.8632 0.2462] DEBUG - Showing Results
      (Development|PrintString "I see you.")
      (AI|Components|Blackboard|SetValueasBool (AI|GetBlackboard (AI|GetAIController (Components|GetOwner))) (Utilities|Name|MakeLiteralName "CanSeePlayer") true))
    (:CastFailed
      (Development|PrintString "I don't even know who you are."))))

(event OnComponentBeginOverlap(Sphere1)
  (params (OverlappedComponent :type Primitive%20Component%20Object%20Reference) (OtherActor :type Actor%20Object%20Reference) (OtherComp :type Primitive%20Component%20Object%20Reference) (OtherBodyIndex :type Integer) (bFromSweep :type Boolean) (SweepResult :type Hit%20Result%20Structure%20%28by%20ref%29))
  (bind _returnvalue (Transformation|GetActorTransform))
  (Utilities|Casting|CastToBP_PigeonCharacter_AB OtherActor)
  (bind _returnvalue_2 (Game|SpawnActorfromClass "/Game/Dev-Directory/Personal-Folders/Wesley/BluePrints_WK/BP_AlertNotificationObject_WK.BP_AlertNotificationObject_WK_C" (Math|Transform|MakeTransform (+ (.location _returnvalue) "0.000000,0.000000,10.000000") (.rotation _returnvalue) (.scale _returnvalue)) "Undefined" "MultiplyWithRoot" 0 0))
  (Audio|PlaySound2D "/Game/Dev-Directory/Personal-Folders/Alex/AlexTestLevel/funny-sound-effect-for-quotjack-in-the-boxquot-sound-ver1-110923.funny-sound-effect-for-quotjack-in-the-boxquot-sound-ver1-110923" 1.0 1.0 0.0 0 0)
  (Utilities|FlowControl|Delay 1.0)
  (Actor|DestroyActor _returnvalue_2))

(fn ConstructionScript)