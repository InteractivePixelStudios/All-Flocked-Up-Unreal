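; Poop meter Blueprint that tracks a current and maximum poop value, starting full on BeginPlay.
; RestorePoop and LosePoop change the current value by fixed amounts, clamped between zero and max.
; IncreaseMaxPoop raises the base max and current value, recomputing max from base plus primary and secondary accessory bonuses.
; AddAccessoryBonus sets either bonus slot, then also applies a fixed IncreaseMaxPoop; the meter functions print debug text.
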(event EventBeginPlay
  ;[1 1 1] At start, set Current poop to Max poop
  (Variables|Default|SetPoopCurrent (Variables|Default|GetPoopMax)))

(event EventTick
  (params (DeltaSeconds :type Float%20%28single-precision%29)))

(fn RestorePoop
  ;[1 1 1] Get Poop restored and add it to current Poop, making sure it doesnt go above Max Poop, and set the value to Current Poop
  (Variables|Default|SetPoopCurrent (Math|Integer|Clamp(Integer) (+ 4 (Variables|Default|GetPoopCurrent)) 0 (Variables|Default|GetPoopMax))) ; Set new Current poop
  ;[1 0.7157 0.04971] Debug
  (Development|PrintText "Poop restored by ")
  (Development|PrintText (Utilities|Text|ToText(Integer) (Math|Integer|Clamp(Integer) (+ 4 (Variables|Default|GetPoopCurrent)) 0 (Variables|Default|GetPoopMax)))))

(fn LosePoop
  ;[1 1 1] Decreases the poop value and makes sure it doesnt go below 0, and set the value to Current poop
  (Variables|Default|SetPoopCurrent (Math|Integer|Clamp(Integer) (- (Variables|Default|GetPoopCurrent) 2) 0 (Variables|Default|GetPoopMax))) ; Set new Current poop
  ;[1 0.7157 0.04971] Debug
  (Development|PrintText "Poop meter lost by ")
  (Development|PrintText (Utilities|Text|ToText(Integer) (Math|Integer|Clamp(Integer) (- (Variables|Default|GetPoopCurrent) 2) 0 (Variables|Default|GetPoopMax))))
  (Development|PrintText "total poop left")
  (Development|PrintText (Utilities|Text|ToText(Integer) (Variables|Default|GetPoopCurrent))))

(fn IncreaseMaxPoop
  (params (MaxPoopIncrease :type Integer))
  ;[1 1 1] When called, increases max poop by the input value and restores that same value to current poop
  (bind _output_get (Variables|Default|SetPoopMaxBase (+ (Variables|Default|GetPoopMaxBase) MaxPoopIncrease)))
  (bind _output_get_2 (Variables|Default|SetPoopMax (+ (+ (Variables|Default|GetPrimaryAccessoryBonus) (Variables|Default|GetSecondaryAccessoryBonus)) _output_get))) ; Set Max Poop to new value
  (Variables|Default|SetPoopCurrent (+ (Variables|Default|GetPoopCurrent) MaxPoopIncrease)) ; set new value to Current Poop
  ;[1 0.7157 0.04971] Debug
  (Development|PrintText "Max Poop increased by ")
  (Development|PrintText (Utilities|Text|ToText(Integer) _output_get_2)))

(fn AddAccessoryBonus
  (params (NewAccesory%20Bonus :type Integer) (IsPrimary :type Boolean))
  (if IsPrimary
    (Variables|Default|SetPrimaryAccessoryBonus NewAccesory%20Bonus)
    (else
      (Variables|Default|SetSecondaryAccessoryBonus NewAccesory%20Bonus)))
  (CallFunction|IncreaseMaxPoop 2))