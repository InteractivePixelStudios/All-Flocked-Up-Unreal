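; Trash can interactable that the pigeon player rummages through once until it is reset after resting at the nest.
; Overlap prints a rummage or wait prompt, and Pickup teleports the player to the can, opens the garbage widget, flags it used and hides the pigeon.
; The widget calls TrashControls to clear the Chamber flag, which Tick polls to update the pigeon's InMenu state and unhide it.
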(event EventTick
  (params (DeltaSeconds :type Float%20%28single-precision%29))
  (if (not (Variables|Default|GetChamber))
    (Utilities|Casting|CastToBP_PigeonCharacter_AB (stale Collision|EventActorBeginOverlap OtherActor))
    ;[0.05613 0.2664 1] helps control, when the player is done with the garbage they come back to the game.
    (if (Variables|Default|GetControllable)
      (Variables|/Game/Dev-Directory/Personal-Folders/Alex/AlexTestLevel/PlayerCharacter/BP_PigeonCharacter_AB.BP_PigeonCharacter_AB_C|SetInMenu (stale Collision|EventActorBeginOverlap _asbp_pigeon_character_ab) (Variables|Default|GetIn%20Menu))
      (if (not false)
        (Variables|Default|SetControllable false)
        (Rendering|SetActorHiddenInGame (stale Collision|EventActorBeginOverlap _asbp_pigeon_character_ab) false)))))

(event Collision|EventActorBeginOverlap
  (params (OtherActor :type Actor%20Object%20Reference))
  ;[1 1 1] Checks to see if the player is overlapping for input message
  (bind _asbp_pigeon_character_ab (Utilities|Casting|CastToBP_PigeonCharacter_AB OtherActor))
  (if (Variables|Default|GetUsed)
    (Development|PrintText "Please wait before you can rummage")
    (else
      (Development|PrintText "Press \"E\" to Rummage through garbage!"))))

(event EventPickup
  ;[1 1 1] teleporting the player to the garbage-can
  (if (not (Variables|Default|GetUsed))
    (Transformation|Teleport (Game|GetPlayerCharacter 0) (Transformation|GetActorLocation) "0, 0, 0")
    ;[1 1 1] Creates pop-up for garbage
    (bind _returnvalue (UserInterface|CreateWidget "/Game/Dev-Directory/Personal-Folders/Jayden/BPW_Garbage_Pick-up.BPW_Garbage_Pick-up_C" (Game|GetPlayerController 0)))
    (bind _output_get (Variables|Default|SetGarbage_widget _returnvalue))
    (UserInterface|Viewport|AddtoViewport _output_get 0)
    ;[0.05613 0.2664 1] Sets the garbage can to be in use and takes away player control. it also hides the player at the moment
    (Variables|Default|SetUsed true)
    (bind _asbp_pigeon_character_ab (Utilities|Casting|CastToBP_PigeonCharacter_AB (stale Collision|EventActorBeginOverlap OtherActor)))
    (Variables|/Game/Dev-Directory/Personal-Folders/Alex/AlexTestLevel/PlayerCharacter/BP_PigeonCharacter_AB.BP_PigeonCharacter_AB_C|SetInMenu _asbp_pigeon_character_ab (Variables|Default|GetIn%20Menu))
    (Variables|Default|SetChamber true)
    (Rendering|SetActorHiddenInGame (stale Collision|EventActorBeginOverlap _asbp_pigeon_character_ab) true)
    (Variables|Default|SetControllable true)))

(fn ConstructionScript)

(fn ResetTrash-Can
  ;[0.05613 0.2664 1] Is called to reset the trash can after resting at nest
  (Variables|Default|SetUsed false))

(fn TrashControls
  ;[0.05613 0.2664 1] Gets called from garbage widget. this is used to help decide if its time to give back controls
  (Variables|Default|SetChamber false))