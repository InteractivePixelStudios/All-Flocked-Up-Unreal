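; Day/night cycle Blueprint that rotates sun and moon directional lights on a 24-unit timer and shows the current phase on the player HUD.
; Once the HUD reference is valid, Tick advances the timer by delta seconds over TimeDilation, pitching the lights 180 degrees apart.
; The timer's upper half counts as day, with its own dilation, HUD text and color.
; SkipTime jumps the timer to the next preset point.
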(event Custom|AdjustForDay
  ;[1 0.02697 0] To adjust the duration of day or night: divide 24 by your desired time in minutes to get the dilation in seconds. Then, multiply the result by 100 to convert it into minutes for accurate timing.
  ;
  ; Example: For 16 min day and 8 min night, the Time Dilation for day would be '150', and for night, '75'.
  ;
  ; 24 / 16 * 100 = 150
  ; 24 / 8 * 100 = 75
  (Variables|Default|SetTimeDilation 1.5))

(event Custom|AdjustForNight
  ;[1 0.02697 0] To adjust the duration of day or night: divide 24 by your desired time in minutes to get the dilation in seconds. Then, multiply the result by 100 to convert it into minutes for accurate timing.
  ;
  ; Example: For 16 min day and 8 min night, the Time Dilation for day would be '150', and for night, '75'.
  ;
  ; 24 / 16 * 100 = 150
  ; 24 / 8 * 100 = 75
  (Variables|Default|SetTimeDilation 0.75))

(event Custom|CheckTime
  (bind _hud_ref (Variables|Default|GetHud%20Ref))
  (bind _daynight (Variables|/Game/Dev-Directory/Personal-Folders/Isaiah/PlayerHUD_Widget.PlayerHUD_Widget_C|GetDayNight _hud_ref))
  ;[1 1 1] Temp solution to inform the player if it's day or night, if they don't have eyes I guess.
  ;;[1 0 0.651] Checks if the timer is Great or Equal to 12 (Day time)
  (if (>= (Variables|Default|GetTimer) 12.0)
    (CallFunction|AdjustforDay)
    ;;[0.2627 0.5529 1] If TRUE, set's the Text to Day and changes the colour to Yellow.
    ;;
    ;; If FALSE, set's the Text to Night and changes the coloiur to Blue.
    (Appearance|SetColorandOpacity _daynight (Utilities|Struct|MakeSlateColor "(R=1.000000,G=0.820144,B=0.055351,A=1.000000)" "UseColor_Specified") :!class /Script/UMG.TextBlock)
    (Variables|/Script/UMG.TextBlock|SetText _daynight "Day")
    (else
      (CallFunction|AdjustforNight)
      (Appearance|SetColorandOpacity _daynight (Utilities|Struct|MakeSlateColor "(R=0.000000,G=0.059855,B=1.000000,A=1.000000)" "UseColor_Specified") :!class /Script/UMG.TextBlock)
      (Variables|/Script/UMG.TextBlock|SetText _daynight "Night"))))

(event Custom|SkipTime
  (if (< (Variables|Default|GetTimer) 12.0)
    (Variables|Default|SetTimer 12.0)
    (elif (< (Variables|Default|GetTimer) 18.0)
      (Variables|Default|SetTimer 18.0)
      (elif (< (Variables|Default|GetTimer) 22.0)
        (Variables|Default|SetTimer 22.0)
        (else
          (Variables|Default|SetTimer 0.1))))))

(event EventTick
  (params (DeltaSeconds :type Float%20%28single-precision%29))
  ;[1 1 1] Main
  ;;[0.2627 0.5529 1] Check if the HUD Ref is not NULL then set Delta Seconds Var = Delta Seconds.
  (if (Utilities|IsValid (Variables|Default|GetHud%20Ref))
    (bind _output_get (Variables|Default|SetDelta%20Seconds DeltaSeconds))
    ;;[1 0 0.651] Adjust Day/Night Text
    (CallFunction|CheckTime)
    ;;[0.2627 1 0.251] Gets Delta Seconds, then divides it by the current Time Dilation, then add's current Timer back into Timer (This is how we pass time)
    (bind _output_get_2 (Variables|Default|SetTimer (+ (/ _output_get (Variables|Default|GetTimeDilation)) (Variables|Default|GetTimer))))
    ;;[1 1 1] Sqquence to run multiple Branches
    (Utilities|FlowControl|Sequence
      (:then_0
        ;;[0.2627 0.5529 1] If Timer is Greater or Equal to 24, reset the day, and set day to FALSE.
        (if (>= _output_get_2 24.0)
          (Variables|Default|SetTimer 0.0)
          (Variables|Default|SetIsDay false)
          (else
            ;;[0.2627 1 0.251] Set the Relative Rotation of the sun.
            (Transformation|SetRelativeRotation (Variables|Default|GetDirectionalLight_Sun) (Math|Rotator|MakeRotator 0.0 (* (/ (Variables|Default|GetTimer) 24.0) 3.6e+02) 0.0) false false)
            ;;[0.2627 1 0.251] Set the Relative Rotation of the moon - 180 degrees so it's in the opposite position of the sun.
            (Transformation|SetRelativeRotation (Variables|Default|GetDirectionalLight_Moon) (Math|Rotator|MakeRotator 0.0 (+ (* (/ (Variables|Default|GetTimer) 24.0) 3.6e+02) 1.8e+02) 0.0) false false))))
      (:then_1
        ;;[0.2627 0.5529 1] If Timer is Great or Equal to 12, set Day to TRUE.
        (if (>= _output_get_2 12.0)
          (Variables|Default|SetIsDay true))))))

(event EventBeginPlay
  ;[1 1 1] Getting Reference to the Player HUD
  (Utilities|FlowControl|Delay 0.2)
  (bind _foundwidgets (Widget|GetAllWidgetsOfClass "/Game/Dev-Directory/Personal-Folders/Isaiah/PlayerHUD_Widget.PlayerHUD_Widget_C" true))
  (Variables|Default|SetHud%20Ref (Utilities|Array|Get(acopy) _foundwidgets)))

(fn ConstructionScript)