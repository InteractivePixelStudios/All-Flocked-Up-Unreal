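; Player audio profile Blueprint that feeds wing flap sounds into a MetaSound player.
; One second after BeginPlay, it passes three wing flap sounds from its data asset to the MSPlayer as the FlapAudioArray parameter.
; A delayed Flap trigger chain exists but is not connected to any event, and Tick is empty.
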(event EventBeginPlay
  (bind _dataasset (Variables|Default|GetDataAsset))
  (Utilities|FlowControl|Delay 1.0)
  (Audio|Parameter|SetObjectArrayParameter (Variables|Default|GetMS_Player) "FlapAudioArray" (Utilities|Array|MakeArray (Variables|/Game/Dev-Directory/Personal-Folders/Isaiah/Audio/Blueprints/BP_DA/BP_VA_Player.BP_VA_Player_C|GetWingFlap1 _dataasset) (Variables|/Game/Dev-Directory/Personal-Folders/Isaiah/Audio/Blueprints/BP_DA/BP_VA_Player.BP_VA_Player_C|GetWingFlap2 _dataasset) (Variables|/Game/Dev-Directory/Personal-Folders/Isaiah/Audio/Blueprints/BP_DA/BP_VA_Player.BP_VA_Player_C|GetWingFlap3 _dataasset))))

(event EventTick
  (params (DeltaSeconds :type Float%20%28single-precision%29)))

(fn ConstructionScript)