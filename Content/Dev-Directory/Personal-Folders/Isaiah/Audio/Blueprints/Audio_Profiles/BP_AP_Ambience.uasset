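; BP_AP_Ambience is an audio profile Blueprint that plays an ambience sound from a DataAsset.
; On BeginPlay it caches the level's first AudioWizard, waits briefly, then injects the DataAsset's wave into the MSAmbience MetaSound through a wave parameter.
; It plays the MetaSound if that wave is valid, otherwise printing a warning.
; Every Tick, it sets the volume from the AudioWizard's ambience and master volumes multiplied together.
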(event Custom|AdjustVolume
  (bind _audiowizard (Variables|Default|GetAudioWizard))
  (Audio|Components|Audio|SetVolumeMultiplier (Variables|Default|GetMS_Ambience) (* (Variables|/Game/Dev-Directory/Personal-Folders/Isaiah/Audio/Blueprints/AudioWizard.AudioWizard_C|GetAmbienceVolume _audiowizard) (Variables|/Game/Dev-Directory/Personal-Folders/Isaiah/Audio/Blueprints/AudioWizard.AudioWizard_C|GetMasterVolume _audiowizard)) :!class /Script/Engine.AudioComponent))

(event EventBeginPlay
  (bind _dataasset (Variables|Default|GetDataAsset))
  (bind _ms_ambience (Variables|Default|GetMS_Ambience))
  (bind _ambience1 (Variables|/Game/Dev-Directory/Personal-Folders/Isaiah/Audio/Blueprints/BP_DA/BP_VA_Ambience.BP_VA_Ambience_C|GetAmbience1 _dataasset))
  (bind _outactors (Actor|GetAllActorsOfClass "/Game/Dev-Directory/Personal-Folders/Isaiah/Audio/Blueprints/AudioWizard.AudioWizard_C"))
  (bind _asaudio_wizard (Utilities|Casting|CastToAudioWizard (Utilities|Array|Get(acopy) _outactors)))
  (Variables|Default|SetAudioWizard _asaudio_wizard)
  (Utilities|FlowControl|Delay 0.1)
  ;[1 1 1] Inject desired audio into the MetaSound from the DataAsset
  (Class|AudioComponent|SetWaveParameter _ms_ambience "A1" _ambience1)
  (if (Utilities|IsValid _ambience1)
    (Audio|Components|Audio|Play _ms_ambience 0.0)
    (else
      (Development|PrintString "No Audio Found in BP_AP_Ambience" true true "(R=1.000000,G=0.084660,B=0.000000,A=1.000000)"))))

(event EventTick
  (params (DeltaSeconds :type Float%20%28single-precision%29))
  (CallFunction|AdjustVolume))

(fn ConstructionScript)