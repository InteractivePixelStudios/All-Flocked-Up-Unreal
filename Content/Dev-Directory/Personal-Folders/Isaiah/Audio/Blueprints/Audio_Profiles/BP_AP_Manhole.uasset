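; Manhole audio profile actor that plays a looping steam hiss and fires a burst when the pigeon character overlaps it.
; BeginPlay caches the level's AudioWizard and feeds hiss and burst waves from a data asset into SteamHiss parameters.
; Tick restarts SteamHiss whenever it stops, and overlap sends it a "Push" trigger with a debug print.
; AdjustAudio, not called here, scales volume by the wizard's manhole and master levels.
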(event Custom|AdjustAudio
  (bind _audiowizard (Variables|Default|GetAudioWizard))
  (Audio|Components|Audio|SetVolumeMultiplier (Variables|Default|GetSteamHiss) (* (Variables|/Game/Dev-Directory/Personal-Folders/Isaiah/Audio/Blueprints/AudioWizard.AudioWizard_C|GetManholeVolume _audiowizard) (Variables|/Game/Dev-Directory/Personal-Folders/Isaiah/Audio/Blueprints/AudioWizard.AudioWizard_C|GetMasterVolume _audiowizard)) :!class /Script/Engine.AudioComponent))

(event Custom|CheckIfPlaying
  (bind _steamhiss (Variables|Default|GetSteamHiss))
  (if (not (Audio|Components|Audio|IsPlaying _steamhiss))
    (Audio|Components|Audio|Play _steamhiss 0.0)))

(event EventBeginPlay
  (bind _steamhiss (Variables|Default|GetSteamHiss))
  (bind _dataasset (Variables|Default|GetDataAsset))
  (bind _outactors (Actor|GetAllActorsOfClass 0))
  (bind _asaudio_wizard (Utilities|Casting|CastToAudioWizard (Utilities|Array|Get(acopy) _outactors)))
  (Variables|Default|SetAudioWizard _asaudio_wizard)
  (Class|AudioComponent|SetWaveParameter _steamhiss "ManholeHiss" (Variables|/Game/Dev-Directory/Personal-Folders/Isaiah/Audio/Blueprints/BP_DA/BP_VA_Environment.BP_VA_Environment_C|GetManhole%20Steam _dataasset))
  (Class|AudioComponent|SetWaveParameter _steamhiss "ManholePush" (Variables|/Game/Dev-Directory/Personal-Folders/Isaiah/Audio/Blueprints/BP_DA/BP_VA_Environment.BP_VA_Environment_C|GetManhole%20Burst _dataasset)))

(event Collision|EventActorBeginOverlap
  (params (OtherActor :type Actor%20Object%20Reference))
  (Utilities|Casting|CastToBP_PigeonCharacter_AB OtherActor)
  (Class|AudioParameterControllerInterface|SetTriggerParameter (Variables|Default|GetSteamHiss) "Push")
  (Development|PrintString "Push Sound Maybe?"))

(event EventTick
  (params (DeltaSeconds :type Float%20%28single-precision%29))
  (CallFunction|CheckifPlaying))

(fn ConstructionScript)