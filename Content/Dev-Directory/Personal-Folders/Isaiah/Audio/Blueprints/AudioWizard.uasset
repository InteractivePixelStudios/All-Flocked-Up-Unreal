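; AudioWizard is a Blueprint that sets up world ambience and AI car audio when play begins.
; It spawns an actor configured with the DA_Ambience data asset at its root location.
; It then finds every existing BP_AICarEnemy and snap-attaches a spawned BP_AP_Car audio actor to each, printing debug messages.
; The search runs only once, so cars spawned later receive no audio from it.
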(event EventBeginPlay
  (Game|SpawnActorfromClass "/Game/Dev-Directory/Personal-Folders/Isaiah/Audio/Blueprints/Audio_Profiles/BP_AP_Ambience.BP_AP_Ambience_C" (Math|Conversions|ToTransform(Vector) (Transformation|GetWorldLocation (Variables|Default|GetDefaultSceneRoot))) "Undefined" "MultiplyWithRoot" 0 "/Game/Dev-Directory/Personal-Folders/Isaiah/Audio/DataAssets/DA_Ambience.DA_Ambience" 0)
  (bind _outactors (Actor|GetAllActorsOfClass "/Game/Dev-Directory/Personal-Folders/Alex/AlexTestLevel/TrafficSystem/BP_AICarEnemy.BP_AICarEnemy_C"))
  (for _array_element _outactors
    (bind _returnvalue (Game|SpawnActorfromClass "/Game/Dev-Directory/Personal-Folders/Isaiah/Audio/Blueprints/Audio_Profiles/BP_AP_Car.BP_AP_Car_C" (Transformation|GetActorTransform _array_element) "AlwaysSpawn" "MultiplyWithRoot" 0 0))
    (Transformation|AttachActorToActor _returnvalue _array_element "None" "SnapToTarget" "SnapToTarget" "SnapToTarget" true)
    (Development|PrintString "I WAS SPAWNED AND ATTACHED TO A CAR" true true "(R=1.000000,G=0.000000,B=0.037496,A=1.000000)" 5.0))
  (Development|PrintString "All Cars Now Have Audio" true true "(R=1.000000,G=0.000000,B=0.037496,A=1.000000)" 5.0))

(fn ConstructionScript)