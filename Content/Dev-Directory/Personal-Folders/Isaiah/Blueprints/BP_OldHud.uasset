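; BP_OldHud is a HUD helper Blueprint in a developer folder, left largely disconnected.
; GetExtras calls two events that search for BP_DayNightCycle and BP_NewHud actors, but neither stores the result.
; Unreachable leftover logic would cache those references, toggle the map with a MapArrow shown while open, and skip or advance the day-night timer.
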(event Custom|Get24HourCycle
  ;[1 1 1] Get Extras
  (bind _outactors (Actor|GetAllActorsOfClass "/Game/Dev-Directory/Personal-Folders/Isaiah/Day-Night-Cycle/BP_DayNightCycle.BP_DayNightCycle_C")))

(event Custom|GetHUDWidget
  ;[1 1 1] Get Extras
  (bind _outactors (Actor|GetAllActorsOfClass "/Game/Dev-Directory/Personal-Folders/Isaiah/Blueprints/BP_NewHud.BP_NewHud_C")))

(event Custom|GetExtras
  ;[1 1 1] Get Extras
  (CallFunction|Get24HourCycle)
  (CallFunction|GetHUDWidget))

(event Input|KeyboardEvents|M
  (params (Key :type Key%20Structure :default "None")))

(event Input|KeyboardEvents|L
  (params (Key :type Key%20Structure :default "None")))

(event Input|KeyboardEvents|K
  (params (Key :type Key%20Structure :default "None")))

(fn ConstructionScript)