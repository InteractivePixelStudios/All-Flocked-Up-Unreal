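; Actor component that tracks the player's gameplay stats in a single PlayerStats struct, covering pickups, pooping, enemies evaded, missions and race times.
; Setter functions rebuild the struct to add to counters, append unique mission names or store race times by race name.
; SetLoadedStats and GetAllStats exchange the whole struct for saved data, and GetPlayerAccuracy derives a rounded poop hit percentage without a zero-division guard.
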(event EventBeginPlay)

(event EventTick
  (params (DeltaSeconds :type Float%20%28single-precision%29)))

(fn SetLoadedStats
  (params (SavedStats :type S%20Player%20Stats%20Structure))
  (Variables|Default|SetPlayerStats SavedStats))

(fn GetAllStats
  (return (Variables|Default|GetPlayerStats)))

(fn SetSeedsCollected
  (params (Seeds :type Integer))
  (Variables|Default|SetPlayerStats (Utilities|Struct|MakeS_PlayerStats (+ (.seedscollected (Variables|Default|GetPlayerStats)) Seeds) (.trinketscollected (Variables|Default|GetPlayerStats)) (.itemscollected (Variables|Default|GetPlayerStats)) (.consumableseaten (Variables|Default|GetPlayerStats)) (.timespooped (Variables|Default|GetPlayerStats)) (.enemiespoopedon (Variables|Default|GetPlayerStats)) (.enemiesevaded (Variables|Default|GetPlayerStats)) (.missionscompleted (Variables|Default|GetPlayerStats)) (.racetimes (Variables|Default|GetPlayerStats)))))

(fn IncrementTrinketsCollected
  (params (TrinketsGained :type Integer))
  (Variables|Default|SetPlayerStats (Utilities|Struct|MakeS_PlayerStats (.seedscollected (Variables|Default|GetPlayerStats)) (+ (.trinketscollected (Variables|Default|GetPlayerStats)) TrinketsGained) (.itemscollected (Variables|Default|GetPlayerStats)) (.consumableseaten (Variables|Default|GetPlayerStats)) (.timespooped (Variables|Default|GetPlayerStats)) (.enemiespoopedon (Variables|Default|GetPlayerStats)) (.enemiesevaded (Variables|Default|GetPlayerStats)) (.missionscompleted (Variables|Default|GetPlayerStats)) (.racetimes (Variables|Default|GetPlayerStats)))))

(fn IncrementItemsCollected
  (bind _result (Math|Integer|IncrementInt (.itemscollected (Variables|Default|GetPlayerStats)))
    (:%20%20
      (Variables|Default|SetPlayerStats (Utilities|Struct|MakeS_PlayerStats (.seedscollected (Variables|Default|GetPlayerStats)) (.trinketscollected (Variables|Default|GetPlayerStats)) _result (.consumableseaten (Variables|Default|GetPlayerStats)) (.timespooped (Variables|Default|GetPlayerStats)) (.enemiespoopedon (Variables|Default|GetPlayerStats)) (.enemiesevaded (Variables|Default|GetPlayerStats)) (.missionscompleted (Variables|Default|GetPlayerStats)) (.racetimes (Variables|Default|GetPlayerStats)))))))

(fn IncrementConsumablesEaten
  (bind _result (Math|Integer|IncrementInt (.consumableseaten (Variables|Default|GetPlayerStats)))
    (:%20%20
      (Variables|Default|SetPlayerStats (Utilities|Struct|MakeS_PlayerStats (.seedscollected (Variables|Default|GetPlayerStats)) (.trinketscollected (Variables|Default|GetPlayerStats)) (.itemscollected (Variables|Default|GetPlayerStats)) _result (.timespooped (Variables|Default|GetPlayerStats)) (.enemiespoopedon (Variables|Default|GetPlayerStats)) (.enemiesevaded (Variables|Default|GetPlayerStats)) (.missionscompleted (Variables|Default|GetPlayerStats)) (.racetimes (Variables|Default|GetPlayerStats)))))))

(fn IncrementTimesPooped
  (bind _result (Math|Integer|IncrementInt (.timespooped (Variables|Default|GetPlayerStats)))
    (:%20%20
      (Variables|Default|SetPlayerStats (Utilities|Struct|MakeS_PlayerStats (.seedscollected (Variables|Default|GetPlayerStats)) (.trinketscollected (Variables|Default|GetPlayerStats)) (.itemscollected (Variables|Default|GetPlayerStats)) (.consumableseaten (Variables|Default|GetPlayerStats)) _result (.enemiespoopedon (Variables|Default|GetPlayerStats)) (.enemiesevaded (Variables|Default|GetPlayerStats)) (.missionscompleted (Variables|Default|GetPlayerStats)) (.racetimes (Variables|Default|GetPlayerStats)))))))

(fn IncrementEnemiesPoopedon
  (bind _result (Math|Integer|IncrementInt (.enemiespoopedon (Variables|Default|GetPlayerStats)))
    (:%20%20
      (Variables|Default|SetPlayerStats (Utilities|Struct|MakeS_PlayerStats (.seedscollected (Variables|Default|GetPlayerStats)) (.trinketscollected (Variables|Default|GetPlayerStats)) (.itemscollected (Variables|Default|GetPlayerStats)) (.consumableseaten (Variables|Default|GetPlayerStats)) (.timespooped (Variables|Default|GetPlayerStats)) _result (.enemiesevaded (Variables|Default|GetPlayerStats)) (.missionscompleted (Variables|Default|GetPlayerStats)) (.racetimes (Variables|Default|GetPlayerStats)))))))

(fn IncrementEnemiesEvaded
  (bind _result (Math|Integer|IncrementInt (.enemiesevaded (Variables|Default|GetPlayerStats)))
    (:%20%20
      (Variables|Default|SetPlayerStats (Utilities|Struct|MakeS_PlayerStats (.seedscollected (Variables|Default|GetPlayerStats)) (.trinketscollected (Variables|Default|GetPlayerStats)) (.itemscollected (Variables|Default|GetPlayerStats)) (.consumableseaten (Variables|Default|GetPlayerStats)) (.timespooped (Variables|Default|GetPlayerStats)) (.enemiespoopedon (Variables|Default|GetPlayerStats)) _result (.missionscompleted (Variables|Default|GetPlayerStats)) (.racetimes (Variables|Default|GetPlayerStats)))))))

(fn AddCompletedMission
  (params (MissionName :type String))
  (Utilities|Array|AddUnique (.missionscompleted (Variables|Default|GetPlayerStats)) MissionName)
  (Variables|Default|SetPlayerStats (Utilities|Struct|MakeS_PlayerStats (.seedscollected (Variables|Default|GetPlayerStats)) (.trinketscollected (Variables|Default|GetPlayerStats)) (.itemscollected (Variables|Default|GetPlayerStats)) (.consumableseaten (Variables|Default|GetPlayerStats)) (.timespooped (Variables|Default|GetPlayerStats)) (.enemiespoopedon (Variables|Default|GetPlayerStats)) (.enemiesevaded (Variables|Default|GetPlayerStats)) (.missionscompleted (Variables|Default|GetPlayerStats)) (.racetimes (Variables|Default|GetPlayerStats)))))

(fn AddRaceTime
  (params (RaceName :type String) (RaceTime :type Float%20%28double-precision%29))
  (Utilities|Map|Add (.racetimes (Variables|Default|GetPlayerStats)) RaceName RaceTime)
  (Variables|Default|SetPlayerStats (Utilities|Struct|MakeS_PlayerStats (.seedscollected (Variables|Default|GetPlayerStats)) (.trinketscollected (Variables|Default|GetPlayerStats)) (.itemscollected (Variables|Default|GetPlayerStats)) (.consumableseaten (Variables|Default|GetPlayerStats)) (.timespooped (Variables|Default|GetPlayerStats)) (.enemiespoopedon (Variables|Default|GetPlayerStats)) (.enemiesevaded (Variables|Default|GetPlayerStats)) (.missionscompleted (Variables|Default|GetPlayerStats)) (.racetimes (Variables|Default|GetPlayerStats)))))

(fn GetPlayerAccuracy
  (bind _playerstats (Variables|Default|GetPlayerStats))
  (return (Math|Float|Round (* (/ (Math|Conversions|ToFloat(Integer) (.enemiespoopedon _playerstats)) (Math|Conversions|ToFloat(Integer) (.timespooped _playerstats))) 1e+02))))