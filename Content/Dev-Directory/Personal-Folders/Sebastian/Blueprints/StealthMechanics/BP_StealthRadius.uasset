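; BP_StealthRadius is a sphere-collision actor that follows an owner and serves as either a detector or detectable radius for stealth mechanics.
; A setup function assigns owner, radius and detector role, and the radius can be resized later.
; When a detector overlaps a non-detector radius, it calls DetectUser or LostUser on its owner's AC_StealthDetector, passing the other radius's owner.
; Tick copies the owner's transform and draws a debug sphere.
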(event OnComponentBeginOverlap(StealthRadius)
  (params (OverlappedComponent :type Primitive%20Component%20Object%20Reference) (OtherActor :type Actor%20Object%20Reference) (OtherComp :type Primitive%20Component%20Object%20Reference) (OtherBodyIndex :type Integer) (bFromSweep :type Boolean) (SweepResult :type Hit%20Result%20Structure%20%28by%20ref%29))
  ;[0.1059 0.1059 0.1059 0.7216] Checks if stealth detector
  (if (Variables|Default|GetDetector)
    ;[0.1059 0.1059 0.1059 0.7216] Check that target is not a fellow detector
    (bind _asbp_stealth_radius (Utilities|Casting|CastToBP_StealthRadius OtherActor))
    (if (not (Variables|BP_StealthRadius_C|GetDetector _asbp_stealth_radius))
      ;[0.1059 0.1059 0.1059 0.7216] Get owners stealth detector and detect user
      (Default|DetectUser (Actor|GetComponentbyClass (Variables|Default|GetOwnerRef) "/Game/Dev-Directory/Personal-Folders/Sebastian/Blueprints/StealthMechanics/AC_StealthDetector.AC_StealthDetector_C") (Variables|BP_StealthRadius_C|GetOwnerRef _asbp_stealth_radius)))))

(event OnComponentEndOverlap(StealthRadius)
  (params (OverlappedComponent :type Primitive%20Component%20Object%20Reference) (OtherActor :type Actor%20Object%20Reference) (OtherComp :type Primitive%20Component%20Object%20Reference) (OtherBodyIndex :type Integer))
  ;[0.1059 0.1059 0.1059 0.7216] Checks if stealth detector
  (if (Variables|Default|GetDetector)
    ;[0.1059 0.1059 0.1059 0.7216] Check that target is not a fellow detector
    (bind _asbp_stealth_radius (Utilities|Casting|CastToBP_StealthRadius OtherActor))
    (if (not (Variables|BP_StealthRadius_C|GetDetector _asbp_stealth_radius))
      ;[0.1059 0.1059 0.1059 0.7216] Get owners stealth detector and lose the user
      (Default|LostUser (Actor|GetComponentbyClass (Variables|Default|GetOwnerRef) "/Game/Dev-Directory/Personal-Folders/Sebastian/Blueprints/StealthMechanics/AC_StealthDetector.AC_StealthDetector_C") (Variables|BP_StealthRadius_C|GetOwnerRef _asbp_stealth_radius)))))

(event EventTick
  (params (DeltaSeconds :type Float%20%28single-precision%29))
  (bind _ownerref (Variables|Default|GetOwnerRef))
  ;[0.1059 0.1059 0.1059 0.7216] Stealth Radius tracks owner
  (Transformation|SetActorTransform self (Transformation|GetActorTransform _ownerref))
  ;[1 0.8632 0.2462] Debug visuals
  (Rendering|Debug|DrawDebugSphere (Transformation|GetActorLocation _ownerref) (Variables|Default|GetRadiusSize) 12 "(R=0.500000,G=0.000000,B=0.210997,A=1.000000)" 0.0))

(fn ConstructionScript)

(fn SetupStealthOwner
  (params (Owner :type Actor%20Object%20Reference) (Radius :type Float%20%28double-precision%29) (IsDetector :type Boolean))
  ;[0.2623 0.552 1] Set Variables and collider sphere radius
  (Variables|Default|SetOwnerRef Owner)
  (bind _output_get (Variables|Default|SetRadiusSize Radius))
  (Variables|Default|SetDetector IsDetector)
  (Components|Sphere|SetSphereRadius (Variables|Default|GetStealthRadius) _output_get true))

(fn ChangeRadius
  (params (New%20Radius :type Float%20%28double-precision%29))
  ;[0.2623 0.552 1] Changes the radius of the collider sphere
  (bind _output_get (Variables|Default|SetRadiusSize New%20Radius))
  (Components|Sphere|SetSphereRadius (Variables|Default|GetStealthRadius) _output_get true))