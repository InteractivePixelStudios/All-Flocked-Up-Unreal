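; BP_BreadConsume is a bread consumable that restores health to the pigeon that consumes it.
; It implements the ConsumableEffect event, writing directly to HealthCurrent on the passed pigeon's BPHealthSystemWK component.
; The event adds a tenth of HealthMax twice in succession, a fifth in total, with no clamp to the maximum in this graph.
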(event EventBeginPlay
  (|CallParentFunction) ; This node is disabled and will not be called.\nDrag off pins to build functionality.
)

(event Collision|EventActorBeginOverlap
  (params (OtherActor :type Actor%20Object%20Reference))
  (|CallParentFunction OtherActor) ; This node is disabled and will not be called.\nDrag off pins to build functionality.
)

(event EventTick
  (params (DeltaSeconds :type Float%20%28single-precision%29))
  (|CallParentFunction DeltaSeconds) ; This node is disabled and will not be called.\nDrag off pins to build functionality.
)

(event EventConsumableEffect
  (params (PigeonRef :type BP%20Pigeon%20Character%20AB%20Object%20Reference%20%28by%20ref%29))
  (bind _bp_healthsystem_wk (Variables|/Game/Dev-Directory/Personal-Folders/Alex/AlexTestLevel/PlayerCharacter/BP_PigeonCharacter_AB.BP_PigeonCharacter_AB_C|GetBP_HealthSystem_WK PigeonRef))
  (bind _bp_healthsystem_wk_2 (Variables|/Game/Dev-Directory/Personal-Folders/Alex/AlexTestLevel/PlayerCharacter/BP_PigeonCharacter_AB.BP_PigeonCharacter_AB_C|GetBP_HealthSystem_WK PigeonRef))
  (Variables|/Game/Dev-Directory/Personal-Folders/Wesley/BluePrints_WK/BP_HealthSystem_WK.BP_HealthSystem_WK_C|SetHealthCurrent _bp_healthsystem_wk (+ (Variables|/Game/Dev-Directory/Personal-Folders/Wesley/BluePrints_WK/BP_HealthSystem_WK.BP_HealthSystem_WK_C|GetHealthCurrent _bp_healthsystem_wk) (/ (Variables|/Game/Dev-Directory/Personal-Folders/Wesley/BluePrints_WK/BP_HealthSystem_WK.BP_HealthSystem_WK_C|GetHealthMax _bp_healthsystem_wk) 10)))
  (Variables|/Game/Dev-Directory/Personal-Folders/Wesley/BluePrints_WK/BP_HealthSystem_WK.BP_HealthSystem_WK_C|SetHealthCurrent _bp_healthsystem_wk_2 (+ (Variables|/Game/Dev-Directory/Personal-Folders/Wesley/BluePrints_WK/BP_HealthSystem_WK.BP_HealthSystem_WK_C|GetHealthCurrent _bp_healthsystem_wk_2) (/ (Variables|/Game/Dev-Directory/Personal-Folders/Wesley/BluePrints_WK/BP_HealthSystem_WK.BP_HealthSystem_WK_C|GetHealthMax _bp_healthsystem_wk_2) 10))))

(fn ConstructionScript
  (|CallParentFunction))