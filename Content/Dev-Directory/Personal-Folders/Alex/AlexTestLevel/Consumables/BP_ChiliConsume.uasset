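; BP_ChiliConsume is a chili consumable that refills the pigeon player's poop resource when its effect fires.
; Its ConsumableEffect event finds the BP_PigeonCharacter_AB via GetActorOfClass, adds a fixed amount to PoopCurrent on its poop system component, and prints the new total.
; The logic applies no clamp, and the default BeginPlay, overlap and Tick events are unused.
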(event EventBeginPlay
  (|CallParentFunction) ; This node is disabled and will not be called.\nDrag off pins to build functionality.
)

(event Collision|EventActorBeginOverlap
  (params (OtherActor :type Actor%20Object%20Reference))
  (|CallParentFunction OtherActor) ; This node is disabled and will not be called.\nDrag off pins to build functionality.
)

(event EventTick
  (params (DeltaSeconds :type Float%20%28single-precision%29))
  (|CallParentFunction DeltaSeconds) ; This node is disabled and will not be called.\nDrag off pins to build functionality.
)

(event EventConsumableEffect
  (bind _returnvalue (Actor|GetActorOfClass "/Game/Dev-Directory/Personal-Folders/Alex/AlexTestLevel/PlayerCharacter/BP_PigeonCharacter_AB.BP_PigeonCharacter_AB_C"))
  (bind _output_get (Variables|/Game/Dev-Directory/Personal-Folders/Jayden/BP_PoopSystem_WK.BP_PoopSystem_WK_C|SetPoopCurrent (Variables|/Game/Dev-Directory/Personal-Folders/Alex/AlexTestLevel/PlayerCharacter/BP_PigeonCharacter_AB.BP_PigeonCharacter_AB_C|GetBP_PoopSystem_WK _returnvalue) (+ (Variables|/Game/Dev-Directory/Personal-Folders/Jayden/BP_PoopSystem_WK.BP_PoopSystem_WK_C|GetPoopCurrent (Variables|/Game/Dev-Directory/Personal-Folders/Alex/AlexTestLevel/PlayerCharacter/BP_PigeonCharacter_AB.BP_PigeonCharacter_AB_C|GetBP_PoopSystem_WK _returnvalue)) 10)))
  (Development|PrintString (Utilities|String|ToString(Integer) _output_get)))

(fn ConstructionScript
  (|CallParentFunction))