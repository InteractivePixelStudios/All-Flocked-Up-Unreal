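; AI enemy car prototype, built on character movement, that seeks out traffic paths.
; On BeginPlay it finds the closest BP_TrafficPath spline, issuing a move-to toward each closer candidate during the search.
; Each tick disables orient-to-movement and calls a steering function, whose yaw-based value is computed only under DebugSteering, alongside debug drawing, and never applied.
; Hits are reported as AI touch events.
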(event EventBeginPlay
  (bind _outactors (Actor|GetAllActorsOfClass "/Game/Dev-Directory/Personal-Folders/Alex/AlexTestLevel/TrafficSystem/BP_TrafficPath.BP_TrafficPath_C"))
  (bind _returnedspline (CallFunction|FindNearestSpline _outactors))
  (Variables|Default|SetDefaultSpline _returnedspline)
  (Variables|Default|SetReturned%20Spline (Variables|Default|GetDefaultSpline))
  (Variables|Default|SetDefaultMaxSpeed (Variables|Default|GetMaxSpeed)))

(event Collision|EventHit
  (params (MyComp :type Primitive%20Component%20Object%20Reference) (Other :type Actor%20Object%20Reference) (OtherComp :type Primitive%20Component%20Object%20Reference) (bSelfMoved :type Boolean) (HitLocation :type Vector :default "0, 0, 0") (HitNormal :type Vector :default "0, 0, 0") (NormalImpulse :type Vector :default "0, 0, 0") (Hit :type Hit%20Result%20Structure%20%28by%20ref%29))
  (Class|AISenseTouch|ReportTouchEvent self Other HitLocation))

(event EventTick
  (params (DeltaSeconds :type Float%20%28single-precision%29))
  (Utilities|IsValid (Variables|Default|GetReturned%20Spline)
    (:Is%20Valid
      (Utilities|FlowControl|Sequence
        (:then_0
          (CallFunction|CalculateSteeringInput (Variables|Default|GetReturned%20Spline))
          (Variables|/Script/Engine.CharacterMovementComponent|SetbOrientRotationToMovement (Variables|Character|GetCharacterMovement) false))))))

(fn ConstructionScript)

(fn FindNearestSpline
  (params (SplineActors :type Array%20of%20BP%20Traffic%20Path%20Object%20References))
  (bind _returnvalue (Transformation|GetActorLocation))
  (LocalVariables|SetDistance 0.0)
  (for (_array_element _array_index) SplineActors
    (if (== _array_index 0)
      (LocalVariables|SetDistance (Math|Vector|Distance(Vector) (Spline|FindLocationClosesttoWorldLocation (Variables|/Game/Dev-Directory/Personal-Folders/Alex/AlexTestLevel/TrafficSystem/BP_TrafficPath.BP_TrafficPath_C|GetSpline _array_element) _returnvalue "World") _returnvalue) :!label _label)
      (bind _output_get (LocalVariables|SetNearestSpline _array_element))
      (AI|Navigation|SimpleMovetoActor 0 _output_get)
      (elif (< (Math|Vector|Distance(Vector) (Spline|FindLocationClosesttoWorldLocation (Variables|/Game/Dev-Directory/Personal-Folders/Alex/AlexTestLevel/TrafficSystem/BP_TrafficPath.BP_TrafficPath_C|GetSpline _array_element) _returnvalue "World") _returnvalue) (LocalVariables|GetDistance))
        (goto _label))))
  (return (LocalVariables|GetNearestSpline)))

(fn CalculateSteeringInput
  (params (Spline :type BP%20Traffic%20Path%20Object%20Reference))
  (bind _returnvalue (Transformation|GetActorLocation))
  (bind _returnvalue_2 (Transformation|GetActorLocation))
  (bind _returnvalue_3 (Transformation|GetActorRotation))
  (bind _returnvalue_4 (+ _returnvalue ""))
  (bind _returnvalue_5 (Spline|FindLocationClosesttoWorldLocation (Variables|/Game/Dev-Directory/Personal-Folders/Alex/AlexTestLevel/TrafficSystem/BP_TrafficPath.BP_TrafficPath_C|GetSpline Spline) _returnvalue_4 "Local"))
  (bind _returnvalue_6 (Math|Rotator|FindLookatRotation _returnvalue_2 _returnvalue_5))
  (bind _returnvalue_7 (Math|Rotator|Delta(Rotator) _returnvalue_6 _returnvalue_3))
  (bind _output_get (Variables|Default|SetOffsetTangentLocation _returnvalue_5))
  (if (Variables|Default|GetDebugSteering)
    (Rendering|Debug|DrawDebugSphere _output_get 25.0 12 "(R=1.000000,G=0.015401,B=0.000000,A=1.000000)" 0.0 1.0)
    (Rendering|Debug|DrawDebugArrow _returnvalue_2 _output_get 1.0 "(R=1.000000,G=0.000000,B=0.015653,A=1.000000)" 0.0 1e+01)
    (Variables|Default|SetYawDelta (.yaw _returnvalue_7))
    (return (Math|Float|MapRangeClamped (.yaw _returnvalue_7) -15.0 15.0 -1.0 1.0))))