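; BP_SaveGame stores quest and player state for saving and loading.
; Active and completed quest lists are copied from the quest log, while each quest's stage and objective progress go into a map keyed by quest ID.
; Loading re-adds active quests and restores their progress from that map, but not the completed list.
; Player position loading applies a saved transform and control rotation; its save function is an empty stub.
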(fn SaveQuestDetails
  (params (Quest :type BP%20Quests%20Base%20Object%20Reference))
  (Utilities|Map|Add (Variables|Default|GetquestProgress) (Variables|/Game/Dev-Directory/Personal-Folders/Alex/AlexTestLevel/QuestSystem/BP_QuestsBase.BP_QuestsBase_C|GetquestID Quest) (Utilities|Struct|MakeS_PlayerSave "0.000000,0.000000,0.000000|0.000000,0.000000,0.000000|1.000000,1.000000,1.000000" 0.0 "0.000000,0.000000,0.000000" (Variables|/Game/Dev-Directory/Personal-Folders/Alex/AlexTestLevel/QuestSystem/BP_QuestsBase.BP_QuestsBase_C|GetcurrentObjectiveProgress Quest) (Variables|/Game/Dev-Directory/Personal-Folders/Alex/AlexTestLevel/QuestSystem/BP_QuestsBase.BP_QuestsBase_C|GetcurrentStage Quest))))

(fn LoadQuests
  (params (Quest%20Log%20Component :type AC%20Quest%20Log%20Object%20Reference))
  (for _array_element (Variables|Default|GetcurrentActiveQuests)
    (bind _returnvalue (Default|AddNewQuest Quest%20Log%20Component _array_element))
    (Variables|/Game/Dev-Directory/Personal-Folders/Alex/AlexTestLevel/QuestSystem/BP_QuestsBase.BP_QuestsBase_C|SetcurrentStage _returnvalue (.CurrentQuestStage (Utilities|Struct|BreakS_PlayerSave (.Value (Utilities|Map|Find (Variables|Default|GetquestProgress) _array_element)))))
    (Variables|/Game/Dev-Directory/Personal-Folders/Alex/AlexTestLevel/QuestSystem/BP_QuestsBase.BP_QuestsBase_C|SetcurrentObjectiveProgress _returnvalue (.QuestProgress (Utilities|Struct|BreakS_PlayerSave (.Value (Utilities|Map|Find (Variables|Default|GetquestProgress) _array_element)))))))

(fn SaveQuestLog
  (params (QuestLog :type AC%20Quest%20Log%20Object%20Reference))
  (Variables|Default|SetcurrentActiveQuests (Variables|/Game/Dev-Directory/Personal-Folders/Alex/AlexTestLevel/QuestSystem/AC_QuestLog.AC_QuestLog_C|GetcurrentActiveQuest QuestLog))
  (Variables|Default|SetcompletedQuests (Variables|/Game/Dev-Directory/Personal-Folders/Alex/AlexTestLevel/QuestSystem/AC_QuestLog.AC_QuestLog_C|GetcompletedQuests QuestLog)))

(fn LoadPlayerPos
  (params (NewParam :type S%20Player%20Save%20Structure))
  (bind (_transform _health _controlrotation) (Utilities|Struct|BreakS_PlayerSave NewParam))
  (bind _playerreference (Variables|Default|GetPlayerReference))
  (Transformation|SetActorTransform _playerreference _transform)
  (Transformation|SetActorRotation _playerreference _controlrotation))

(fn SavePlayerPos
  (params (Player%20Ref :type BP%20Pigeon%20Character%20AB%20Object%20Reference))
  (return))