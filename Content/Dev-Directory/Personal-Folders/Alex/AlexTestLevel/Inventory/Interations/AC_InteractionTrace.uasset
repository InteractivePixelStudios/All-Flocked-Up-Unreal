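; Actor component that lets the player focus and interact with BP_InterationArea objects in view.
; Each tick, a camera-forward line trace updates the focused area and toggles its focus, cancelling interaction when focus is lost.
; Interact input either fires immediately or runs a looping timer that fills the WB_E widget's progress for timed holds.
; Completion calls InteractOnServer, which sends an interface interact message to the area's parent actor.
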(event Custom|TryToInteract
  (params (In :type Boolean))
  (if In
    (if (Variables|Default|GetisTracing)
      (bind _output_get (Variables|Default|SetInteract%20Duration (Variables|/Game/Dev-Directory/Personal-Folders/Alex/AlexTestLevel/Inventory/Interations/BP_InterationArea.BP_InterationArea_C|GetInteractDuration (Variables|Default|GetFocusedTrace))))
      (if (> _output_get 0.0)
        (bind _ref (Class|BIInteration|GetInteractionWidgetRef(Message) (Actor|GetParentActor (Variables|Default|GetFocusedTrace))))
        (bind _aswb_e (Utilities|Casting|CastToWB_E (UserInterface|GetWidget _ref)))
        (Variables|Default|SetCurrentIntercationWidgetRef _aswb_e)
        (bind _returnvalue (Utilities|Time|SetTimerbyEvent (delegate Custom|UpdateInteractionProgress) (Variables|Default|GetUpdateInteractionInterval) true))
        (Variables|Default|SetInteractionTimer _returnvalue)
        (else
          (CallFunction|InteractonServer (Variables|Default|GetFocusedTrace)))))
    (else
      (CallFunction|StopInteraction))))

(event Custom|InteractOnServer
  (params (InteractionArea :type BP%20Interation%20Area%20Object%20Reference))
  (Class|BIInteration|InterfaceInteract(Message) (Actor|GetParentActor InteractionArea)))

(event Custom|UpdateInteractionProgress
  (bind _output_get (Variables|Default|SetInteractionProgress (+ (Variables|Default|GetInteractionProgress) (* (/ 1.0 (Variables|Default|GetInteract%20Duration)) (Variables|Default|GetUpdateInteractionInterval)))))
  (Default|SetPercent (Variables|Default|GetCurrentIntercationWidgetRef) _output_get)
  (if (>= (Variables|Default|GetInteractionProgress) 1.0)
    (CallFunction|StopInteraction)
    (CallFunction|InteractonServer (Variables|Default|GetFocusedTrace))))

(event EventTick
  (params (DeltaSeconds :type Float%20%28single-precision%29))
  (CallFunction|Trace))

(fn Trace
  (bind _returnvalue (Game|GetPlayerCameraManager 0))
  (bind _returnvalue_2 (Transformation|GetActorLocation _returnvalue))
  (bind (_outhit _returnvalue_3) (Collision|LineTraceByChannel _returnvalue_2 (+ _returnvalue_2 (* (Math|Vector|GetForwardVector (Transformation|GetActorRotation _returnvalue)) (Variables|Default|GetTraceLength))) "TraceTypeQuery1" false 0 "None"))
  (if _returnvalue_3
    (if (!= (Variables|Default|GetFocusedActor) (.HitActor (Collision|BreakHitResult _outhit)))
      (Variables|Default|SetFocusedActor (.HitActor (Collision|BreakHitResult _outhit)))
      (CallFunction|TraceInteractionArea (== (Utilities|GetClass (.HitActor (Collision|BreakHitResult _outhit))) "/Game/Dev-Directory/Personal-Folders/Alex/AlexTestLevel/Inventory/Interations/BP_InterationArea.BP_InterationArea_C")))
    (else
      (CallFunction|TraceInteractionArea false))))

(fn TraceInteractionArea
  (params (Trace :type Boolean))
  (if Trace
    (if (Variables|Default|GetisTracing)
      (Default|ToggleFocus (Variables|Default|GetFocusedTrace) false))
    (bind _asbp_interation_area (Utilities|Casting|CastToBP_InterationArea (Variables|Default|GetFocusedActor)))
    (bind _output_get (Variables|Default|SetFocusedTrace _asbp_interation_area))
    (Default|ToggleFocus _output_get true)
    (Variables|Default|SetisTracing true)
    (elif (Variables|Default|GetisTracing)
      (Variables|Default|SetisTracing false)
      (Default|ToggleFocus (Variables|Default|GetFocusedTrace) false)
      (Variables|Default|SetFocusedActor 0)
      (Variables|Default|SetFocusedTrace 0)
      (CallFunction|StopInteraction))))

(fn StopInteraction
  (if (> (Variables|Default|GetInteractionProgress) 0.0)
    (Utilities|Time|ClearandInvalidateTimerbyHandle (Variables|Default|GetInteractionTimer))
    (Default|SetPercent (Variables|Default|GetCurrentIntercationWidgetRef) 0.0)
    (Variables|Default|SetInteractionProgress 0.0)
    (Variables|Default|SetCurrentIntercationWidgetRef 0)))