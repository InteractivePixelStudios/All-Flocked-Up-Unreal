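; Inventory component for the player's pigeon character that picks up, stacks and drops items in a name-keyed map.
; IA_Pick sphere-traces from the pawn toward the camera's aim, storing and destroying any A_MasterPickUpItem hit.
; Removal functions respawn item actors: single drops use the aim trace, multiple drops probe around the player for unblocked spots.
; BeginPlay caches four merchant table items, but AddItemFromShop is an unfinished stub.
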(event Input|EnhancedActionEvents|EnhancedInputActionIA_Pick
  (params (ActionValue :type Boolean) (ElapsedSeconds :type Float%20%28double-precision%29) (TriggeredSeconds :type Float%20%28double-precision%29) (InputAction :type Input%20Action%20Object%20Reference :default "/Game/Dev-Directory/Personal-Folders/Alex/AlexTestLevel/EnhancedInput/IA_Pick.IA_Pick"))
  (bind _connectedactor (Variables|Default|GetConnectedActor))
  (bind _groundcamera (Variables|/Game/Dev-Directory/Personal-Folders/Alex/AlexTestLevel/PlayerCharacter/BP_PigeonCharacter_AB.BP_PigeonCharacter_AB_C|GetGroundCamera _connectedactor))
  (:Completed
    (bind (_outhit _returnvalue) (Collision|SphereTraceByChannel (Transformation|GetActorLocation (Game|Player|GetPlayerPawn 0)) (+ (+ (Transformation|GetWorldLocation _groundcamera) (* (Math|Vector|GetForwardVector _groundcamera) (+ (Variables|/Script/Engine.SpringArmComponent|GetTargetArmLength (Variables|/Game/Dev-Directory/Personal-Folders/Alex/AlexTestLevel/PlayerCharacter/BP_PigeonCharacter_AB.BP_PigeonCharacter_AB_C|GetGroundSpringArm _connectedactor)) 1.5e+02))) "0.000000,0.000000,35.000000") 15.0 "TraceTypeQuery1" false 0 "ForDuration"))
    (if _returnvalue
      (bind _added_ (CallFunction|TryAddItem (.HitActor (Collision|BreakHitResult _outhit))))
      (if _added_
        (Actor|DestroyActor (.HitActor (Collision|BreakHitResult _outhit)))))))

(event EventBeginPlay
  (bind _asbp_pigeon_character_ab (Utilities|Casting|CastToBP_PigeonCharacter_AB (Game|Player|GetPlayerPawn 0)))
  (Variables|Default|SetConnectedActor _asbp_pigeon_character_ab)
  (CallFunction|GetShopItems))

(fn TryAddItem
  (params (HitActor :type Actor%20Object%20Reference))
  (bind _asa_master_pick_up_item (Utilities|Casting|CastToA_MasterPickUpItem HitActor)
    (:then
      (bind _output_get (LocalVariables|SetCurrectItem (Default|GetItemData _asa_master_pick_up_item)))
      (if (CallFunction|IsItemAlreadyinInventory _output_get)
        (CallFunction|IncreaseItemAmount (LocalVariables|GetCurrectItem))
        (else
          (CallFunction|AddItemtoInventory (LocalVariables|GetCurrectItem))))
      (Development|PrintString (Utilities|String|Append (.Name (Utilities|Struct|BreakS_ItemData (LocalVariables|GetCurrectItem))) "Added"))
      (return true))
    (:CastFailed
      (LocalVariables|SetCurrectItem "")
      (return false))))

(fn IsItemAlreadyinInventory
  (params (Item :type S%20Item%20Data%20Structure))
  (return (Utilities|Map|Contains (Variables|Default|GetInventory) (.Name (Utilities|Struct|BreakS_ItemData Item)))))

(fn AddItemtoInventory
  (params (Item :type S%20Item%20Data%20Structure))
  (Utilities|Map|Add (Variables|Default|GetInventory) (.Name (Utilities|Struct|BreakS_ItemData Item)) Item))

(fn IncreaseItemAmount
  (params (Item :type S%20Item%20Data%20Structure))
  (LocalVariables|SetItemName (.Name (Utilities|Struct|BreakS_ItemData Item)))
  (bind _result (Math|Integer|IncrementInt (.Amount (Utilities|Struct|BreakS_ItemData (.Value (Utilities|Map|Find (Variables|Default|GetInventory) (LocalVariables|GetItemName))))))
    (:%20%20
      (bind _structout (Utilities|Struct|SetmembersinS_ItemData (.Value (Utilities|Map|Find (Variables|Default|GetInventory) (LocalVariables|GetItemName))) _result))
      (Utilities|Map|Add (Variables|Default|GetInventory) (LocalVariables|GetItemName) _structout))))

(fn RemoveSingleItem
  (params (Key :type String%20%28by%20ref%29))
  (bind _inventory (Variables|Default|GetInventory))
  (bind (_value _returnvalue) (Utilities|Map|Find _inventory Key))
  (bind _amount (Utilities|Struct|BreakS_ItemData _value))
  (if _returnvalue
    (if (> _amount 1)
      (bind _structout (Utilities|Struct|SetmembersinS_ItemData _value (- _amount 1)))
      (Utilities|Map|Add (Variables|Default|GetInventory) Key _structout)
      (bind _impactpoint (CallFunction|TracefromAbove))
      (CallFunction|SpawnItem (.ItemClass (Utilities|Struct|BreakS_ItemData _structout)) _impactpoint)
      (return false _structout)
      (else
        (bind _output_get (LocalVariables|SetDeletedItem _value))
        (Utilities|Map|Remove (Variables|Default|GetInventory) Key)
        (bind _impactpoint_2 (CallFunction|TracefromAbove))
        (CallFunction|SpawnItem (.ItemClass (Utilities|Struct|BreakS_ItemData _output_get)) _impactpoint_2)
        (return true "")))))

(fn TracefromAbove
  (bind _connectedactor (Variables|Default|GetConnectedActor))
  (bind _groundcamera (Variables|/Game/Dev-Directory/Personal-Folders/Alex/AlexTestLevel/PlayerCharacter/BP_PigeonCharacter_AB.BP_PigeonCharacter_AB_C|GetGroundCamera _connectedactor))
  (bind (_outhit _returnvalue) (Collision|SphereTraceByChannel (Transformation|GetActorLocation (Game|Player|GetPlayerPawn 0)) (+ (+ (Transformation|GetWorldLocation _groundcamera) (* (Math|Vector|GetForwardVector _groundcamera) (+ (Variables|/Script/Engine.SpringArmComponent|GetTargetArmLength (Variables|/Game/Dev-Directory/Personal-Folders/Alex/AlexTestLevel/PlayerCharacter/BP_PigeonCharacter_AB.BP_PigeonCharacter_AB_C|GetGroundSpringArm _connectedactor)) 1.5e+02))) "0.000000,0.000000,25.000000") 5.0 "TraceTypeQuery1" false 0 "ForDuration"))
  (if _returnvalue
    (return (.ImpactPoint (Collision|BreakHitResult _outhit)))
    (else
      (return (.TraceEnd (Collision|BreakHitResult _outhit))))))

(fn SpawnItem
  (params (Class :type Actor%20Class%20Reference) (Position :type Vector))
  (Game|SpawnActorfromClass Class (Math|Transform|MakeTransform (+ Position "0.000000,0.000000,50.000000")) "Undefined" "MultiplyWithRoot" 0 0))

(fn TraceAroundPlayer
  (bind (_start _end) (CallFunction|GetStartEndTrace (* (Transformation|GetActorForwardVector (Variables|Default|GetConnectedActor)) 1e+02)))
  (bind (_outhit _returnvalue) (Collision|SphereTraceByChannel (- _start "0.000000,0.000000,50.000000") (- _end "0.000000,0.000000,50.000000") 1e+01 "TraceTypeQuery1" false 0 "ForDuration"))
  (if _returnvalue
    (bind (_start_2 _end_2) (CallFunction|GetStartEndTrace (* (Transformation|GetActorRightVector (Variables|Default|GetConnectedActor)) 1e+02)))
    (bind (_outhit_2 _returnvalue_2) (Collision|SphereTraceByChannel (- _start_2 "0.000000,0.000000,50.000000") (- _end_2 "0.000000,0.000000,50.000000") 1e+01 "TraceTypeQuery1" false 0 "ForDuration"))
    (if _returnvalue_2
      (bind (_start_3 _end_3) (CallFunction|GetStartEndTrace (* (Transformation|GetActorRightVector (Variables|Default|GetConnectedActor)) -1e+02)))
      (bind (_outhit_3 _returnvalue_3) (Collision|SphereTraceByChannel (- _start_3 "0.000000,0.000000,50.000000") (- _end_3 "0.000000,0.000000,50.000000") 1e+01 "TraceTypeQuery1" false 0 "ForDuration"))
      (if _returnvalue_3
        (bind (_start_4 _end_4) (CallFunction|GetStartEndTrace (* (Transformation|GetActorForwardVector (Variables|Default|GetConnectedActor)) -1e+02)))
        (bind (_outhit_4 _returnvalue_4) (Collision|SphereTraceByChannel (- _start_4 "0.000000,0.000000,50.000000") (- _end_4 "0.000000,0.000000,50.000000") 1e+01 "TraceTypeQuery1" false 0 "ForDuration"))
        (if _returnvalue_4
          (return (.ImpactPoint (Collision|BreakHitResult _outhit_4)))
          (else
            (return (.TraceEnd (Collision|BreakHitResult _outhit_4)))))
        (else
          (return (.TraceEnd (Collision|BreakHitResult _outhit_3)))))
      (else
        (return (.TraceEnd (Collision|BreakHitResult _outhit_2)))))
    (else
      (return (.TraceEnd (Collision|BreakHitResult _outhit))))))

(fn RemoveItemAll
  (params (ItemName :type String))
  (bind _inventory (Variables|Default|GetInventory))
  (bind (_value _returnvalue) (Utilities|Map|Find _inventory ItemName))
  (bind _amount (Utilities|Struct|BreakS_ItemData _value))
  (if _returnvalue
    (LocalVariables|SetDeletedItem _value)
    (bind _output_get (LocalVariables|SetDropAmount _amount))
    (for _index (range 1 _output_get)
      (bind _structout (Utilities|Struct|SetmembersinS_ItemData (LocalVariables|GetDeletedItem) (- _amount 1)))
      (Utilities|Map|Add (Variables|Default|GetInventory) ItemName _structout)
      (bind _position (CallFunction|TraceAroundPlayer))
      (CallFunction|SpawnItem (.ItemClass (Utilities|Struct|BreakS_ItemData (LocalVariables|GetDeletedItem))) _position))
    (Utilities|Map|Remove (Variables|Default|GetInventory) ItemName)
    (return)))

(fn GetStartEndTrace
  (params (VectorDirection :type Vector))
  (bind _connectedactor (Variables|Default|GetConnectedActor))
  (bind _mesh (Variables|/Script/Engine.Character|GetMesh _connectedactor))
  (bind _returnvalue (Transformation|GetWorldLocation _mesh))
  (return (+ _returnvalue "0.000000,0.000000,100.000000") (+ (+ _returnvalue VectorDirection) "0.000000,0.000000,100.000000")))

(fn RemoveItembyAmount
  (params (Item :type String) (AmountToDrop :type Integer))
  (bind _inventory (Variables|Default|GetInventory))
  (bind _inventory_2 (Variables|Default|GetInventory))
  (bind (_value _returnvalue) (Utilities|Map|Find _inventory Item))
  (bind _value_2 (Utilities|Map|Find _inventory_2 Item))
  (if _returnvalue
    (LocalVariables|SetFoundItem _value)
    (for _index (range 0 (- AmountToDrop 1))
      (bind _structout (Utilities|Struct|SetmembersinS_ItemData (LocalVariables|GetFoundItem) (- (.Amount (Utilities|Struct|BreakS_ItemData _value)) 1)))
      (Utilities|Map|Add (Variables|Default|GetInventory) Item _structout)
      (bind _position (CallFunction|TraceAroundPlayer))
      (CallFunction|SpawnItem (.ItemClass (Utilities|Struct|BreakS_ItemData (LocalVariables|GetFoundItem))) _position))
    (if (== (.Amount (Utilities|Struct|BreakS_ItemData _value_2)) 0)
      (Utilities|Map|Remove (Variables|Default|GetInventory) Item)
      (return "")
      (else
        (return _value_2)))))

(fn AddItemfromShop
  (for _array_element (Variables|Default|GetShopItemArray)
    _))

(fn GetShopItems
  (bind _returnvalue (Actor|GetActorOfClass "/Game/Dev-Directory/Personal-Folders/Alex/AlexTestLevel/InteractWithMerchant/EdgarAllanCrow/BP_MerchantTable.BP_MerchantTable_C"))
  (Variables|Default|SetShopItemArray (Utilities|Array|MakeArray (Variables|/Game/Dev-Directory/Personal-Folders/Alex/AlexTestLevel/InteractWithMerchant/EdgarAllanCrow/BP_MerchantTable.BP_MerchantTable_C|GetItem1 _returnvalue) (Variables|/Game/Dev-Directory/Personal-Folders/Alex/AlexTestLevel/InteractWithMerchant/EdgarAllanCrow/BP_MerchantTable.BP_MerchantTable_C|GetItem2 _returnvalue) (Variables|/Game/Dev-Directory/Personal-Folders/Alex/AlexTestLevel/InteractWithMerchant/EdgarAllanCrow/BP_MerchantTable.BP_MerchantTable_C|GetItem3 _returnvalue) (Variables|/Game/Dev-Directory/Personal-Folders/Alex/AlexTestLevel/InteractWithMerchant/EdgarAllanCrow/BP_MerchantTable.BP_MerchantTable_C|GetItem4 _returnvalue))))