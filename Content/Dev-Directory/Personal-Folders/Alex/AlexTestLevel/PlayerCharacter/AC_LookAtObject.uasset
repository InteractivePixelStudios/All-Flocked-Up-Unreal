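; Actor component prototype for turning a player character bone, likely the head, toward a cat.
; BeginPlay caches the bone's world rotation from the player mesh.
; Each tick runs a zero-length sphere trace at the player controller's location and, on hitting BP_Cat, stores a look-at rotation to the impact.
; The work looks unfinished: the stored rotation is never applied and the passed start rotation is unused.
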(event Custom|TurnHeadToObject
  (CallFunction|LookatObject (Variables|Default|GetBoneStartRotation)))

(event EventBeginPlay
  (CallFunction|GetRigBone))

(event EventTick
  (params (DeltaSeconds :type Float%20%28single-precision%29))
  (CallFunction|TurnHeadtoObject))

(fn GetRigBone
  (Variables|Default|SetBoneStartRotation (.Rotation (Math|Transform|BreakTransform (Transformation|GetBoneTransform (Variables|/Script/Engine.Character|GetMesh (Game|GetPlayerCharacter 0)) (Variables|Default|GetBoneToMove) "RTS_World")))))

(fn LookatObject
  (params (StartingLookRotation :type Rotator))
  (bind _returnvalue (Game|GetPlayerController 0))
  (bind _returnvalue_2 (Transformation|GetActorLocation _returnvalue))
  (bind _outhit (Collision|SphereTraceByChannel _returnvalue_2 _returnvalue_2 2e+01 "TraceTypeQuery1" false 0 "None"))
  (if (== (.hitactor _outhit) "/Game/Dev-Directory/Personal-Folders/Max/Cat/BP_Cat.BP_Cat")
    (Variables|Default|SetBoneEndRotation (Math|Rotator|FindLookatRotation _returnvalue_2 (.location _outhit)))))