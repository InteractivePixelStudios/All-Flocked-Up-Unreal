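; Player pigeon poop-firing component, triggered by the IA_Poo input or CallPoop while the pigeon's poop system has ammo.
; Flight state, polled on Tick, selects a drop from the aerial fire point or an aimed shot from the ground point with projectile movement activated.
; Each mode has its own one-second cooldown, and each shot consumes poop.
; ChiliPoops enables projectile particles for five seconds, then fires automatically before clearing the power-up.
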(event Custom|ChiliPoops
  ;[1 1 1] Chili Poop Powerup
  (Variables|Default|SetHasChiliPower true)
  (Utilities|FlowControl|Delay 5.0)
  (CallFunction|CallPoop)
  (Variables|Default|SetHasChiliPower false))

(event Custom|CallPoop
  ;[1 1 1] Aerial Poo Drop
  (bind _asbp_pigeon_character_ab (Utilities|Casting|CastToBP_PigeonCharacter_AB (Game|GetPlayerCharacter 0)))
  (if (> (Variables|/Game/Dev-Directory/Personal-Folders/Jayden/BP_PoopSystem_WK.BP_PoopSystem_WK_C|GetPoopCurrent (Variables|/Game/Dev-Directory/Personal-Folders/Alex/AlexTestLevel/PlayerCharacter/BP_PigeonCharacter_AB.BP_PigeonCharacter_AB_C|GetBP_PoopSystem_WK _asbp_pigeon_character_ab)) 0)
    (if (stale EventTick _output_get)
      ;;[1 1 1] Poop is spawned at the ProjectileSpawnPoint on the Player
      (Utilities|FlowControl|DoOnce false :!label _label
        (:Completed
          (bind _returnvalue (Game|SpawnActorfromClass "/Game/Dev-Directory/Personal-Folders/Max/Blueprints/BP_PoopFunction.BP_PoopFunction_C" (Math|Transform|MakeTransform (Math|Vector|MakeVector (.x (Transformation|GetWorldLocation (Variables|/Game/Dev-Directory/Personal-Folders/Alex/AlexTestLevel/PlayerCharacter/BP_PigeonCharacter_AB.BP_PigeonCharacter_AB_C|GetArialPoopFirePoint _asbp_pigeon_character_ab))) (.y (Transformation|GetWorldLocation (Variables|/Game/Dev-Directory/Personal-Folders/Alex/AlexTestLevel/PlayerCharacter/BP_PigeonCharacter_AB.BP_PigeonCharacter_AB_C|GetArialPoopFirePoint _asbp_pigeon_character_ab))) (.z (Transformation|GetWorldLocation (Variables|/Game/Dev-Directory/Personal-Folders/Alex/AlexTestLevel/PlayerCharacter/BP_PigeonCharacter_AB.BP_PigeonCharacter_AB_C|GetArialPoopFirePoint _asbp_pigeon_character_ab)))) "0, 0, 0" "0.200000,0.200000,0.200000") "AdjustIfPossibleButAlwaysSpawn" "MultiplyWithRoot" 0 0))
          (if (Variables|Default|GetHasChiliPower)
            (Components|Activation|Activate (Variables|/Game/Dev-Directory/Personal-Folders/Max/Blueprints/BP_PoopFunction.BP_PoopFunction_C|GetParticleSystem _returnvalue) false))
          (Default|LosePoop (Variables|/Game/Dev-Directory/Personal-Folders/Alex/AlexTestLevel/PlayerCharacter/BP_PigeonCharacter_AB.BP_PigeonCharacter_AB_C|GetBP_PoopSystem_WK _asbp_pigeon_character_ab))
          (Utilities|FlowControl|Delay 1.0)
          (goto _label Reset)))
      (else
        ;[1 1 1] Grounded Poo Shoot
        (Utilities|FlowControl|DoOnce false :!label _label_2
          (:Completed
            (bind _returnvalue_2 (Game|SpawnActorfromClass "/Game/Dev-Directory/Personal-Folders/Max/Blueprints/BP_PoopFunction.BP_PoopFunction_C" (Math|Transform|MakeTransform (Math|Vector|MakeVector (.x (Transformation|GetWorldLocation (Variables|/Game/Dev-Directory/Personal-Folders/Alex/AlexTestLevel/PlayerCharacter/BP_PigeonCharacter_AB.BP_PigeonCharacter_AB_C|GetGroundPoopFirePoint _asbp_pigeon_character_ab))) (.y (Transformation|GetWorldLocation (Variables|/Game/Dev-Directory/Personal-Folders/Alex/AlexTestLevel/PlayerCharacter/BP_PigeonCharacter_AB.BP_PigeonCharacter_AB_C|GetGroundPoopFirePoint _asbp_pigeon_character_ab))) (.z (Transformation|GetWorldLocation (Variables|/Game/Dev-Directory/Personal-Folders/Alex/AlexTestLevel/PlayerCharacter/BP_PigeonCharacter_AB.BP_PigeonCharacter_AB_C|GetGroundPoopFirePoint _asbp_pigeon_character_ab)))) (Transformation|GetWorldRotation (Variables|/Game/Dev-Directory/Personal-Folders/Alex/AlexTestLevel/PlayerCharacter/BP_PigeonCharacter_AB.BP_PigeonCharacter_AB_C|GetGroundPoopFirePoint _asbp_pigeon_character_ab)) "0.200000,0.200000,0.200000") "AdjustIfPossibleButAlwaysSpawn" "MultiplyWithRoot" 0 0))
            (Components|Activation|Activate (Variables|/Game/Dev-Directory/Personal-Folders/Max/Blueprints/BP_PoopFunction.BP_PoopFunction_C|GetProjectileMovement _returnvalue_2) false)
            (if (Variables|Default|GetHasChiliPower)
              (Components|Activation|Activate (Variables|/Game/Dev-Directory/Personal-Folders/Max/Blueprints/BP_PoopFunction.BP_PoopFunction_C|GetParticleSystem _returnvalue_2) false))
            (Default|LosePoop (Variables|/Game/Dev-Directory/Personal-Folders/Alex/AlexTestLevel/PlayerCharacter/BP_PigeonCharacter_AB.BP_PigeonCharacter_AB_C|GetBP_PoopSystem_WK _asbp_pigeon_character_ab))
            (Utilities|FlowControl|Delay 1.0)
            (goto _label_2 Reset)))))
    (else
      (Development|PrintString "No Poop Left" true true "(R=1.000000,G=0.000000,B=0.000000,A=1.000000)"))))

(event Input|EnhancedActionEvents|EnhancedInputActionIA_Poo
  (params (ActionValue :type Boolean) (ElapsedSeconds :type Float%20%28double-precision%29) (TriggeredSeconds :type Float%20%28double-precision%29) (InputAction :type Input%20Action%20Object%20Reference :default "/Game/Dev-Directory/Personal-Folders/Max/Character/Inputs/IA_Poo.IA_Poo"))
  ;[1 1 1] Aerial Poo Drop
  ;;[1 1 1] Player Input
  (bind _asbp_pigeon_character_ab (Utilities|Casting|CastToBP_PigeonCharacter_AB (Game|GetPlayerCharacter 0)))
  (if (> (Variables|/Game/Dev-Directory/Personal-Folders/Jayden/BP_PoopSystem_WK.BP_PoopSystem_WK_C|GetPoopCurrent (Variables|/Game/Dev-Directory/Personal-Folders/Alex/AlexTestLevel/PlayerCharacter/BP_PigeonCharacter_AB.BP_PigeonCharacter_AB_C|GetBP_PoopSystem_WK _asbp_pigeon_character_ab)) 0)
    (if (stale EventTick _output_get)
      ;;[1 1 1] Poop is spawned at the ProjectileSpawnPoint on the Player
      (Utilities|FlowControl|DoOnce false :!label _label
        (:Completed
          (bind _returnvalue (Game|SpawnActorfromClass "/Game/Dev-Directory/Personal-Folders/Max/Blueprints/BP_PoopFunction.BP_PoopFunction_C" (Math|Transform|MakeTransform (Math|Vector|MakeVector (.x (Transformation|GetWorldLocation (Variables|/Game/Dev-Directory/Personal-Folders/Alex/AlexTestLevel/PlayerCharacter/BP_PigeonCharacter_AB.BP_PigeonCharacter_AB_C|GetArialPoopFirePoint _asbp_pigeon_character_ab))) (.y (Transformation|GetWorldLocation (Variables|/Game/Dev-Directory/Personal-Folders/Alex/AlexTestLevel/PlayerCharacter/BP_PigeonCharacter_AB.BP_PigeonCharacter_AB_C|GetArialPoopFirePoint _asbp_pigeon_character_ab))) (.z (Transformation|GetWorldLocation (Variables|/Game/Dev-Directory/Personal-Folders/Alex/AlexTestLevel/PlayerCharacter/BP_PigeonCharacter_AB.BP_PigeonCharacter_AB_C|GetArialPoopFirePoint _asbp_pigeon_character_ab)))) "0, 0, 0" "0.200000,0.200000,0.200000") "AdjustIfPossibleButAlwaysSpawn" "MultiplyWithRoot" 0 0))
          (if (Variables|Default|GetHasChiliPower)
            (Components|Activation|Activate (Variables|/Game/Dev-Directory/Personal-Folders/Max/Blueprints/BP_PoopFunction.BP_PoopFunction_C|GetParticleSystem _returnvalue) false))
          (Default|LosePoop (Variables|/Game/Dev-Directory/Personal-Folders/Alex/AlexTestLevel/PlayerCharacter/BP_PigeonCharacter_AB.BP_PigeonCharacter_AB_C|GetBP_PoopSystem_WK _asbp_pigeon_character_ab))
          (Utilities|FlowControl|Delay 1.0)
          (goto _label Reset)))
      (else
        ;[1 1 1] Grounded Poo Shoot
        (Utilities|FlowControl|DoOnce false :!label _label_2
          (:Completed
            (bind _returnvalue_2 (Game|SpawnActorfromClass "/Game/Dev-Directory/Personal-Folders/Max/Blueprints/BP_PoopFunction.BP_PoopFunction_C" (Math|Transform|MakeTransform (Math|Vector|MakeVector (.x (Transformation|GetWorldLocation (Variables|/Game/Dev-Directory/Personal-Folders/Alex/AlexTestLevel/PlayerCharacter/BP_PigeonCharacter_AB.BP_PigeonCharacter_AB_C|GetGroundPoopFirePoint _asbp_pigeon_character_ab))) (.y (Transformation|GetWorldLocation (Variables|/Game/Dev-Directory/Personal-Folders/Alex/AlexTestLevel/PlayerCharacter/BP_PigeonCharacter_AB.BP_PigeonCharacter_AB_C|GetGroundPoopFirePoint _asbp_pigeon_character_ab))) (.z (Transformation|GetWorldLocation (Variables|/Game/Dev-Directory/Personal-Folders/Alex/AlexTestLevel/PlayerCharacter/BP_PigeonCharacter_AB.BP_PigeonCharacter_AB_C|GetGroundPoopFirePoint _asbp_pigeon_character_ab)))) (Transformation|GetWorldRotation (Variables|/Game/Dev-Directory/Personal-Folders/Alex/AlexTestLevel/PlayerCharacter/BP_PigeonCharacter_AB.BP_PigeonCharacter_AB_C|GetGroundPoopFirePoint _asbp_pigeon_character_ab)) "0.200000,0.200000,0.200000") "AdjustIfPossibleButAlwaysSpawn" "MultiplyWithRoot" 0 0))
            (Components|Activation|Activate (Variables|/Game/Dev-Directory/Personal-Folders/Max/Blueprints/BP_PoopFunction.BP_PoopFunction_C|GetProjectileMovement _returnvalue_2) false)
            (if (Variables|Default|GetHasChiliPower)
              (Components|Activation|Activate (Variables|/Game/Dev-Directory/Personal-Folders/Max/Blueprints/BP_PoopFunction.BP_PoopFunction_C|GetParticleSystem _returnvalue_2) false))
            (Default|LosePoop (Variables|/Game/Dev-Directory/Personal-Folders/Alex/AlexTestLevel/PlayerCharacter/BP_PigeonCharacter_AB.BP_PigeonCharacter_AB_C|GetBP_PoopSystem_WK _asbp_pigeon_character_ab))
            (Utilities|FlowControl|Delay 1.0)
            (goto _label_2 Reset)))))
    (else
      (Development|PrintString "No Poop Left" true true "(R=1.000000,G=0.000000,B=0.000000,A=1.000000)"))))

(event EventTick
  (params (DeltaSeconds :type Float%20%28single-precision%29))
  (bind _pigeonref (Variables|Default|GetPigeonRef)
    (:then
      (bind _output_get (Variables|Default|SetIsFlying (Variables|/Game/Dev-Directory/Personal-Folders/Sebastian/Blueprints/PlayerMechanics/BP_PlayerFlightControl_SO.BP_PlayerFlightControl_SO_C|GetisFlying (Variables|/Game/Dev-Directory/Personal-Folders/Alex/AlexTestLevel/PlayerCharacter/BP_PigeonCharacter_AB.BP_PigeonCharacter_AB_C|GetBP_PlayerFlightControl_SO _pigeonref)))))
    (:else)))