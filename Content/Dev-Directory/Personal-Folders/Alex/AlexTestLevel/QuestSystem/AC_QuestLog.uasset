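; Quest log component that records active and completed quests, presumably for the player, and manages their on-screen tracker.
; Adding a quest stores its ID, spawns a BP_QuestsBase actor and starts its countdown.
; Completion moves the ID to the completed list, flags the actor turned in and calls OnQuestCompleted, while turn-in first prints the stage's XP reward.
; TrackQuest creates or updates a single WBP_QuestTracker widget.
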(event EventBeginPlay)

(event EventTick
  (params (DeltaSeconds :type Float%20%28single-precision%29)))

(fn AddNewQuest
  (params (QuestID :type Name))
  ;[1 1 1] Adds a new Quest to the Quest Log
  ;;[0.2627 0.5529 1] Gets current active quest and adds unique to ensure no duplicate quests
  (Utilities|Array|AddUnique (Variables|Default|GetcurrentActiveQuest) QuestID)
  ;;[0.2627 0.5529 1] Gets Current active quest
  (bind _returnvalue (Game|SpawnActorfromClass "/Game/Dev-Directory/Personal-Folders/Alex/AlexTestLevel/QuestSystem/BP_QuestsBase.BP_QuestsBase_C" (Math|Transform|MakeTransform "0, 0, 0" "0, 0, 0" "1.000000,1.000000,1.000000") "Undefined" "MultiplyWithRoot" 0 QuestID 0))
  (Utilities|Array|Add (Variables|Default|GetcurrentActiveQuests) _returnvalue)
  (Default|CountdownTime _returnvalue)
  ;[0.2314 0.1137 0.5529] Returns the questBase
  (return _returnvalue))

(fn CompleteQuest
  (params (QuestID :type Name%20%28by%20ref%29))
  ;[0.2627 0.5529 1] Adds to complete quest array
  (Utilities|Array|AddUnique (Variables|Default|GetcompletedQuests) QuestID)
  ;[0.2627 0.5529 1] Removes from the current active quest array
  (Utilities|Array|RemoveItem (Variables|Default|GetcurrentActiveQuest) QuestID)
  ;[0.2314 0.1137 0.5529] Gets the quest actor, sets isQuestTurnedIn to true and calls OnQuestCompleted
  (bind _array_element (CallFunction|GetQuestActor QuestID))
  (Variables|/Game/Dev-Directory/Personal-Folders/Alex/AlexTestLevel/QuestSystem/BP_QuestsBase.BP_QuestsBase_C|SetisQuestTurnedIn _array_element true)
  (Default|CallOnQuestCompleted _array_element))

(fn QueryActiveQuest
  (params (QuestID :type Name))
  ;[0.2314 0.1137 0.5529] Queries the Active quest to see if player already has quest
  (return (Utilities|Array|ContainsItem (Variables|Default|GetcurrentActiveQuest) QuestID)))

(fn TrackQuest
  (params (QuestActorRef :type BP%20Quests%20Base%20Object%20Reference))
  ;[0.2627 0.5529 1] Gets the tracker widgets and adds it to the viewport
  (bind _tracker (Variables|Default|GetTracker)
    (:then
      (Default|Update _tracker QuestActorRef))
    (:else
      (bind _returnvalue (UserInterface|CreateWidget "/Game/Dev-Directory/Personal-Folders/Alex/AlexTestLevel/QuestSystem/UI/WBP_QuestTracker.WBP_QuestTracker_C" 0 QuestActorRef))
      (bind _output_get (Variables|Default|SetTracker _returnvalue))
      (UserInterface|Viewport|AddtoViewport _output_get -1))))

(fn GetQuestActor
  (params (QuestID :type Name))
  ;[0.2627 0.5529 1] Loops through currentActiveQuest array and checks if the questID matches the questID from the questlog component
  (for _array_element (Variables|Default|GetcurrentActiveQuests)
    ;[0.2314 0.1137 0.5529] if true, returns that array element
    (if (== (Variables|/Game/Dev-Directory/Personal-Folders/Alex/AlexTestLevel/QuestSystem/BP_QuestsBase.BP_QuestsBase_C|GetquestID _array_element) QuestID)
      (return _array_element))))

(fn TurninQuest
  (params (QuestID :type Name))
  (Utilities|FlowControl|Sequence
    (:then_0
      ;[0.2627 0.5529 1] Gets the quest actor, turns in the quest and shows a debug log for xprewards
      (bind _array_element (CallFunction|GetQuestActor QuestID))
      (Development|PrintString (Utilities|String|ToString(Text) (Utilities|Text|FormatText "XP={a}" (.XPReward (Utilities|Struct|BreakS_StageDetails (Variables|/Game/Dev-Directory/Personal-Folders/Alex/AlexTestLevel/QuestSystem/BP_QuestsBase.BP_QuestsBase_C|GetcurrentStageDetails _array_element)))))))
    (:then_1
      ;[0.6875 0.1683 0.1683 0.7216] For AutoCompleteQuest
      (CallFunction|CompleteQuest QuestID))))

(fn QueryCompletedQuest
  (params (QuestID :type Name))
  (bind _completedquests (Variables|Default|GetcompletedQuests))
  (bind _returnvalue (Utilities|Array|ContainsItem _completedquests QuestID))
  ;[0.2627 0.5529 1] Queries the Active quest to see if player already has quest and if the quest has already been turned in
  (bind _array_element (CallFunction|GetQuestActor QuestID))
  (Utilities|IsValid _array_element
    (:Is%20Valid
      (return _returnvalue (Variables|/Game/Dev-Directory/Personal-Folders/Alex/AlexTestLevel/QuestSystem/BP_QuestsBase.BP_QuestsBase_C|GetisQuestTurnedIn _array_element)))
    (:Is%20Not%20Valid
      (return _returnvalue true))))