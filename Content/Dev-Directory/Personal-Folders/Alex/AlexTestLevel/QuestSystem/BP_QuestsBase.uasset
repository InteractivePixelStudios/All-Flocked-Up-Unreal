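; Base quest actor that tracks one quest's staged objectives and time limit for the pigeon character.
; It loads stages from DT_QuestData, counts objective IDs broadcast by the character, shows notifications, advances stages and auto-turns in to AC_QuestLog.
; Tick runs and debug-prints a countdown that shows a failure widget and clears progress at zero.
; A separate function, uncalled here, spawns BP_Breadcrumb at every BP_CollectibleSpawn.
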(event Custom|CountdownTime
  (CallFunction|QuestCountdownTimer))

(event EventBeginPlay
  (CallFunction|GetQuestDetails)
  ;[0.2627 0.5529 1] Gets the quest details and binds event to OnObjectiveIDCalled
  (CallFunction|GetQuestTime)
  (EventDispatchers|BindEventtoOnObjectiveIDCalled (CallFunction|GetPigeonCharacter) (EventDispatchers|CreateEvent :!event OnObjectiveIDHeard))
  ;[0.2627 0.5529 1] Checks if ALL objectives are completed and sets the isCompleted bool true
  (bind _return (CallFunction|AreAllObjectivesComplete))
  (Variables|Default|SetisCompleted _return))

(event Collision|EventActorBeginOverlap
  (params (OtherActor :type Actor%20Object%20Reference)))

(event EventTick
  (params (DeltaSeconds :type Float%20%28single-precision%29))
  (CallFunction|CountdownTime)
  (Development|PrintString (Utilities|String|ToString(Float) (Variables|Default|GetQuestTimer)) true false "(R=0.000000,G=0.660000,B=1.000000,A=1.000000)" 0.01))

(fn ConstructionScript)

(fn OnObjectiveIDHeard
  (params (ObjectiveID :type Name))
  (bind _returnvalue (Utilities|String|ToString(Name) ObjectiveID))
  (bind _returnvalue_2 (Utilities|String|ToString(Name) ObjectiveID))
  (bind _currentobjectiveprogress (Variables|Default|GetcurrentObjectiveProgress))
  (bind (_value _returnvalue_3) (Utilities|Map|Find _currentobjectiveprogress _returnvalue))
  ;[1 1 1] gets the objectiveID of questgiver and adds the objectives to the currentObjectiveProgress map. When objectives are completed, it cannot be called again from for that questID
  ;;[0.2627 0.5529 1] Checks for objective id matches
  ;;[0.1059 0.1059 0.1059 0.7216] Ensures only set amount can be triggered
  (if (< _value (.Quantity (Utilities|Struct|BreakS_ObjectiveDetails (CallFunction|GetObjectiveDatabyID (Utilities|String|ToString(Name) ObjectiveID)))))
    ;;[0.2627 1 0.251] Adds 1 if match is found
    (if _returnvalue_3
      (Utilities|Map|Add (Variables|Default|GetcurrentObjectiveProgress) _returnvalue_2 (+ _value 1))
      ;;[1 1 1] Calls IsObjectiveComplete
      (CallFunction|IsObjectiveCompleted _returnvalue_2)
      ;;[1 1 1] Calls OnObjectiveIDHeard
      (Default|CallOnObjectiveHeard)
      (return)
      (else
        (return)))))

(fn GetQuestDetails
  ;[0.2627 0.5529 1] Gets and sets quest id in data table
  (bind _returnvalue (Utilities|GetDataTableRow "/Game/Dev-Directory/Personal-Folders/Alex/AlexTestLevel/QuestSystem/DT_QuestData.DT_QuestData" (Variables|Default|GetquestID))
    (:then
      (bind _output_get (Variables|Default|SetquestDetails _returnvalue))
      ;[0.2627 0.5529 1] sets current stage details
      (bind _output_get_2 (Variables|Default|SetcurrentStageDetails (Utilities|Array|Get(acopy) (.Stages (Utilities|Struct|BreakS_QuestDetails _output_get)) (Variables|Default|GetcurrentStage))))
      ;[0.6875 0.1683 0.1683 0.7216] clears progress array
      (Utilities|Map|Clear (Variables|Default|GetcurrentObjectiveProgress))
      ;[0.2314 0.1137 0.5529] Adds objectives to array
      (for _array_element (.Objectives (Utilities|Struct|BreakS_StageDetails _output_get_2))
        (Utilities|Map|Add (Variables|Default|GetcurrentObjectiveProgress) (.ObjectiveID (Utilities|Struct|BreakS_ObjectiveDetails _array_element)) 0)))))

(fn GetObjectiveDatabyID
  (params (ObjectiveID :type String))
  ;[0.2314 0.1137 0.5529] Loops through the objectives array and gets the objective ID. If it matches the stored data it returns it.
  (for _array_element (.Objectives (Utilities|Struct|BreakS_StageDetails (Variables|Default|GetcurrentStageDetails)))
    (if (Utilities|Enum|Equal(Enum) (.ObjectiveID (Utilities|Struct|BreakS_ObjectiveDetails _array_element)) ObjectiveID)
      (return _array_element))))

(fn IsObjectiveCompleted
  (params (ObjectiveID :type String))
  (bind _array_element (CallFunction|GetObjectiveDatabyID ObjectiveID))
  (bind (_objectivename _description _objectivetype _objectiveid _quantity) (Utilities|Struct|BreakS_ObjectiveDetails _array_element))
  ;[0.6875 0.1683 0.1683 0.7216] Creates the widget and adds it to the viewport
  (if (>= (.Value (Utilities|Map|Find (Variables|Default|GetcurrentObjectiveProgress) ObjectiveID)) _quantity)
    (bind _returnvalue (UserInterface|CreateWidget "/Game/Dev-Directory/Personal-Folders/Alex/AlexTestLevel/QuestSystem/UI/WBP_QuestNotification.WBP_QuestNotification_C" 0 _description))
    (UserInterface|Viewport|AddtoViewport _returnvalue 0)
    ;[0.2627 0.5529 1] Checks if all the objectives in the current stage are complete and increments the current stage to the next.
    (bind _return (CallFunction|AreAllObjectivesComplete))
    (if _return
      (bind _result (Math|Integer|IncrementInt (Variables|Default|GetcurrentStage))
        (:%20%20
          ;[0.2627 0.5529 1] Checks if the index is valid in the for the save
          (if (Utilities|Array|IsValidIndex (.stages (Variables|Default|GetquestDetails)) _result)
            ;[0.2314 0.1137 0.5529] if true, it gets the quest details
            (CallFunction|GetQuestDetails)
            (else
              ;[0.2627 0.5529 1] if all objectives ate completed this turns in the quest and completes it.
              (Variables|Default|SetisCompleted true)
              (if (.autocomplete (Variables|Default|GetquestDetails))
                (Default|TurninQuest (Actor|GetComponentbyClass (Game|GetPlayerCharacter 0) "/Game/Dev-Directory/Personal-Folders/Alex/AlexTestLevel/QuestSystem/AC_QuestLog.AC_QuestLog_C") (Variables|Default|GetquestID))))))))))

(fn AreAllObjectivesComplete
  ;[0.2627 0.5529 1] Gets the objective ID from S_ObjectiveDetails
  (for _array_element (.objectives (Variables|Default|GetcurrentStageDetails))
    ;[0.2314 0.1137 0.5529] If you dont that means the quest is not complete, Once quantity fufilled it sets all complete to true and returns that bool value
    (if (not (>= (.Value (Utilities|Map|Find (Variables|Default|GetcurrentObjectiveProgress) (.ObjectiveID (Utilities|Struct|BreakS_ObjectiveDetails _array_element)))) (.Quantity (Utilities|Struct|BreakS_ObjectiveDetails (CallFunction|GetObjectiveDatabyID (.ObjectiveID (Utilities|Struct|BreakS_ObjectiveDetails _array_element)))))))
      (bind _output_get (LocalVariables|SetlocalAllComplete false))
      (return _output_get)))
  ;[0.6875 0.1683 0.1683 0.7216] If all quests are complete it returns early
  (return (LocalVariables|GetlocalAllComplete)))

(fn QuestCountdownTimer
  (bind _output_get (Variables|Default|SetQuestTimer (Math|Float|Clamp(Float) (- (Variables|Default|GetQuestTimer) (Utilities|Time|GetWorldDeltaSeconds)) 0.0 (Variables|Default|GetQuestMaxTime))))
  (if (<= _output_get 0.0)
    (if (!= (Variables|Default|GetisQuestFail) true)
      (Variables|Default|SetisQuestFail true)
      (bind _returnvalue (UserInterface|CreateWidget "/Game/Dev-Directory/Personal-Folders/Alex/AlexTestLevel/QuestSystem/UI/WBP_QuestFailed.WBP_QuestFailed_C" 0 "QUEST FAILED!"))
      (UserInterface|Viewport|AddtoViewport _returnvalue 0)
      (Utilities|Map|Clear (Variables|Default|GetcurrentObjectiveProgress)))))

(fn GetQuestTime
  (bind _output_get (Variables|Default|SetQuestMaxTime (.questtime (Variables|Default|GetquestDetails))))
  (Variables|Default|SetQuestTimer _output_get))

(fn ActivateQuestItems
  (bind _outactors (Actor|GetAllActorsOfClass "/Game/Dev-Directory/Personal-Folders/Alex/AlexTestLevel/Collectibles(Quests)/BP_CollectibleSpawn.BP_CollectibleSpawn_C"))
  (for _array_element _outactors
    (Game|SpawnActorfromClass "/Game/Dev-Directory/Personal-Folders/Alex/AlexTestLevel/Collectibles(Quests)/BP_Breadcrumb.BP_Breadcrumb_C" (Transformation|GetActorTransform _array_element) "Undefined" "MultiplyWithRoot" 0 0)))