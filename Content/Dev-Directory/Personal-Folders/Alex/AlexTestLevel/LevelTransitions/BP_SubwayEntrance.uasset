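; BP_SubwayEntrance is a subway entrance interactable that opens the level transition menu for the pigeon character.
; Box overlaps with BP_PigeonCharacter_AB toggle CanInteract and print leftover "Merchant" debug messages.
; When in range, the Pickup event creates WBP_LevelTransition, pauses the game and switches to UI-only input with cursor.
; WidgetRef, the focus target, is assigned only in unreachable code, alongside unused widget removal logic.
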(event OnComponentBeginOverlap(Box)
  (params (OverlappedComponent :type Primitive%20Component%20Object%20Reference) (OtherActor :type Actor%20Object%20Reference) (OtherComp :type Primitive%20Component%20Object%20Reference) (OtherBodyIndex :type Integer) (bFromSweep :type Boolean) (SweepResult :type Hit%20Result%20Structure%20%28by%20ref%29))
  (Utilities|Casting|CastToBP_PigeonCharacter_AB OtherActor)
  (Variables|Default|SetbCanInteract true) ; Sets interactivity to true
  (Development|PrintString "Merchant can be interacted with"))

(event OnComponentEndOverlap(Box)
  (params (OverlappedComponent :type Primitive%20Component%20Object%20Reference) (OtherActor :type Actor%20Object%20Reference) (OtherComp :type Primitive%20Component%20Object%20Reference) (OtherBodyIndex :type Integer))
  (Utilities|Casting|CastToBP_PigeonCharacter_AB OtherActor)
  (Variables|Default|SetbCanInteract false)
  (Development|PrintString "Merchant interact range left"))

(event EventBeginPlay)

(event Collision|EventActorBeginOverlap
  (params (OtherActor :type Actor%20Object%20Reference)))

(event EventTick
  (params (DeltaSeconds :type Float%20%28single-precision%29)))

(event EventPickup
  (bind _returnvalue (Game|GetPlayerController 0))
  (Input|EnableInput _returnvalue)
  (if (Variables|Default|GetbCanInteract)
    (bind _returnvalue_2 (UserInterface|CreateWidget "/Game/Dev-Directory/Personal-Folders/Alex/AlexTestLevel/LevelTransitions/WBP_LevelTransition.WBP_LevelTransition_C" _returnvalue))
    (UserInterface|Viewport|AddtoViewport _returnvalue_2 0)
    (Game|SetGamePaused true)
    (Input|SetInputModeUIOnly _returnvalue (Variables|Default|GetWidgetRef) "DoNotLock" false)
    (Variables|/Script/Engine.PlayerController|SetbShowMouseCursor _returnvalue true)))

(fn ConstructionScript)