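; Base actor for a pickup item that the pigeon character carries to hide, raising its stealth stat while held.
; A box overlap caches the pigeon, then Pickup lifts and tilts the item, attaches it to the pigeon's ArialPoopFirePoint and adds stealth.
; RemoveItem detaches it at the pigeon's transform, briefly enables mesh physics with cube collision off, then removes the bonus.
; IsHiding gates both events, and debug prints show the stat.
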(event OnComponentBeginOverlap(Box)
  (params (OverlappedComponent :type Primitive%20Component%20Object%20Reference) (OtherActor :type Actor%20Object%20Reference) (OtherComp :type Primitive%20Component%20Object%20Reference) (OtherBodyIndex :type Integer) (bFromSweep :type Boolean) (SweepResult :type Hit%20Result%20Structure%20%28by%20ref%29))
  ;[1 1 1] Attach Item
  (bind _asbp_pigeon_character_ab (Utilities|Casting|CastToBP_PigeonCharacter_AB OtherActor))
  (Development|PrintString (Utilities|String|ToString(Float) (Variables|/Game/Dev-Directory/Personal-Folders/Alex/AlexTestLevel/PlayerCharacter/BP_PigeonCharacter_AB.BP_PigeonCharacter_AB_C|GetbaseStealthStat _asbp_pigeon_character_ab))))

(event Custom|RemoveItem
  ;[1 1 1] Detach Item
  (if (Variables|Default|GetisHiding)
    (Transformation|DetachFromActor "KeepWorld" "KeepRelative" "KeepRelative")
    (Transformation|SetActorTransform (Math|Transform|MakeTransform (Math|Vector|MakeVector (.x (.location (Transformation|GetActorTransform (stale OnComponentBeginOverlap(Box) _asbp_pigeon_character_ab)))) (.y (.location (Transformation|GetActorTransform (stale OnComponentBeginOverlap(Box) _asbp_pigeon_character_ab)))) (.z (.location (Transformation|GetActorTransform (stale OnComponentBeginOverlap(Box) _asbp_pigeon_character_ab))))) (Math|Rotator|MakeRotator (.roll (.rotation (Transformation|GetActorTransform (stale OnComponentBeginOverlap(Box) _asbp_pigeon_character_ab)))) (.pitch (.rotation (Transformation|GetActorTransform (stale OnComponentBeginOverlap(Box) _asbp_pigeon_character_ab)))) (.yaw (.rotation (Transformation|GetActorTransform (stale OnComponentBeginOverlap(Box) _asbp_pigeon_character_ab))))) "1.000000,1.000000,1.000000"))
    (Collision|SetCollisionEnabled (Variables|Default|GetCube) "NoCollision")
    (Physics|SetSimulatePhysics (Variables|Default|GetStaticMesh) true)
    (Utilities|FlowControl|Delay 1.0)
    (Collision|SetCollisionEnabled (Variables|Default|GetCube) "QueryAndPhysics")
    (Physics|SetSimulatePhysics (Variables|Default|GetStaticMesh) false)
    (Variables|Default|SetisHiding false)
    (Variables|/Game/Dev-Directory/Personal-Folders/Alex/AlexTestLevel/PlayerCharacter/BP_PigeonCharacter_AB.BP_PigeonCharacter_AB_C|SetbaseStealthStat (stale OnComponentBeginOverlap(Box) _asbp_pigeon_character_ab) (- (Variables|/Game/Dev-Directory/Personal-Folders/Alex/AlexTestLevel/PlayerCharacter/BP_PigeonCharacter_AB.BP_PigeonCharacter_AB_C|GetbaseStealthStat (stale OnComponentBeginOverlap(Box) _asbp_pigeon_character_ab)) 1e+01))
    (Development|PrintString (Utilities|String|ToString(Float) (- (Variables|/Game/Dev-Directory/Personal-Folders/Alex/AlexTestLevel/PlayerCharacter/BP_PigeonCharacter_AB.BP_PigeonCharacter_AB_C|GetbaseStealthStat (stale OnComponentBeginOverlap(Box) _asbp_pigeon_character_ab)) 1e+01)))))

(event EventBeginPlay)

(event Collision|EventActorBeginOverlap
  (params (OtherActor :type Actor%20Object%20Reference)))

(event EventPickup
  (bind _returnvalue (Transformation|GetActorLocation))
  (bind _returnvalue_2 (Transformation|GetActorRotation))
  (bind _returnvalue_3 (Transformation|GetActorLocation))
  (bind _returnvalue_4 (Transformation|GetActorRotation))
  (if (not (Variables|Default|GetisHiding))
    (Transformation|SetActorTransform (Math|Transform|MakeTransform (Math|Vector|MakeVector (.x _returnvalue) (.y _returnvalue) (+ (.z _returnvalue) 2.5)) (Math|Rotator|MakeRotator (+ (.roll _returnvalue_2) 1e+01) (.pitch _returnvalue_2) (.yaw _returnvalue_2)) "1.000000,1.000000,1.000000"))
    (Utilities|FlowControl|Delay 0.5)
    (Transformation|SetActorTransform (Math|Transform|MakeTransform (Math|Vector|MakeVector (.x _returnvalue_3) (.y _returnvalue_3) (.z _returnvalue_3)) (Math|Rotator|MakeRotator (- (.roll _returnvalue_4) 45.0) (- (.pitch _returnvalue_4) -15.0) (.yaw _returnvalue_4)) "1.000000,1.000000,1.000000"))
    (bind _returnvalue_5 (Transformation|AttachComponentToComponent (Variables|Default|GetDefaultSceneRoot) (Variables|/Game/Dev-Directory/Personal-Folders/Alex/AlexTestLevel/PlayerCharacter/BP_PigeonCharacter_AB.BP_PigeonCharacter_AB_C|GetArialPoopFirePoint (stale OnComponentBeginOverlap(Box) _asbp_pigeon_character_ab)) "None" "SnapToTarget" "KeepRelative" "KeepRelative" false))
    (Variables|Default|SetisHiding _returnvalue_5)
    (Variables|/Game/Dev-Directory/Personal-Folders/Alex/AlexTestLevel/PlayerCharacter/BP_PigeonCharacter_AB.BP_PigeonCharacter_AB_C|SetbaseStealthStat (stale OnComponentBeginOverlap(Box) _asbp_pigeon_character_ab) (+ (Variables|/Game/Dev-Directory/Personal-Folders/Alex/AlexTestLevel/PlayerCharacter/BP_PigeonCharacter_AB.BP_PigeonCharacter_AB_C|GetbaseStealthStat (stale OnComponentBeginOverlap(Box) _asbp_pigeon_character_ab)) 1e+01))
    (Development|PrintString (Utilities|String|ToString(Float) (+ (Variables|/Game/Dev-Directory/Personal-Folders/Alex/AlexTestLevel/PlayerCharacter/BP_PigeonCharacter_AB.BP_PigeonCharacter_AB_C|GetbaseStealthStat (stale OnComponentBeginOverlap(Box) _asbp_pigeon_character_ab)) 1e+01)))))

(fn ConstructionScript)