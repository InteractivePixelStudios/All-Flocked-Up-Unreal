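; Red-tailed hawk enemy AI that perches at the nearest BP_PerchLocation until pawn sensing spots a pawn, then chases the player.
; Tick traces toward the player for the move target and launches the hawk when it is not above the hit; FollowPlayer triggers Attack and a delayed return to perch.
; Capsule hits damage the pigeon player, and sphere overlap shows a brief alert with sound.
; RandomRoam is never called here.
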(event OnSeePawn(PawnSensing)
  (params (Pawn :type Pawn%20Object%20Reference))
  ;[1 1 1] Set Can See Player on Pawn sensing
  (Variables|Default|SetIsSeeingPlayer true))

(event OnComponentBeginOverlap(Sphere)
  (params (OverlappedComponent :type Primitive%20Component%20Object%20Reference) (OtherActor :type Actor%20Object%20Reference) (OtherComp :type Primitive%20Component%20Object%20Reference) (OtherBodyIndex :type Integer) (bFromSweep :type Boolean) (SweepResult :type Hit%20Result%20Structure%20%28by%20ref%29))
  (bind _returnvalue (Transformation|GetActorTransform))
  (Utilities|Casting|CastToBP_PigeonCharacter_AB OtherActor)
  (bind _returnvalue_2 (Game|SpawnActorfromClass "/Game/Dev-Directory/Personal-Folders/Wesley/BluePrints_WK/BP_AlertNotificationObject_WK.BP_AlertNotificationObject_WK_C" (Math|Transform|MakeTransform (+ (.location _returnvalue) "0.000000,0.000000,10.000000") (.rotation _returnvalue) (.scale _returnvalue)) "Undefined" "MultiplyWithRoot" 0 0))
  (Audio|PlaySound2D "/Game/Dev-Directory/Personal-Folders/Alex/AlexTestLevel/funny-sound-effect-for-quotjack-in-the-boxquot-sound-ver1-110923.funny-sound-effect-for-quotjack-in-the-boxquot-sound-ver1-110923" 1.0 1.0 0.0 0 0)
  (Utilities|FlowControl|Delay 1.0)
  (Actor|DestroyActor _returnvalue_2))

(event OnComponentHit(CapsuleComponent)
  (params (HitComponent :type Primitive%20Component%20Object%20Reference) (OtherActor :type Actor%20Object%20Reference) (OtherComp :type Primitive%20Component%20Object%20Reference) (NormalImpulse :type Vector :default "0, 0, 0") (Hit :type Hit%20Result%20Structure%20%28by%20ref%29))
  ;[1 1 1] Player takes damage on collision
  (bind _asbp_pigeon_character_ab (Utilities|Casting|CastToBP_PigeonCharacter_AB OtherActor))
  (Default|LoseHealth (Variables|/Game/Dev-Directory/Personal-Folders/Alex/AlexTestLevel/PlayerCharacter/BP_PigeonCharacter_AB.BP_PigeonCharacter_AB_C|GetBP_HealthSystem_WK _asbp_pigeon_character_ab) 1)
  (Utilities|FlowControl|Delay 1.0))

(event Custom|RandomRoam
  ;[1 1 1] Random Roam Logic
  (AI|AIMoveTo (Variables|Default|GetAC_Redtail) self (.RandomLocation (AI|Navigation|GetRandomReachablePointinRadius (Transformation|GetActorLocation) 2e+02 0 0)) 0 5.0 false
    (:OnSuccess
      (CallFunction|RandomRoam))))

(event Custom|Perch
  (bind _returnvalue (Transformation|GetActorLocation))
  (bind _perchreference (Variables|Default|GetPerchReference))
  (bind _returnvalue_2 (Actor|FindNearestActor _returnvalue _perchreference))
  ;[1 1 1] Perch Logic
  (Utilities|FlowControl|Sequence
    (:then_0
      (AI|AIMoveTo self (Transformation|GetActorLocation _returnvalue_2) _returnvalue_2 0.1 false
        (:OnSuccess
          (Components|Movement|StopMovementImmediately (Variables|Character|GetCharacterMovement)))))))

(event Custom|FollowPlayer
  ;[1 1 1] Follow Player Logic
  (Variables|Default|SetCanAttack true)
  (if (Variables|Default|GetIsSeeingPlayer)
    (Utilities|FlowControl|Sequence
      (:then_0
        (AI|AIMoveTo self (Variables|Default|GetNewLocation) (Game|GetPlayerCharacter 0) 0.1 false
          (:OnSuccess
            (if (Variables|Default|GetCanAttack)
              (Variables|Default|SetCanAttack false)
              (CallFunction|Attack)))))
      (:then_1
        (Utilities|FlowControl|RetriggerableDelay 3.0)
        (CallFunction|Perch)))
    (else
      (Variables|Default|SetIsSeeingPlayer false))))

(event EventBeginPlay
  ;[1 1 1] Get Perch Locations and set AI to perch
  (bind _outactors (Actor|GetAllActorsOfClass "/Game/Dev-Directory/Personal-Folders/Damon/AITesting/AIFunctionality/RedTailHawkAI/BP_PerchLocation.BP_PerchLocation_C"))
  (Variables|Default|SetPerchReference _outactors)
  (CallFunction|Perch))

(event EventTick
  (params (DeltaSeconds :type Float%20%28single-precision%29))
  (bind _returnvalue (Transformation|GetActorLocation))
  (bind _output_get (Variables|Default|SetPlayerLocation (Transformation|GetActorLocation (Game|GetPlayerCharacter 0))))
  (bind _outhit (Collision|LineTraceByChannel (Transformation|GetActorLocation) _output_get "TraceTypeQuery1" false 0 "ForOneFrame"))
  (Variables|Default|SetNewLocation (.location _outhit))
  ;[1 1 1] Event tick to check if seeing player
  (if (Variables|Default|GetIsSeeingPlayer)
    (CallFunction|FollowPlayer)
    (if (> (.Z (Math|Vector|BreakVector _returnvalue)) (.Z (Math|Vector|BreakVector (Variables|Default|GetNewLocation))))
      (CallFunction|FollowPlayer :!label _label)
      (else
        (Utilities|FlowControl|Sequence
          (:then_0
            (Character|LaunchCharacter (+ (* (Math|Vector|Normalize (+ _returnvalue (Variables|Default|GetNewLocation)) 1.0) "0.000000,0.000000,500.000000") (Math|Vector|GetForwardVector (Transformation|GetActorRotation))) true true)
            (CallFunction|FollowPlayer))
          (:then_1
            (goto _label)))))
    (else
      (CallFunction|Perch))))

(fn ConstructionScript)

(fn Attack
  (bind _capsulecomponent (Variables|Collision|GetCapsuleComponent))
  (if (<= (Math|Vector|Distance(Vector) (Transformation|GetActorLocation (Game|GetPlayerController 0)) (Transformation|GetWorldLocation _capsulecomponent)) 0.5)
    (Variables|/Script/Engine.MovementComponent|SetVelocity (Variables|Character|GetCharacterMovement) (* (Transformation|GetComponentVelocity _capsulecomponent) 2))))