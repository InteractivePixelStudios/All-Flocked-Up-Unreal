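; BP_Carlos is an AI test actor that turns to face the player.
; Tick continuously interpolates its yaw toward the player's location, holding pitch and roll at zero.
; A Detection overlap calls EngagePlayer when the player character is BP_PigeonCharacter_AB, setting ShouldRotateToPlayer, which ending an overlap clears.
; Tick reads neither that flag nor the rotation saved at BeginPlay, so turning is not gated by detection.
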(event OnComponentBeginOverlap(Detection)
  (params (OverlappedComponent :type Primitive%20Component%20Object%20Reference) (OtherActor :type Actor%20Object%20Reference) (OtherComp :type Primitive%20Component%20Object%20Reference) (OtherBodyIndex :type Integer) (bFromSweep :type Boolean) (SweepResult :type Hit%20Result%20Structure%20%28by%20ref%29))
  (Utilities|Casting|CastToBP_PigeonCharacter_AB (Game|GetPlayerCharacter 0))
  (CallFunction|EngagePlayer))

(event Custom|EngagePlayer
  (Variables|Default|SetShouldRotateToPlayer true))

(event EventTick
  (params (DeltaSeconds :type Float%20%28single-precision%29))
  (Transformation|SetActorRotation (Math|Interpolation|RInterpTo (Transformation|GetActorRotation) (Math|Rotator|MakeRotator 0.0 0.0 (.Yaw (Math|Rotator|BreakRotator (Math|Rotator|FindLookatRotation (Transformation|GetActorLocation) (Transformation|GetActorLocation (Game|GetPlayerCharacter 0)))))) 0.0 0.0)))

(event Collision|EventActorEndOverlap
  (params (OtherActor :type Actor%20Object%20Reference))
  (Variables|Default|SetShouldRotateToPlayer false))

(event EventBeginPlay
  (Variables|Default|SetOriginalRotation (Transformation|GetActorRotation)))

(fn ConstructionScript)