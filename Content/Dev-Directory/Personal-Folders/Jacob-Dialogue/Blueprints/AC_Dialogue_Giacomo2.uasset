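; Dialogue component, apparently a test for Giacomo, that overrides Dialogue to play a scripted conversation with linear and branching examples.
; Each line's speaker, text and response options come from a hardcoded row in DDT_Test_JS, fed to AddDialogue, whose State and OptionIndex gate the next nested lookup.
; The third line splits into two short branches that both clear dialogue progress and close the conversation.
; Only a missing first row is logged.
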(event EventBeginPlay)

(event EventTick
  (params (DeltaSeconds :type Float%20%28single-precision%29)))

(fn Dialogue
  (|CallParentFunction)
  ;[1 1 1] Linear dialogue example
  (bind _returnvalue (Utilities|GetDataTableRow "/Game/Dev-Directory/Personal-Folders/Jacob-Dialogue/Blueprints/DataTableTest/DDT_Test_JS.DDT_Test_JS" "1.0")
    (:then
      (switch int (Variables|Default|GetDialogueTreeIndex)
        (:0
          ;;[1 1 1] Creates new dialogue with Add Dialogue method and using an array, create branches in dialogue.
          (bind (_state _optionindex) (CallFunction|AddDialogue (.SpeakerName (Utilities|Struct|BreakDialogueDataStruct_JS _returnvalue)) (.DialogueText (Utilities|Struct|BreakDialogueDataStruct_JS _returnvalue)) (.ResponseOptions (Utilities|Struct|BreakDialogueDataStruct_JS _returnvalue))))
          (switch Utilities|FlowControl|Switch|SwitchonEnum_DialogueState _state
            (:NewEnumerator0
              (switch int _optionindex
                (:0
                  (bind _returnvalue_2 (Utilities|GetDataTableRow "/Game/Dev-Directory/Personal-Folders/Jacob-Dialogue/Blueprints/DataTableTest/DDT_Test_JS.DDT_Test_JS" "1.1")
                    (:then
                      (bind (_state_2 _optionindex_2) (CallFunction|AddDialogue (.SpeakerName (Utilities|Struct|BreakDialogueDataStruct_JS _returnvalue_2)) (.DialogueText (Utilities|Struct|BreakDialogueDataStruct_JS _returnvalue_2)) (.ResponseOptions (Utilities|Struct|BreakDialogueDataStruct_JS _returnvalue_2))))
                      (switch Utilities|FlowControl|Switch|SwitchonEnum_DialogueState _state_2
                        (:NewEnumerator0
                          (switch int _optionindex_2
                            (:0
                              (bind _returnvalue_3 (Utilities|GetDataTableRow "/Game/Dev-Directory/Personal-Folders/Jacob-Dialogue/Blueprints/DataTableTest/DDT_Test_JS.DDT_Test_JS" "1.2")
                                (:then
                                  (bind (_state_3 _optionindex_3) (CallFunction|AddDialogue (.SpeakerName (Utilities|Struct|BreakDialogueDataStruct_JS _returnvalue_3)) (.DialogueText (Utilities|Struct|BreakDialogueDataStruct_JS _returnvalue_3)) (.ResponseOptions (Utilities|Struct|BreakDialogueDataStruct_JS _returnvalue_3))))
                                  ;[1 1 1] Branching Dialogue Example
                                  (switch Utilities|FlowControl|Switch|SwitchonEnum_DialogueState _state_3
                                    (:NewEnumerator0
                                      (switch int _optionindex_3
                                        (:0
                                          (bind _returnvalue_4 (Utilities|GetDataTableRow "/Game/Dev-Directory/Personal-Folders/Jacob-Dialogue/Blueprints/DataTableTest/DDT_Test_JS.DDT_Test_JS" "1.3")
                                            (:then
                                              (bind (_state_4 _optionindex_4) (CallFunction|AddDialogue (.SpeakerName (Utilities|Struct|BreakDialogueDataStruct_JS _returnvalue_4)) (.DialogueText (Utilities|Struct|BreakDialogueDataStruct_JS _returnvalue_4)) (.ResponseOptions (Utilities|Struct|BreakDialogueDataStruct_JS _returnvalue_4))))
                                              (switch Utilities|FlowControl|Switch|SwitchonEnum_DialogueState _state_4
                                                (:NewEnumerator0
                                                  (switch int _optionindex_4
                                                    (:0
                                                      (bind _returnvalue_5 (Utilities|GetDataTableRow "/Game/Dev-Directory/Personal-Folders/Jacob-Dialogue/Blueprints/DataTableTest/DDT_Test_JS.DDT_Test_JS" "1.5")
                                                        (:then
                                                          (bind (_state_5 _optionindex_5) (CallFunction|AddDialogue (.SpeakerName (Utilities|Struct|BreakDialogueDataStruct_JS _returnvalue_5)) (.DialogueText (Utilities|Struct|BreakDialogueDataStruct_JS _returnvalue_5)) (.ResponseOptions (Utilities|Struct|BreakDialogueDataStruct_JS _returnvalue_5))))
                                                          (switch Utilities|FlowControl|Switch|SwitchonEnum_DialogueState _state_5
                                                            (:NewEnumerator0
                                                              (switch int _optionindex_5
                                                                (:0
                                                                  _)))))))))))))
                                        (:1
                                          (bind _returnvalue_6 (Utilities|GetDataTableRow "/Game/Dev-Directory/Personal-Folders/Jacob-Dialogue/Blueprints/DataTableTest/DDT_Test_JS.DDT_Test_JS" "1.4")
                                            (:then
                                              (bind (_state_6 _optionindex_6) (CallFunction|AddDialogue (.SpeakerName (Utilities|Struct|BreakDialogueDataStruct_JS _returnvalue_6)) (.DialogueText (Utilities|Struct|BreakDialogueDataStruct_JS _returnvalue_6)) (.ResponseOptions (Utilities|Struct|BreakDialogueDataStruct_JS _returnvalue_6))))
                                              (switch Utilities|FlowControl|Switch|SwitchonEnum_DialogueState _state_6
                                                (:NewEnumerator0
                                                  (switch int _optionindex_6
                                                    (:0
                                                      (bind _returnvalue_7 (Utilities|GetDataTableRow "/Game/Dev-Directory/Personal-Folders/Jacob-Dialogue/Blueprints/DataTableTest/DDT_Test_JS.DDT_Test_JS" "1.6")
                                                        (:then
                                                          (bind (_state_7 _optionindex_7) (CallFunction|AddDialogue (.SpeakerName (Utilities|Struct|BreakDialogueDataStruct_JS _returnvalue_7)) (.DialogueText (Utilities|Struct|BreakDialogueDataStruct_JS _returnvalue_7)) (.ResponseOptions (Utilities|Struct|BreakDialogueDataStruct_JS _returnvalue_7))))
                                                          (switch Utilities|FlowControl|Switch|SwitchonEnum_DialogueState _state_7
                                                            (:NewEnumerator0
                                                              (switch int _optionindex_7
                                                                (:0
                                                                  _))))))))))))))
                                      ;;[1 1 1] Exits Dialogue
                                      (CallFunction|ClearDialogueProgress)
                                      (CallFunction|CloseConversation))))))))))))))))))
    (:RowNotFound
      (Utilities|String|LogString "Data Table Row Not Found"))))