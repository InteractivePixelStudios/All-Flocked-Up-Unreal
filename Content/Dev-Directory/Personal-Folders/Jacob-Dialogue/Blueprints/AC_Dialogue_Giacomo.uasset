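; Actor component defining a branching conversation with the NPC Giacomo, who asks the player to do assigned tasks.
; The Dialogue override calls its parent, then chains AddDialogue nodes, branching on the selected option index whenever a node returns Passthrough.
; Agreeing leads to a pass response, refusing to a fail response with debug prints on both.
; Leave options and branch endings share an exit that clears dialogue progress and closes the conversation.
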(event EventBeginPlay)

(event EventTick
  (params (DeltaSeconds :type Float%20%28single-precision%29)))

(fn Dialogue
  (params (DialogueRow :type Name :default "None"))
  (|CallParentFunction "None")
  (switch int (Variables|Default|GetDialogueTreeIndex)
    (:0
      ;[1 1 1] Creates new dialogue with Add Dialogue method and using an array, create branches in dialogue.
      (bind (_state _optionindex) (CallFunction|AddDialogue "Giacomo" "\"Do your assigned tasks please!\"" (Utilities|Array|MakeArray "\"Okay\"" "\"NO!!! I HATE WORK!\"" "Leave")))
      (switch Utilities|FlowControl|Switch|SwitchonEnum_DialogueState _state
        (:NewEnumerator0
          ;[1 1 1] Branches dialogue based on previous option selected.
          (switch int _optionindex
            (:0
              (Development|PrintString "Selecting \"Okay\"")
              (bind (_state_2 _optionindex_2) (CallFunction|AddDialogue "Giacomo" "\"You pass :)!\"" (Utilities|Array|MakeArray "Continue" "Leave")))
              (switch Utilities|FlowControl|Switch|SwitchonEnum_DialogueState _state_2
                (:NewEnumerator0
                  (switch int _optionindex_2
                    (:0
                      (bind _state_3 (CallFunction|AddDialogue "You" "Yay!" (Utilities|Array|MakeArray "Leave")))
                      (switch Utilities|FlowControl|Switch|SwitchonEnum_DialogueState _state_3
                        (:NewEnumerator0
                          _)))
                    (:1
                      _)))))
            (:1
              (Development|PrintString "Selecting \"I HATE WORK\"")
              (bind _state_4 (CallFunction|AddDialogue "Giacomo" "\"YOU FAIL!\"" (Utilities|Array|MakeArray "aw shoot")))
              (switch Utilities|FlowControl|Switch|SwitchonEnum_DialogueState _state_4
                (:NewEnumerator0
                  _)))
            (:2
              _))
          ;[1 1 1] Exits Dialogue
          (CallFunction|ClearDialogueProgress)
          (CallFunction|CloseConversation))))))