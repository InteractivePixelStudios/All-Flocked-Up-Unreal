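; Base NPC actor for dialogue, with a name label set at construction and shown or hidden with interactable state.
; Interact opens a conversation through the dialogue component and plays a timeline that lerps the NPC and player yaw to face each other.
; Each update also pitches and yaw-offsets the player camera to a side chosen from its starting world yaw.
; Closing the conversation notifies the interact instigator.
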(event EventInteract
  (params (Instigator :type Actor%20Object%20Reference))
  (Variables|Default|SetInteractInstigator Instigator)
  (Default|OpenConversation (Variables|Default|GetAC_Dialogue_Base) (Variables|Default|GetConversationStartRow))
  (Variables|Default|SetPlayerStartRotation (Transformation|GetActorRotation (Game|Player|GetPlayerPawn 0)))
  (Variables|Default|SetPlayerCameraRotation (Pawn|GetControlRotation (Game|GetPlayerController 0) :!class /Script/Engine.Controller))
  (bind _turnalpha (Timeline|TurnTimeline Play)
    (:Update
      (CallFunction|NPCLookatPlayer _turnalpha)
      (CallFunction|PlayerLookatNPC _turnalpha))
    (:Finished
      (CallFunction|NPCLookatPlayer 1.0)
      (CallFunction|PlayerLookatNPC 1.0))))

(event EventConversationClosed
  (Class|BPIInteractable|ConversationClosed(Message) (Variables|Default|GetInteractInstigator)))

(event EventBeginPlay
  (Variables|Default|SetOriginalRotation (Transformation|GetActorRotation)))

(event EventSetInteractableState
  (params (CanShowInteract :type Boolean))
  ;[1 1 1] Sets character name visibility when nearby
  (Development|PrintString "set interactable state event")
  (if CanShowInteract
    (Rendering|SetVisibility (Variables|Default|GetTXT_CharacterName) true false)
    (else
      (Rendering|SetVisibility (Variables|Default|GetTXT_CharacterName) false false))))

(fn ConstructionScript
  ;[1 1 1] Update Character Name
  (Rendering|Components|TextRender|SetText (Variables|Default|GetTXT_CharacterName) (Variables|Default|GetCharacterName)))

(fn NPCLookatPlayer
  (params (TurnAlpha :type Float%20%28double-precision%29))
  (Transformation|SetActorRotation (Math|Rotator|MakeRotator 0.0 0.0 (Math|Float|Lerp (.yaw (Variables|Default|GetOriginalRotation)) (.yaw (Math|Rotator|FindLookatRotation (Transformation|GetActorLocation) (Transformation|GetActorLocation (Game|Player|GetPlayerPawn 0)))) TurnAlpha))))

(fn PlayerLookatNPC
  (params (Turn%20Alpha :type Float%20%28double-precision%29))
  (bind _returnvalue (Game|Player|GetPlayerPawn 0))
  (bind _returnvalue_2 (Transformation|GetActorLocation))
  (bind _playerstartrotation (Variables|Default|GetPlayerStartRotation))
  (bind _returnvalue_3 (Transformation|GetActorLocation _returnvalue))
  (bind _returnvalue_4 (Math|Rotator|FindLookatRotation _returnvalue_3 _returnvalue_2))
  (bind _returnvalue_5 (Math|Float|Lerp (.yaw _playerstartrotation) (.yaw _returnvalue_4) Turn%20Alpha))
  (Transformation|SetActorRotation (Game|Player|GetPlayerPawn 0) (Math|Rotator|MakeRotator 0.0 0.0 _returnvalue_5))
  (CallFunction|AdjustPlayerCamera _returnvalue_5))

(fn AdjustPlayerCamera
  (params (Z-Rotation :type Float%20%28double-precision%29))
  (bind _playercamerarotation (Variables|Default|GetPlayerCameraRotation))
  (if (and (<= (.yaw _playercamerarotation) 2.7e+02) (>= (.yaw _playercamerarotation) 9e+01))
    ;[0.2623 0.552 1] Set Camera to right side of player
    (Pawn|SetControlRotation (Game|GetPlayerController 0) (Math|Rotator|MakeRotator (.roll (Variables|Default|GetPlayerCameraRotation)) (Variables|Default|GetCameraPitchAngle) (- Z-Rotation (Variables|Default|GetCameraYawAngle))))
    (else
      ;[0.2623 0.552 1] Set Camera to left side of player
      (Pawn|SetControlRotation (Game|GetPlayerController 0) (Math|Rotator|MakeRotator (.roll (Variables|Default|GetPlayerCameraRotation)) (Variables|Default|GetCameraPitchAngle) (+ Z-Rotation (Variables|Default|GetCameraYawAngle)))))))