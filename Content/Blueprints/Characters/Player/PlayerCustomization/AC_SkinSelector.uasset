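; AC_SkinSelector is a player customization component that opens and closes the skin selector screen.
; Opening adds WBP_SkinSelector to the viewport and spawns a BP_BackdropPlane offset from the player controller's transform; closing removes both and restores game-only input with the cursor hidden.
; BeginPlay caches the player mesh's first material, unused in this graph.
; The UI-only input and cursor setup for opening is disconnected, so it never runs.
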(event Custom|OpenSkinSelector
  (bind _returnvalue (Game|GetPlayerController 0))
  (bind _returnvalue_2 (Transformation|GetActorTransform _returnvalue))
  (bind _returnvalue_3 (UserInterface|CreateWidget "/Game/Blueprints/Characters/Player/PlayerCustomization/WBP_SkinSelector.WBP_SkinSelector_C" _returnvalue))
  (UserInterface|Viewport|AddtoViewport _returnvalue_3 0)
  (bind _returnvalue_4 (Game|SpawnActorfromClass "/Game/Blueprints/GameplaySystems/HelperMechanics/BP_BackdropPlane.BP_BackdropPlane_C" (Math|Transform|MakeTransform (+ (.location _returnvalue_2) "50.000000,40.000000,-25.000000") (.rotation _returnvalue_2) (.scale _returnvalue_2)) "AlwaysSpawn" "OverrideRootScale" 0 0))
  (Variables|Default|SetBackdropRef _returnvalue_4))

(event Custom|CloseSkinSelector
  (bind _returnvalue (Game|GetPlayerController 0))
  (Widget|RemovefromParent (stale Custom|OpenSkinSelector _returnvalue_3))
  (Input|SetInputModeGameOnly _returnvalue true)
  (Variables|/Script/Engine.PlayerController|SetbShowMouseCursor _returnvalue false)
  (Actor|DestroyActor (Variables|Default|GetBackdropRef)))

(event EventBeginPlay
  (Variables|Default|SetCurrentMaterial (Rendering|Material|GetMaterial (Variables|/Script/Engine.Character|GetMesh (Game|GetPlayerCharacter 0)) 0)))

(event EventTick
  (params (DeltaSeconds :type Float%20%28single-precision%29)))