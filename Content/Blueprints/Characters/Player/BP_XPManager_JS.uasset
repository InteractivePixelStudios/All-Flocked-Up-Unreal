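; Player XP manager that tracks experience and level, with IncreaseXP feeding CollectXP until MaxLevel is reached.
; Reaching XPThreshold triggers at most one LevelUp per gain, which carries over surplus XP, raises the threshold linearly and calls OnLevelUp on RegisteredListeners.
; OnLoadGame rebuilds progression by replaying LevelUp from level 2 to the saved level, re-notifying listeners, then restores saved XP.
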(event EventBeginPlay)

(event EventTick
  (params (DeltaSeconds :type Float%20%28single-precision%29)))

(event EventIncreaseXP
  (params (XP%20amount :type Integer))
  (CallFunction|CollectXP XP%20amount))

(event EventOnLevelUp)

(fn CollectXP
  (params (XPAmount :type Integer))
  ;[1 1 1] XP Increase Debug
  ;[1 1 1] XP Increase Override if max level is reached
  (if (not (== (Variables|Default|GetPlayerLevel) (Variables|Default|GetMaxLevel)))
    ;[1 1 1] Increase Current XP
    (bind _output_get (Variables|Default|SetCurrentXP (+ XPAmount (Variables|Default|GetCurrentXP))))
    ;[1 1 1] Check if XP Threshold reached
    (if (>= _output_get (Variables|Default|GetXPThreshold)) ; If current XP is equal to or greater than level up threshold, level up!
      (CallFunction|LevelUp))))

(fn LevelUp
  ;[1 1 1] Level Up Logic Plus Debug
  (Variables|Default|SetCurrentXP (- (Variables|Default|GetCurrentXP) (Variables|Default|GetXPThreshold))) ; Subtracts the XP threshold from current xp.
  (Variables|Default|SetPlayerLevel (+ (Variables|Default|GetPlayerLevel) 1)) ; increment player lvl
  (Variables|Default|SetXPThreshold (+ (Variables|Default|GetXPThreshold) 1.0)) ; Increases the XP Threshold required for the next level
  ;[1 1 1] Calling each Component on pigeon that has XP Interface
  (for _array_element (Variables|Default|GetRegisteredListeners)
    (Default|OnLevelUp _array_element)))

(fn OnLoadGame
  (params (XP :type Integer) (Level :type Integer))
  ;[1 1 1] On load
  (for _index (range 2 Level)
    (CallFunction|LevelUp))
  (Variables|Default|SetCurrentXP (Math|Conversions|ToFloat(Integer) XP)))