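; Player pigeon character Blueprint that switches between jumping and flying movement through Enhanced Input.
; A second jump press within a short retriggerable-delay window starts flying, where further flaps spend stamina on upward impulses.
; While flying, Tick applies forward glide and custom gravity forces until a ground box overlap restores falling mode and refills stamina.
; Move input off the ground pushes along control yaw and turns the controller.
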(event Input|EnhancedActionEvents|EnhancedInputActionIA_FlapUp
  (params (ActionValue :type Boolean) (ElapsedSeconds :type Float%20%28double-precision%29) (TriggeredSeconds :type Float%20%28double-precision%29) (InputAction :type Input%20Action%20Object%20Reference :default "/Game/Blueprints/Characters/Player/IA_FlapUp.IA_FlapUp"))
  (bind _charactermovement (Variables|Character|GetCharacterMovement))
  ;[1 1 1] Flapping Up
  (:Started
    (if (Variables|Default|GetisFlying)
      (if (> (Variables|Default|Getstamina) 1.0)
        (bind _result (Math|Float|DecrementFloat (Variables|Default|Getstamina))
          (:%20%20
            (Variables|Default|Setstamina _result)
            (Physics|AddImpulse _charactermovement (Math|Vector|MakeVector 0.0 0.0 (Variables|Default|GetflightFlapUpForce)) false))))
      (else
        (bind _result_2 (Math|Integer|IncrementInt (Variables|Default|GetjumpCount))
          (:%20%20
            (if (== _result_2 2)
              (Pawn|Components|CharacterMovement|SetMovementMode _charactermovement "MOVE_Flying" 0)
              (Variables|Default|SetisFlying true)
              (else
                (Character|Jump)
                (Utilities|FlowControl|RetriggerableDelay 0.5)
                (Variables|Default|SetjumpCount 0))))))))
  (:Completed
    (Character|StopJumping)))

(event Input|EnhancedActionEvents|EnhancedInputActionIA_FlyMove
  (params (ActionValue :type Vector%202D%20Structure) (ElapsedSeconds :type Float%20%28double-precision%29) (TriggeredSeconds :type Float%20%28double-precision%29) (InputAction :type Input%20Action%20Object%20Reference :default "/Game/Blueprints/Characters/Player/IA_FlyMove.IA_FlyMove"))
  ;[1 1 1] Fly Movement Input
  (if (not (AI|Components|NavMovement|IsMovingonGround (Pawn|GetMovementComponent)))
    (Pawn|Input|AddMovementInput (Math|Vector|GetForwardVector (Math|Rotator|MakeRotator 0.0 0.0 (.yaw (Pawn|GetControlRotation :!class /Script/Engine.Pawn)))) (.y ActionValue) false)
    (Pawn|Input|AddControllerYawInput (.x ActionValue))))

(event EventBeginPlay
  ;[1 1 1] Initial Controller Setup
  (bind _asplayer_controller (Utilities|Casting|CastToPlayerController (Pawn|GetController)))
  (Utilities|IsValid (PlayerController|LocalPlayerSubsystems|GetEnhancedInputLocalPlayerSubsystem _asplayer_controller)
    (:Is%20Valid
      (Input|AddMappingContext (PlayerController|LocalPlayerSubsystems|GetEnhancedInputLocalPlayerSubsystem _asplayer_controller) "/Game/Blueprints/Characters/Player/IMC_FlyControls.IMC_FlyControls" 0 "(bIgnoreAllPressedKeysUntilRelease=True,bForceImmediately=False,bNotifyUserSettings=False)")
      (Variables|/Script/Engine.CharacterMovementComponent|SetMaxFlySpeed (Variables|Character|GetCharacterMovement) (Variables|Default|GetflightSpeed)))))

(event EventTick
  (params (DeltaSeconds :type Float%20%28single-precision%29))
  ;[1 1 1] Gravity and Glide while flying
  (if (Variables|Default|GetisFlying)
    (Physics|AddForce (Variables|Character|GetCharacterMovement) (- (* (Math|Vector|GetForwardVector (Math|Rotator|MakeRotator 0.0 0.0 (.yaw (Pawn|GetControlRotation :!class /Script/Engine.Pawn)))) (Variables|Default|GetflightForwardGlideSpeed)) (Math|Vector|MakeVector 0.0 0.0 (Variables|Default|GetflightGravity))))
    (bind _returnvalue (Collision|BoxOverlapActors (Transformation|GetWorldLocation (Variables|Default|GetGroundCheck)) "1.000000,1.000000,0.500000" (Utilities|Array|MakeArray "ObjectTypeQuery1") 0 (Utilities|Array|MakeArray self) :!class /Script/Engine.KismetSystemLibrary))
    (if _returnvalue
      (Variables|Default|SetisFlying false)
      (Pawn|Components|CharacterMovement|SetMovementMode (Variables|Character|GetCharacterMovement) "MOVE_Falling" 0)
      (Variables|Default|Setstamina (Variables|Default|GetMAX_STAMINA)))))

(fn ConstructionScript)