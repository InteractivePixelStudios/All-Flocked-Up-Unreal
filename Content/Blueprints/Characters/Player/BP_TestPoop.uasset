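; BP_TestPoop is a short-lived poop actor that marks and damages what it overlaps, ignoring pigeon characters and stealth radius actors.
; On a valid sphere overlap it spawns a temporary poop decal at its own location, applies damage and destroys itself.
; The damage amount carries StunDuration rather than a conventional damage value.
; Without a hit, it destroys itself a few seconds after BeginPlay.
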(event OnComponentBeginOverlap(Sphere)
  (params (OverlappedComponent :type Primitive%20Component%20Object%20Reference) (OtherActor :type Actor%20Object%20Reference) (OtherComp :type Primitive%20Component%20Object%20Reference) (OtherBodyIndex :type Integer) (bFromSweep :type Boolean) (SweepResult :type Hit%20Result%20Structure%20%28by%20ref%29))
  (if (!= OtherActor self)
    (Utilities|Casting|CastToBP_PigeonCharacter_AB OtherActor
      (:CastFailed
        (Utilities|Casting|CastToBP_StealthRadius OtherActor
          (:CastFailed
            (Rendering|Decal|SpawnDecalatLocation "/Game/Art/ImportedArtwork/poop1_Mat.poop1_Mat" "10.000000,10.000000,10.000000" (.location (Transformation|GetActorTransform)) "-90.000000,0.000000,0.000000" 1e+01)
            (Game|Damage|ApplyDamage OtherActor (Variables|Default|GetStunDuration) 0 0)
            (Actor|DestroyActor)))))))

(event EventBeginPlay
  (Utilities|FlowControl|Delay 3.0)
  (Actor|DestroyActor))

(fn ConstructionScript)