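; BP_PoopFunction is the pigeon's poop projectile, which splats and damages what it hits.
; On BeginPlay it finds the pigeon character, triggers the dropping sound through its BPAPPlayerV2, and self-destructs after five seconds.
; Hits on anything but the player pawn trigger the splat sound or effect, leave a temporary decal, destroy the actor and spawn two Niagara splatters.
; StunDuration is passed as the damage amount.
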(event OnComponentHit(PoopObject)
  (params (HitComponent :type Primitive%20Component%20Object%20Reference) (OtherActor :type Actor%20Object%20Reference) (OtherComp :type Primitive%20Component%20Object%20Reference) (NormalImpulse :type Vector :default "0, 0, 0") (Hit :type Hit%20Result%20Structure%20%28by%20ref%29))
  (if (!= OtherActor (Game|Player|GetPlayerPawn 0))
    (Default|TriggerSplat (Variables|/Game/Blueprints/Characters/Player/BP_PigeonCharacter_AB.BP_PigeonCharacter_AB_C|GetBP_AP_PlayerV2 (Utilities|Array|Get(acopy) (stale EventBeginPlay _outactors))))
    (Rendering|Decal|SpawnDecalatLocation "/Game/Art/ImportedArtwork/poop1_Mat.poop1_Mat" "10.000000,10.000000,10.000000" (.impactpoint Hit) "-90.000000,0.000000,0.000000" 1e+01)
    (Game|Damage|ApplyDamage OtherActor (Variables|Default|GetStunDuration) 0 0)
    (Actor|DestroyActor)
    (Niagara|SpawnSystematLocation "/Game/Art/VFX/Player/PoopSplatter/VFX_PoopSplatter.VFX_PoopSplatter" (.impactpoint Hit))
    (Niagara|SpawnSystematLocation "/Game/DevTestMaps/Personal-Folders/Armaan/NS_PoopSplatter.NS_PoopSplatter" (.impactpoint Hit))))

(event EventBeginPlay
  (bind _outactors (Actor|GetAllActorsOfClass "/Game/Blueprints/Characters/Player/BP_PigeonCharacter_AB.BP_PigeonCharacter_AB_C"))
  (Default|TriggerDookySound (Variables|/Game/Blueprints/Characters/Player/BP_PigeonCharacter_AB.BP_PigeonCharacter_AB_C|GetBP_AP_PlayerV2 (Utilities|Array|Get(acopy) _outactors)))
  (Utilities|FlowControl|Delay 5.0)
  (Actor|DestroyActor))

(fn ConstructionScript)