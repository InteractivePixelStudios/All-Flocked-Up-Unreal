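; Player flight controller that turns a double jump within a short window into winged gliding through the CharacterMovementComponent's Flying mode.
; While flying, Tick applies custom gravity plus forward glide force, and a box overlap below the character ends flight and refills stamina.
; Enhanced Input drives stamina-limited flap impulses, forward-down dives, stalls that drop the glide force, and yaw rotation.
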(event Input|EnhancedActionEvents|EnhancedInputActionIA_FlapUp
  (params (ActionValue :type Boolean) (ElapsedSeconds :type Float%20%28double-precision%29) (TriggeredSeconds :type Float%20%28double-precision%29) (InputAction :type Input%20Action%20Object%20Reference :default "/Game/Blueprints/Characters/Player/IAactionsSebastian/IA_FlapUp.IA_FlapUp"))
  (:Started
    (if (Variables|Default|GetisFlying)
      ;[1 1 1] Check if player has the stamina to Flap wings
      (if (> (Variables|Default|Getstamina) 1.0)
        ;[1 1 1] Decrement Stamina and add upward force to the player
        (bind _result (Math|Float|DecrementFloat (Variables|Default|Getstamina))
          (:%20%20
            (Variables|Default|Setstamina _result)
            (Physics|AddImpulse (Variables|Default|GetcharacterMovementComponent) (Math|Vector|MakeVector 0.0 0.0 (Variables|Default|GetflightFlapUpForce)) false)))))))

(event Input|EnhancedActionEvents|EnhancedInputActionIA_Jump
  (params (ActionValue :type Boolean) (ElapsedSeconds :type Float%20%28double-precision%29) (TriggeredSeconds :type Float%20%28double-precision%29) (InputAction :type Input%20Action%20Object%20Reference :default "/Game/Blueprints/Characters/Player/EnhancedInput/IA_Jump.IA_Jump"))
  (:Started
    ;[1 1 1] If not flying increment jump to attempt to fly
    (if (not (Variables|Default|GetisFlying))
      (bind _result (Math|Integer|IncrementInt (Variables|Default|GetjumpCount))
        (:%20%20
          ;[1 1 1] If jumped twice then set player to flying
          (if (== _result 2)
            (Pawn|Components|CharacterMovement|SetMovementMode (Variables|Default|GetcharacterMovementComponent) "MOVE_Flying" 0)
            (Variables|Default|SetisFlying true)
            (else
              ;[1 1 1] Else reset jump count after half second
              (Utilities|FlowControl|RetriggerableDelay 0.5)
              (Variables|Default|SetjumpCount 0))))))))

(event Input|EnhancedActionEvents|EnhancedInputActionIA_FlyMove
  (params (ActionValue :type Float%20%28double-precision%29) (ElapsedSeconds :type Float%20%28double-precision%29) (TriggeredSeconds :type Float%20%28double-precision%29) (InputAction :type Input%20Action%20Object%20Reference :default "/Game/Blueprints/Characters/Player/IAactionsSebastian/IA_FlyMove.IA_FlyMove"))
  (bind _charactermovementcomponent (Variables|Default|GetcharacterMovementComponent))
  (bind _returnvalue (Class|PawnMovementComponent|GetPawnOwner _charactermovementcomponent))
  (bind _returnvalue_2 (Pawn|GetControlRotation _returnvalue :!class /Script/Engine.Pawn))
  (bind _returnvalue_3 (Math|Vector|GetForwardVector (Math|Rotator|MakeRotator 0.0 0.0 (.yaw _returnvalue_2))))
  (:Triggered
    (if (Variables|Default|GetisFlying) ; Check the player is flying
      ;[1 0.1197 0] If Action Value Y is > 0 player will dive, < 0 player stalls
      (if (> ActionValue 0.0)
        ;[1 1 1] Player will dive forward and down by the dive speed value
        (Pawn|Input|AddMovementInput (Class|PawnMovementComponent|GetPawnOwner (Variables|Default|GetcharacterMovementComponent)) (Math|Vector|MakeVector (.x _returnvalue_3) (.y _returnvalue_3) -1.0) (Variables|Default|GetdiveSpeed) false)
        (else
          ;[1 1 1] Set Air Stall to true
          (Variables|Default|SetairStall true)))))
  (:Completed
    ;[1 0.1566 0] Reset Air Stall
    (Variables|Default|SetairStall false)))

(event Input|EnhancedActionEvents|EnhancedInputActionIA_FlyRotate
  (params (ActionValue :type Float%20%28double-precision%29) (ElapsedSeconds :type Float%20%28double-precision%29) (TriggeredSeconds :type Float%20%28double-precision%29) (InputAction :type Input%20Action%20Object%20Reference :default "/Game/Blueprints/Characters/Player/IA_FlyRotate.IA_FlyRotate"))
  (bind _returnvalue (Game|Player|GetPlayerPawn 0))
  (bind _returnvalue_2 (Transformation|GetActorRotation _returnvalue))
  ;[1 1 1] Rotate Player Character Left/Right
  (Transformation|SetActorRotation _returnvalue (Math|Rotator|MakeRotator (.roll _returnvalue_2) (.pitch _returnvalue_2) (+ (.yaw _returnvalue_2) ActionValue))))

(event EventBeginPlay
  ;[1 1 1] Set Base Variables
  (CallFunction|GetParentCharacterController)
  (Variables|Default|Setstamina (Variables|Default|GetMAX_STAMINA)))

(event EventTick
  (params (DeltaSeconds :type Float%20%28single-precision%29))
  ;[1 1 1] If flying apply gravity and forward glide while checking if the player hit the ground
  (if (Variables|Default|GetisFlying)
    (CallFunction|FallandGlide)
    (bind _groundcheck (CallFunction|GroundCheck))
    ;[1 1 1] When player hits the ground set flying to false and make the character fall to the ground
    (if _groundcheck
      (Variables|Default|SetisFlying false)
      (Pawn|Components|CharacterMovement|SetMovementMode (Variables|Default|GetcharacterMovementComponent) "MOVE_Falling" 0)
      ;[1 1 1] Reset Stamina once on ground
      (Variables|Default|Setstamina (Variables|Default|GetMAX_STAMINA)))))

(fn GetParentCharacterController
  ;[1 1 1] Get and set Character Movement Component from Character Component
  (Variables|Default|SetcharacterMovementComponent (Variables|/Script/Engine.Character|GetCharacterMovement (Game|GetPlayerCharacter 0))))

(fn FallandGlide
  (bind _charactermovementcomponent (Variables|Default|GetcharacterMovementComponent))
  (if (Variables|Default|GetairStall)
    ;[1 1 1] When stalled just apply downward gravity
    (Physics|AddForce _charactermovementcomponent (Math|Vector|MakeVector 0.0 0.0 (* (Variables|Default|GetflightGravity) -1.0)))
    (else
      ;[1 1 1] Apply glide speed and gravity to the direction
      (Physics|AddForce _charactermovementcomponent (- (* (Math|Vector|GetForwardVector (Math|Rotator|MakeRotator 0.0 0.0 (.yaw (Class|CharacterMovementComponent|GetLastUpdateRotation (Variables|Default|GetcharacterMovementComponent))))) (Variables|Default|GetflightForwardGlideSpeed)) (Math|Vector|MakeVector 0.0 0.0 (Variables|Default|GetflightGravity)))))))

(fn GroundCheck
  (bind _returnvalue (Game|GetPlayerCharacter 0))
  ;[1 1 1] Create box and check for collisions with terrain
  (bind _returnvalue_2 (Collision|BoxOverlapActors (- (Transformation|GetActorLocation _returnvalue) "0.000000,0.000000,100.000000") "25.000000,25.000000,15.000000" (Utilities|Array|MakeArray "ObjectTypeQuery1") 0 (Utilities|Array|MakeArray _returnvalue) :!class /Script/Engine.KismetSystemLibrary))
  ;[1 1 1] Return results of overlap check
  (return _returnvalue_2))