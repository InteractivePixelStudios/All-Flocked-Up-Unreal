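; Actor component for stealth users that gives its owner a detection radius through a spawned BP_StealthRadius actor.
; BeginPlay spawns that actor at the owner's transform and registers the owner as a non-detector with the current DetectionRadius.
; SetUpStealthUser stores a given radius and repeats the spawn, replacing the stored reference without destroying the earlier actor.
; ResizeRadius updates DetectionRadius and forwards it to the referenced radius actor.
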(event EventBeginPlay
  (bind _returnvalue (Components|GetOwner))
  ;[0.2623 0.552 1] Spawns and sets stealth radius parent and radius
  (bind _returnvalue_2 (Game|SpawnActorfromClass "/Game/Blueprints/Characters/Player/Stealth/BP_StealthRadius.BP_StealthRadius_C" (Transformation|GetActorTransform _returnvalue) "Undefined" "MultiplyWithRoot" 0 0))
  (bind _output_get (Variables|Default|SetStealthRadiusRef _returnvalue_2))
  (Default|SetupStealthOwner _output_get _returnvalue (Variables|Default|GetDetectionRadius) false))

(fn SetUpStealthUser
  (params (RadiusOfDetection :type Float%20%28double-precision%29))
  (bind _returnvalue (Components|GetOwner))
  (Variables|Default|SetDetectionRadius RadiusOfDetection)
  ;[0.2623 0.552 1] Spawn Stealth Radius and set up owner/radius
  (bind _returnvalue_2 (Game|SpawnActorfromClass "/Game/Blueprints/Characters/Player/Stealth/BP_StealthRadius.BP_StealthRadius_C" (Transformation|GetActorTransform _returnvalue) "Undefined" "MultiplyWithRoot" 0 0))
  (bind _output_get (Variables|Default|SetStealthRadiusRef _returnvalue_2))
  (Default|SetupStealthOwner _output_get _returnvalue (Variables|Default|GetDetectionRadius) false))

(fn ResizeRadius
  (params (New%20Radius :type Float%20%28double-precision%29))
  ;[0.2623 0.552 1] Change Radius size and call Stealth Radius function
  (bind _output_get (Variables|Default|SetDetectionRadius New%20Radius))
  (Default|ChangeRadius (Variables|Default|GetStealthRadiusRef) _output_get))