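; AC_StealthDetector is an actor component that gives its owner a stealth detection radius.
; On BeginPlay it spawns a BP_StealthRadius at the owner's transform and sets it up with the owner, DetectionRadius and the detector flag.
; DetectUser and LostUser are placeholder responses that print the detected user's name, or the lost user's name and last seen location.
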(event EventBeginPlay
  (bind _returnvalue (Components|GetOwner))
  ;[0.2623 0.552 1] Spawns and sets stealth radius parent and radius
  (bind _returnvalue_2 (Game|SpawnActorfromClass "/Game/Blueprints/Characters/Player/Stealth/BP_StealthRadius.BP_StealthRadius_C" (Transformation|GetActorTransform _returnvalue) "Undefined" "MultiplyWithRoot" 0 0))
  (bind _output_get (Variables|Default|SetStealthRadiusRef _returnvalue_2))
  (Default|SetupStealthOwner _output_get _returnvalue (Variables|Default|GetDetectionRadius) true))

(fn DetectUser
  (params (User :type Actor%20Object%20Reference))
  (Development|PrintString (Utilities|String|Append "User Detected: " (Utilities|GetDisplayName User))))

(fn LostUser
  (params (User :type Actor%20Object%20Reference))
  (Development|PrintString (Utilities|String|Append (Utilities|GetDisplayName User) " Last seen at location: " (Utilities|String|ToString(Vector) (Transformation|GetActorLocation User)))))