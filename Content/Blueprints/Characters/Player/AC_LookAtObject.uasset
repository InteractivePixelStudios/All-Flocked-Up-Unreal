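; Actor component, apparently an unfinished head look-at for the player pigeon character.
; BeginPlay caches and prints the socket rotation of BoneToMove on the pigeon's mesh.
; Every tick it passes that start rotation to LookAtObject, which only casts the player pawn and looks up a BP_Cat actor.
; No bone rotation is applied, and the "looking at cat" debug print is disconnected.
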(event Custom|TurnHeadToObject
  (CallFunction|LookatObject (Variables|Default|GetBoneStartRotation)))

(event EventBeginPlay
  (CallFunction|GetRigBone))

(event EventTick
  (params (DeltaSeconds :type Float%20%28single-precision%29))
  (CallFunction|TurnHeadtoObject))

(fn GetRigBone
  (bind _asbp_pigeon_character_ab (Utilities|Casting|CastToBP_PigeonCharacter_AB (Game|Player|GetPlayerPawn 0)))
  (bind _output_get (Variables|Default|SetBoneStartRotation (Transformation|GetSocketRotation (Variables|/Script/Engine.Character|GetMesh _asbp_pigeon_character_ab) (Variables|Default|GetBoneToMove))))
  (Development|PrintString "got bone")
  (Development|PrintString (Utilities|String|ToString(Rotator) _output_get))
  (return _output_get))

(fn LookatObject
  (params (StartingLookRotation :type Rotator))
  (bind _asbp_pigeon_character_ab (Utilities|Casting|CastToBP_PigeonCharacter_AB (Game|Player|GetPlayerPawn 0)))
  (Actor|GetActorOfClass "/Game/Blueprints/Characters/Enemies/Cat/BP_Cat.BP_Cat_C"))