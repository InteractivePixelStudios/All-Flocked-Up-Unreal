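; Player component that handles the pigeon character's poop attack, both as an aerial drop and a grounded shot.
; IA_Poo checks the poop count, spawns BP_PoopFunction at the fire point matching the flight state polled on Tick, spends one poop and applies a one-second cooldown.
; ChiliPoops grants five seconds of particle-enhanced poop, ending with an automatic poop.
; A debug key provides rough aiming by flipping the player's pitch.
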(event Custom|ChiliPoops
  ;[1 1 1] Chili Poop Powerup
  (Variables|Default|SetHasChiliPower true)
  (Utilities|FlowControl|Delay 5.0)
  (CallFunction|CallPoop)
  (Variables|Default|SetHasChiliPower false))

(event Custom|CallPoop
  ;[1 1 1] Aerial Poo Drop
  ;;[1 1 1] Is The Player Flying?
  (bind _asbp_pigeon_character_ab (Utilities|Casting|CastToBP_PigeonCharacter_AB (Game|GetPlayerCharacter 0)))
  (if (> (Variables|/Game/Blueprints/Characters/Player/BP_PoopSystem_WK.BP_PoopSystem_WK_C|GetPoopCurrent (Variables|/Game/Blueprints/Characters/Player/BP_PigeonCharacter_AB.BP_PigeonCharacter_AB_C|GetBP_PoopSystem_WK _asbp_pigeon_character_ab)) 0)
    (if (Variables|Default|GetIsFlying)
      ;;[1 1 1] Poop is spawned at the ProjectileSpawnPoint on the Player
      (Utilities|FlowControl|DoOnce false :!label _label
        (:Completed
          (bind _returnvalue (Game|SpawnActorfromClass "/Game/Blueprints/Characters/Player/BP_PoopFunction.BP_PoopFunction_C" (Math|Transform|MakeTransform (Math|Vector|MakeVector (.x (Transformation|GetWorldLocation (Variables|/Game/Blueprints/Characters/Player/BP_PigeonCharacter_AB.BP_PigeonCharacter_AB_C|GetArialPoopFirePoint _asbp_pigeon_character_ab))) (- (.y (Transformation|GetWorldLocation (Variables|/Game/Blueprints/Characters/Player/BP_PigeonCharacter_AB.BP_PigeonCharacter_AB_C|GetArialPoopFirePoint _asbp_pigeon_character_ab))) 1.0) (.z (Transformation|GetWorldLocation (Variables|/Game/Blueprints/Characters/Player/BP_PigeonCharacter_AB.BP_PigeonCharacter_AB_C|GetArialPoopFirePoint _asbp_pigeon_character_ab)))) "0, 0, 0" "0.200000,0.200000,0.200000") "AdjustIfPossibleButAlwaysSpawn" "MultiplyWithRoot" 0 0))
          (if (Variables|Default|GetHasChiliPower)
            (Components|Activation|Activate (Variables|/Game/Blueprints/Characters/Player/BP_PoopFunction.BP_PoopFunction_C|GetParticleSystem _returnvalue) false))
          (Default|LosePoop (Variables|/Game/Blueprints/Characters/Player/BP_PigeonCharacter_AB.BP_PigeonCharacter_AB_C|GetBP_PoopSystem_WK _asbp_pigeon_character_ab))
          (Utilities|FlowControl|Delay 1.0)
          (goto _label Reset)))
      (else
        ;[1 1 1] Grounded Poo Shoot
        (Utilities|FlowControl|DoOnce false :!label _label_2
          (:Completed
            (bind _returnvalue_2 (Game|SpawnActorfromClass "/Game/Blueprints/Characters/Player/BP_PoopFunction.BP_PoopFunction_C" (Math|Transform|MakeTransform (Math|Vector|MakeVector (.x (Transformation|GetWorldLocation (Variables|/Game/Blueprints/Characters/Player/BP_PigeonCharacter_AB.BP_PigeonCharacter_AB_C|GetGroundPoopFirePoint _asbp_pigeon_character_ab))) (- (.y (Transformation|GetWorldLocation (Variables|/Game/Blueprints/Characters/Player/BP_PigeonCharacter_AB.BP_PigeonCharacter_AB_C|GetGroundPoopFirePoint _asbp_pigeon_character_ab))) 1.0) (.z (Transformation|GetWorldLocation (Variables|/Game/Blueprints/Characters/Player/BP_PigeonCharacter_AB.BP_PigeonCharacter_AB_C|GetGroundPoopFirePoint _asbp_pigeon_character_ab)))) (Transformation|GetWorldRotation (Variables|/Game/Blueprints/Characters/Player/BP_PigeonCharacter_AB.BP_PigeonCharacter_AB_C|GetGroundPoopFirePoint _asbp_pigeon_character_ab)) "0.200000,0.200000,0.200000") "AdjustIfPossibleButAlwaysSpawn" "MultiplyWithRoot" 0 0))
            (if (Variables|Default|GetHasChiliPower)
              (Components|Activation|Activate (Variables|/Game/Blueprints/Characters/Player/BP_PoopFunction.BP_PoopFunction_C|GetParticleSystem _returnvalue_2) false))
            (Default|LosePoop (Variables|/Game/Blueprints/Characters/Player/BP_PigeonCharacter_AB.BP_PigeonCharacter_AB_C|GetBP_PoopSystem_WK _asbp_pigeon_character_ab))
            (Utilities|FlowControl|Delay 1.0)
            (goto _label_2 Reset)))))))

(event Custom|RotatePlayerToPoop
  (params (DeltaSeconds :type Float%20%28single-precision%29))
  (bind _returnvalue (Game|GetPlayerCharacter 0))
  (bind _returnvalue_2 (Game|GetPlayerCharacter 0))
  (bind _returnvalue_3 (Transformation|GetActorRotation _returnvalue))
  (bind _returnvalue_4 (Transformation|GetActorRotation _returnvalue_2))
  (bind (_roll _pitch _yaw) (Math|Rotator|BreakRotator _returnvalue_3))
  (bind (_roll_2 _pitch_2 _yaw_2) (Math|Rotator|BreakRotator _returnvalue_4))
  ;[1 1 1] Aiming
  (if (Variables|Default|GetIsAiming)
    (Transformation|SetActorRotation _returnvalue_2 (Math|Rotator|MakeRotator _roll_2 (+ _pitch_2 1.8e+02) _yaw_2))
    (Development|PrintString "Hello")
    (else
      (Transformation|SetActorRotation _returnvalue (Math|Rotator|MakeRotator _roll (+ _pitch 1.8e+02) _yaw))
      (Development|PrintString "Hello"))))

(event Input|EnhancedActionEvents|EnhancedInputActionIA_Poo
  (params (ActionValue :type Boolean) (ElapsedSeconds :type Float%20%28double-precision%29) (TriggeredSeconds :type Float%20%28double-precision%29) (InputAction :type Input%20Action%20Object%20Reference :default "/Game/Blueprints/Characters/Player/MaxInputs/IA_Poo.IA_Poo"))
  ;[1 1 1] Aerial Poo Drop
  ;;[1 1 1] Player Input
  ;;[1 1 1] Is The Player Flying?
  (bind _asbp_pigeon_character_ab (Utilities|Casting|CastToBP_PigeonCharacter_AB (Game|GetPlayerCharacter 0)))
  (if (> (Variables|/Game/Blueprints/Characters/Player/BP_PoopSystem_WK.BP_PoopSystem_WK_C|GetPoopCurrent (Variables|/Game/Blueprints/Characters/Player/BP_PigeonCharacter_AB.BP_PigeonCharacter_AB_C|GetBP_PoopSystem_WK _asbp_pigeon_character_ab)) 0)
    (if (Variables|Default|GetIsFlying)
      ;;[1 1 1] Poop is spawned at the ProjectileSpawnPoint on the Player
      (Utilities|FlowControl|DoOnce false :!label _label
        (:Completed
          (bind _returnvalue (Game|SpawnActorfromClass "/Game/Blueprints/Characters/Player/BP_PoopFunction.BP_PoopFunction_C" (Math|Transform|MakeTransform (Math|Vector|MakeVector (.x (Transformation|GetWorldLocation (Variables|/Game/Blueprints/Characters/Player/BP_PigeonCharacter_AB.BP_PigeonCharacter_AB_C|GetArialPoopFirePoint _asbp_pigeon_character_ab))) (- (.y (Transformation|GetWorldLocation (Variables|/Game/Blueprints/Characters/Player/BP_PigeonCharacter_AB.BP_PigeonCharacter_AB_C|GetArialPoopFirePoint _asbp_pigeon_character_ab))) 1.0) (.z (Transformation|GetWorldLocation (Variables|/Game/Blueprints/Characters/Player/BP_PigeonCharacter_AB.BP_PigeonCharacter_AB_C|GetArialPoopFirePoint _asbp_pigeon_character_ab)))) "0, 0, 0" "0.200000,0.200000,0.200000") "AdjustIfPossibleButAlwaysSpawn" "MultiplyWithRoot" 0 0))
          (if (Variables|Default|GetHasChiliPower)
            (Components|Activation|Activate (Variables|/Game/Blueprints/Characters/Player/BP_PoopFunction.BP_PoopFunction_C|GetParticleSystem _returnvalue) false))
          (Default|LosePoop (Variables|/Game/Blueprints/Characters/Player/BP_PigeonCharacter_AB.BP_PigeonCharacter_AB_C|GetBP_PoopSystem_WK _asbp_pigeon_character_ab))
          (Utilities|FlowControl|Delay 1.0)
          (goto _label Reset)))
      (else
        ;[1 1 1] Grounded Poo Shoot
        (Utilities|FlowControl|DoOnce false :!label _label_2
          (:Completed
            (bind _returnvalue_2 (Game|SpawnActorfromClass "/Game/Blueprints/Characters/Player/BP_PoopFunction.BP_PoopFunction_C" (Math|Transform|MakeTransform (Math|Vector|MakeVector (.x (Transformation|GetWorldLocation (Variables|/Game/Blueprints/Characters/Player/BP_PigeonCharacter_AB.BP_PigeonCharacter_AB_C|GetGroundPoopFirePoint _asbp_pigeon_character_ab))) (- (.y (Transformation|GetWorldLocation (Variables|/Game/Blueprints/Characters/Player/BP_PigeonCharacter_AB.BP_PigeonCharacter_AB_C|GetGroundPoopFirePoint _asbp_pigeon_character_ab))) 1.0) (.z (Transformation|GetWorldLocation (Variables|/Game/Blueprints/Characters/Player/BP_PigeonCharacter_AB.BP_PigeonCharacter_AB_C|GetGroundPoopFirePoint _asbp_pigeon_character_ab)))) (Transformation|GetWorldRotation (Variables|/Game/Blueprints/Characters/Player/BP_PigeonCharacter_AB.BP_PigeonCharacter_AB_C|GetGroundPoopFirePoint _asbp_pigeon_character_ab)) "0.200000,0.200000,0.200000") "AdjustIfPossibleButAlwaysSpawn" "MultiplyWithRoot" 0 0))
            (if (Variables|Default|GetHasChiliPower)
              (Components|Activation|Activate (Variables|/Game/Blueprints/Characters/Player/BP_PoopFunction.BP_PoopFunction_C|GetParticleSystem _returnvalue_2) false))
            (Default|LosePoop (Variables|/Game/Blueprints/Characters/Player/BP_PigeonCharacter_AB.BP_PigeonCharacter_AB_C|GetBP_PoopSystem_WK _asbp_pigeon_character_ab))
            (Utilities|FlowControl|Delay 1.0)
            (goto _label_2 Reset)))))))

(event EventTick
  (params (DeltaSeconds :type Float%20%28single-precision%29))
  (bind _pigeonref (Variables|Default|GetPigeonRef)
    (:then
      (Variables|Default|SetIsFlying (Variables|/Game/Blueprints/Characters/Player/ActorComponents/BP_PlayerFlightControl_SO.BP_PlayerFlightControl_SO_C|GetisFlying (Variables|/Game/Blueprints/Characters/Player/BP_PigeonCharacter_AB.BP_PigeonCharacter_AB_C|GetBP_PlayerFlightControl_SO _pigeonref))))
    (:else)))

(event Input|KeyboardEvents|DebugKeyH
  (params (Key :type Key%20Structure :default "None") (ActionValue :type Input%20Action%20Value%20Structure))
  ;[1 1 1] Aiming
  (:Pressed
    ;;[0.05613 0.2664 1] Rotate to pigeons forward
    (Variables|Default|SetIsAiming true)
    (CallFunction|RotatePlayertoPoop 0.0))
  (:Released
    (Variables|Default|SetIsAiming false)))