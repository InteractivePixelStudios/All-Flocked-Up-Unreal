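; Player actor component that handles the pigeon character's perch controls, relaying movement and leave requests to the referenced perch.
; When move input starts while the perch reports perching, it sets the perch's right or left direction from the X axis and calls its player-input handler.
; The LeavingPerch event asks the perch to release through JumpOffPerch.
; BeginPlay caches the pigeon pawn, and Tick continuously advances a spline distance by speed.
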(event Custom|LeavingPerch
  (CallFunction|JumpOffPerch))

(event Input|EnhancedActionEvents|EnhancedInputActionIA_Move
  (params (ActionValue :type Vector%202D%20Structure) (ElapsedSeconds :type Float%20%28double-precision%29) (TriggeredSeconds :type Float%20%28double-precision%29) (InputAction :type Input%20Action%20Object%20Reference :default "/Game/Blueprints/Characters/Player/EnhancedInput/IA_Move.IA_Move"))
  (:Started
    (bind _perchref (Variables|Default|GetPerchRef)
      (:then
        (if (Variables|/Game/Blueprints/GameplaySystems/Perch/BP_PlayerPerchSpot.BP_PlayerPerchSpot_C|GetPerching _perchref)
          (if (== (.x ActionValue) 1.0)
            (Variables|/Game/Blueprints/GameplaySystems/Perch/BP_PlayerPerchSpot.BP_PlayerPerchSpot_C|SetMovingRight _perchref true)
            (Default|CallPlayerInput _perchref)
            (else
              (Variables|/Game/Blueprints/GameplaySystems/Perch/BP_PlayerPerchSpot.BP_PlayerPerchSpot_C|SetMovingRight _perchref false)
              (Default|CallPlayerInput _perchref)))))
      (:else))))

(event EventBeginPlay
  (bind _asbp_pigeon_character_ab (Utilities|Casting|CastToBP_PigeonCharacter_AB (Game|Player|GetPlayerPawn 0)))
  (Variables|Default|SetPigeonRef _asbp_pigeon_character_ab))

(event EventTick
  (params (DeltaSeconds :type Float%20%28single-precision%29))
  (Variables|Default|SetDistanceAlongSpline (+ (* DeltaSeconds (Variables|Default|GetSplineSpeed)) (Variables|Default|GetDistanceAlongSpline))))

(fn JumpOffPerch
  (bind _perchref (Variables|Default|GetPerchRef)
    (:then
      (Default|CallLeavePerch _perchref))
    (:else)))