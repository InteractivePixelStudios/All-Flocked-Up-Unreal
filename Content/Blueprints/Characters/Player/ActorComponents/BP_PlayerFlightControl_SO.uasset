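; Player flight component for the pigeon character: a double jump starts flight, and further jumps spend stamina to flap upward.
; Tick applies custom gravity and forward glide to movement velocity, with input for steering, slow diving, air braking and full dives.
; The sprint input triggers a timed hover-stall that arcs up and back before dropping out of flight.
; A box overlap detects landing to restore walking and stamina recharge, while the mesh tilts to match each maneuver.
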(event Custom|Stall
  (Variables|Default|SetAirStall false)
  (Variables|Default|SetisFlying false)
  (CallFunction|ReturntoWalkState)
  (Utilities|FlowControl|Delay 1.5)
  (Default|SetStaminatoCharge (Variables|Default|GetstaminaSystem)))

(event Custom|InitiateFlightMode
  (bind _playerref (Variables|Default|GetPlayerRef))
  (bind _playerref_2 (Variables|Default|GetPlayerRef))
  (bind _playerref_3 (Variables|Default|GetPlayerRef))
  (if (Variables|/Game/Blueprints/Characters/Player/BP_PigeonCharacter_AB.BP_PigeonCharacter_AB_C|GetIsAiming _playerref_2)
    (Default|StopAiming _playerref_2))
  (if (not (Variables|Default|GetisFlying))
    (Default|StopSprint _playerref)
    (Variables|/Game/Blueprints/Characters/Player/BP_PigeonCharacter_AB.BP_PigeonCharacter_AB_C|SetisCrouching _playerref false)
    (Default|CancelCrouch _playerref)
    (Pawn|Components|CharacterMovement|SetMovementMode (Variables|Default|GetcharacterMovementComponent) "MOVE_Flying" 0)
    (Variables|Default|SetisFlying true)
    (Components|Activation|Activate (Variables|/Game/Blueprints/Characters/Player/BP_PigeonCharacter_AB.BP_PigeonCharacter_AB_C|GetWingRight _playerref_3) false)
    (Components|Activation|Activate (Variables|/Game/Blueprints/Characters/Player/BP_PigeonCharacter_AB.BP_PigeonCharacter_AB_C|GetWingLeft _playerref_3) false)
    (Utilities|FlowControl|Delay 0.5)
    (Variables|Default|SetWDiveCooldown true)))

(event Input|EnhancedActionEvents|EnhancedInputActionIA_FlapUp
  (params (ActionValue :type Boolean) (ElapsedSeconds :type Float%20%28double-precision%29) (TriggeredSeconds :type Float%20%28double-precision%29) (InputAction :type Input%20Action%20Object%20Reference :default "/Game/Blueprints/Characters/Player/IAactionsSebastian/IA_FlapUp.IA_FlapUp")))

(event Input|EnhancedActionEvents|EnhancedInputActionIA_Jump
  (params (ActionValue :type Boolean) (ElapsedSeconds :type Float%20%28double-precision%29) (TriggeredSeconds :type Float%20%28double-precision%29) (InputAction :type Input%20Action%20Object%20Reference :default "/Game/Blueprints/Characters/Player/EnhancedInput/IA_Jump.IA_Jump"))
  (bind _playerref (Variables|Default|GetPlayerRef))
  (bind _charactermovementcomponent (Variables|Default|GetcharacterMovementComponent))
  (:Started
    (if (not (Variables|/Game/Blueprints/Characters/Player/BP_PigeonCharacter_AB.BP_PigeonCharacter_AB_C|GetInMenu _playerref))
      ;[1 1 1] If not flying increment jump to attempt to fly
      (if (Math|Boolean|ORBoolean (Variables|Default|GetisFlying) (Variables|/Game/Blueprints/Characters/Player/BP_PigeonCharacter_AB.BP_PigeonCharacter_AB_C|GetisCrouching _playerref) (Variables|/Game/Blueprints/Characters/Player/BP_PigeonCharacter_AB.BP_PigeonCharacter_AB_C|GetIsAiming _playerref) (Variables|/Game/Blueprints/Characters/Player/BP_PigeonCharacter_AB.BP_PigeonCharacter_AB_C|GetisEnvHiding _playerref))
        (if (and (Variables|Default|GetisFlying) (!= (Variables|Default|GetFullDive) true))
          ;[1 1 1] Check if player has the stamina to Flap wings
          (bind _usedstamina (Default|UseStamina (Variables|Default|GetstaminaSystem) 1.0))
          ;[1 1 1] If stamina was used, flap upwards
          (if _usedstamina
            (Variables|Default|SetIsFlapping true)
            (Variables|/Script/Engine.MovementComponent|SetVelocity _charactermovementcomponent (Math|Vector|MakeVector (.x (Variables|/Script/Engine.MovementComponent|GetVelocity _charactermovementcomponent)) (.y (Variables|/Script/Engine.MovementComponent|GetVelocity _charactermovementcomponent)) (Variables|Default|GetFlapUpVelocity)))
            (Utilities|FlowControl|Delay 0.5)
            (Variables|Default|SetIsFlapping false)))
        (else
          (bind _result (Math|Integer|IncrementInt (Variables|Default|GetjumpCount))
            (:%20%20
              ;[1 1 1] If jumped twice then set player to flying
              (if (== _result 2)
                (Default|UseStamina (Variables|Default|GetstaminaSystem) 1.0)
                (CallFunction|InitiateFlightMode)
                (Variables|/Script/Engine.MovementComponent|SetVelocity (Variables|Default|GetcharacterMovementComponent) (Math|Vector|MakeVector (.x (Variables|/Script/Engine.MovementComponent|GetVelocity (Variables|Default|GetcharacterMovementComponent))) (.y (Variables|/Script/Engine.MovementComponent|GetVelocity (Variables|Default|GetcharacterMovementComponent))) (Variables|Default|GetFlapUpVelocity)))
                (else
                  ;[1 1 1] Else reset jump count after half second
                  (Utilities|FlowControl|RetriggerableDelay 0.5)
                  (Variables|Default|SetjumpCount 0))))))))))

(event Input|EnhancedActionEvents|EnhancedInputActionIA_FlyMove
  (params (ActionValue :type Float%20%28double-precision%29) (ElapsedSeconds :type Float%20%28double-precision%29) (TriggeredSeconds :type Float%20%28double-precision%29) (InputAction :type Input%20Action%20Object%20Reference :default "/Game/Blueprints/Characters/Player/IAactionsSebastian/IA_FlyMove.IA_FlyMove"))
  (bind _charactermovementcomponent (Variables|Default|GetcharacterMovementComponent))
  (bind _playermeshref (Variables|Default|GetPlayerMeshRef))
  (bind _playermeshref_2 (Variables|Default|GetPlayerMeshRef))
  (bind _returnvalue (Transformation|GetWorldRotation _playermeshref))
  (bind _returnvalue_2 (Transformation|GetWorldRotation _playermeshref_2))
  (:Triggered
    (if (and (Variables|Default|GetisFlying) (Variables|Default|GetWDiveCooldown)) ; Check the player is flying
      ;[1 0.1197 0] If Action Value Y is > 0 player will dive, < 0 player stalls
      (if (> ActionValue 0.0)
        ;[1 1 1] Player will dive forward and down with a small increase in gravity
        (Variables|Default|SetDiving true)
        (Variables|/Script/Engine.MovementComponent|SetVelocity _charactermovementcomponent (Math|Vector|MakeVector (.x (Variables|/Script/Engine.MovementComponent|GetVelocity _charactermovementcomponent)) (.y (Variables|/Script/Engine.MovementComponent|GetVelocity _charactermovementcomponent)) (+ (.z (Variables|/Script/Engine.MovementComponent|GetVelocity _charactermovementcomponent)) (* (/ (Variables|Default|GetGravity) 4.0) (Utilities|Time|GetWorldDeltaSeconds)))))
        (Variables|Default|SetForwardGlideSpeed (Variables|Default|GetDiveGlideSpeed))
        (Transformation|SetWorldRotation _playermeshref (Math|Rotator|MakeRotator (.roll _returnvalue) (Math|Float|Lerp (.pitch _returnvalue) (Variables|Default|GetMeshSlowDiveAngle) 0.1) (.yaw _returnvalue)) false false)
        (else
          ;[1 1 1] Set Air Stall to true
          (Variables|Default|SetAirStall true)
          (Transformation|SetWorldRotation _playermeshref_2 (Math|Rotator|MakeRotator (.roll _returnvalue_2) (Math|Float|Lerp (.pitch _returnvalue_2) (Variables|Default|GetMeshStallAngle) 0.1) (.yaw _returnvalue_2)) false false)))))
  (:Completed
    ;[1 0.1566 0] Reset Air Stall and Diving
    (Variables|Default|SetDiving false)
    (Variables|Default|SetAirStall false)
    (Variables|Default|SetForwardGlideSpeed (Variables|Default|GetBaseGlideSpeed))))

(event Input|EnhancedActionEvents|EnhancedInputActionIA_FlyRotate
  (params (ActionValue :type Float%20%28double-precision%29) (ElapsedSeconds :type Float%20%28double-precision%29) (TriggeredSeconds :type Float%20%28double-precision%29) (InputAction :type Input%20Action%20Object%20Reference :default "/Game/Blueprints/Characters/Player/IA_FlyRotate.IA_FlyRotate"))
  (bind _returnvalue (Game|Player|GetPlayerPawn 0))
  (bind _playermeshref (Variables|Default|GetPlayerMeshRef))
  (bind _fullstall (Variables|Default|GetFullStall))
  (bind _returnvalue_2 (Transformation|GetActorRotation _returnvalue))
  (bind _returnvalue_3 (Transformation|GetWorldRotation _playermeshref))
  (:Triggered
    (if (not _fullstall)
      ;[1 1 1] Rotate Player Character Left/Right
      (Transformation|SetActorRotation _returnvalue (Math|Rotator|MakeRotator (.roll _returnvalue_2) (.pitch _returnvalue_2) (+ (.yaw _returnvalue_2) (* ActionValue (Variables|Default|GetRotateSpeed)))))
      (if (Variables|Default|GetisFlying)
        (Transformation|SetWorldRotation _playermeshref (Math|Rotator|MakeRotator (Math|Float|Lerp (.roll _returnvalue_3) (* ActionValue (Variables|Default|GetMeshRotateAngle)) 0.1) (.pitch _returnvalue_3) (.yaw _returnvalue_3)) false false))))
  (:Started
    (if (not _fullstall)
      (Variables|Default|SetIsTurning true)))
  (:Canceled
    (Variables|Default|SetIsTurning false :!label _label))
  (:Completed
    (goto _label)))

(event Input|EnhancedActionEvents|EnhancedInputActionIA_SprintToggle
  (params (ActionValue :type Boolean) (ElapsedSeconds :type Float%20%28double-precision%29) (TriggeredSeconds :type Float%20%28double-precision%29) (InputAction :type Input%20Action%20Object%20Reference :default "/Game/Blueprints/Characters/Player/EnhancedInput/IA_SprintToggle.IA_SprintToggle"))
  (bind _playermeshref (Variables|Default|GetPlayerMeshRef))
  (bind _returnvalue (Transformation|GetWorldRotation _playermeshref))
  (:Started
    (if (Variables|Default|GetisFlying)
      (Variables|Default|SetStallStartZHeight (.z (Transformation|GetActorLocation (Components|GetOwner))))
      (Variables|Default|SetAirStall true)
      (Variables|Default|SetFullStall true)
      (Variables|/Script/Engine.MovementComponent|SetVelocity (Variables|Default|GetcharacterMovementComponent) "0, 0, 0")
      (Transformation|SetWorldRotation _playermeshref (Math|Rotator|MakeRotator 0.0 (.pitch _returnvalue) (.yaw _returnvalue)) false false))))

(event Input|EnhancedActionEvents|EnhancedInputActionIA_Dive
  (params (ActionValue :type Boolean) (ElapsedSeconds :type Float%20%28double-precision%29) (TriggeredSeconds :type Float%20%28double-precision%29) (InputAction :type Input%20Action%20Object%20Reference :default "/Game/Blueprints/Characters/Player/IA_Dive.IA_Dive"))
  (if (Variables|Default|GetisFlying)
    (Variables|Default|SetFullDive true)
    (CallFunction|Dive self)))

(event EventBeginPlay
  ;[1 1 1] Set Base Variables
  (CallFunction|GetParentComponents)
  (CallFunction|CalculateFlapVelocity))

(event EventTick
  (params (DeltaSeconds :type Float%20%28single-precision%29))
  (if (Variables|Default|GetisFlying)
    ;[1 1 1] If flying apply gravity and forward glide while checking if the player hit the ground
    (if (!= (Variables|Default|GetFullStall) true)
      (CallFunction|FallandGlide DeltaSeconds)
      (CallFunction|RotateBack)
      ;[1 1 1] When player hits the ground set flying to false and make the character fall to the ground
      (bind _groundcheck (CallFunction|GroundCheck))
      (if _groundcheck
        (Variables|Default|SetisFlying false)
        (CallFunction|ReturntoWalkState)
        ;[1 1 1] Reset Stamina once on ground
        (Default|SetStaminatoCharge (Variables|Default|GetstaminaSystem))
        (elif (Variables|Default|GetFullDive)
          (CallFunction|DiveRotate)
          (if (<= (.z (Transformation|GetComponentVelocity (Variables|/Script/Engine.Character|GetCapsuleComponent (Variables|Default|GetPlayerRef)))) 1e+01)
            (CallFunction|ReturntoWalkState))))
      (else
        (CallFunction|AirStallAnim DeltaSeconds)))
    (else
      (CallFunction|RotateBack))))

(fn GetParentComponents
  (bind _returnvalue (Components|GetOwner))
  ;[1 1 1] Get and set Character Movement Component from Character Component
  (Variables|Default|SetcharacterMovementComponent (Variables|/Script/Engine.Character|GetCharacterMovement (Game|GetPlayerCharacter 0)))
  ;[1 1 1] Get and set Stamina System Component from player
  (Variables|Default|SetstaminaSystem (Actor|GetComponentbyClass _returnvalue "/Game/Blueprints/Characters/Player/ActorComponents/BP_StaminaSystem_SO.BP_StaminaSystem_SO_C"))
  (bind _asbp_pigeon_character_ab (Utilities|Casting|CastToBP_PigeonCharacter_AB _returnvalue))
  (bind _output_get (Variables|Default|SetPlayerRef _asbp_pigeon_character_ab))
  (Variables|Default|SetPlayerMeshRef (Variables|/Script/Engine.Character|GetMesh _output_get)))

(fn FallandGlide
  (params (DeltaTime :type Float%20%28double-precision%29))
  (bind _returnvalue (Components|GetOwner))
  (bind _slowdownrate (Variables|Default|GetSlowDownRate))
  (bind _forwardglidespeed (Variables|Default|GetForwardGlideSpeed))
  (bind _charactermovementcomponent (Variables|Default|GetcharacterMovementComponent))
  (bind _returnvalue_2 (Transformation|GetActorForwardVector _returnvalue))
  (bind _returnvalue_3 (* _slowdownrate DeltaTime))
  (bind _returnvalue_4 (* _returnvalue_2 _forwardglidespeed))
  (Variables|/Script/Engine.MovementComponent|SetVelocity (Variables|Default|GetcharacterMovementComponent) (Math|Vector|MakeVector (.x (Variables|/Script/Engine.MovementComponent|GetVelocity (Variables|Default|GetcharacterMovementComponent))) (.y (Variables|/Script/Engine.MovementComponent|GetVelocity (Variables|Default|GetcharacterMovementComponent))) (+ (.z (Variables|/Script/Engine.MovementComponent|GetVelocity (Variables|Default|GetcharacterMovementComponent))) (* (Variables|Default|GetGravity) DeltaTime))))
  (if (not (Variables|Default|GetFullDive))
    (if (Variables|Default|GetAirStall)
      (Variables|/Script/Engine.MovementComponent|SetVelocity (Variables|Default|GetcharacterMovementComponent) (Math|Vector|MakeVector (Math|Float|Lerp (.x (Variables|/Script/Engine.MovementComponent|GetVelocity (Variables|Default|GetcharacterMovementComponent))) 0.0 _returnvalue_3) (Math|Float|Lerp (.y (Variables|/Script/Engine.MovementComponent|GetVelocity (Variables|Default|GetcharacterMovementComponent))) 0.0 _returnvalue_3) (.z (Variables|/Script/Engine.MovementComponent|GetVelocity (Variables|Default|GetcharacterMovementComponent)))))
      (else
        ;[1 1 1] Apply glide speed to the direction
        (Variables|/Script/Engine.MovementComponent|SetVelocity _charactermovementcomponent (Math|Vector|MakeVector (.x _returnvalue_4) (.y _returnvalue_4) (.z (Variables|/Script/Engine.MovementComponent|GetVelocity _charactermovementcomponent))))))))

(fn GroundCheck
  (bind _returnvalue (Game|GetPlayerCharacter 0))
  ;[1 1 1] Create box and check for collisions with terrain
  (bind _returnvalue_2 (Collision|BoxOverlapActors (- (Transformation|GetActorLocation _returnvalue) "0.000000,0.000000,12.000000") "15.000000,15.000000,10.000000" (Utilities|Array|MakeArray "ObjectTypeQuery1") 0 (Utilities|Array|MakeArray _returnvalue) :!class /Script/Engine.KismetSystemLibrary))
  ;[1 1 1] Return results of overlap check
  (return _returnvalue_2))

(fn Dive
  (bind _returnvalue (Components|GetOwner))
  (bind _returnvalue_2 (Transformation|GetActorForwardVector _returnvalue))
  (bind _returnvalue_3 (* _returnvalue_2 1e+03))
  (if (Variables|Default|GetisFlying)
    (Variables|/Script/Engine.MovementComponent|SetVelocity (Variables|Default|GetcharacterMovementComponent) (Math|Vector|MakeVector (.x _returnvalue_3) (.y _returnvalue_3) (Variables|Default|GetDiveVelocity)))))

(fn CalculateFlapVelocity
  (Variables|Default|SetFlapUpVelocity (Math|Float|Sqrt (* (Variables|Default|GetJumpHeight) (* (Math|Float|Absolute(Float) (Variables|Default|GetGravity)) 2.0)))))

(fn RotateBack
  (bind _playermeshref (Variables|Default|GetPlayerMeshRef))
  (bind _returnvalue (Transformation|GetWorldRotation _playermeshref))
  (bind _returnvalue_2 (Transformation|GetWorldRotation _playermeshref))
  (if (not (Variables|/Game/Blueprints/Characters/Player/BP_PigeonCharacter_AB.BP_PigeonCharacter_AB_C|GetIsAiming (Variables|Default|GetPlayerRef)))
    (if (Variables|Default|GetIsTurning)
      _
      (else
        (Transformation|SetWorldRotation _playermeshref (Math|Rotator|MakeRotator (Math|Float|Lerp (.roll _returnvalue_2) 0.0 0.1) (.pitch _returnvalue_2) (.yaw _returnvalue_2)) false false)))
    (if (not (Math|Boolean|ANDBoolean (Variables|Default|GetFullDive) (Variables|Default|GetDiving) (Variables|Default|GetAirStall)))
      (Transformation|SetWorldRotation _playermeshref (Math|Rotator|MakeRotator (.roll _returnvalue) (Math|Float|Lerp (.pitch _returnvalue) 0.0 0.1) (.yaw _returnvalue)) false false))))

(fn AirStallAnim
  (params (DeltaTime :type Float%20%28double-precision%29))
  (bind _returnvalue (Components|GetOwner))
  (bind _returnvalue_2 (Components|GetOwner))
  (bind _stallstartzheight (Variables|Default|GetStallStartZHeight))
  (bind _stallstartzheight_2 (Variables|Default|GetStallStartZHeight))
  (bind _returnvalue_3 (Transformation|GetActorLocation _returnvalue_2))
  (bind _returnvalue_4 (Transformation|GetActorLocation _returnvalue))
  (bind _output_get (Variables|Default|SetCurrentStallTime (+ DeltaTime (Variables|Default|GetCurrentStallTime))))
  (if (< _output_get (/ (Variables|Default|GetStallTime) 2.0))
    (Transformation|SetActorLocation _returnvalue_2 (Math|Vector|MakeVector (.x _returnvalue_3) (.y _returnvalue_3) (Math|Float|Lerp _stallstartzheight_2 (+ _stallstartzheight_2 (* (Variables|Default|GetStallHeight) 2.0)) (/ (Variables|Default|GetCurrentStallTime) (Variables|Default|GetStallTime)))) false false)
    (else
      (Transformation|SetActorLocation _returnvalue (Math|Vector|MakeVector (.x _returnvalue_4) (.y _returnvalue_4) (Math|Float|Lerp (+ (* (Variables|Default|GetStallHeight) 2.0) _stallstartzheight) _stallstartzheight (/ (Variables|Default|GetCurrentStallTime) (Variables|Default|GetStallTime)))) false false)
      (if (>= (Variables|Default|GetCurrentStallTime) (Variables|Default|GetStallTime))
        (Variables|Default|SetCurrentStallTime 0.0)
        (Variables|Default|SetFullStall false)
        (CallFunction|Stall)))))

(fn ReturntoWalkState
  (bind _playermeshref (Variables|Default|GetPlayerMeshRef))
  (bind _playerref (Variables|Default|GetPlayerRef))
  (Components|Activation|Deactivate (Variables|/Game/Blueprints/Characters/Player/BP_PigeonCharacter_AB.BP_PigeonCharacter_AB_C|GetWingRight _playerref))
  (Components|Activation|Deactivate (Variables|/Game/Blueprints/Characters/Player/BP_PigeonCharacter_AB.BP_PigeonCharacter_AB_C|GetWingLeft _playerref))
  (Variables|Default|SetisFlying false)
  (Pawn|Components|CharacterMovement|SetMovementMode (Variables|Default|GetcharacterMovementComponent) "MOVE_Falling" 0)
  (bind _asbp_pigeon_character_ab (Utilities|Casting|CastToBP_PigeonCharacter_AB (Game|Player|GetPlayerPawn 0)))
  (Default|ResizeRadius (Variables|/Game/Blueprints/Characters/Player/BP_PigeonCharacter_AB.BP_PigeonCharacter_AB_C|GetAC_StealthUser _asbp_pigeon_character_ab) (Variables|/Game/Blueprints/Characters/Player/BP_PigeonCharacter_AB.BP_PigeonCharacter_AB_C|GetWalkingStealthRadius _asbp_pigeon_character_ab))
  (Variables|Default|SetWDiveCooldown false)
  (Transformation|SetWorldRotation _playermeshref (Math|Rotator|MakeRotator 0.0 0.0 (.yaw (Transformation|GetWorldRotation _playermeshref))) false false)
  (Variables|Default|SetFullDive false))

(fn DiveRotate
  (bind _playermeshref (Variables|Default|GetPlayerMeshRef))
  (bind _returnvalue (Transformation|GetWorldRotation _playermeshref))
  (Transformation|SetWorldRotation _playermeshref (Math|Rotator|MakeRotator (.roll _returnvalue) (Math|Float|Lerp (.pitch _returnvalue) (Variables|Default|GetMeshDiveAngle) 0.2) (.yaw _returnvalue)) false false))