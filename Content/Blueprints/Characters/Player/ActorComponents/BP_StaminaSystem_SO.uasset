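; Player stamina component that handles spending, regeneration, level-up growth and accessory bonuses.
; UseStamina deducts affordable costs, returns success and pauses recharge until SetStaminaToCharge re-enables it.
; Tick uses Delay nodes to pace clamped regen after an initial wait, or skips that wait and uses a separate rate when fully depleted.
; SetAccessoryBonus rebuilds max and regen stats from base values plus primary and secondary accessory arrays.
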(event EventBeginPlay
  ;[1 1 1] At start set stamina to max amount
  (Variables|Default|Setstamina (Variables|Default|GetmaxStamina)))

(event EventTick
  (params (DeltaSeconds :type Float%20%28single-precision%29))
  (bind _regenticktime (Variables|Default|GetregenTickTime))
  ;[1 1 1] Check if stamina can charge
  (if (Variables|Default|GetstaminaCanCharge)
    ;[1 1 1] If stamina is depleted charge faster
    (if (Variables|Default|GetstaminaDepleted)
      ;[1 1 1] Start regenerating after tick time amount with increased rate
      (Utilities|FlowControl|Delay _regenticktime)
      (CallFunction|RechargeStamina (Variables|Default|GetdepletedStaminaRegenSpeed))
      (else
        (if (Variables|Default|Getdelayed)
          ;[1 1 1] Once delayed regenerate at tick time
          (Utilities|FlowControl|Delay _regenticktime)
          (else
            ;[1 1 1] With stamina not depleted delay the first regeneration
            (Utilities|FlowControl|Delay (Variables|Default|GettimeToStartRegen))
            (Variables|Default|Setdelayed true)))
        ;[1 1 1] Recharge stamina at normal speed
        (CallFunction|RechargeStamina (Variables|Default|GetstaminaRegenSpeed))))))

(event EventOnLevelUp
  ;[1 1 1] On Level Up
  (bind _result (Math|Float|IncrementFloat (Variables|Default|GetmaxStamina)) ; Increment Max by 1
    (:%20%20
      (Variables|Default|SetmaxStamina _result)
      (Development|PrintString "Max Stamina is now ")
      (Development|PrintString (Utilities|String|ToString(Float) (Variables|Default|GetmaxStamina)))
      (Variables|Default|SetstaminaCanCharge true))))

(fn UseStamina
  (params (staminaUsed :type Float%20%28double-precision%29))
  (if (>= (- (Variables|Default|Getstamina) staminaUsed) 0.0)
    ;[1 1 1] Reset all bools since stamina is being used
    (Variables|Default|SetstaminaCanCharge false)
    (Variables|Default|Setdelayed false)
    (Variables|Default|SetstaminaDepleted false)
    ;[1 1 1] Subtract stamina used from stamina
    (bind _output_get (Variables|Default|Setstamina (- (Variables|Default|Getstamina) staminaUsed)))
    ;[1 1 1] Check if stamina was fully depleted
    (if (== _output_get 0.0)
      (Variables|Default|SetstaminaDepleted true))
    ;[1 1 1] Return true, stamina was used
    (return true)
    (else
      ;[1 1 1] Returns false, no stamina used
      (return false))))

(fn SetStaminatoCharge
  ;[1 1 1] Function allows stamina to begin charging
  (Variables|Default|SetstaminaCanCharge true))

(fn RechargeStamina
  (params (rechargeRate :type Float%20%28double-precision%29))
  ;[1 1 1] Add recharge rate to stamina and clamp to Max Stamina amount
  (Variables|Default|Setstamina (Math|Float|Clamp(Float) (+ (Variables|Default|Getstamina) rechargeRate) 0.0 (Variables|Default|GetmaxStamina)))
  ;[1 1 1] Once max stamina reached, reset all bools for next use
  (if (== (Variables|Default|Getstamina) (Variables|Default|GetmaxStamina))
    (Variables|Default|SetstaminaCanCharge false)
    (Variables|Default|SetstaminaDepleted false)
    (Variables|Default|Setdelayed false)))

(fn SetAccessoryBonus
  (params (IsPrimary :type Boolean) (MaxStaminaBonus :type Float%20%28double-precision%29) (RegenSpeedBonus :type Float%20%28double-precision%29) (TickTimeBonus :type Float%20%28double-precision%29) (TimeToStartBonus :type Float%20%28double-precision%29))
  (bind _array (Utilities|Array|MakeArray MaxStaminaBonus RegenSpeedBonus TickTimeBonus TimeToStartBonus))
  (if IsPrimary
    (Variables|Default|SetPrimaryAccessory _array)
    (else
      (Variables|Default|SetSecondaryAccessory _array)))
  (for (_array_element _array_index) (Variables|Default|GetStamineBaseStats)
    (switch int _array_index
      (:Default
        (Development|PrintString "Nothing Happened"))
      (:0
        (Variables|Default|SetmaxStamina (+ _array_element (+ (Utilities|Array|Get(acopy) (Variables|Default|GetPrimaryAccessory) _array_index) (Utilities|Array|Get(acopy) (Variables|Default|GetSecondaryAccessory) _array_index)))))
      (:1
        (Variables|Default|SetstaminaRegenSpeed (+ _array_element (+ (Utilities|Array|Get(acopy) (Variables|Default|GetPrimaryAccessory) _array_index) (Utilities|Array|Get(acopy) (Variables|Default|GetSecondaryAccessory) _array_index)))))
      (:2
        (Variables|Default|SetregenTickTime (+ _array_element (+ (Utilities|Array|Get(acopy) (Variables|Default|GetPrimaryAccessory) _array_index) (Utilities|Array|Get(acopy) (Variables|Default|GetSecondaryAccessory) _array_index)))))
      (:3
        (Variables|Default|SettimeToStartRegen (+ _array_element (+ (Utilities|Array|Get(acopy) (Variables|Default|GetPrimaryAccessory) _array_index) (Utilities|Array|Get(acopy) (Variables|Default|GetSecondaryAccessory) _array_index))))))))