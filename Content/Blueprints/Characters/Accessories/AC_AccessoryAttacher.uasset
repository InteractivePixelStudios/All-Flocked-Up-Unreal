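; Component that attaches and removes cosmetic accessories on the pigeon player character.
; Attach looks up a row in DT_AccessoryTable, spawns its accessory class and snaps it to the named mesh socket, so only scale survives from the row's transform.
; Detach finds tracked accessories matching the row's class and destroys them.
; Debug keys open and close a test accessory widget.
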(event Custom|AttachToPlayer
  (params (IncomingRow :type Name))
  (bind _rowname (CallFunction|GetRowName IncomingRow))
  (bind (_accessoryname _socketname _transform _accessoryclass _output_get) (CallFunction|GetAccessoryInfo _rowname))
  (bind _returnvalue (Game|SpawnActorfromClass _output_get _transform "Undefined" "MultiplyWithRoot" 0 0))
  (Transformation|AttachComponentToComponent _returnvalue (Variables|/Script/Engine.Character|GetMesh (Variables|Default|GetPigeonRef)) _socketname "SnapToTarget" "SnapToTarget" "KeepWorld" false)
  (Utilities|Array|AddUnique (Variables|Default|GetAttachedAccessories) _returnvalue)
  (Development|PrintString "WhatHappens"))

(event Custom|DetachFromPlayer
  (params (IncomingRow :type Name))
  (bind _attachedaccessories (Variables|Default|GetAttachedAccessories))
  (bind _rowname (CallFunction|GetRowName IncomingRow))
  (bind _output_get (CallFunction|GetAccessoryInfo _rowname))
  (for (_array_element _array_index) (Variables|Default|GetAttachedAccessories)
    (if (== _output_get (Utilities|GetClass _array_element))
      (bind _output_get_2 (Variables|Default|SetTempACC (Utilities|Array|Get(acopy) _attachedaccessories _array_index)))
      (Utilities|Array|RemoveIndex _attachedaccessories _array_index)
      (Actor|DestroyActor _output_get_2))))

(event EventBeginPlay
  (Variables|Default|SetPigeonRef (CallFunction|GetPigeonCharacter)))

(event Input|KeyboardEvents|6
  (params (Key :type Key%20Structure :default "None"))
  (:Pressed
    (bind _returnvalue (UserInterface|CreateWidget "/Game/Blueprints/Characters/Accessories/WBP_TestAccessoryWidget.WBP_TestAccessoryWidget_C"))
    (UserInterface|Viewport|AddtoViewport _returnvalue 0)
    (Variables|/Script/Engine.PlayerController|SetbShowMouseCursor (Game|GetPlayerController 0) true)))

(event Input|KeyboardEvents|7
  (params (Key :type Key%20Structure :default "None"))
  (:Pressed
    (bind _foundwidgets (Widget|GetAllWidgetsOfClass "/Game/Blueprints/Characters/Accessories/WBP_TestAccessoryWidget.WBP_TestAccessoryWidget_C" true))
    (Default|CloseWidget _foundwidgets)
    (Variables|/Script/Engine.PlayerController|SetbShowMouseCursor (Game|GetPlayerController 0) true)))

(fn GetAccessoryInfo
  (params (RowName :type Name))
  (bind _returnvalue (Utilities|GetDataTableRow "/Game/Blueprints/Characters/Accessories/DT_AccessoryTable.DT_AccessoryTable" RowName)
    (:then
      (bind _output_get (Variables|Default|SetAccessory%20Name (.accessoryname _returnvalue)))
      (bind _output_get_2 (Variables|Default|SetSocket%20Name (.socketname _returnvalue)))
      (bind _output_get_3 (Variables|Default|SetTransform%20Offset (.transformoffset _returnvalue)))
      (bind _output_get_4 (Variables|Default|SetOut%20Row%20Accessory%20Class (.accessoryclass _returnvalue)))
      (return _output_get _output_get_2 _output_get_3 0 _output_get_4))))

(fn GetRowName
  (params (IncomingRow :type Name))
  (bind _output_get (Variables|Default|SetIncomingRow IncomingRow))
  (return _output_get))

(fn GetChildClass)