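; BP_Trash_Pick-up is a single-use garbage can the pigeon player can climb into.
; Pickup teleports and hides the pigeon, sets InMenu, marks the can used, and opens the BPW_Garbage_Pickup widget with a back-reference and ObjectiveID.
; ReleasePlayer restores control and visibility, placing the pigeon just above the can.
; ResetTrashCan re-arms it after resting at the nest; SpawnGarbage is an empty stub.
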(event Custom|ReleasePlayer
  (bind _asbp_pigeon_character_ab (Utilities|Casting|CastToBP_PigeonCharacter_AB (Game|Player|GetPlayerPawn 0)))
  ;[0.05613 0.2664 1] helps control, when the player is done with the garbage they come back to the game.
  (Variables|/Game/Blueprints/Characters/Player/BP_PigeonCharacter_AB.BP_PigeonCharacter_AB_C|SetInMenu _asbp_pigeon_character_ab false)
  (Transformation|Teleport _asbp_pigeon_character_ab (+ (Transformation|GetActorLocation) "0.000000,0.000000,50.000000") (Transformation|GetActorRotation _asbp_pigeon_character_ab))
  (Rendering|SetActorHiddenInGame _asbp_pigeon_character_ab false))

(event EventPickup
  (bind _returnvalue (Game|GetPlayerCharacter 0))
  ;[1 1 1] teleporting the player to the garbage-can
  (if (not (Variables|Default|GetUsed))
    (Transformation|Teleport _returnvalue (Transformation|GetActorLocation) (Transformation|GetActorRotation _returnvalue))
    (bind _returnvalue_2 (UserInterface|CreateWidget "/Game/Blueprints/Characters/Consumables/BPW_Garbage_Pick-up.BPW_Garbage_Pick-up_C" (Game|GetPlayerController 0)))
    ;[1 1 1] Creates pop-up for garbage
    (Variables|/Game/Blueprints/Characters/Consumables/BPW_Garbage_Pick-up.BPW_Garbage_Pick-up_C|SetGarbageRef _returnvalue_2 self)
    (UserInterface|Viewport|AddtoViewport _returnvalue_2 0)
    (Variables|/Game/Blueprints/Characters/Consumables/BPW_Garbage_Pick-up.BPW_Garbage_Pick-up_C|SetObjective%20ID _returnvalue_2 (Variables|Default|GetObjective%20ID))
    ;[0.05613 0.2664 1] Sets the garbage can to be in use and takes away player control. it also hides the player at the moment
    (Variables|Default|SetUsed true)
    (bind _asbp_pigeon_character_ab (Utilities|Casting|CastToBP_PigeonCharacter_AB (Game|Player|GetPlayerPawn 0)))
    (Variables|/Game/Blueprints/Characters/Player/BP_PigeonCharacter_AB.BP_PigeonCharacter_AB_C|SetInMenu _asbp_pigeon_character_ab true)
    (Rendering|SetActorHiddenInGame _asbp_pigeon_character_ab true)))

(fn ConstructionScript)

(fn ResetTrash-Can
  ;[0.05613 0.2664 1] Is called to reset the trash can after resting at nest
  (Variables|Default|SetUsed false))

(fn SpawnGarbage
  (params (IsInTrash :type Boolean)))