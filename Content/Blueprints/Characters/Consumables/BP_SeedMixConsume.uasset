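; BP_SeedMixConsume is a seed mix consumable that restores several of the pigeon's resources when consumed.
; Its ConsumableEffect event adds a fifth of max health and a tenth each of max stamina and max poop to the pigeon's current values.
; It writes directly to the health, stamina and poop system components, with no clamping in this Blueprint.
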(event EventBeginPlay
  (|CallParentFunction) ; This node is disabled and will not be called.\nDrag off pins to build functionality.
)

(event Collision|EventActorBeginOverlap
  (params (OtherActor :type Actor%20Object%20Reference))
  (|CallParentFunction OtherActor) ; This node is disabled and will not be called.\nDrag off pins to build functionality.
)

(event EventTick
  (params (DeltaSeconds :type Float%20%28single-precision%29))
  (|CallParentFunction DeltaSeconds) ; This node is disabled and will not be called.\nDrag off pins to build functionality.
)

(event EventConsumableEffect
  (params (PigeonRef :type BP%20Pigeon%20Character%20AB%20Object%20Reference%20%28by%20ref%29))
  (bind _bp_healthsystem_wk (Variables|/Game/Blueprints/Characters/Player/BP_PigeonCharacter_AB.BP_PigeonCharacter_AB_C|GetBP_HealthSystem_WK PigeonRef))
  (bind _bp_staminasystem_so (Variables|/Game/Blueprints/Characters/Player/BP_PigeonCharacter_AB.BP_PigeonCharacter_AB_C|GetBP_StaminaSystem_SO PigeonRef))
  (bind _bp_poopsystem_wk (Variables|/Game/Blueprints/Characters/Player/BP_PigeonCharacter_AB.BP_PigeonCharacter_AB_C|GetBP_PoopSystem_WK PigeonRef))
  (Variables|/Game/Blueprints/Characters/Player/ActorComponents/BP_HealthSystem_WK.BP_HealthSystem_WK_C|SetHealthCurrent _bp_healthsystem_wk (+ (Variables|/Game/Blueprints/Characters/Player/ActorComponents/BP_HealthSystem_WK.BP_HealthSystem_WK_C|GetHealthCurrent _bp_healthsystem_wk) (/ (Variables|/Game/Blueprints/Characters/Player/ActorComponents/BP_HealthSystem_WK.BP_HealthSystem_WK_C|GetHealthMax _bp_healthsystem_wk) 5)))
  (Variables|/Game/Blueprints/Characters/Player/ActorComponents/BP_StaminaSystem_SO.BP_StaminaSystem_SO_C|Setstamina _bp_staminasystem_so (+ (Variables|/Game/Blueprints/Characters/Player/ActorComponents/BP_StaminaSystem_SO.BP_StaminaSystem_SO_C|Getstamina _bp_staminasystem_so) (/ (Variables|/Game/Blueprints/Characters/Player/ActorComponents/BP_StaminaSystem_SO.BP_StaminaSystem_SO_C|GetmaxStamina _bp_staminasystem_so) 1e+01)))
  (Variables|/Game/Blueprints/Characters/Player/BP_PoopSystem_WK.BP_PoopSystem_WK_C|SetPoopCurrent _bp_poopsystem_wk (+ (Variables|/Game/Blueprints/Characters/Player/BP_PoopSystem_WK.BP_PoopSystem_WK_C|GetPoopCurrent _bp_poopsystem_wk) (/ (Variables|/Game/Blueprints/Characters/Player/BP_PoopSystem_WK.BP_PoopSystem_WK_C|GetPoopMax _bp_poopsystem_wk) 10))))

(fn ConstructionScript
  (|CallParentFunction))