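; BP_PickupEXP is an experience pickup that awards one XP when collected.
; On BeginPlay it finds the actor tagged XPManagerHolder and caches its XP manager component, with debug prints checking validity and the XP interface.
; Overlap by the pigeon character only prints an "E" prompt.
; The Pickup event destroys the actor and sends IncreaseXP to the manager.
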(event Collision|EventActorBeginOverlap
  (params (OtherActor :type Actor%20Object%20Reference))
  ;[1 1 1] Checks to see if the player is overlapping for input message
  (Utilities|Casting|CastToBP_PigeonCharacter_AB OtherActor)
  (Development|PrintText "Press \"E\" to pickup"))

(event EventPickup
  ;[1 1 1] Checks to see if the player picked up the object and deletes it
  (Actor|DestroyActor)
  ;;[1 1 1] debug message
  (Development|PrintString "item picked")
  ;[1 1 1] Sends call to XPManager
  (CallFunction|IncreaseXP 1))

(event EventBeginPlay
  (Development|PrintString "I am block!")
  (bind _outactors (Actor|GetAllActorswithTag "XPManagerHolder"))
  (Utilities|IsValid (Actor|GetComponentbyClass (Utilities|Array|Get(acopy) _outactors) 0)
    (:Is%20Valid
      (Development|PrintString "Component IS VALID" true true "(R=0.000000,G=0.660000,B=1.000000,A=1.000000)" 1e+01)
      (Development|PrintString "XP Manager Implements Interaface" (Utilities|DoesObjectImplementInterface (Actor|GetComponentbyClass (Utilities|Array|Get(acopy) _outactors) 0) "/Game/Blueprints/Characters/Player/BPI_XPInterface_JS.BPI_XPInterface_JS_C") true "(R=0.000000,G=0.660000,B=1.000000,A=1.000000)" 1e+01)
      (Variables|Default|SetXPManager (Actor|GetComponentbyClass (Utilities|Array|Get(acopy) _outactors) 0)))
    (:Is%20Not%20Valid
      (Development|PrintString "Component not valid"))))

(fn ConstructionScript)