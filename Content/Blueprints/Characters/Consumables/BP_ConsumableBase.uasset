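; Base pickup actor for consumables, collected when the player pigeon character overlaps its collider.
; At full health it adds a stackable item to the pigeon's inventory, hardcoded as bread even in this base class.
; Otherwise it calls ConsumableEffect on the pigeon immediately.
; Either way it plays a quiet pickup sound and destroys itself.
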(event OnComponentBeginOverlap(ConsumableCollider)
  (params (OverlappedComponent :type Primitive%20Component%20Object%20Reference) (OtherActor :type Actor%20Object%20Reference) (OtherComp :type Primitive%20Component%20Object%20Reference) (OtherBodyIndex :type Integer) (bFromSweep :type Boolean) (SweepResult :type Hit%20Result%20Structure%20%28by%20ref%29))
  (bind _defaultsceneroot (Variables|Default|GetDefaultSceneRoot))
  (bind _asbp_pigeon_character_ab (Utilities|Casting|CastToBP_PigeonCharacter_AB OtherActor))
  (if (== (Variables|/Game/Blueprints/Characters/Player/ActorComponents/BP_HealthSystem_WK.BP_HealthSystem_WK_C|GetHealthCurrent (Variables|/Game/Blueprints/Characters/Player/BP_PigeonCharacter_AB.BP_PigeonCharacter_AB_C|GetBP_HealthSystem_WK _asbp_pigeon_character_ab)) (Variables|/Game/Blueprints/Characters/Player/ActorComponents/BP_HealthSystem_WK.BP_HealthSystem_WK_C|GetHealthMax (Variables|/Game/Blueprints/Characters/Player/BP_PigeonCharacter_AB.BP_PigeonCharacter_AB_C|GetBP_HealthSystem_WK _asbp_pigeon_character_ab)))
    (Default|AddItemtoInventory (Variables|/Game/Blueprints/Characters/Player/BP_PigeonCharacter_AB.BP_PigeonCharacter_AB_C|GetAC_Inventory _asbp_pigeon_character_ab) (Utilities|Struct|MakeS_ItemData "BREAD" "IT'S BREAD!" "NewEnumerator0" 0 true 1 "/Game/Blueprints/Characters/Consumables/BP_BreadConsume.BP_BreadConsume_C") (Variables|/Game/Blueprints/GameplaySystems/Inventory/AC_Inventory.AC_Inventory_C|GetInventory (Variables|/Game/Blueprints/Characters/Player/BP_PigeonCharacter_AB.BP_PigeonCharacter_AB_C|GetAC_Inventory _asbp_pigeon_character_ab)))
    (else
      (CallFunction|ConsumableEffect _asbp_pigeon_character_ab)))
  (Audio|SpawnSoundAttached "/Game/Audio/Audio/SFX/Waves/Pickup/item-pick-up-38258.item-pick-up-38258" _defaultsceneroot "None" (Transformation|GetWorldLocation _defaultsceneroot) "0, 0, 0" "KeepWorldPosition" false 0.03 1.2 0.1 0 0)
  (Actor|DestroyActor))

(event EventBeginPlay)

(event Collision|EventActorBeginOverlap
  (params (OtherActor :type Actor%20Object%20Reference)))

(event EventTick
  (params (DeltaSeconds :type Float%20%28single-precision%29)))

(fn ConstructionScript)