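; Coffee consumable that gives the pigeon a temporary stamina regeneration boost.
; Its ConsumableEffect event adds a fifth of the base regen speed to the current value on the pigeon's stamina system.
; After a fixed Delay it sets regen speed back to the base value, discarding any other modifiers rather than subtracting its own bonus.
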(event EventBeginPlay
  (|CallParentFunction) ; This node is disabled and will not be called.\nDrag off pins to build functionality.
)

(event Collision|EventActorBeginOverlap
  (params (OtherActor :type Actor%20Object%20Reference))
  (|CallParentFunction OtherActor) ; This node is disabled and will not be called.\nDrag off pins to build functionality.
)

(event EventTick
  (params (DeltaSeconds :type Float%20%28single-precision%29))
  (|CallParentFunction DeltaSeconds) ; This node is disabled and will not be called.\nDrag off pins to build functionality.
)

(event EventConsumableEffect
  (params (PigeonRef :type BP%20Pigeon%20Character%20AB%20Object%20Reference%20%28by%20ref%29))
  (bind _bp_staminasystem_so (Variables|/Game/Blueprints/Characters/Player/BP_PigeonCharacter_AB.BP_PigeonCharacter_AB_C|GetBP_StaminaSystem_SO PigeonRef))
  (bind _staminaregenspeedbase (Variables|/Game/Blueprints/Characters/Player/ActorComponents/BP_StaminaSystem_SO.BP_StaminaSystem_SO_C|GetstaminaRegenSpeedBase _bp_staminasystem_so))
  (Variables|/Game/Blueprints/Characters/Player/ActorComponents/BP_StaminaSystem_SO.BP_StaminaSystem_SO_C|SetstaminaRegenSpeed _bp_staminasystem_so (+ (Variables|/Game/Blueprints/Characters/Player/ActorComponents/BP_StaminaSystem_SO.BP_StaminaSystem_SO_C|GetstaminaRegenSpeed _bp_staminasystem_so) (/ _staminaregenspeedbase 5.0)))
  (Utilities|FlowControl|Delay 1e+01)
  (Variables|/Game/Blueprints/Characters/Player/ActorComponents/BP_StaminaSystem_SO.BP_StaminaSystem_SO_C|SetstaminaRegenSpeed _bp_staminasystem_so _staminaregenspeedbase))

(fn ConstructionScript
  (|CallParentFunction))