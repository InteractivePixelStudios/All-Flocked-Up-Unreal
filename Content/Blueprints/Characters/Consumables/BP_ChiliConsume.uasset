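; BP_ChiliConsume is a chili consumable that refills the pigeon's poop meter.
; It implements the ConsumableEffect event, adding a fixed amount to PoopCurrent on the pigeon's BPPoopSystemWK with no clamp in this graph.
; The new value is printed with PrintString; the construction script only calls its parent, and the other events are disabled stubs.
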(event EventBeginPlay
  (|CallParentFunction) ; This node is disabled and will not be called.\nDrag off pins to build functionality.
)

(event Collision|EventActorBeginOverlap
  (params (OtherActor :type Actor%20Object%20Reference))
  (|CallParentFunction OtherActor) ; This node is disabled and will not be called.\nDrag off pins to build functionality.
)

(event EventTick
  (params (DeltaSeconds :type Float%20%28single-precision%29))
  (|CallParentFunction DeltaSeconds) ; This node is disabled and will not be called.\nDrag off pins to build functionality.
)

(event EventConsumableEffect
  (params (PigeonRef :type BP%20Pigeon%20Character%20AB%20Object%20Reference%20%28by%20ref%29))
  (bind _bp_poopsystem_wk (Variables|/Game/Blueprints/Characters/Player/BP_PigeonCharacter_AB.BP_PigeonCharacter_AB_C|GetBP_PoopSystem_WK PigeonRef))
  (bind _output_get (Variables|/Game/Blueprints/Characters/Player/BP_PoopSystem_WK.BP_PoopSystem_WK_C|SetPoopCurrent _bp_poopsystem_wk (+ (Variables|/Game/Blueprints/Characters/Player/BP_PoopSystem_WK.BP_PoopSystem_WK_C|GetPoopCurrent _bp_poopsystem_wk) 10)))
  (Development|PrintString (Utilities|String|ToString(Integer) _output_get)))

(fn ConstructionScript
  (|CallParentFunction))