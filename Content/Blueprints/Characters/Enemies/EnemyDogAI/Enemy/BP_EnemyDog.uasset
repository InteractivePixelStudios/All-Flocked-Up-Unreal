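; Enemy dog character that runs its AI behavior until damaged, then flees and is removed from the world.
; BeginPlay caches the mesh's ABP_CatAnims instance and the AIC_Dog controller, then flags its behavior as started.
; Damage reports the objective ID to the pigeon character and moves the dog to a random navigable point, destroying it on arrival or shortly after failure.
; RunAwayDestroy, unused here, starts a short move but destroys the dog immediately.
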(event EventBeginPlay
  (|CallParentFunction)
  (bind _asabp_cat_anims (Utilities|Casting|CastToABP_CatAnims (Components|SkeletalMesh|GetAnimInstance (Variables|Character|GetMesh))))
  (Variables|Default|SetCatAnimRef _asabp_cat_anims)
  (bind _asaic_dog (Utilities|Casting|CastToAIC_Dog (AI|GetAIController self)))
  (bind _output_get (Variables|Default|SetAs%20AIC%20Dog _asaic_dog))
  (Variables|/Game/Blueprints/Characters/Enemies/EnemyDogAI/Enemy/AIC_Dog.AIC_Dog_C|SetBehaviorStarted _output_get true))

(event EventOnTakeAnyDamageEvent
  (params (DamagedActor :type Actor%20Object%20Reference) (Damage :type Float%20%28single-precision%29) (DamageType :type Damage%20Type%20Object%20Reference) (InstigatedBy :type Controller%20Object%20Reference) (DamageCauser :type Actor%20Object%20Reference))
  (Default|CallOnObjectiveIDCalled (CallFunction|GetPigeonCharacter) (Variables|Default|GetObjective%20ID))
  (bind _randomlocation (Class|NavigationSystemV1|GetRandomLocationinNavigableRadius (Transformation|GetActorLocation) 2e+03 0 0))
  (AI|AIMoveTo (Variables|Character|GetCharacterMovement) self _randomlocation 0 1.0 true
    (:OnSuccess
      _)
    (:OnFail
      (Utilities|FlowControl|Delay 5.0)))
  (Actor|DestroyActor))

(fn ConstructionScript)

(fn RunAway&Destroy
  (AI|Navigation|SimpleMovetoLocation (AI|GetAIController self) (.RandomLocation (AI|Navigation|GetRandomReachablePointinRadius (Transformation|GetActorLocation) 1e+02 0 0)))
  (Actor|DestroyActor))