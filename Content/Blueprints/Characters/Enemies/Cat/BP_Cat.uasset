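; Enemy cat character that spots the player pigeon, pounces and damages it on contact with a cooldown.
; PawnSensing hisses at any seen pawn, then alerts and flags the AI controller unless pigeon stealth is high; Tick clears this beyond sight radius.
; Pounce launches an angled force toward a given location, while poop overlapping the capsule triggers retreat to a random nearby point.
; BeginPlay caches controller and anim references and hands MSCat to BPAPCat2.
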(event OnSeePawn(PawnSensing)
  (params (Pawn :type Pawn%20Object%20Reference))
  (Default|CallHiss)
  (bind _asbp_pigeon_character_ab (Utilities|Casting|CastToBP_PigeonCharacter_AB Pawn))
  (if (not (>= (Variables|/Game/Blueprints/Characters/Player/BP_PigeonCharacter_AB.BP_PigeonCharacter_AB_C|GetbaseStealthStat _asbp_pigeon_character_ab) 15.0))
    (Variables|Default|SetCanSeePlayer true)
    (Default|SetCanSeePlayer (Variables|Default|GetControllerRef) true)
    (if (Variables|Default|GetCanAlert)
      (CallFunction|Alert))))

(event OnComponentBeginOverlap(AttackCollider)
  (params (OverlappedComponent :type Primitive%20Component%20Object%20Reference) (OtherActor :type Actor%20Object%20Reference) (OtherComp :type Primitive%20Component%20Object%20Reference) (OtherBodyIndex :type Integer) (bFromSweep :type Boolean) (SweepResult :type Hit%20Result%20Structure%20%28by%20ref%29))
  (bind _asbp_pigeon_character_ab (Utilities|Casting|CastToBP_PigeonCharacter_AB OtherActor))
  (if (Variables|Default|GetCanAttack)
    (Variables|Default|SetCanAttack false)
    ;[0.1059 0.1059 0.1059 0.7216] Apply Damage to the player then delay ability to damage
    (Game|Damage|ApplyDamage _asbp_pigeon_character_ab (Variables|Default|GetAttackDamage) 0 0)
    (Default|CallAttack)
    (Utilities|FlowControl|Delay (Variables|Default|GetAttackCooldown))
    (Variables|Default|SetCanAttack true)))

(event OnComponentBeginOverlap(CapsuleComponent)
  (params (OverlappedComponent :type Primitive%20Component%20Object%20Reference) (OtherActor :type Actor%20Object%20Reference) (OtherComp :type Primitive%20Component%20Object%20Reference) (OtherBodyIndex :type Integer) (bFromSweep :type Boolean) (SweepResult :type Hit%20Result%20Structure%20%28by%20ref%29))
  (Utilities|Casting|CastToBP_PoopFunction OtherActor)
  (CallFunction|EnemyRetreat)
  (Development|PrintString "retreating"))

(event Custom|Pounce
  (params (PlayerLocation :type Vector))
  (bind _returnvalue (Transformation|GetActorLocation))
  (bind _returnvalue_2 (Math|Vector|GetUnitDirection(Vector) _returnvalue PlayerLocation))
  (Default|CallPounceAnim (Variables|Default|GetCatAnimRef))
  (Variables|/Script/Engine.MovementComponent|SetVelocity (Variables|Character|GetCharacterMovement) "0, 0, 0")
  (Physics|AddForce (Variables|Character|GetCharacterMovement) (* (Math|Vector|MakeVector (.x _returnvalue_2) (.y _returnvalue_2) 0.5) (Variables|Default|GetPounceForce))))

(event Custom|GetRefs
  (bind _bp_ap_cat2 (Variables|Default|GetBP_AP_Cat2))
  (Variables|/Game/Audio/Audio/Blueprints/Audio_Profiles/AudioPrfiles(v2)/BP_AP_Cat2.BP_AP_Cat2_C|SetCatRef _bp_ap_cat2 self)
  (Variables|/Game/Audio/Audio/Blueprints/Audio_Profiles/AudioPrfiles(v2)/BP_AP_Cat2.BP_AP_Cat2_C|SetMS_Cat _bp_ap_cat2 (Variables|Default|GetMS_Cat))
  (if (Utilities|IsValid (Variables|Default|GetBP_AP_Cat2))
    (if (not (Utilities|IsValid (Variables|Default|GetMS_Cat)))
      (Utilities|FlowControl|Delay 0.2 :!label _label)
      (CallFunction|GetRefs))
    (else
      (goto _label))))

(event Custom|EnemyRetreat
  (AI|AIMoveTo (Class|PawnMovementComponent|GetPawnOwner (Variables|Character|GetCharacterMovement)) (.RandomLocation (AI|Navigation|GetRandomReachablePointinRadius (Transformation|GetActorLocation) 2e+02 0 0)) self 5.0 false))

(event EventBeginPlay
  (|CallParentFunction)
  (bind _asai_cat (Utilities|Casting|CastToAI_Cat (AI|GetAIController self)))
  (Variables|Default|SetControllerRef _asai_cat)
  (bind _asabp_cat_anims (Utilities|Casting|CastToABP_CatAnims (Components|SkeletalMesh|GetAnimInstance (Variables|Character|GetMesh))))
  (Variables|Default|SetCatAnimRef _asabp_cat_anims)
  (Components|Activation|Activate (Variables|Default|GetMS_Cat) false)
  (Utilities|FlowControl|Delay 1.0)
  (CallFunction|GetRefs))

(event EventTick
  (params (DeltaSeconds :type Float%20%28single-precision%29))
  (if (Variables|Default|GetCanSeePlayer)
    (if (> (Math|Vector|Distance(Vector) (Transformation|GetActorLocation (Game|Player|GetPlayerPawn 0)) (Transformation|GetActorLocation)) (Variables|/Script/AIModule.PawnSensingComponent|GetSightRadius (Variables|Default|GetPawnSensing)))
      (bind _output_get (Variables|Default|SetCanSeePlayer false))
      (Default|SetCanSeePlayer (Variables|Default|GetControllerRef) _output_get)
      (CallFunction|ResetAlert))))

(fn ConstructionScript)