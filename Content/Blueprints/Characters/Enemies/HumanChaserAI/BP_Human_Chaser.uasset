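; BP_Human_Chaser is a human chaser enemy character that alerts when the pigeon character comes near.
; A sphere overlap with the pigeon spawns an alert notification object just above the actor's origin, plays a 2D sound, then destroys the object after a short delay.
; Pawn sensing sets the PlayerInRange blackboard key when the seen pawn casts to BP_Human_Chaser, not to the pigeon; nothing here clears it.
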(event OnSeePawn(PawnSensing)
  (params (Pawn :type Pawn%20Object%20Reference))
  (Utilities|Casting|CastToBP_Human_Chaser Pawn)
  (AI|Components|Blackboard|SetValueasBool (AI|GetBlackboard (AI|GetAIController 0)) (Utilities|Name|MakeLiteralName "PlayerInRange") true))

(event OnComponentBeginOverlap(Sphere)
  (params (OverlappedComponent :type Primitive%20Component%20Object%20Reference) (OtherActor :type Actor%20Object%20Reference) (OtherComp :type Primitive%20Component%20Object%20Reference) (OtherBodyIndex :type Integer) (bFromSweep :type Boolean) (SweepResult :type Hit%20Result%20Structure%20%28by%20ref%29))
  (bind _returnvalue (Transformation|GetActorTransform))
  (Utilities|Casting|CastToBP_PigeonCharacter_AB OtherActor)
  (bind _returnvalue_2 (Game|SpawnActorfromClass "/Game/Blueprints/Characters/Enemies/BP_AlertNotificationObject_WK.BP_AlertNotificationObject_WK_C" (Math|Transform|MakeTransform (+ (.location _returnvalue) "0.000000,0.000000,10.000000") (.rotation _returnvalue) (.scale _returnvalue)) "Undefined" "MultiplyWithRoot" 0 0))
  (Audio|PlaySound2D "/Game/Audio/SFX/funny-sound-effect-for-quotjack-in-the-boxquot-sound-ver1-110923.funny-sound-effect-for-quotjack-in-the-boxquot-sound-ver1-110923" 1.0 1.0 0.0 0 0)
  (Utilities|FlowControl|Delay 1.0)
  (Actor|DestroyActor _returnvalue_2))

(event EventBeginPlay)

(fn ConstructionScript)