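; BP_BaseEnemy is a base enemy character that can carry a consumable item and reacts to taking damage.
; On BeginPlay it caches the pigeon character and shows any held item's mesh.
; Damage drops the item as a spawned actor, reports ObjectiveID to the pigeon and halts movement, using the damage amount as stun seconds before moving to a random navigable point.
; Alert spawns a notification above the capsule and clears CanAlert until ResetAlert.
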(event Custom|Alert
  (bind _self self)
  (bind _returnvalue (Transformation|GetActorTransform _self))
  (Variables|Default|SetCanAlert false)
  (Game|SpawnActorfromClass "/Game/Blueprints/Characters/Enemies/BP_AlertNotificationObject_WK.BP_AlertNotificationObject_WK_C" (Math|Transform|MakeTransform (Math|Vector|MakeVector (.x (.location _returnvalue)) (.y (.location _returnvalue)) (+ (.z (.location _returnvalue)) (.z (.BoxExtent (Collision|GetComponentBounds (Variables|Collision|GetCapsuleComponent)))))) (.rotation _returnvalue) (.scale _returnvalue)) "Undefined" "MultiplyWithRoot" 0 0))

(event Custom|OnTakeAnyDamage_Event
  (params (DamagedActor :type Actor%20Object%20Reference) (Damage :type Float%20%28single-precision%29) (DamageType :type Damage%20Type%20Object%20Reference) (InstigatedBy :type Controller%20Object%20Reference) (DamageCauser :type Actor%20Object%20Reference))
  (bind _charactermovement (Variables|Character|GetCharacterMovement))
  (Pawn|Components|CharacterMovement|DisableMovement _charactermovement)
  (CallFunction|DropItem)
  (Default|CallOnObjectiveIDCalled (CallFunction|GetPigeonCharacter) (Variables|Default|GetObjective%20ID))
  (Utilities|FlowControl|RetriggerableDelay Damage)
  (Pawn|Components|CharacterMovement|SetMovementMode _charactermovement "MOVE_Walking" 0)
  (bind _randomlocation (Class|NavigationSystemV1|GetRandomLocationinNavigableRadius (Transformation|GetActorLocation) 2e+03 0 0))
  (AI|AIMoveTo (Variables|Character|GetCharacterMovement) self _randomlocation 0 1.0 true
    (:OnSuccess
      _)
    (:OnFail
      _))
  (Utilities|FlowControl|Delay 5.0))

(event Custom|ResetAlert
  (Variables|Default|SetCanAlert true))

(event EventBeginPlay
  (bind _holditempoint (Variables|Default|GetHoldItemPoint))
  (bind _helditem (Variables|Default|GetHeldItem))
  (bind _consumablemesh (Variables|/Game/Blueprints/Characters/Consumables/BP_ConsumableBase.BP_ConsumableBase_C|GetConsumableMesh _helditem))
  (EventDispatchers|AssignOnTakeAnyDamage (delegate Custom|OnTakeAnyDamage_Event))
  (bind _returnvalue (Actor|GetActorOfClass "/Game/Blueprints/Characters/Player/BP_PigeonCharacter_AB.BP_PigeonCharacter_AB_C"))
  (Variables|Default|SetPigeonRef _returnvalue)
  (if (Variables|Default|GetHasItem)
    (Components|StaticMesh|SetStaticMesh _holditempoint (Variables|/Script/Engine.StaticMeshComponent|GetStaticMesh _consumablemesh))
    (Rendering|Material|SetMaterial _holditempoint 0 (Rendering|Material|GetMaterial _consumablemesh 0))))

(fn ConstructionScript)

(fn GetQuestBaseRef
  (bind _returnvalue (Actor|GetActorOfClass "/Game/Blueprints/GameplaySystems/Quest/QuestSystem/BP_QuestsBase.BP_QuestsBase_C"))
  (Variables|Default|SetQuestBaseRef _returnvalue))

(fn DropItem
  (bind _holditempoint (Variables|Default|GetHoldItemPoint))
  (if (Variables|Default|GetHasItem)
    (Variables|Default|SetHasItem false)
    (Game|SpawnActorfromClass (Utilities|GetClass (Variables|Default|GetHeldItem)) (Transformation|GetWorldTransform (Variables|Default|GetHoldItemPoint)) "Undefined" "MultiplyWithRoot" 0 0)
    (Components|StaticMesh|SetStaticMesh _holditempoint 0)
    (Rendering|Material|SetMaterial _holditempoint 0 0)))

(fn RunAway)