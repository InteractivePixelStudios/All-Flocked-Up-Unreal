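; AI controller for the human chase enemy, running a behavior tree that hunts the pigeon player character.
; On begin play it writes the enemy's patrol-point flag to the blackboard.
; Pawn sensing flags the pigeon as seen unless its stealth stat is high enough, updating the blackboard target and alerting the enemy if able.
; Tick clears sight and resets the alert once the player leaves the sight radius.
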(event OnSeePawn(PawnSensing)
  (params (Pawn :type Pawn%20Object%20Reference))
  (bind _ownerref (Variables|Default|GetOwnerRef))
  (bind _asbp_pigeon_character_ab (Utilities|Casting|CastToBP_PigeonCharacter_AB Pawn))
  (Variables|Default|SetTargetRef _asbp_pigeon_character_ab)
  (if (not (>= (Variables|/Game/Blueprints/Characters/Player/BP_PigeonCharacter_AB.BP_PigeonCharacter_AB_C|GetbaseStealthStat _asbp_pigeon_character_ab) 15.0))
    (bind _output_get (Variables|Default|SetCanSeePlayer true))
    (CallFunction|SetCanSeePlayer _asbp_pigeon_character_ab _output_get)
    (if (Variables|/Game/Blueprints/Characters/Enemies/HumanChase/BP_BaseEnemy.BP_BaseEnemy_C|GetCanAlert _ownerref)
      (Default|Alert _ownerref))))

(event EventBeginPlay
  (AI|RunBehaviorTree "/Game/Blueprints/Characters/Enemies/HumanChase/BT_ChaseAI.BT_ChaseAI")
  (bind _asbp_enemy_chase_human (Utilities|Casting|CastToBP_EnemyChaseHuman (Pawn|GetControlledPawn)))
  (AI|Components|Blackboard|SetValueasBool (Variables|Default|GetBlackboard) (Variables|/Game/Blueprints/Characters/Enemies/HumanChase/BP_EnemyChaseHuman.BP_EnemyChaseHuman_C|GetBBPatrol%20Point%20Bool _asbp_enemy_chase_human) (Variables|/Game/Blueprints/Characters/Enemies/HumanChase/BP_EnemyChaseHuman.BP_EnemyChaseHuman_C|GetPatrolPoints _asbp_enemy_chase_human))
  (Variables|Default|SetOwnerRef _asbp_enemy_chase_human))

(event EventTick
  (params (DeltaSeconds :type Float%20%28single-precision%29))
  (if (Variables|Default|GetCanSeePlayer)
    (if (> (Math|Vector|Distance(Vector) (Transformation|GetActorLocation (Variables|Default|GetTargetRef)) (Transformation|GetActorLocation (Variables|Default|GetOwnerRef))) (Variables|/Script/AIModule.PawnSensingComponent|GetSightRadius (Variables|Default|GetPawnSensing)))
      (bind _output_get (Variables|Default|SetCanSeePlayer false))
      (CallFunction|SetCanSeePlayer 0 _output_get)
      (Default|ResetAlert (Variables|Default|GetOwnerRef)))))

(fn ConstructionScript)

(fn SetCanSeePlayer
  (params (PlayerTarget :type Pawn%20Object%20Reference) (CanSeePlayer :type Boolean))
  (bind _blackboard (Variables|Default|GetBlackboard))
  (AI|Components|Blackboard|SetValueasBool _blackboard (Variables|Default|GetBBCanSeePlayer) CanSeePlayer)
  (AI|Components|Blackboard|SetValueasObject _blackboard (Variables|Default|GetBBPlayerTarget) PlayerTarget))