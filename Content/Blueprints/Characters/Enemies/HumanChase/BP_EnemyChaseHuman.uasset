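; Human chasing enemy Blueprint that builds a modular character with randomized clothing.
; The construction script slaves the clothing, brows, nose and headgear meshes to the body mesh via leader pose.
; On BeginPlay, after the parent's logic, it picks random shirt, pants, shoes and headgear meshes from the DT_Clothes data table.
; Each tick it snaps HoldItemPoint to the right mitten bone's world location and rotation.
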(event EventBeginPlay
  (|CallParentFunction)
  (CallFunction|RandomClothes))

(event EventTick
  (params (DeltaSeconds :type Float%20%28single-precision%29))
  (bind _mesh (Variables|Character|GetMesh))
  (bind _returnvalue (Transformation|GetBoneTransform _mesh "MaleNPC_Right_Mitten1_DEF" "RTS_World"))
  (Transformation|SetWorldTransform (Variables|Default|GetHoldItemPoint) (Math|Transform|MakeTransform (.location _returnvalue) (.rotation _returnvalue) "1.000000,1.000000,1.000000") false false))

(fn ConstructionScript
  (bind _mesh (Variables|Character|GetMesh))
  (Components|SkinnedMesh|SetLeaderPoseComponent (Variables|Default|GetShoes) _mesh false false)
  (Components|SkinnedMesh|SetLeaderPoseComponent (Variables|Default|GetPants) _mesh false false)
  (Components|SkinnedMesh|SetLeaderPoseComponent (Variables|Default|GetShirt) _mesh false false)
  (Components|SkinnedMesh|SetLeaderPoseComponent (Variables|Default|GetBrows) _mesh false false)
  (Components|SkinnedMesh|SetLeaderPoseComponent (Variables|Default|GetNose) _mesh false false)
  (Components|SkinnedMesh|SetLeaderPoseComponent (Variables|Default|GetHeadGear) _mesh false false))

(fn RandomClothes
  (bind _returnvalue (Utilities|GetDataTableRow "/Game/Art/Characters/Enemies/Human/NPCs/DT_Clothes.DT_Clothes" "Clothes")
    (:then
      (Components|SkeletalMesh|SetSkeletalMeshAsset (Variables|Default|GetShirt) (Utilities|Array|Get(acopy) (.shirts _returnvalue) (Math|Random|RandomIntegerinRange 0 (- (Utilities|Array|Length (.shirts _returnvalue)) 1))))
      (Components|SkeletalMesh|SetSkeletalMeshAsset (Variables|Default|GetPants) (Utilities|Array|Get(acopy) (.pants _returnvalue) (Math|Random|RandomIntegerinRange 0 (- (Utilities|Array|Length (.pants _returnvalue)) 1))))
      (Components|SkeletalMesh|SetSkeletalMeshAsset (Variables|Default|GetShoes) (Utilities|Array|Get(acopy) (.shoes _returnvalue) (Math|Random|RandomIntegerinRange 0 (- (Utilities|Array|Length (.shoes _returnvalue)) 1))))
      (Components|SkeletalMesh|SetSkeletalMeshAsset (Variables|Default|GetHeadGear) (Utilities|Array|Get(acopy) (.headgear _returnvalue) (Math|Random|RandomIntegerinRange 0 (- (Utilities|Array|Length (.headgear _returnvalue)) 1)))))))