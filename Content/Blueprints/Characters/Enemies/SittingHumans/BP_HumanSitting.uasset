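; Modular seated human character that gets a randomized outfit and face when play begins.
; The construction script makes clothing, headgear, brow and nose meshes follow the Human mesh through leader pose.
; On BeginPlay, RandomClothes reads the Clothes row of DT_Clothes and assigns each part a random skeletal mesh from its matching array.
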(event EventBeginPlay
  (CallFunction|RandomClothes))

(fn ConstructionScript
  (bind _human (Variables|Default|GetHuman))
  (Components|SkinnedMesh|SetLeaderPoseComponent (Variables|Default|GetShoes) _human false false)
  (Components|SkinnedMesh|SetLeaderPoseComponent (Variables|Default|GetPants) _human false false)
  (Components|SkinnedMesh|SetLeaderPoseComponent (Variables|Default|GetShirt) _human false false)
  (Components|SkinnedMesh|SetLeaderPoseComponent (Variables|Default|GetBrows) _human false false)
  (Components|SkinnedMesh|SetLeaderPoseComponent (Variables|Default|GetNose) _human false false)
  (Components|SkinnedMesh|SetLeaderPoseComponent (Variables|Default|GetHeadGear) _human false false))

(fn RandomClothes
  (bind _returnvalue (Utilities|GetDataTableRow "/Game/Art/Characters/Enemies/Human/NPCs/DT_Clothes.DT_Clothes" "Clothes")
    (:then
      (Components|SkeletalMesh|SetSkeletalMeshAsset (Variables|Default|GetShirt) (Utilities|Array|Get(acopy) (.shirts _returnvalue) (Math|Random|RandomIntegerinRange 0 (- (Utilities|Array|Length (.shirts _returnvalue)) 1))))
      (Components|SkeletalMesh|SetSkeletalMeshAsset (Variables|Default|GetPants) (Utilities|Array|Get(acopy) (.pants _returnvalue) (Math|Random|RandomIntegerinRange 0 (- (Utilities|Array|Length (.pants _returnvalue)) 1))))
      (Components|SkeletalMesh|SetSkeletalMeshAsset (Variables|Default|GetShoes) (Utilities|Array|Get(acopy) (.shoes _returnvalue) (Math|Random|RandomIntegerinRange 0 (- (Utilities|Array|Length (.shoes _returnvalue)) 1))))
      (Components|SkeletalMesh|SetSkeletalMeshAsset (Variables|Default|GetHeadGear) (Utilities|Array|Get(acopy) (.headgear _returnvalue) (Math|Random|RandomIntegerinRange 0 (- (Utilities|Array|Length (.headgear _returnvalue)) 1))))
      (Components|SkeletalMesh|SetSkeletalMeshAsset (Variables|Default|GetBrows) (Utilities|Array|Get(acopy) (.brows _returnvalue) (Math|Random|RandomIntegerinRange 0 (- (Utilities|Array|Length (.brows _returnvalue)) 1))))
      (Components|SkeletalMesh|SetSkeletalMeshAsset (Variables|Default|GetNose) (Utilities|Array|Get(acopy) (.noses _returnvalue) (Math|Random|RandomIntegerinRange 0 (- (Utilities|Array|Length (.noses _returnvalue)) 1)))))))