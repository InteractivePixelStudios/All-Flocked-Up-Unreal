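; Red-tailed hawk enemy that perches until pawn sensing spots the pigeon player, then alerts and gives chase.
; BeginPlay caches BP_PerchLocation actors and flies to the nearest; Tick re-perches or follows, launching upward when not above the player.
; FollowPlayer uses AIMoveTo, triggers a close-range velocity-boost Attack, and retreats to perch through a retriggerable delay.
; Capsule hits damage the pigeon's health; RandomRoam is defined but not started here.
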(event OnSeePawn(PawnSensing)
  (params (Pawn :type Pawn%20Object%20Reference))
  ;[1 1 1] Set Can See Player on Pawn sensing
  (Utilities|Casting|CastToBP_PigeonCharacter_AB Pawn)
  (Variables|Default|SetIsSeeingPlayer true)
  (if (Variables|Default|GetCanAlert)
    (CallFunction|Alert)))

(event OnComponentHit(CapsuleComponent)
  (params (HitComponent :type Primitive%20Component%20Object%20Reference) (OtherActor :type Actor%20Object%20Reference) (OtherComp :type Primitive%20Component%20Object%20Reference) (NormalImpulse :type Vector :default "0, 0, 0") (Hit :type Hit%20Result%20Structure%20%28by%20ref%29))
  ;[1 1 1] Player takes damage on collision
  (bind _asbp_pigeon_character_ab (Utilities|Casting|CastToBP_PigeonCharacter_AB OtherActor))
  (Default|LoseHealth (Variables|/Game/Blueprints/Characters/Player/BP_PigeonCharacter_AB.BP_PigeonCharacter_AB_C|GetBP_HealthSystem_WK _asbp_pigeon_character_ab) 1)
  (Utilities|FlowControl|Delay 1.0))

(event Custom|RandomRoam
  ;[1 1 1] Random Roam Logic
  (AI|AIMoveTo (Variables|Default|GetAC_Redtail) self (.RandomLocation (AI|Navigation|GetRandomReachablePointinRadius (Transformation|GetActorLocation) 2e+02 0 0)) 0 5.0 false
    (:OnSuccess
      (CallFunction|RandomRoam))))

(event Custom|Perch
  (bind _returnvalue (Transformation|GetActorLocation))
  (bind _perchreference (Variables|Default|GetPerchReference))
  (bind _returnvalue_2 (Actor|FindNearestActor _returnvalue _perchreference))
  ;[1 1 1] Perch Logic
  (Utilities|FlowControl|Sequence
    (:then_0
      (AI|AIMoveTo self (Transformation|GetActorLocation _returnvalue_2) _returnvalue_2 0.1 false
        (:OnSuccess
          (Components|Movement|StopMovementImmediately (Variables|Character|GetCharacterMovement)))))))

(event Custom|FollowPlayer
  ;[1 1 1] Follow Player Logic
  (Variables|Default|SetCanAttack true)
  (if (Variables|Default|GetIsSeeingPlayer)
    (Utilities|FlowControl|Sequence
      (:then_0
        (AI|AIMoveTo self (Variables|Default|GetPlayerLocation) (Game|GetPlayerCharacter 0) 0.1 false
          (:OnSuccess
            (if (Variables|Default|GetCanAttack)
              (Variables|Default|SetCanAttack false)
              (CallFunction|Attack)))))
      (:then_1
        (Utilities|FlowControl|RetriggerableDelay 3.0)
        (CallFunction|Perch)))
    (else
      (Variables|Default|SetIsSeeingPlayer false)
      (CallFunction|ResetAlert))))

(event EventBeginPlay
  ;[1 1 1] Get Perch Locations and set AI to perch
  (|CallParentFunction)
  (bind _outactors (Actor|GetAllActorsOfClass "/Game/Blueprints/Characters/Enemies/RedTailHawkAI/BP_PerchLocation.BP_PerchLocation_C"))
  (Variables|Default|SetPerchReference _outactors)
  (CallFunction|Perch))

(event EventTick
  (params (DeltaSeconds :type Float%20%28single-precision%29))
  (bind _returnvalue (Transformation|GetActorLocation))
  (bind _returnvalue_2 (Game|GetPlayerController 0))
  (bind _returnvalue_3 (Game|GetPlayerCharacter 0))
  (bind _returnvalue_4 (Transformation|GetActorLocation _returnvalue_3))
  (bind _returnvalue_5 (Transformation|GetActorLocation _returnvalue_2))
  (bind (_x _y _z) (Math|Vector|BreakVector _returnvalue))
  (bind (_x_2 _y_2 _z_2) (Math|Vector|BreakVector _returnvalue_4))
  (Variables|Default|SetPlayerLocation _returnvalue_5)
  (bind _outhit (Collision|LineTraceByChannel (Transformation|GetActorLocation) _returnvalue_5 "TraceTypeQuery2" false 0 "ForOneFrame"))
  (Variables|Default|SetNewLocation (.location _outhit))
  ;[1 1 1] Event tick to check if seeing player
  (if (Variables|Default|GetIsSeeingPlayer)
    (CallFunction|FollowPlayer)
    (if (> _z _z_2)
      (CallFunction|FollowPlayer :!label _label)
      (else
        (Utilities|FlowControl|Sequence
          (:then_0
            (Character|LaunchCharacter (+ (* (Math|Vector|Normalize (+ _returnvalue _returnvalue_4) 1.0) (Math|Vector|GetForwardVector (Transformation|GetActorRotation))) (Math|Vector|MakeVector (- _x_2 _x) 0.0 3.5e+02)) true true)
            (CallFunction|FollowPlayer))
          (:then_1
            (goto _label)))))
    (else
      (CallFunction|Perch)
      (CallFunction|ResetAlert))))

(fn ConstructionScript)

(fn Attack
  (bind _capsulecomponent (Variables|Default|GetCapsuleComponent))
  (if (<= (Math|Vector|Distance(Vector) (Transformation|GetActorLocation (Game|GetPlayerController 0)) (Transformation|GetWorldLocation _capsulecomponent)) 0.5)
    (Variables|/Script/Engine.MovementComponent|SetVelocity (Variables|Character|GetCharacterMovement) (* (Transformation|GetComponentVelocity _capsulecomponent) 2))))