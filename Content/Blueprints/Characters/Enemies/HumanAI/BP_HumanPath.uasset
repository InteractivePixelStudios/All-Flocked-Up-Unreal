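; BP_HumanPath is a spline-based looping path actor, filed with the human AI enemy Blueprints.
; The Pathing event advances the PathPoint index and wraps it to zero when it reaches the spline's point count.
; GetLocationofSlinePoint returns the world location of the current point.
; The construction script calls that getter without using the result.
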(event Custom|Pathing
  (bind _output_get (Variables|Default|SetPathPoint (+ (Variables|Default|GetPathPoint) 1)))
  (if (== _output_get (Spline|GetNumberOfSplinePoints (Variables|Default|GetSpline)))
    (Variables|Default|SetPathPoint 0)))

(event EventBeginPlay)

(event Collision|EventActorBeginOverlap
  (params (OtherActor :type Actor%20Object%20Reference)))

(event EventTick
  (params (DeltaSeconds :type Float%20%28single-precision%29)))

(fn ConstructionScript
  (CallFunction|GetLocationofSlinePoint))

(fn GetLocationofSlinePoint
  (return (Spline|GetLocationatSplinePoint (Variables|Default|GetSpline) (Variables|Default|GetPathPoint) "World")))