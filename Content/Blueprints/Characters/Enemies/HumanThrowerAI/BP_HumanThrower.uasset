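; Human thrower enemy that spots the pigeon player unless its stealth stat is high enough, then turns to face it.
; Pawn sensing sets CanSeePlayer on its AI_HumanThrower controller and can trigger an alert; Tick rotates the capsule toward the player and resets the alert beyond sight radius.
; Modular clothing and face meshes follow the body via leader pose and are randomized from DT_Clothes on BeginPlay.
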(event OnSeePawn(PawnSensing)
  (params (Pawn :type Pawn%20Object%20Reference))
  (bind _asbp_pigeon_character_ab (Utilities|Casting|CastToBP_PigeonCharacter_AB Pawn))
  (if (not (>= (Variables|/Game/Blueprints/Characters/Player/BP_PigeonCharacter_AB.BP_PigeonCharacter_AB_C|GetbaseStealthStat _asbp_pigeon_character_ab) 15.0))
    (bind _output_get (Variables|Default|SetCanSeePlayer true))
    (Default|SetCanSeePlayer (Variables|Default|GetControllerRef) _output_get)
    (if (Variables|Default|GetCanAlert)
      (CallFunction|Alert))))

(event EventBeginPlay
  (bind _bp_ap_human (Variables|Default|GetBP_AP_Human))
  (|CallParentFunction)
  (bind _asai_human_thrower (Utilities|Casting|CastToAI_HumanThrower (AI|GetAIController self)))
  (Variables|Default|SetControllerRef _asai_human_thrower)
  (CallFunction|RandomClothes)
  (Variables|/Game/Audio/Audio/Blueprints/Audio_Profiles/AudioPrfiles(v2)/BP_AP_Human.BP_AP_Human_C|SetMS_Human _bp_ap_human (Variables|Default|GetMS_Human))
  (Variables|/Game/Audio/Audio/Blueprints/Audio_Profiles/AudioPrfiles(v2)/BP_AP_Human.BP_AP_Human_C|SetHumanReference _bp_ap_human self))

(event EventTick
  (params (DeltaSeconds :type Float%20%28single-precision%29))
  (if (Variables|Default|GetCanSeePlayer)
    (if (> (Math|Vector|Distance(Vector) (Transformation|GetActorLocation (Game|Player|GetPlayerPawn 0)) (Transformation|GetActorLocation)) (Variables|/Script/AIModule.PawnSensingComponent|GetSightRadius (Variables|Default|GetPawnSensing)))
      (bind _output_get (Variables|Default|SetCanSeePlayer false))
      (Default|SetCanSeePlayer (Variables|Default|GetControllerRef) _output_get)
      (CallFunction|ResetAlert)
      (else
        (Transformation|SetWorldRotation (Variables|Default|GetCapsuleComponent) (Math|Rotator|MakeRotator 0.0 0.0 (.yaw (Math|Rotator|FindLookatRotation (Transformation|GetActorLocation self) (Transformation|GetActorLocation (Game|Player|GetPlayerPawn 0))))) false false)))))

(fn ConstructionScript
  (bind _mesh (Variables|Character|GetMesh))
  (Components|SkinnedMesh|SetLeaderPoseComponent (Variables|Default|GetShoes) _mesh false false)
  (Components|SkinnedMesh|SetLeaderPoseComponent (Variables|Default|GetPants) _mesh false false)
  (Components|SkinnedMesh|SetLeaderPoseComponent (Variables|Default|GetShirt) _mesh false false)
  (Components|SkinnedMesh|SetLeaderPoseComponent (Variables|Default|GetBrows) _mesh false false)
  (Components|SkinnedMesh|SetLeaderPoseComponent (Variables|Default|GetNose) _mesh false false)
  (Components|SkinnedMesh|SetLeaderPoseComponent (Variables|Default|GetHeadGear) _mesh false false))

(fn RandomClothes
  (bind _returnvalue (Utilities|GetDataTableRow "/Game/Art/Characters/Enemies/Human/NPCs/DT_Clothes.DT_Clothes" "Clothes")
    (:then
      (Components|SkeletalMesh|SetSkeletalMeshAsset (Variables|Default|GetShirt) (Utilities|Array|Get(acopy) (.shirts _returnvalue) (Math|Random|RandomIntegerinRange 0 (- (Utilities|Array|Length (.shirts _returnvalue)) 1))))
      (Components|SkeletalMesh|SetSkeletalMeshAsset (Variables|Default|GetPants) (Utilities|Array|Get(acopy) (.pants _returnvalue) (Math|Random|RandomIntegerinRange 0 (- (Utilities|Array|Length (.pants _returnvalue)) 1))))
      (Components|SkeletalMesh|SetSkeletalMeshAsset (Variables|Default|GetShoes) (Utilities|Array|Get(acopy) (.shoes _returnvalue) (Math|Random|RandomIntegerinRange 0 (- (Utilities|Array|Length (.shoes _returnvalue)) 1))))
      (Components|SkeletalMesh|SetSkeletalMeshAsset (Variables|Default|GetHeadGear) (Utilities|Array|Get(acopy) (.headgear _returnvalue) (Math|Random|RandomIntegerinRange 0 (- (Utilities|Array|Length (.headgear _returnvalue)) 1))))
      (Components|SkeletalMesh|SetSkeletalMeshAsset (Variables|Default|GetBrows) (Utilities|Array|Get(acopy) (.brows _returnvalue) (Math|Random|RandomIntegerinRange 0 (- (Utilities|Array|Length (.brows _returnvalue)) 1))))
      (Components|SkeletalMesh|SetSkeletalMeshAsset (Variables|Default|GetNose) (Utilities|Array|Get(acopy) (.noses _returnvalue) (Math|Random|RandomIntegerinRange 0 (- (Utilities|Array|Length (.noses _returnvalue)) 1)))))))