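; BP_SittingHuman is a modular human character, filed under enemies, that gets a randomized outfit and face at spawn.
; The construction script makes the shoes, pants, shirt, brow, nose and hat meshes follow the main Mesh as leader pose, so they animate together.
; On BeginPlay, RandomClothes reads the Clothes row of DT_Clothes and picks a random skeletal mesh for each part from its array.
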(event EventBeginPlay
  (CallFunction|RandomClothes))

(event Collision|EventActorBeginOverlap
  (params (OtherActor :type Actor%20Object%20Reference)))

(event EventTick
  (params (DeltaSeconds :type Float%20%28single-precision%29)))

(fn ConstructionScript
  (bind _mesh (Variables|Default|GetMesh))
  (Components|SkinnedMesh|SetLeaderPoseComponent (Variables|Default|GetShoes) _mesh false false)
  (Components|SkinnedMesh|SetLeaderPoseComponent (Variables|Default|GetPants) _mesh false false)
  (Components|SkinnedMesh|SetLeaderPoseComponent (Variables|Default|GetShirt) _mesh false false)
  (Components|SkinnedMesh|SetLeaderPoseComponent (Variables|Default|GetBrow) _mesh false false)
  (Components|SkinnedMesh|SetLeaderPoseComponent (Variables|Default|GetNose) _mesh false false)
  (Components|SkinnedMesh|SetLeaderPoseComponent (Variables|Default|GetHat) _mesh false false))

(fn RandomClothes
  (bind _returnvalue (Utilities|GetDataTableRow "/Game/Art/Characters/Enemies/Human/NPCs/DT_Clothes.DT_Clothes" "Clothes")
    (:then
      (Components|SkeletalMesh|SetSkeletalMeshAsset (Variables|Default|GetShirt) (Utilities|Array|Get(acopy) (.shirts _returnvalue) (Math|Random|RandomIntegerinRange 0 (- (Utilities|Array|Length (.shirts _returnvalue)) 1))))
      (Components|SkeletalMesh|SetSkeletalMeshAsset (Variables|Default|GetPants) (Utilities|Array|Get(acopy) (.pants _returnvalue) (Math|Random|RandomIntegerinRange 0 (- (Utilities|Array|Length (.pants _returnvalue)) 1))))
      (Components|SkeletalMesh|SetSkeletalMeshAsset (Variables|Default|GetShoes) (Utilities|Array|Get(acopy) (.shoes _returnvalue) (Math|Random|RandomIntegerinRange 0 (- (Utilities|Array|Length (.shoes _returnvalue)) 1))))
      (Components|SkeletalMesh|SetSkeletalMeshAsset (Variables|Default|GetHat) (Utilities|Array|Get(acopy) (.headgear _returnvalue) (Math|Random|RandomIntegerinRange 0 (- (Utilities|Array|Length (.headgear _returnvalue)) 1))))
      (Components|SkeletalMesh|SetSkeletalMeshAsset (Variables|Default|GetBrow) (Utilities|Array|Get(acopy) (.brows _returnvalue) (Math|Random|RandomIntegerinRange 0 (- (Utilities|Array|Length (.brows _returnvalue)) 1))))
      (Components|SkeletalMesh|SetSkeletalMeshAsset (Variables|Default|GetNose) (Utilities|Array|Get(acopy) (.noses _returnvalue) (Math|Random|RandomIntegerinRange 0 (- (Utilities|Array|Length (.noses _returnvalue)) 1)))))))