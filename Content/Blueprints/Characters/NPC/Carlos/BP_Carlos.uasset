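; Carlos is a stationary NPC turret that shoots at the pigeon player character while it is inside his Detection volume.
; Overlap events set an in-range flag, and Tick triggers FireProjectile after a short delay whenever shooting is allowed.
; Shots spawn BP_CarlosProjectile aimed at a position predicted from player velocity, followed by a cooldown.
; Out of range, he eases back to his starting rotation; the rotation that tracks the player is disconnected.
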(event OnComponentBeginOverlap(Detection)
  (params (OverlappedComponent :type Primitive%20Component%20Object%20Reference) (OtherActor :type Actor%20Object%20Reference) (OtherComp :type Primitive%20Component%20Object%20Reference) (OtherBodyIndex :type Integer) (bFromSweep :type Boolean) (SweepResult :type Hit%20Result%20Structure%20%28by%20ref%29))
  ;[1 1 1] Calls FireProjectile event to shoot at player when entering radius
  (Utilities|Casting|CastToBP_PigeonCharacter_AB OtherActor)
  (Variables|Default|SetIsPlayerInRange true))

(event OnComponentEndOverlap(Detection)
  (params (OverlappedComponent :type Primitive%20Component%20Object%20Reference) (OtherActor :type Actor%20Object%20Reference) (OtherComp :type Primitive%20Component%20Object%20Reference) (OtherBodyIndex :type Integer))
  ;[1 1 1] Stops FireProjectile once player leaves radius
  (Utilities|Casting|CastToBP_PigeonCharacter_AB OtherActor)
  (Variables|Default|SetIsPlayerInRange false))

(event Custom|FireProjectile
  (bind _returnvalue (Game|GetPlayerCharacter 0))
  ;[1 1 1] Fires projectile using predictive logic
  (Variables|Default|SetCanShoot false)
  (Variables|Default|SetPlayerVelocity (Variables|/Script/Engine.MovementComponent|GetVelocity (Variables|/Script/Engine.Character|GetCharacterMovement _returnvalue)))
  (Variables|Default|SetPredictedOffset (* (Variables|Default|GetPlayerVelocity) (Variables|Default|GetPredictionTime)))
  (Variables|Default|SetPredictedLocation (+ (Transformation|GetActorLocation _returnvalue) (Variables|Default|GetPredictedOffset)))
  (bind _output_get (Variables|Default|SetSpawnLocation (Transformation|GetWorldLocation (Variables|Default|GetProjectileSpawn))))
  (Variables|Default|SetProjectileRotation (Math|Rotator|FindLookatRotation _output_get (Variables|Default|GetPredictedLocation)))
  (Game|SpawnActorfromClass "/Game/Blueprints/Characters/NPC/Carlos/BP_CarlosProjectile.BP_CarlosProjectile_C" (Math|Transform|MakeTransform (Variables|Default|GetSpawnLocation) (Variables|Default|GetProjectileRotation) "1.000000,1.000000,1.000000") "Undefined" "MultiplyWithRoot" 0 0)
  (Utilities|FlowControl|Delay 2.0)
  (Variables|Default|SetCanShoot true))

(event EventTick
  (params (DeltaSeconds :type Float%20%28single-precision%29))
  ;[1 1 1] Calls branch to track whether player is seen within detection radius, uses yaw rotation to track
  (if (Variables|Default|GetIsPlayerInRange)
    (Variables|Default|SetTargetLocation (Transformation|GetActorLocation (Game|GetPlayerCharacter 0)))
    (if (Variables|Default|GetCanShoot)
      (Utilities|FlowControl|Delay 1.0)
      (CallFunction|FireProjectile))
    (else
      (Transformation|SetActorRotation (Math|Interpolation|RInterpTo (Transformation|GetActorRotation) (Variables|Default|GetOriginalRotation) (Utilities|Time|GetWorldDeltaSeconds) 1e+01)))))

(event EventBeginPlay
  ;[1 1 1] Sets Carlos' current rotation as original rotation
  (Variables|Default|SetOriginalRotation (Transformation|GetActorRotation)))

(fn ConstructionScript)