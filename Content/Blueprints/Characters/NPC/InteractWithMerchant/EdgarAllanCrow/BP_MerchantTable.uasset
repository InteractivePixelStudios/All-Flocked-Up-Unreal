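; Merchant table actor that sells four randomly drawn items from DT_MerchantShop to the pigeon player for Trinkets.
; Items spawn on four slots, and each slot's box overlap sets the current item and checks affordability.
; Pickup opens a paused merchant widget, while BuyItem deducts Trinkets, adds the item to inventory and retires that slot.
; ResetItems, triggered here by a debug key, restocks the table on a self-repeating delay.
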(event OnComponentBeginOverlap(Box3)
  (params (OverlappedComponent :type Primitive%20Component%20Object%20Reference) (OtherActor :type Actor%20Object%20Reference) (OtherComp :type Primitive%20Component%20Object%20Reference) (OtherBodyIndex :type Integer) (bFromSweep :type Boolean) (SweepResult :type Hit%20Result%20Structure%20%28by%20ref%29))
  (CallFunction|CheckArrayforCollider (Variables|Default|GetBox3))
  (Utilities|Casting|CastToBP_PigeonCharacter_AB OtherActor)
  (Variables|Default|SetbCanInteract true) ; Sets interactivity to true
  (Development|PrintString "Merchant can be interacted with")
  (CallFunction|GetPlayerTrinkets)
  (CallFunction|GetCurrentItemSlot)
  (CallFunction|CompareTrinketsVsCost))

(event OnComponentBeginOverlap(Box1)
  (params (OverlappedComponent :type Primitive%20Component%20Object%20Reference) (OtherActor :type Actor%20Object%20Reference) (OtherComp :type Primitive%20Component%20Object%20Reference) (OtherBodyIndex :type Integer) (bFromSweep :type Boolean) (SweepResult :type Hit%20Result%20Structure%20%28by%20ref%29))
  (CallFunction|CheckArrayforCollider (Variables|Default|GetBox1))
  (Utilities|Casting|CastToBP_PigeonCharacter_AB OtherActor)
  (Variables|Default|SetbCanInteract true) ; Sets interactivity to true
  (Development|PrintString "Merchant can be interacted with")
  (CallFunction|GetPlayerTrinkets)
  (CallFunction|GetCurrentItemSlot)
  (CallFunction|CompareTrinketsVsCost))

(event OnComponentEndOverlap(Box1)
  (params (OverlappedComponent :type Primitive%20Component%20Object%20Reference) (OtherActor :type Actor%20Object%20Reference) (OtherComp :type Primitive%20Component%20Object%20Reference) (OtherBodyIndex :type Integer))
  (Utilities|Casting|CastToBP_PigeonCharacter_AB OtherActor)
  (Variables|Default|SetbCanInteract false)
  (Development|PrintString "Merchant interact range left"))

(event OnComponentBeginOverlap(Box)
  (params (OverlappedComponent :type Primitive%20Component%20Object%20Reference) (OtherActor :type Actor%20Object%20Reference) (OtherComp :type Primitive%20Component%20Object%20Reference) (OtherBodyIndex :type Integer) (bFromSweep :type Boolean) (SweepResult :type Hit%20Result%20Structure%20%28by%20ref%29))
  (CallFunction|CheckArrayforCollider (Variables|Default|GetBox))
  (Utilities|Casting|CastToBP_PigeonCharacter_AB OtherActor)
  (Variables|Default|SetbCanInteract true) ; Sets interactivity to true
  (Development|PrintString "Merchant can be interacted with")
  (CallFunction|GetPlayerTrinkets)
  (CallFunction|GetCurrentItemSlot)
  (CallFunction|CompareTrinketsVsCost))

(event OnComponentEndOverlap(Box)
  (params (OverlappedComponent :type Primitive%20Component%20Object%20Reference) (OtherActor :type Actor%20Object%20Reference) (OtherComp :type Primitive%20Component%20Object%20Reference) (OtherBodyIndex :type Integer))
  (Utilities|Casting|CastToBP_PigeonCharacter_AB OtherActor)
  (Variables|Default|SetbCanInteract false)
  (Development|PrintString "Merchant interact range left"))

(event OnComponentBeginOverlap(Box2)
  (params (OverlappedComponent :type Primitive%20Component%20Object%20Reference) (OtherActor :type Actor%20Object%20Reference) (OtherComp :type Primitive%20Component%20Object%20Reference) (OtherBodyIndex :type Integer) (bFromSweep :type Boolean) (SweepResult :type Hit%20Result%20Structure%20%28by%20ref%29))
  (CallFunction|CheckArrayforCollider (Variables|Default|GetBox2))
  (Utilities|Casting|CastToBP_PigeonCharacter_AB OtherActor)
  (Variables|Default|SetbCanInteract true) ; Sets interactivity to true
  (Development|PrintString "Merchant can be interacted with")
  (CallFunction|GetPlayerTrinkets)
  (CallFunction|GetCurrentItemSlot)
  (CallFunction|CompareTrinketsVsCost))

(event OnComponentEndOverlap(Box2)
  (params (OverlappedComponent :type Primitive%20Component%20Object%20Reference) (OtherActor :type Actor%20Object%20Reference) (OtherComp :type Primitive%20Component%20Object%20Reference) (OtherBodyIndex :type Integer))
  (Utilities|Casting|CastToBP_PigeonCharacter_AB OtherActor)
  (Variables|Default|SetbCanInteract false)
  (Development|PrintString "Merchant interact range left"))

(event OnComponentEndOverlap(Box3)
  (params (OverlappedComponent :type Primitive%20Component%20Object%20Reference) (OtherActor :type Actor%20Object%20Reference) (OtherComp :type Primitive%20Component%20Object%20Reference) (OtherBodyIndex :type Integer))
  (Utilities|Casting|CastToBP_PigeonCharacter_AB OtherActor)
  (Variables|Default|SetbCanInteract false)
  (Development|PrintString "Merchant interact range left"))

(event Custom|BuyingItem_Event
  (CallFunction|BuyItem)
  (Development|PrintString "buying"))

(event Custom|ResetItems
  (CallFunction|RemoveItems)
  (CallFunction|PopulateTable)
  (Utilities|FlowControl|Delay (Variables|Default|GetTimeForNewItems))
  (CallFunction|ResetItems))

(event EventBeginPlay
  (CallFunction|GetColliders)
  (CallFunction|PopulateTable)
  (CallFunction|GetPlayerTrinkets))

(event Collision|EventActorBeginOverlap
  (params (OtherActor :type Actor%20Object%20Reference)))

(event EventTick
  (params (DeltaSeconds :type Float%20%28single-precision%29)))

(event EventPickup
  (bind _returnvalue (Game|GetPlayerController 0))
  (Input|EnableInput _returnvalue)
  (if (Variables|Default|GetbCanInteract)
    (CallFunction|CreateWidget _returnvalue _returnvalue _returnvalue)))

(event Input|KeyboardEvents|DebugKeyR
  (params (Key :type Key%20Structure :default "None") (ActionValue :type Input%20Action%20Value%20Structure))
  (:Pressed
    (CallFunction|BuyItem)))

(event Input|KeyboardEvents|DebugKeyV
  (params (Key :type Key%20Structure :default "None") (ActionValue :type Input%20Action%20Value%20Structure))
  (:Pressed
    (CallFunction|ResetItems)))

(fn ConstructionScript)

(fn PopulateTable
  (bind _itemslot1 (Variables|Default|GetItemSlot1))
  (bind _itemslot2 (Variables|Default|GetItemSlot2))
  (bind _itemslot3 (Variables|Default|GetItemSlot3))
  (bind _itemslot4 (Variables|Default|GetItemSlot4))
  (CallFunction|GetColliders)
  (bind _returnvalue (Utilities|GetDataTableRow "/Game/Blueprints/Characters/NPC/InteractWithMerchant/EdgarAllanCrow/DT_MerchantShop.DT_MerchantShop" (Utilities|String|StringToName (Utilities|String|ToString(Integer) (Math|Random|RandomInteger 15))))
    (:then
      (Variables|Default|SetSlot1Class (.itemactorclass _returnvalue))
      (Variables|Default|SetSlot1Cost (.cost _returnvalue))
      (Variables|Default|SetSlot1Type (.itemtype _returnvalue))
      (Variables|Default|SetSlot1Name (.itemname _returnvalue))
      (bind _returnvalue_2 (Game|SpawnActorfromClass (.itemactorclass _returnvalue) (Transformation|GetSocketTransform _itemslot1 "None" "RTS_World") "Undefined" "OverrideRootScale" 0 0))
      (Collision|SetActorEnableCollision _returnvalue_2 false)
      (bind _output_get (Variables|Default|SetItem1 _returnvalue_2))
      (Transformation|AttachComponentToComponent _output_get _itemslot1 "None" "KeepWorld" "KeepWorld" "KeepRelative" true)
      (bind _returnvalue_3 (Utilities|GetDataTableRow "/Game/Blueprints/Characters/NPC/InteractWithMerchant/EdgarAllanCrow/DT_MerchantShop.DT_MerchantShop" (Utilities|String|StringToName (Utilities|String|ToString(Integer) (Math|Random|RandomInteger 15))))
        (:then
          (Variables|Default|SetSlot2Class (.itemactorclass _returnvalue_3))
          (Variables|Default|SetSlot2Cost (.cost _returnvalue_3))
          (Variables|Default|SetSlot2Type (.itemtype _returnvalue_3))
          (Variables|Default|SetSlot2Name (.itemname _returnvalue_3))
          (bind _returnvalue_4 (Game|SpawnActorfromClass (.itemactorclass _returnvalue_3) (Transformation|GetSocketTransform _itemslot2 "None" "RTS_World") "Undefined" "OverrideRootScale" 0 0))
          (Collision|SetActorEnableCollision _returnvalue_4 false)
          (bind _output_get_2 (Variables|Default|SetItem2 _returnvalue_4))
          (Transformation|AttachComponentToComponent _output_get_2 _itemslot2 "None" "KeepWorld" "KeepWorld" "KeepWorld" true)
          (bind _returnvalue_5 (Utilities|GetDataTableRow "/Game/Blueprints/Characters/NPC/InteractWithMerchant/EdgarAllanCrow/DT_MerchantShop.DT_MerchantShop" (Utilities|String|StringToName (Utilities|String|ToString(Integer) (Math|Random|RandomInteger 15))))
            (:then
              (Variables|Default|SetSlot3Class (.itemactorclass _returnvalue_5))
              (Variables|Default|SetSlot3Cost (.cost _returnvalue_5))
              (Variables|Default|SetSlot3Type (.itemtype _returnvalue_5))
              (Variables|Default|SetSlot3Name (.itemname _returnvalue_5))
              (bind _returnvalue_6 (Game|SpawnActorfromClass (.itemactorclass _returnvalue_5) (Transformation|GetSocketTransform _itemslot3 "None" "RTS_World") "Undefined" "OverrideRootScale" 0 0))
              (Collision|SetActorEnableCollision _returnvalue_6 false)
              (bind _output_get_3 (Variables|Default|SetItem3 _returnvalue_6))
              (Transformation|AttachComponentToComponent _output_get_3 _itemslot3 "None" "KeepWorld" "KeepWorld" "KeepRelative" true)
              (bind _returnvalue_7 (Utilities|GetDataTableRow "/Game/Blueprints/Characters/NPC/InteractWithMerchant/EdgarAllanCrow/DT_MerchantShop.DT_MerchantShop" (Utilities|String|StringToName (Utilities|String|ToString(Integer) (Math|Random|RandomInteger 15))))
                (:then
                  (Variables|Default|SetSlot4Class (.itemactorclass _returnvalue_7))
                  (Variables|Default|SetSlot4Cost (.cost _returnvalue_7))
                  (Variables|Default|SetSlot4Type (.itemtype _returnvalue_7))
                  (Variables|Default|SetSlot4Name (.itemname _returnvalue_7))
                  (bind _returnvalue_8 (Game|SpawnActorfromClass (.itemactorclass _returnvalue_7) (Transformation|GetSocketTransform _itemslot4 "None" "RTS_World") "Undefined" "OverrideRootScale" 0 0))
                  (Collision|SetActorEnableCollision _returnvalue_8 false)
                  (bind _output_get_4 (Variables|Default|SetItem4 _returnvalue_8))
                  (Transformation|AttachComponentToComponent _output_get_4 _itemslot4 "None" "KeepWorld" "KeepWorld" "KeepRelative" true))))))))))

(fn GetPlayerTrinkets
  (Variables|Default|SetPlayerCurrentTrinkets (Variables|/Game/Blueprints/Characters/Player/BP_PigeonCharacter_AB.BP_PigeonCharacter_AB_C|GetTrinkets (CallFunction|GetPigeonCharacter))))

(fn BuyItem
  (if (Variables|Default|GetCanAffordItem)
    (bind _returnvalue (Actor|GetActorOfClass "/Game/Blueprints/Characters/Player/BP_PigeonCharacter_AB.BP_PigeonCharacter_AB_C"))
    (switch Utilities|FlowControl|Switch|SwitchonE_MerchantState (Variables|Default|GetEnumRef)
      (:NewEnumerator0
        (CallFunction|RemoveTrinketsfromPlayer)
        (Default|AddItemtoInventory (Variables|/Game/Blueprints/Characters/Player/BP_PigeonCharacter_AB.BP_PigeonCharacter_AB_C|GetAC_Inventory _returnvalue) (Utilities|Struct|MakeS_ItemData (Utilities|String|ToString(Text) (Variables|Default|GetSlot1Name)) "It's an Item!" "NewEnumerator0" 1 true 1 (Variables|Default|GetSlot1Class)) (Variables|/Game/Blueprints/GameplaySystems/Inventory/AC_Inventory.AC_Inventory_C|GetInventory (Variables|/Game/Blueprints/Characters/Player/BP_PigeonCharacter_AB.BP_PigeonCharacter_AB_C|GetAC_Inventory _returnvalue)))
        (Actor|DestroyActor (Variables|Default|GetItem1))
        (Utilities|Array|RemoveItem (Variables|Default|GetBoxColliderArray) (Variables|Default|GetBox)))
      (:NewEnumerator1
        (CallFunction|RemoveTrinketsfromPlayer)
        (Default|AddItemtoInventory (Variables|/Game/Blueprints/Characters/Player/BP_PigeonCharacter_AB.BP_PigeonCharacter_AB_C|GetAC_Inventory _returnvalue) (Utilities|Struct|MakeS_ItemData (Utilities|String|ToString(Text) (Variables|Default|GetSlot2Name)) "It's an Item!" "NewEnumerator0" 1 true 1 (Variables|Default|GetSlot2Class)) (Variables|/Game/Blueprints/GameplaySystems/Inventory/AC_Inventory.AC_Inventory_C|GetInventory (Variables|/Game/Blueprints/Characters/Player/BP_PigeonCharacter_AB.BP_PigeonCharacter_AB_C|GetAC_Inventory _returnvalue)))
        (Actor|DestroyActor (Variables|Default|GetItem2))
        (Utilities|Array|RemoveItem (Variables|Default|GetBoxColliderArray) (Variables|Default|GetBox1)))
      (:NewEnumerator2
        (CallFunction|RemoveTrinketsfromPlayer)
        (Default|AddItemtoInventory (Variables|/Game/Blueprints/Characters/Player/BP_PigeonCharacter_AB.BP_PigeonCharacter_AB_C|GetAC_Inventory _returnvalue) (Utilities|Struct|MakeS_ItemData (Utilities|String|ToString(Text) (Variables|Default|GetSlot3Name)) "It's an Item!" "NewEnumerator0" 1 true 1 (Variables|Default|GetSlot3Class)) (Variables|/Game/Blueprints/GameplaySystems/Inventory/AC_Inventory.AC_Inventory_C|GetInventory (Variables|/Game/Blueprints/Characters/Player/BP_PigeonCharacter_AB.BP_PigeonCharacter_AB_C|GetAC_Inventory _returnvalue)))
        (Actor|DestroyActor (Variables|Default|GetItem3))
        (Utilities|Array|RemoveItem (Variables|Default|GetBoxColliderArray) (Variables|Default|GetBox2)))
      (:NewEnumerator3
        (CallFunction|RemoveTrinketsfromPlayer)
        (Default|AddItemtoInventory (Variables|/Game/Blueprints/Characters/Player/BP_PigeonCharacter_AB.BP_PigeonCharacter_AB_C|GetAC_Inventory _returnvalue) (Utilities|Struct|MakeS_ItemData (Utilities|String|ToString(Text) (Variables|Default|GetSlot4Name)) "It's an Item!" "NewEnumerator0" 1 true 1 (Variables|Default|GetSlot4Class)) (Variables|/Game/Blueprints/GameplaySystems/Inventory/AC_Inventory.AC_Inventory_C|GetInventory (Variables|/Game/Blueprints/Characters/Player/BP_PigeonCharacter_AB.BP_PigeonCharacter_AB_C|GetAC_Inventory _returnvalue)))
        (Actor|DestroyActor (Variables|Default|GetItem4))
        (Utilities|Array|RemoveItem (Variables|Default|GetBoxColliderArray) (Variables|Default|GetBox3))))))

(fn GetColliders
  (bind _output_get (Variables|Default|SetBoxColliderArray (Utilities|Array|MakeArray (Variables|Default|GetBox) (Variables|Default|GetBox1) (Variables|Default|GetBox2) (Variables|Default|GetBox3))))
  (for _array_element _output_get
    (Collision|SetCollisionEnabled _array_element "QueryAndProbe")))

(fn RemoveItems
  (Actor|DestroyActor (Variables|Default|GetItem1))
  (Actor|DestroyActor (Variables|Default|GetItem2))
  (Actor|DestroyActor (Variables|Default|GetItem3))
  (Actor|DestroyActor (Variables|Default|GetItem4)))

(fn GetCurrentItemSlot
  (for _array_element (Variables|Default|GetBoxColliderArray)
    (if (Collision|IsOverlappingActor _array_element (Game|GetPlayerCharacter 0) :!class /Script/Engine.PrimitiveComponent)
      (if (== _array_element (Variables|Default|GetBox))
        (Variables|Default|SetEnumRef "NewEnumerator0")
        (CallFunction|GetInfoforWidget (Variables|Default|GetSlot1Name) (Variables|Default|GetSlot1Type) (Variables|Default|GetSlot1Cost))
        (elif (== _array_element (Variables|Default|GetBox1))
          (Variables|Default|SetEnumRef "NewEnumerator1")
          (CallFunction|GetInfoforWidget (Variables|Default|GetSlot2Name) (Variables|Default|GetSlot2Type) (Variables|Default|GetSlot2Cost))
          (elif (== _array_element (Variables|Default|GetBox2))
            (Variables|Default|SetEnumRef "NewEnumerator2")
            (CallFunction|GetInfoforWidget (Variables|Default|GetSlot3Name) (Variables|Default|GetSlot3Type) (Variables|Default|GetSlot3Cost))
            (elif (== _array_element (Variables|Default|GetBox3))
              (Variables|Default|SetEnumRef "NewEnumerator3")
              (CallFunction|GetInfoforWidget (Variables|Default|GetSlot4Name) (Variables|Default|GetSlot4Type) (Variables|Default|GetSlot4Cost)))))))))

(fn CreateWidget
  (params (PlayerController :type Player%20Controller%20Object%20Reference) (self2 :type Player%20Controller%20Object%20Reference) (OwningPlayer :type Player%20Controller%20Object%20Reference))
  (bind _returnvalue (UserInterface|CreateWidget "/Game/Blueprints/Characters/NPC/InteractWithMerchant/WBP_MerchantWidget.WBP_MerchantWidget_C" OwningPlayer))
  (UserInterface|Viewport|AddtoViewport _returnvalue 0)
  (Game|SetGamePaused true)
  (Input|SetInputModeUIOnly PlayerController (Variables|Default|GetMechantWidgetRef) "DoNotLock" false)
  (Variables|/Script/Engine.PlayerController|SetbShowMouseCursor self2 true))

(fn GetInfoforWidget
  (params (Name :type Text) (Description :type Text) (Cost :type Integer))
  (bind _output_get (Variables|Default|SetCurrentName Name))
  (bind _output_get_2 (Variables|Default|SetCurrentDescript Description))
  (bind _output_get_3 (Variables|Default|SetCurrentCost Cost))
  (return _output_get _output_get_2 _output_get_3))

(fn SendtoWidget
  (return (Variables|Default|GetCurrentName) (Variables|Default|GetCurrentDescript) (Variables|Default|GetCurrentCost)))

(fn CompareTrinketsVsCost
  (if (>= (Variables|Default|GetPlayerCurrentTrinkets) (Variables|Default|GetCurrentCost))
    (Variables|Default|SetCanAffordItem true)
    (else
      (Variables|Default|SetCanAffordItem false))))

(fn RemoveTrinketsfromPlayer
  (Variables|/Game/Blueprints/Characters/Player/BP_PigeonCharacter_AB.BP_PigeonCharacter_AB_C|SetTrinkets (Variables|Default|GetPlayerRef) (- (Variables|Default|GetPlayerCurrentTrinkets) (Variables|Default|GetCurrentCost))))

(fn CheckArrayforCollider
  (params (ItemToFind :type Box%20Component%20Object%20Reference%20%28by%20ref%29))
  (if (Utilities|Array|ContainsItem (Variables|Default|GetBoxColliderArray) ItemToFind)
    (return)
    (else
      (Collision|SetCollisionEnabled ItemToFind "NoCollision")
      (Development|PrintString "Already Purchased"))))