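; Test game mode that provides debug cheat toggles for the pigeon character's level, XP, health, poop and stamina.
; It caches the pigeon on BeginPlay, then checks every toggle each Tick, pinning enabled stats to their maximum, or to the threshold for XP.
; When off, level is continually set to DebugLevel, which is overwritten each enabled tick.
; The other stats self-assign when off, leaving their saved debug values unused.
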(event Custom|StaminaToggled
  (bind _pigeonref (Variables|Default|GetPigeonRef))
  (bind _bp_staminasystem_so (Variables|/Game/Blueprints/Characters/Player/BP_PigeonCharacter_AB.BP_PigeonCharacter_AB_C|GetBP_StaminaSystem_SO _pigeonref))
  ;[1 1 1] StaminaToggle
  (if (Variables|Default|GetStaminaToggle)
    (Variables|Default|SetDebugStamina (Variables|/Game/Blueprints/Characters/Player/ActorComponents/BP_StaminaSystem_SO.BP_StaminaSystem_SO_C|Getstamina _bp_staminasystem_so))
    (Variables|/Game/Blueprints/Characters/Player/ActorComponents/BP_StaminaSystem_SO.BP_StaminaSystem_SO_C|Setstamina _bp_staminasystem_so (Variables|/Game/Blueprints/Characters/Player/ActorComponents/BP_StaminaSystem_SO.BP_StaminaSystem_SO_C|GetmaxStamina _bp_staminasystem_so))
    (else
      (Variables|/Game/Blueprints/Characters/Player/ActorComponents/BP_StaminaSystem_SO.BP_StaminaSystem_SO_C|Setstamina _bp_staminasystem_so (Variables|/Game/Blueprints/Characters/Player/ActorComponents/BP_StaminaSystem_SO.BP_StaminaSystem_SO_C|Getstamina _bp_staminasystem_so)))))

(event Custom|LevelToggled
  (bind _pigeonref (Variables|Default|GetPigeonRef))
  (bind _bp_xpmanager_js (Variables|/Game/Blueprints/Characters/Player/BP_PigeonCharacter_AB.BP_PigeonCharacter_AB_C|GetBP_XPManager_JS _pigeonref))
  ;[1 1 1] LevelToggle
  (if (Variables|Default|GetLevelToggle)
    (bind _output_get (Variables|Default|SetDebugLevel (Variables|/Game/Blueprints/Characters/Player/BP_XPManager_JS.BP_XPManager_JS_C|GetPlayerLevel _bp_xpmanager_js)))
    (Variables|/Game/Blueprints/Characters/Player/BP_XPManager_JS.BP_XPManager_JS_C|SetPlayerLevel _bp_xpmanager_js (Variables|/Game/Blueprints/Characters/Player/BP_XPManager_JS.BP_XPManager_JS_C|GetMaxLevel _bp_xpmanager_js))
    (else
      (Variables|/Game/Blueprints/Characters/Player/BP_XPManager_JS.BP_XPManager_JS_C|SetPlayerLevel _bp_xpmanager_js _output_get))))

(event Custom|XPToggled
  (bind _pigeonref (Variables|Default|GetPigeonRef))
  (bind _bp_xpmanager_js (Variables|/Game/Blueprints/Characters/Player/BP_PigeonCharacter_AB.BP_PigeonCharacter_AB_C|GetBP_XPManager_JS _pigeonref))
  ;[1 1 1] XPToggle
  (if (Variables|Default|GetXPToggle)
    (Variables|Default|SetDebugXP (Variables|/Game/Blueprints/Characters/Player/BP_XPManager_JS.BP_XPManager_JS_C|GetCurrentXP _bp_xpmanager_js))
    (Variables|/Game/Blueprints/Characters/Player/BP_XPManager_JS.BP_XPManager_JS_C|SetCurrentXP _bp_xpmanager_js (Variables|/Game/Blueprints/Characters/Player/BP_XPManager_JS.BP_XPManager_JS_C|GetXPThreshold _bp_xpmanager_js))
    (else
      (Variables|/Game/Blueprints/Characters/Player/BP_XPManager_JS.BP_XPManager_JS_C|SetCurrentXP _bp_xpmanager_js (Variables|/Game/Blueprints/Characters/Player/BP_XPManager_JS.BP_XPManager_JS_C|GetCurrentXP _bp_xpmanager_js)))))

(event Custom|HealthToggled
  (bind _pigeonref (Variables|Default|GetPigeonRef))
  (bind _bp_healthsystem_wk (Variables|/Game/Blueprints/Characters/Player/BP_PigeonCharacter_AB.BP_PigeonCharacter_AB_C|GetBP_HealthSystem_WK _pigeonref))
  ;[1 1 1] HealthToggle
  (if (Variables|Default|GetHealthToggle)
    (Variables|Default|SetDebugHealth (Variables|/Game/Blueprints/Characters/Player/ActorComponents/BP_HealthSystem_WK.BP_HealthSystem_WK_C|GetHealthCurrent _bp_healthsystem_wk))
    (Variables|/Game/Blueprints/Characters/Player/ActorComponents/BP_HealthSystem_WK.BP_HealthSystem_WK_C|SetHealthCurrent _bp_healthsystem_wk (Variables|/Game/Blueprints/Characters/Player/ActorComponents/BP_HealthSystem_WK.BP_HealthSystem_WK_C|GetHealthMax _bp_healthsystem_wk))
    (else
      (Variables|/Game/Blueprints/Characters/Player/ActorComponents/BP_HealthSystem_WK.BP_HealthSystem_WK_C|SetHealthCurrent _bp_healthsystem_wk (Variables|/Game/Blueprints/Characters/Player/ActorComponents/BP_HealthSystem_WK.BP_HealthSystem_WK_C|GetHealthCurrent _bp_healthsystem_wk)))))

(event Custom|PoopToggled
  (bind _pigeonref (Variables|Default|GetPigeonRef))
  (bind _bp_poopsystem_wk (Variables|/Game/Blueprints/Characters/Player/BP_PigeonCharacter_AB.BP_PigeonCharacter_AB_C|GetBP_PoopSystem_WK _pigeonref))
  ;[1 1 1] PoopToggle
  (if (Variables|Default|GetPoopToggle)
    (Variables|Default|SetDebugPoop (Variables|/Game/Blueprints/Characters/Player/BP_PoopSystem_WK.BP_PoopSystem_WK_C|GetPoopCurrent _bp_poopsystem_wk))
    (Variables|/Game/Blueprints/Characters/Player/BP_PoopSystem_WK.BP_PoopSystem_WK_C|SetPoopCurrent _bp_poopsystem_wk (Variables|/Game/Blueprints/Characters/Player/BP_PoopSystem_WK.BP_PoopSystem_WK_C|GetPoopMax _bp_poopsystem_wk))
    (else
      (Variables|/Game/Blueprints/Characters/Player/BP_PoopSystem_WK.BP_PoopSystem_WK_C|SetPoopCurrent _bp_poopsystem_wk (Variables|/Game/Blueprints/Characters/Player/BP_PoopSystem_WK.BP_PoopSystem_WK_C|GetPoopCurrent _bp_poopsystem_wk)))))

(event EventBeginPlay
  (Variables|Default|SetPigeonRef (CallFunction|GetPigeonCharacter)))

(event EventTick
  (params (DeltaSeconds :type Float%20%28single-precision%29))
  (CallFunction|LevelToggled)
  (CallFunction|XPToggled)
  (CallFunction|HealthToggled)
  (CallFunction|PoopToggled)
  (CallFunction|StaminaToggled))

(fn ConstructionScript)