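; Spawner for a timed stick-collection objective that gets the pigeon player's nest built.
; SpawnSticks scatters sticks in a box, re-rolling positions that are too close, then creates a timer UI and an arrow pointer.
; CollectStick retargets the pointer and adds bonus time while sticks remain.
; Tick counts down, either resetting on timeout or building the nest and signaling the objective ID once all are collected.
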(event EventBeginPlay
  (bind _asbp_pigeon_character_ab (Utilities|Casting|CastToBP_PigeonCharacter_AB (Game|GetPlayerCharacter 0)))
  (Variables|Default|SetPigeonRef _asbp_pigeon_character_ab))

(event EventTick
  (params (DeltaSeconds :type Float%20%28single-precision%29))
  ;[0.2623 0.552 1] When collecting adjust time with seconds passed and set current time remaining
  (if (Variables|Default|GetPlayerCollecting)
    (bind _output_get (Variables|Default|SetCurrentTime (- (Variables|Default|GetCurrentTime) DeltaSeconds)))
    ;[0.2623 0.552 1] Update the time in the widget
    (Default|UpdateTime (Variables|Default|GetUIRef) _output_get)
    (if (<= _output_get 0.0)
      (if (> (Utilities|Array|Length (Variables|Default|GetSticks)) 0)
        ;[0.2623 0.552 1] On failure reset the spawner and remove the timer widget
        (CallFunction|ResetSpawner)
        (Widget|RemovefromParent (Variables|Default|GetUIRef))
        (Actor|DestroyActor (Variables|Default|GetPointerRef)))
      (elif (== (Variables|Default|GetTotalSticks) (Variables|Default|GetSticksCollected))
        ;[0.1059 0.1059 0.1059 0.7216] Build the nest
        (Default|NestBuilt (Variables|Default|GetNestRef))
        ;[0.2623 0.552 1] Set player to no longer collecting and remove the timer widget from player
        (Variables|Default|SetPlayerCollecting false)
        (Widget|RemovefromParent (Variables|Default|GetUIRef))
        (Actor|DestroyActor (Variables|Default|GetPointerRef))
        (Default|CallOnObjectiveIDCalled (Variables|Default|GetPigeonRef) (Variables|Default|GetObjective%20ID))))))

(fn ConstructionScript
  ;[0.2623 0.552 1] Sets spawn bounds as constructed to show in editor view
  (Components|Box|SetBoxExtent (Variables|Default|GetStickSpawnArea) (Variables|Default|GetStickSpawnAreaSize) true))

(fn SpawnSticks
  (params (NestRef :type BP%20Base%20Nest%20Object%20Reference) (TimeToCollect :type Float%20%28double-precision%29) (NumberOfSticksToSpawn :type Integer))
  (bind _stickspawnarea (Variables|Default|GetStickSpawnArea))
  (bind _sticks (Variables|Default|GetSticks))
  (bind _stickspawnarea_2 (Variables|Default|GetStickSpawnArea))
  (if (not (Variables|Default|GetPlayerCollecting))
    (Variables|Default|SetTotalSticks NumberOfSticksToSpawn)
    ;[0.2623 0.552 1] Spawn the arrow pointer and set the reference
    (bind _returnvalue (Game|SpawnActorfromClass "/Game/Blueprints/GameplaySystems/HelperMechanics/BP_ArrowPointer.BP_ArrowPointer_C" (Transformation|GetActorTransform self) "Undefined" "MultiplyWithRoot" 0 0))
    (Variables|Default|SetPointerRef _returnvalue)
    ;[0.2623 0.552 1] Add/Set timer widget to player character
    (bind _returnvalue_2 (UserInterface|CreateWidget "/Game/Blueprints/GameplaySystems/Nest/WBP_NestTimerUI.WBP_NestTimerUI_C" (Game|GetPlayerController 0)))
    (bind _output_get (Variables|Default|SetUIRef _returnvalue_2))
    (UserInterface|Viewport|AddtoViewport _output_get 0)
    ;[0.2623 0.552 1] Set Reference to nest calling spawn, and set current time to start counting down from
    (Variables|Default|SetNestRef NestRef)
    (Variables|Default|SetCurrentTime TimeToCollect)
    ;[0.1059 0.1059 0.1059 0.7216] Loops through all sticks to spawn
    (for _index (range 1 (Variables|Default|GetTotalSticks))
      ;[0.2623 0.552 1] Spawn stick at random location within spawn bounds and set the sticks spawner reference for collection
      (bind _returnvalue_3 (Game|SpawnActorfromClass "/Game/Blueprints/GameplaySystems/Nest/BP_Stick.BP_Stick_C" (Math|Transform|MakeTransform (Math|Random|RandomPointinBoundingBox (Transformation|GetWorldLocation _stickspawnarea_2) (Components|Box|GetScaledBoxExtent _stickspawnarea_2)) "0, 0, 0" "1.000000,1.000000,1.000000") "AdjustIfPossibleButAlwaysSpawn" "MultiplyWithRoot" 0 0))
      (Default|SetSpawnerRef _returnvalue_3 self)
      (if (Variables|Default|GetFirstStick)
        ;[0.2623 0.552 1] If first stick add to array without check
        (Utilities|Array|Add (Variables|Default|GetSticks) _returnvalue_3)
        (Variables|Default|SetFirstStick false)
        (else
          ;[0.1059 0.1059 0.1059 0.7216] After stick is spawned, check to make sure its random location is spaced from other sticks
          (for _array_element _sticks :!label _label
            (if (< (Math|Vector|Distance2D(Vector) (Math|Vector2D|MakeVector2D (.x (Transformation|GetActorLocation _returnvalue_3)) (.y (Transformation|GetActorLocation _returnvalue_3))) (Math|Vector2D|MakeVector2D (.x (Transformation|GetActorLocation _array_element)) (.y (Transformation|GetActorLocation _array_element)))) (Variables|Default|GetStickMinimumSpacingDistance))
              ;[0.2623 0.552 1] If not far away enough from another stick, re-loop and try a new position
              (Transformation|SetActorLocation _returnvalue_3 (Math|Random|RandomPointinBoundingBox (Transformation|GetWorldLocation _stickspawnarea) (Components|Box|GetScaledBoxExtent _stickspawnarea)) false true)
              (goto _label)))
          ;[0.2623 0.552 1] If stick is in appropriate spot add to array
          (Utilities|Array|Add _sticks _returnvalue_3))))
    ;[0.2623 0.552 1] On completion of spawning set collecting to true to start timer
    (Variables|Default|SetPlayerCollecting true)
    ;[0.2623 0.552 1] Set the current target for the point to the first stick spawned
    (Default|SetOwnerandTarget (Variables|Default|GetPointerRef) (Utilities|Array|Get(acopy) (Variables|Default|GetSticks)) (Game|Player|GetPlayerPawn 0))
    ;[0.2623 0.552 1] Update the stick UI
    (Default|UpdateSticks (Variables|Default|GetUIRef) (Variables|Default|GetSticksCollected) (Variables|Default|GetTotalSticks))))

(fn ResetSpawner
  ;[0.2623 0.552 1] Reset tracking variables after failing to collect
  (Variables|Default|SetPlayerCollecting false)
  (Variables|Default|SetCurrentTime (Variables|Default|GetCollectTimeAmount))
  ;[0.1059 0.1059 0.1059 0.7216] Loop through and destroy remaining sticks on map
  (for _array_element (Variables|Default|GetSticks)
    (Actor|DestroyActor _array_element)))

(fn CollectStick
  (params (Stick :type BP%20Stick%20Object%20Reference))
  (bind _sticks (Variables|Default|GetSticks))
  (Development|PrintString "Stick Collected" true true "(R=1.000000,G=0.000000,B=0.046735,A=1.000000)")
  ;[0.1059 0.1059 0.1059 0.7216] Removes a collected stick from the array
  (Utilities|Array|RemoveItem _sticks Stick)
  (Math|Integer|IncrementInt (Variables|Default|GetSticksCollected)
    (:%20%20
      ;[0.2623 0.552 1] When stick is collected, and sticks remain, set new target for the pointer
      (if (> (Utilities|Array|Length _sticks) 0)
        (Default|SetNewTarget (Variables|Default|GetPointerRef) (Utilities|Array|Get(acopy) _sticks))
        ;[0.1059 0.1059 0.1059 0.7216] Update the UI stick collection
        (Default|UpdateSticks (Variables|Default|GetUIRef) (Variables|Default|GetSticksCollected) (Variables|Default|GetTotalSticks))
        (Variables|Default|SetCurrentTime (+ (Variables|Default|GetCurrentTime) 1.5))))))