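; Base nest actor that the pigeon player builds from collected sticks and names as a player-made respawn point.
; While inactive, it has its stick spawner spawn the needed sticks with a collection time.
; On completion it activates and opens a naming widget in UI-only input; the entered name fills its respawn info and refreshes the respawn manager.
; Material, visibility and inventory functions are empty stubs here.
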(event EventBeginPlay
  (bind _asbp_pigeon_character_ab (Utilities|Casting|CastToBP_PigeonCharacter_AB (Game|GetPlayerCharacter 0)))
  (Variables|Default|SetPigeonRef _asbp_pigeon_character_ab))

(fn ConstructionScript)

(fn SetActive
  (params (Is%20Active :type Boolean))
  (Variables|Default|SetActive Is%20Active))

(fn SpawnSticks
  (if (not (Variables|Default|GetActive))
    (Default|SpawnSticks (Variables|Default|GetStickSpawnerLocation) self (Variables|Default|GetTime%20to%20Collect) (Variables|Default|GetSticksNeeded))))

(fn AccessInventory)

(fn SwapMaterials)

(fn MakeVisible)

(fn MakeInvisible)

(fn NestBuilt
  ;[1 1 1] Swaps from shimmer material and sets nest to active
  (CallFunction|SwapMaterials)
  (CallFunction|SetActive true)
  (CallFunction|MakeVisible)
  (CallFunction|InputNewNestName)
  (Variables|Default|SetBuildComplete true))

(fn SetNestName
  (params (NameInputText :type String))
  (Variables|Default|SetRespawn%20Point%20Info (Utilities|Struct|MakeS_RespawnPoint NameInputText true true))
  (bind _returnvalue (Actor|GetActorOfClass "/Game/Blueprints/GameplaySystems/Respawn/BP_RespawnManager.BP_RespawnManager_C"))
  (Default|RefreshRespawnPointArray _returnvalue))

(fn InputNewNestName
  (bind _returnvalue (Game|GetPlayerController 0))
  (Utilities|IsValid (Variables|Default|GetNamerRef)
    (:Is%20Valid
      _)
    (:Is%20Not%20Valid
      (bind _returnvalue_2 (UserInterface|CreateWidget "/Game/Blueprints/GameplaySystems/Nest/UW_NestNamer_WK.UW_NestNamer_WK_C" 0 0 0))
      (Variables|Default|SetNamerRef _returnvalue_2)))
  (UserInterface|Viewport|AddtoViewport (Variables|Default|GetNamerRef) 0)
  (Input|SetInputModeUIOnly _returnvalue 0 "DoNotLock" true)
  (Components|Movement|StopMovementImmediately (Variables|/Script/Engine.Character|GetCharacterMovement (Variables|Default|GetPigeonRef)))
  (Variables|/Game/Blueprints/GameplaySystems/Nest/UW_NestNamer_WK.UW_NestNamer_WK_C|SetNestToName (Variables|Default|GetNamerRef) self)
  (Variables|/Script/Engine.PlayerController|SetbShowMouseCursor _returnvalue true))