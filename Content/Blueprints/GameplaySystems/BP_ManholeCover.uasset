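; BP_ManholeCover is a manhole updraft that lifts the pigeon player upward and reports an objective ID on overlap.
; Unless the pigeon is in a full dive or the boost is cooling down, a timeline teleports its Z to just above the trigger box and initiates flight mode if needed.
; Timeline completion and overlap exit both start the delayed re-arm.
; The construction script sizes and raises the box from BoxExtent.
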(event OnComponentEndOverlap(Box)
  (params (OverlappedComponent :type Primitive%20Component%20Object%20Reference) (OtherActor :type Actor%20Object%20Reference) (OtherComp :type Primitive%20Component%20Object%20Reference) (OtherBodyIndex :type Integer))
  (Utilities|Casting|CastToBP_PigeonCharacter_AB OtherActor)
  (Utilities|Time|SetTimerbyEvent (delegate Custom|DelayBoost) 0.1))

(event OnComponentBeginOverlap(Box)
  (params (OverlappedComponent :type Primitive%20Component%20Object%20Reference) (OtherActor :type Actor%20Object%20Reference) (OtherComp :type Primitive%20Component%20Object%20Reference) (OtherBodyIndex :type Integer) (bFromSweep :type Boolean) (SweepResult :type Hit%20Result%20Structure%20%28by%20ref%29))
  (bind _asbp_pigeon_character_ab (Utilities|Casting|CastToBP_PigeonCharacter_AB OtherActor))
  (Default|CallOnObjectiveIDCalled (CallFunction|GetPigeonCharacter) (Variables|Default|GetObjective%20ID))
  (if (and (Variables|Default|GetCanBoost) (!= (Variables|/Game/Blueprints/Characters/Player/ActorComponents/BP_PlayerFlightControl_SO.BP_PlayerFlightControl_SO_C|GetFullDive (Variables|/Game/Blueprints/Characters/Player/BP_PigeonCharacter_AB.BP_PigeonCharacter_AB_C|GetBP_PlayerFlightControl_SO _asbp_pigeon_character_ab)) true))
    (Variables|Default|SetCanBoost false)
    (bind _output_get (Variables|Default|SetOrignalPlayerLocation (.z (Transformation|GetActorLocation _asbp_pigeon_character_ab))))
    (bind _alpha (Timeline|Boost PlayFromStart)
      (:Update
        (Transformation|SetActorLocation _asbp_pigeon_character_ab (Math|Vector|MakeVector (.x (Transformation|GetActorLocation _asbp_pigeon_character_ab)) (.y (Transformation|GetActorLocation _asbp_pigeon_character_ab)) (Math|Float|Lerp _output_get (+ (.z (Transformation|GetWorldLocation (Variables|Default|GetManhole))) (* (.z (Components|Box|GetScaledBoxExtent (Variables|Default|GetBox))) 2.0) 72.0) _alpha)) false true)
        (if (not (Variables|/Game/Blueprints/Characters/Player/ActorComponents/BP_PlayerFlightControl_SO.BP_PlayerFlightControl_SO_C|GetisFlying (Variables|/Game/Blueprints/Characters/Player/BP_PigeonCharacter_AB.BP_PigeonCharacter_AB_C|GetBP_PlayerFlightControl_SO _asbp_pigeon_character_ab)))
          (Utilities|FlowControl|Delay 0.1)
          (Default|InitiateFlightMode (Variables|/Game/Blueprints/Characters/Player/BP_PigeonCharacter_AB.BP_PigeonCharacter_AB_C|GetBP_PlayerFlightControl_SO _asbp_pigeon_character_ab))))
      (:Finished
        (CallFunction|DelayBoost)))))

(event Custom|DelayBoost
  (Utilities|FlowControl|Delay 2.0)
  (Variables|Default|SetCanBoost true))

(fn ConstructionScript
  (bind _box (Variables|Default|GetBox))
  (bind _boxextent (Variables|Default|GetboxExtent))
  (bind _returnvalue (Components|Box|GetScaledBoxExtent _box))
  (Components|Box|SetBoxExtent _box (Math|Vector|MakeVector (.x _returnvalue) (.y _returnvalue) _boxextent) true)
  (Transformation|SetRelativeLocation _box (Math|Vector|MakeVector 0.0 0.0 _boxextent) false false))