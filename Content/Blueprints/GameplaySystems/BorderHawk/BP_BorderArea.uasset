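; BP_BorderArea is a boundary volume that punishes the pigeon player for entering it, themed as a border hawk.
; On box overlap it stores the pigeon's transform and shows the WBP_BorderHawk widget.
; After a short delay it returns the pigeon to walk state, deals heavy damage through its health system, then removes all hawk widgets.
; End overlap only casts, with no further effect.
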(event OnComponentBeginOverlap(Box)
  (params (OverlappedComponent :type Primitive%20Component%20Object%20Reference) (OtherActor :type Actor%20Object%20Reference) (OtherComp :type Primitive%20Component%20Object%20Reference) (OtherBodyIndex :type Integer) (bFromSweep :type Boolean) (SweepResult :type Hit%20Result%20Structure%20%28by%20ref%29))
  (bind _asbp_pigeon_character_ab (Utilities|Casting|CastToBP_PigeonCharacter_AB OtherActor))
  (Variables|Default|SetStarting%20Pos (Transformation|GetActorTransform _asbp_pigeon_character_ab))
  (bind _returnvalue (UserInterface|CreateWidget "/Game/Blueprints/GameplaySystems/BorderHawk/WBP_BorderHawk.WBP_BorderHawk_C" (Game|GetPlayerController 0)))
  (Variables|Default|SetWidgetRef _returnvalue)
  (UserInterface|Viewport|AddtoViewport _returnvalue 0)
  (Utilities|FlowControl|Delay 0.6)
  (Default|ReturntoWalkState (Variables|/Game/Blueprints/Characters/Player/BP_PigeonCharacter_AB.BP_PigeonCharacter_AB_C|GetBP_PlayerFlightControl_SO _asbp_pigeon_character_ab))
  (Default|LoseHealth (Variables|/Game/Blueprints/Characters/Player/BP_PigeonCharacter_AB.BP_PigeonCharacter_AB_C|GetBP_HealthSystem_WK _asbp_pigeon_character_ab) 100)
  (bind _foundwidgets (Widget|GetAllWidgetsOfClass "/Game/Blueprints/GameplaySystems/BorderHawk/WBP_BorderHawk.WBP_BorderHawk_C" true))
  (for _array_element _foundwidgets
    (Widget|RemovefromParent _array_element)))

(event OnComponentEndOverlap(Box)
  (params (OverlappedComponent :type Primitive%20Component%20Object%20Reference) (OtherActor :type Actor%20Object%20Reference) (OtherComp :type Primitive%20Component%20Object%20Reference) (OtherBodyIndex :type Integer))
  (Utilities|Casting|CastToBP_PigeonCharacter_AB OtherActor))

(event EventBeginPlay)

(event Collision|EventActorBeginOverlap
  (params (OtherActor :type Actor%20Object%20Reference)))

(event EventTick
  (params (DeltaSeconds :type Float%20%28single-precision%29)))

(fn ConstructionScript)