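; Quest location marker that reports a location objective and announces the area's name when the pigeon player character enters it.
; Box overlap passes the ObjectiveID to the character's CallOnObjectiveIDCalled, then shows a WBP_LocationNotify widget with LocationName if the capsule is overlapping the box.
; The Sphere component is destroyed on BeginPlay, leaving the box as the trigger.
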(event OnComponentBeginOverlap(Box)
  (params (OverlappedComponent :type Primitive%20Component%20Object%20Reference) (OtherActor :type Actor%20Object%20Reference) (OtherComp :type Primitive%20Component%20Object%20Reference) (OtherBodyIndex :type Integer) (bFromSweep :type Boolean) (SweepResult :type Hit%20Result%20Structure%20%28by%20ref%29))
  ;[0.6875 0.1683 0.1683 0.7216] Checks in the player overlaps the collision and calls the OnObjectiveIDCalled for location quests and displays the location widget
  (Variables|Default|SetisShown false)
  (bind _asbp_pigeon_character_ab (Utilities|Casting|CastToBP_PigeonCharacter_AB OtherActor))
  (Default|CallOnObjectiveIDCalled _asbp_pigeon_character_ab (Utilities|String|StringToName (Variables|Default|GetobjectiveID)))
  (if (Class|PrimitiveComponent|IsOverlappingComponent (Variables|/Script/Engine.Character|GetCapsuleComponent _asbp_pigeon_character_ab) (Variables|Default|GetBox))
    (bind _returnvalue (UserInterface|CreateWidget "/Game/Blueprints/GameplaySystems/Quest/QuestSystem/UI/WBP_LocationNotify.WBP_LocationNotify_C" 0 (Variables|Default|GetlocationName)))
    (Utilities|IsValid _returnvalue
      (:Is%20Valid
        (UserInterface|Viewport|AddtoViewport _returnvalue 0)))))

(event EventBeginPlay
  (Components|DestroyComponent (Variables|Default|GetSphere)))

(event EventTick
  (params (DeltaSeconds :type Float%20%28single-precision%29)))

(fn ConstructionScript)