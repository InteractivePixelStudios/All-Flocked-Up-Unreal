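; Base quest actor that runs one staged quest from DT_QuestData for the pigeon player.
; Objective IDs broadcast by the pigeon raise per-objective counts, showing notifications and advancing stages while the HUD handles the quest arrow.
; The last stage completes the quest and, with AutoComplete, turns it in via AC_QuestLog; quest 00103 also destroys "Destroy"-tagged actors with feather VFX.
; CountdownTime ticks down the quest timer, failing the quest at zero.
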(event Custom|CountdownTime
  (CallFunction|QuestCountdownTimer))

(event Custom|DestroyAtEnd
  (bind _outactors (Actor|GetAllActorswithTag "Destroy"))
  (for _array_element _outactors
    (bind _returnvalue (Niagara|SpawnSystematLocation "/Game/Art/VFX/Player/FeatherPoof/VFX_Feathers.VFX_Feathers" (Transformation|GetActorLocation _array_element) "0, 0, 0" "1.000000,1.000000,1.000000" false))
    (Actor|DestroyActor _array_element)
    (Development|PrintString "check1")
    (Utilities|FlowControl|Delay 0.2)
    (Components|DestroyComponent _returnvalue)))

(event EventBeginPlay
  (CallFunction|GetQuestDetails)
  ;[0.2627 0.5529 1] Gets the quest details and binds event to OnObjectiveIDCalled
  (CallFunction|GetQuestTime)
  (EventDispatchers|BindEventtoOnObjectiveIDCalled (CallFunction|GetPigeonCharacter) (EventDispatchers|CreateEvent :!event OnObjectiveIDHeard))
  ;[0.2627 0.5529 1] Checks if ALL objectives are completed and sets the isCompleted bool true
  (bind _return (CallFunction|AreAllObjectivesComplete))
  (Variables|Default|SetisCompleted _return)
  (bind _returnvalue (Actor|GetActorOfClass "/Game/UI/HUD/BP_NewHud.BP_NewHud_C"))
  (bind _output_get (Variables|Default|SetHUDRef _returnvalue))
  (Default|GetQuestLocation _output_get (Utilities|String|ToString(Name) (Variables|Default|GetquestID)))
  (Default|ShowQuestArrow _output_get))

(event Collision|EventActorBeginOverlap
  (params (OtherActor :type Actor%20Object%20Reference)))

(fn ConstructionScript)

(fn OnObjectiveIDHeard
  (params (ObjectiveID :type Name))
  (bind _returnvalue (Utilities|String|ToString(Name) ObjectiveID))
  (bind _returnvalue_2 (Utilities|String|ToString(Name) ObjectiveID))
  (bind _currentobjectiveprogress (Variables|Default|GetcurrentObjectiveProgress))
  (bind (_value _returnvalue_3) (Utilities|Map|Find _currentobjectiveprogress _returnvalue))
  ;[1 1 1] gets the objectiveID of questgiver and adds the objectives to the currentObjectiveProgress map. When objectives are completed, it cannot be called again from for that questID
  ;;[0.2627 0.5529 1] Checks for objective id matches
  ;;[0.1059 0.1059 0.1059 0.7216] Ensures only set amount can be triggered
  (if (< _value (.Quantity (Utilities|Struct|BreakS_ObjectiveDetails (CallFunction|GetObjectiveDatabyID (Utilities|String|ToString(Name) ObjectiveID)))))
    ;;[0.2627 1 0.251] Adds 1 if match is found
    (if _returnvalue_3
      (Utilities|Map|Add (Variables|Default|GetcurrentObjectiveProgress) _returnvalue_2 (+ _value 1))
      ;;[1 1 1] Calls IsObjectiveComplete
      (CallFunction|IsObjectiveCompleted _returnvalue_2)
      ;;[1 1 1] Calls OnObjectiveIDHeard
      (Default|CallOnObjectiveHeard)
      (return)
      (else
        (return)))))

(fn GetQuestDetails
  ;[0.2627 0.5529 1] Gets and sets quest id in data table
  (bind _returnvalue (Utilities|GetDataTableRow "/Game/Blueprints/GameplaySystems/Quest/QuestSystem/DT_QuestData.DT_QuestData" (Variables|Default|GetquestID))
    (:then
      (bind _output_get (Variables|Default|SetquestDetails _returnvalue))
      ;[0.2627 0.5529 1] sets current stage details
      (bind _output_get_2 (Variables|Default|SetcurrentStageDetails (Utilities|Array|Get(acopy) (.Stages (Utilities|Struct|BreakS_QuestDetails _output_get)) (Variables|Default|GetcurrentStage))))
      ;[0.6875 0.1683 0.1683 0.7216] clears progress array
      (Utilities|Map|Clear (Variables|Default|GetcurrentObjectiveProgress))
      ;[0.2314 0.1137 0.5529] Adds objectives to array
      (for _array_element (.Objectives (Utilities|Struct|BreakS_StageDetails _output_get_2))
        (Utilities|Map|Add (Variables|Default|GetcurrentObjectiveProgress) (.ObjectiveID (Utilities|Struct|BreakS_ObjectiveDetails _array_element)) 0)
        (bind _hudref (Variables|Default|GetHUDRef)
          (:then
            (Default|GetQuestLocation _hudref (.ObjectiveID (Utilities|Struct|BreakS_ObjectiveDetails _array_element)))
            (Default|ShowQuestArrow _hudref))
          (:else))))))

(fn GetObjectiveDatabyID
  (params (ObjectiveID :type String))
  ;[0.2314 0.1137 0.5529] Loops through the objectives array and gets the objective ID. If it matches the stored data it returns it.
  (for _array_element (.Objectives (Utilities|Struct|BreakS_StageDetails (Variables|Default|GetcurrentStageDetails)))
    (if (Utilities|Enum|Equal(Enum) (.ObjectiveID (Utilities|Struct|BreakS_ObjectiveDetails _array_element)) ObjectiveID)
      (return _array_element))))

(fn IsObjectiveCompleted
  (params (ObjectiveID :type String))
  (bind _array_element (CallFunction|GetObjectiveDatabyID ObjectiveID))
  (bind _questid (Variables|Default|GetquestID))
  (bind _hudref (Variables|Default|GetHUDRef))
  (bind (_objectivename _description _objectivetype _objectiveid _quantity) (Utilities|Struct|BreakS_ObjectiveDetails _array_element))
  (Variables|/Game/UI/HUD/BP_NewHud.BP_NewHud_C|SetInQuest (Variables|Default|GetHUDRef) true)
  ;[0.6875 0.1683 0.1683 0.7216] Creates the widget and adds it to the viewport
  (if (>= (.Value (Utilities|Map|Find (Variables|Default|GetcurrentObjectiveProgress) ObjectiveID)) _quantity)
    (bind _returnvalue (UserInterface|CreateWidget "/Game/Blueprints/GameplaySystems/Quest/QuestSystem/UI/WBP_QuestNotification.WBP_QuestNotification_C" 0 _description))
    (UserInterface|Viewport|AddtoViewport _returnvalue 0)
    ;[0.2627 0.5529 1] Checks if all the objectives in the current stage are complete and increments the current stage to the next.
    (bind _return (CallFunction|AreAllObjectivesComplete))
    (if _return
      (bind _result (Math|Integer|IncrementInt (Variables|Default|GetcurrentStage))
        (:%20%20
          ;[0.2627 0.5529 1] Checks if the index is valid in the for the save
          (if (Utilities|Array|IsValidIndex (.stages (Variables|Default|GetquestDetails)) _result)
            ;[0.2314 0.1137 0.5529] if true, it gets the quest details
            (CallFunction|GetQuestDetails)
            (else
              ;[0.2627 0.5529 1] if all objectives ate completed this turns in the quest and completes it.
              (Variables|Default|SetisCompleted true)
              (Variables|/Game/UI/HUD/BP_NewHud.BP_NewHud_C|SetInQuest _hudref false)
              (Default|HideQuestArrow _hudref)
              (if (.autocomplete (Variables|Default|GetquestDetails))
                (Default|TurninQuest (Actor|GetComponentbyClass (CallFunction|GetPigeonCharacter) "/Game/Blueprints/GameplaySystems/Quest/QuestSystem/AC_QuestLog.AC_QuestLog_C") _questid)
                (if (== _questid "00103")
                  (CallFunction|DestroyatEnd))))))))))

(fn AreAllObjectivesComplete
  ;[0.2627 0.5529 1] Gets the objective ID from S_ObjectiveDetails
  (for _array_element (.objectives (Variables|Default|GetcurrentStageDetails))
    ;[0.2314 0.1137 0.5529] If you dont that means the quest is not complete, Once quantity fufilled it sets all complete to true and returns that bool value
    (if (not (>= (.Value (Utilities|Map|Find (Variables|Default|GetcurrentObjectiveProgress) (.ObjectiveID (Utilities|Struct|BreakS_ObjectiveDetails _array_element)))) (.Quantity (Utilities|Struct|BreakS_ObjectiveDetails (CallFunction|GetObjectiveDatabyID (.ObjectiveID (Utilities|Struct|BreakS_ObjectiveDetails _array_element)))))))
      (bind _output_get (LocalVariables|SetlocalAllComplete false))
      (return _output_get)))
  ;[0.6875 0.1683 0.1683 0.7216] If all quests are complete it returns early
  (return (LocalVariables|GetlocalAllComplete)))

(fn QuestCountdownTimer
  (bind _output_get (Variables|Default|SetQuestTimer (Math|Float|Clamp(Float) (- (Variables|Default|GetQuestTimer) (Utilities|Time|GetWorldDeltaSeconds)) 0.0 (Variables|Default|GetQuestMaxTime))))
  (if (<= _output_get 0.0)
    (if (!= (Variables|Default|GetisQuestFail) true)
      (Variables|Default|SetisQuestFail true)
      (bind _returnvalue (UserInterface|CreateWidget "/Game/Blueprints/GameplaySystems/Quest/QuestSystem/UI/WBP_QuestFailed.WBP_QuestFailed_C" 0 "QUEST FAILED!"))
      (UserInterface|Viewport|AddtoViewport _returnvalue 0)
      (Utilities|Map|Clear (Variables|Default|GetcurrentObjectiveProgress)))))

(fn GetQuestTime
  (bind _output_get (Variables|Default|SetQuestMaxTime (.questtime (Variables|Default|GetquestDetails))))
  (Variables|Default|SetQuestTimer _output_get))

(fn ActivateQuestItems)

(fn ShowArrowtoLocation
  (params (ObjectiveID :type Name%20%28by%20ref%29) (PigeonRef :type BP%20Pigeon%20Character%20AB%20Object%20Reference%20%28by%20ref%29))
  (if (Utilities|Enum|Equal(Enum) (.ObjectiveType (Utilities|Struct|BreakS_ObjectiveDetails (CallFunction|GetObjectiveDatabyID (Utilities|String|ToString(Name) ObjectiveID)))) "NewEnumerator0")
    (bind _returnvalue (Actor|GetActorOfClass "/Game/Blueprints/GameplaySystems/Quest/QuestSystem/QuestBuilders/BP_QuestLocationMarker.BP_QuestLocationMarker_C"))
    (Variables|Default|SetTarget _returnvalue)
    (if (Actor|ActorHasTag _returnvalue ObjectiveID)
      _
      (else
        _))
    (bind _returnvalue_2 (Game|SpawnActorfromClass "/Game/Blueprints/GameplaySystems/Quest/QuestSystem/QuestBuilders/BP_QuestArrow.BP_QuestArrow_C" (Transformation|GetActorTransform PigeonRef) "AlwaysSpawn" "MultiplyWithRoot" 0 0 0))
    (Default|SetOwnerandTarget _returnvalue_2 (Variables|Default|GetTarget) PigeonRef)
    (Rendering|SetVisibility (Variables|/Game/Blueprints/GameplaySystems/Quest/QuestSystem/QuestBuilders/BP_QuestArrow.BP_QuestArrow_C|GetArrowBody _returnvalue_2) true false)
    (Rendering|SetVisibility (Variables|/Game/Blueprints/GameplaySystems/Quest/QuestSystem/QuestBuilders/BP_QuestArrow.BP_QuestArrow_C|GetCone _returnvalue_2) true false)
    (return)
    (else
      (return))))