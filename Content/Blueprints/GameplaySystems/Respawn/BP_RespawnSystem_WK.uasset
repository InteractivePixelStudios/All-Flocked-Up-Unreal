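; Respawn component for the pigeon player character that runs the respawn selection screen and returns the player to play.
; StartRespawn waits, shows a fading UW_PickRespawn widget, then switches to UI input and the RespawnManager's view.
; RespawnPlayer resets mesh physics, teleports above the manager's current respawn point, and restores camera, control, health and stamina.
; An older UW_RespawnMap widget path remains disconnected.
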(event Custom|Respawn%20Player
  (bind _returnvalue (Game|GetPlayerController 0))
  (bind _player_ref (Variables|Default|GetPlayer%20Ref))
  (bind _player_ref_2 (Variables|Default|GetPlayer%20Ref))
  (bind _mesh (Variables|/Script/Engine.Character|GetMesh _player_ref_2))
  (bind _bp_healthsystem_wk (Variables|/Game/Blueprints/Characters/Player/BP_PigeonCharacter_AB.BP_PigeonCharacter_AB_C|GetBP_HealthSystem_WK _player_ref))
  (bind _bp_staminasystem_so (Variables|/Game/Blueprints/Characters/Player/BP_PigeonCharacter_AB.BP_PigeonCharacter_AB_C|GetBP_StaminaSystem_SO _player_ref))
  ;[0.231 0.1121 0.5521] Teleports player to selected respawn point
  (Collision|SetCollisionEnabled _mesh "QueryOnly")
  (Physics|SetSimulatePhysics _mesh false)
  (Transformation|ResetRelativeTransform _mesh)
  (Transformation|SetRelativeLocation _mesh "0.000000,0.000000,-21.000000" false false)
  (Transformation|AttachComponentToComponent (Variables|/Game/Blueprints/Characters/Player/BP_PigeonCharacter_AB.BP_PigeonCharacter_AB_C|GetGroundSpringArm _player_ref_2) (Variables|/Game/Blueprints/Characters/Player/BP_PigeonCharacter_AB.BP_PigeonCharacter_AB_C|GetCube _player_ref_2) "None" "KeepRelative" "KeepRelative" "KeepRelative" true)
  (bind _newparam (Default|GetCurrentRespawnPoint (Variables|Default|GetRespawnManager)))
  (Transformation|SetActorLocation (Game|Player|GetPlayerPawn 0) (Math|Vector|MakeVector (.X (Math|Vector|BreakVector (Transformation|GetActorLocation _newparam))) (.Y (Math|Vector|BreakVector (Transformation|GetActorLocation _newparam))) (+ (.Z (Math|Vector|BreakVector (Transformation|GetActorLocation _newparam))) 5e+01)) false false)
  (Widget|RemovefromParent (Variables|Default|GetDebug%20Reference))
  ;[1 1 1] Returns camera and control to the player
  (Variables|Default|SetIsRespawning false)
  (Variables|/Script/Engine.PlayerController|SetbShowMouseCursor _returnvalue false)
  (Input|SetInputModeGameOnly _returnvalue false)
  (Input|EnableInput _player_ref _returnvalue)
  (Game|Player|SetViewTargetwithBlend _returnvalue _player_ref 0.0 "VTBlend_Linear" 0.0 false)
  (Default|TurnUIonOff _player_ref true)
  (Default|RestoreHealth _bp_healthsystem_wk (Variables|/Game/Blueprints/Characters/Player/ActorComponents/BP_HealthSystem_WK.BP_HealthSystem_WK_C|GetHealthMax _bp_healthsystem_wk))
  (Variables|/Game/Blueprints/Characters/Player/ActorComponents/BP_StaminaSystem_SO.BP_StaminaSystem_SO_C|Setstamina _bp_staminasystem_so (Variables|/Game/Blueprints/Characters/Player/ActorComponents/BP_StaminaSystem_SO.BP_StaminaSystem_SO_C|GetmaxStamina _bp_staminasystem_so)))

(event Custom|Start%20Respawn
  (bind _returnvalue (Game|GetPlayerController 0))
  (Utilities|FlowControl|Delay 3.0)
  (Utilities|IsValid (Variables|Default|GetPause%20Reference)
    (:Is%20Valid
      _)
    (:Is%20Not%20Valid
      ;[1 1 1] If widget doesn't exist, make one
      (bind _returnvalue_2 (UserInterface|CreateWidget "/Game/Blueprints/GameplaySystems/Respawn/UW_PickRespawn.UW_PickRespawn_C"))
      (Variables|Default|SetDebug%20Reference _returnvalue_2)))
  (if (not (Variables|Default|GetIsRespawning))
    (UserInterface|Viewport|AddtoViewport (Variables|Default|GetDebug%20Reference) 0)
    (Default|FadeinOut (Variables|Default|GetDebug%20Reference) true)
    (Utilities|FlowControl|Delay 3.0)
    ;[1 1 1] Takes away player control and enters respawn UI
    (Variables|Default|SetIsRespawning true)
    (Variables|/Script/Engine.PlayerController|SetbShowMouseCursor _returnvalue true)
    (Input|SetInputModeUIOnly _returnvalue 0 "DoNotLock" false)
    (Input|EnableInput _returnvalue 0)
    (Game|Player|SetViewTargetwithBlend _returnvalue (Variables|Default|GetRespawnManager) 0.0 "VTBlend_Linear" 0.0 false)
    (Default|FadeinOut (Variables|Default|GetDebug%20Reference) false)
    (Utilities|FlowControl|Delay 1.0)
    (Input|EnableInput _returnvalue 0)))

(event EventBeginPlay
  (bind _returnvalue (Actor|GetActorOfClass "/Game/Blueprints/GameplaySystems/Respawn/BP_RespawnManager.BP_RespawnManager_C"))
  (Variables|Default|SetRespawnManager _returnvalue)
  (bind _asbp_pigeon_character_ab (Utilities|Casting|CastToBP_PigeonCharacter_AB (Components|GetOwner)))
  (Variables|Default|SetPlayer%20Ref _asbp_pigeon_character_ab))

(event EventTick
  (params (DeltaSeconds :type Float%20%28single-precision%29)))