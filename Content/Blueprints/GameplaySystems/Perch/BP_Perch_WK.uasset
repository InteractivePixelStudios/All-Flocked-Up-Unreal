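; Perch actor that lets the player pigeon land on and hop between points along a spline.
; On BeginPlay it spawns an overlap box with a debug outline at each spline point.
; Overlapping a box returns the pigeon from flight to walk state, and SetNewPerch later steps the clamped point index.
; Both trigger a timeline that lerps the pigeon to the point with a jump-curve arc, switching movement from Flying to Falling on arrival.
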(event Custom|Attempt%20Perch
  (params (OverlappedComponent :type Primitive%20Component%20Object%20Reference) (OtherActor :type Actor%20Object%20Reference) (OtherComp :type Primitive%20Component%20Object%20Reference) (OtherBodyIndex :type Integer) (bFromSweep :type Boolean) (SweepResult :type Hit%20Result%20Structure%20%28by%20ref%29))
  (bind _asbox_collision (Utilities|Casting|CastToBoxComponent OverlappedComponent))
  (bind _asbp_pigeon_character_ab (Utilities|Casting|CastToBP_PigeonCharacter_AB OtherActor))
  (if (not (Variables|Default|GetIs%20Perched))
    (Variables|Default|SetIs%20Perched true)
    (Variables|Default|SetIs%20Changing%20Perch true)
    (Variables|Default|SetCurrent%20Perch%20Point%20Location (Transformation|GetWorldLocation OverlappedComponent))
    (Variables|Default|SetCurrent%20Perch%20Point (Utilities|Array|FindItem (Variables|Default|GetSpline%20Boxs) _asbox_collision))
    (Variables|/Game/Blueprints/Characters/Player/BP_PigeonCharacter_AB.BP_PigeonCharacter_AB_C|SetPerch%20ref _asbp_pigeon_character_ab self)
    (Default|ReturntoWalkState (Variables|/Game/Blueprints/Characters/Player/BP_PigeonCharacter_AB.BP_PigeonCharacter_AB_C|GetBP_PlayerFlightControl_SO _asbp_pigeon_character_ab))
    (CallFunction|MovetoNewPerch)))

(event Custom|Set%20New%20Perch
  (params (Input :type Float%20%28double-precision%29))
  (if (not (Variables|Default|GetIs%20Changing%20Perch))
    (Variables|Default|SetIs%20Changing%20Perch true)
    (bind _output_get (Variables|Default|SetCurrent%20Perch%20Point (Math|Integer|Clamp(Integer) (+ (Variables|Default|GetCurrent%20Perch%20Point) Input) 0 (- (Variables|Default|GetTotal%20Spline%20Points) 1))))
    (Variables|Default|SetCurrent%20Perch%20Point%20Location (Transformation|GetWorldLocation (Utilities|Array|Get(acopy) (Variables|Default|GetSpline%20Boxs) _output_get)))
    (CallFunction|MovetoNewPerch)))

(event Custom|Move%20To%20New%20Perch
  (bind _current_perch_point_location (Variables|Default|GetCurrent%20Perch%20Point%20Location))
  (bind _asbp_pigeon_character_ab (Utilities|Casting|CastToBP_PigeonCharacter_AB (Game|GetPlayerCharacter 0)))
  (Pawn|Components|CharacterMovement|SetMovementMode (Variables|/Script/Engine.Character|GetCharacterMovement _asbp_pigeon_character_ab) "MOVE_Flying" 0)
  (bind (_direction _travel_speed _jump_curve) (Timeline|Timeline PlayFromStart)
    (:Update
      (Transformation|SetActorLocation _asbp_pigeon_character_ab (Math|Vector|MakeVector (.x (Math|Vector|Lerp(Vector) (Transformation|GetActorLocation _asbp_pigeon_character_ab) _current_perch_point_location _travel_speed)) (.y (Math|Vector|Lerp(Vector) (Transformation|GetActorLocation _asbp_pigeon_character_ab) _current_perch_point_location _travel_speed)) (+ (.z _jump_curve) (.z (Math|Vector|Lerp(Vector) (Transformation|GetActorLocation _asbp_pigeon_character_ab) _current_perch_point_location _travel_speed)))) false false))
    (:Finished
      (Variables|Default|SetIs%20Changing%20Perch false)
      (Transformation|SetActorLocation _asbp_pigeon_character_ab _current_perch_point_location false false)
      (Pawn|Components|CharacterMovement|SetMovementMode (Variables|/Script/Engine.Character|GetCharacterMovement _asbp_pigeon_character_ab) "MOVE_Falling" 0))))

(event Custom|Leave%20Perch
  (Variables|Default|SetIs%20Perched false))

(event EventBeginPlay
  (bind _spline (Variables|Default|GetSpline))
  (bind _box_half_extent (Variables|Default|GetBox%20Half%20Extent))
  (bind _returnvalue (/ _box_half_extent 2.0))
  (bind _output_get (Variables|Default|SetTotal%20Spline%20Points (Spline|GetNumberOfSplinePoints _spline)))
  (for _index (range 0 _output_get)
    (bind _returnvalue_2 (AddComponent|AddBoxComponent false (Spline|GetTransformatSplinePoint _spline _index "Local" false)))
    (Rendering|Debug|DrawDebugBox (Spline|GetLocationatSplinePoint _spline _index "World") (Math|Vector|MakeVector _box_half_extent (/ _box_half_extent 2.0) _returnvalue) "(R=1.000000,G=0.028412,B=0.000000,A=1.000000)" "0, 0, 0" 1e+05 1.0)
    (Components|Box|SetBoxExtent _returnvalue_2 (Math|Vector|MakeVector _box_half_extent _box_half_extent _returnvalue) true)
    (Collision|BindEventtoOnComponentBeginOverlap _returnvalue_2 (delegate Custom|Attempt%20Perch))
    (Utilities|Array|Add (Variables|Default|GetSpline%20Boxs) _returnvalue_2)))

(event Collision|EventActorBeginOverlap
  (params (OtherActor :type Actor%20Object%20Reference)))

(event EventTick
  (params (DeltaSeconds :type Float%20%28single-precision%29)))

(fn ConstructionScript)