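; Perch spot actor that snaps the pigeon character onto a box that can shift along a spline.
; Box overlap starts landing and hands this spot to the pigeon's perch component.
; While landing, Tick pulls the pigeon to the box, locks it, then after a delay sets the box to a spline point.
; Otherwise Tick runs the leave logic, which offsets the player controller actor, not the pawn; perch input is an empty stub.
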(event OnComponentBeginOverlap(Box)
  (params (OverlappedComponent :type Primitive%20Component%20Object%20Reference) (OtherActor :type Actor%20Object%20Reference) (OtherComp :type Primitive%20Component%20Object%20Reference) (OtherBodyIndex :type Integer) (bFromSweep :type Boolean) (SweepResult :type Hit%20Result%20Structure%20%28by%20ref%29))
  (bind _asbp_pigeon_character_ab (Utilities|Casting|CastToBP_PigeonCharacter_AB OtherActor))
  (bind _output_get (Variables|Default|SetAs%20BP%20Pigeon%20Character%20AB _asbp_pigeon_character_ab))
  (Variables|Default|SetLanding true)
  (Variables|Default|SetPerching true)
  (bind _output_get_2 (Variables|Default|SetPerchRef self))
  (Variables|/Game/Blueprints/Characters/Player/ActorComponents/AC_PlayerPerch.AC_PlayerPerch_C|SetPerchRef (Variables|/Game/Blueprints/Characters/Player/BP_PigeonCharacter_AB.BP_PigeonCharacter_AB_C|GetAC_PlayerPerch _output_get) _output_get_2))

(event Custom|CallLeavePerch
  (Variables|Default|SetLeaving true)
  (Variables|Default|SetPerching false)
  (Variables|Default|SetLanding false)
  (CallFunction|MoveOffPerch))

(event Custom|CallMoveAlongSpline
  (CallFunction|MoveAlongSpline 0.0))

(event Custom|CallPlayerInput
  (CallFunction|PlayerMoveInput)
  (Utilities|FlowControl|Delay 0.2))

(event EventBeginPlay)

(event Collision|EventActorBeginOverlap
  (params (OtherActor :type Actor%20Object%20Reference)))

(event EventTick
  (params (DeltaSeconds :type Float%20%28single-precision%29))
  (if (Variables|Default|GetLanding)
    (CallFunction|Perch)
    (Utilities|FlowControl|Delay 0.5)
    (CallFunction|MoveAlongSpline DeltaSeconds)
    (else
      (CallFunction|CallLeavePerch))))

(fn ConstructionScript)

(fn Perch
  (bind _as_bp_pigeon_character_ab (Variables|Default|GetAs%20BP%20Pigeon%20Character%20AB))
  (if (Variables|Default|GetPerching)
    (bind _returnvalue (Transformation|SetActorLocation _as_bp_pigeon_character_ab (.location (Class|KismetMathLibrary|TInterpto (Math|Conversions|ToTransform(Vector) (Transformation|GetActorLocation _as_bp_pigeon_character_ab)) (Math|Conversions|ToTransform(Vector) (Transformation|GetWorldLocation (Variables|Default|GetBox))) 0.0 0.0)) true false))
    (if _returnvalue
      (CallFunction|PerchLock))))

(fn MoveOffPerch
  (if (Variables|Default|GetLeaving)
    (Transformation|SetActorLocation (Game|GetPlayerController 0) (+ (Transformation|GetWorldLocation (Variables|Default|GetBox)) "0.000000,30.000000,30.000000") false true)))

(fn MoveAlongSpline
  (params (DeltaSeconds :type Float%20%28double-precision%29))
  (bind _spline (Variables|Default|GetSpline))
  (bind _spline_2 (Variables|Default|GetSpline))
  (bind _returnvalue (Spline|GetNumberOfSplinePoints _spline))
  (bind _output_get (Variables|Default|SetSplinePoints _returnvalue))
  (bind _output_get_2 (Variables|Default|SetCurrent%20Point (Math|Integer|Clamp(Integer) _output_get 1 _returnvalue)))
  (if (Variables|Default|GetMovingRight)
    (Transformation|SetRelativeTransform (Variables|Default|GetBox) (Math|Transform|MakeTransform (.location (Spline|GetTransformatSplinePoint _spline_2 _output_get_2 "Local" true)) (.rotation (Spline|GetTransformatSplinePoint _spline_2 _output_get_2 "Local" true)) (.scale (Spline|GetTransformatSplinePoint _spline_2 _output_get_2 "Local" true))) false false)
    (bind _output_get_3 (Variables|Default|SetCurrent%20Point (+ (Variables|Default|GetCurrent%20Point) 1)))
    (Development|PrintString (Utilities|String|ToString(Integer) _output_get_3))
    (else
      (Transformation|SetRelativeTransform (Variables|Default|GetBox) (Math|Transform|MakeTransform (Math|Vector|NegateVector (.location (Spline|GetTransformatSplinePoint _spline_2 _output_get_2 "Local" false))) (.rotation (Spline|GetTransformatSplinePoint _spline_2 _output_get_2 "Local" false)) (.scale (Spline|GetTransformatSplinePoint _spline_2 _output_get_2 "Local" false))) false false)
      (bind _output_get_4 (Variables|Default|SetCurrent%20Point (- (Variables|Default|GetCurrent%20Point) 1)))
      (Development|PrintString (Utilities|String|ToString(Integer) _output_get_4)))))

(fn PerchLock
  (if (Variables|Default|GetPerching)
    (Transformation|SetActorLocation (Variables|Default|GetAs%20BP%20Pigeon%20Character%20AB) (Transformation|GetWorldLocation (Variables|Default|GetBox)) false true)))

(fn PlayerMoveInput)