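; Manager actor that controls when the level's fireflies appear and when they are removed.
; On BeginPlay it caches every placed BP_Fireflies actor and hides them.
; SpawnFlies reveals the cached actors rather than spawning new ones.
; DestroyFlies calls DestroyAfterQuest, which hides and destroys them all.
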(event Custom|DestroyFlies
  (CallFunction|DestroyAfterQuest))

(event Custom|SpawnFlies
  (CallFunction|SpawnFireflies))

(event EventBeginPlay
  (bind _outactors (Actor|GetAllActorsOfClass "/Game/Blueprints/GameplaySystems/Fireflies/BP_Fireflies.BP_Fireflies_C"))
  (bind _output_get (Variables|Default|SetFireFliesRef _outactors))
  (for _array_element _output_get
    (Rendering|SetActorHiddenInGame _array_element true)))

(event Collision|EventActorBeginOverlap
  (params (OtherActor :type Actor%20Object%20Reference)))

(event EventTick
  (params (DeltaSeconds :type Float%20%28single-precision%29)))

(fn ConstructionScript)

(fn SpawnFireflies
  (for _array_element (Variables|Default|GetFireFliesRef)
    (Rendering|SetActorHiddenInGame _array_element false)))

(fn DestroyAfterQuest
  (for _array_element (Variables|Default|GetFireFliesRef)
    (Rendering|SetActorHiddenInGame _array_element true)
    (Actor|DestroyActor _array_element)))