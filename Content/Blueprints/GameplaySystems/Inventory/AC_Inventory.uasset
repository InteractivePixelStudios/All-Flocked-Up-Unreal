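; Inventory component for the pigeon player character, managing Inventory and Stash maps of stackable items keyed by name.
; Adds increment existing stacks or create entries until an item cap diverts to the stash transfer, which only moves items already held.
; Drops spawn actors at points found by sphere-tracing around the player.
; It caches merchant table items at BeginPlay, but shop adding is an empty loop and consumable use is hard-coded to bread.
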(event EventBeginPlay
  (bind _asbp_pigeon_character_ab (Utilities|Casting|CastToBP_PigeonCharacter_AB (Game|Player|GetPlayerPawn 0)))
  (Variables|Default|SetConnectedActor _asbp_pigeon_character_ab)
  (CallFunction|GetShopItems))

(fn TryAddItem
  (params (Storage :type Map%20of%20Strings%20to%20Structs) (CurrectItem1 :type S%20Item%20Data%20Structure))
  (bind _output_get (LocalVariables|SetCurrectItem CurrectItem1))
  (if (CallFunction|IsItemAlreadyinInventory _output_get Storage)
    (CallFunction|IncreaseItemAmount (LocalVariables|GetCurrectItem) Storage)
    (else
      (CallFunction|AddItemtoInventory (LocalVariables|GetCurrectItem) Storage)))
  (Development|PrintString (Utilities|String|Append (.Name (Utilities|Struct|BreakS_ItemData (LocalVariables|GetCurrectItem))) "Added"))
  (return true))

(fn IsItemAlreadyinInventory
  (params (Item :type S%20Item%20Data%20Structure) (Storage :type Map%20of%20Strings%20to%20Structs))
  (return (Utilities|Map|Contains Storage (.Name (Utilities|Struct|BreakS_ItemData Item)))))

(fn AddItemtoInventory
  (params (Item :type S%20Item%20Data%20Structure) (Target%20Destination :type Map%20of%20Strings%20to%20Structs))
  (if (>= (Variables|Default|GetTotalItems) 5)
    (CallFunction|TransferItemtoStash Item)
    (else
      (Utilities|Map|Add Target%20Destination (.Name (Utilities|Struct|BreakS_ItemData Item)) Item)
      (Variables|Default|SetTotalItems (+ (Variables|Default|GetTotalItems) 1)))))

(fn IncreaseItemAmount
  (params (Item :type S%20Item%20Data%20Structure) (Storage :type Map%20of%20Strings%20to%20Structs))
  (LocalVariables|SetItemName (.Name (Utilities|Struct|BreakS_ItemData Item)))
  (bind _result (Math|Integer|IncrementInt (.Amount (Utilities|Struct|BreakS_ItemData (.Value (Utilities|Map|Find Storage (LocalVariables|GetItemName))))))
    (:%20%20
      (bind _structout (Utilities|Struct|SetmembersinS_ItemData (.Value (Utilities|Map|Find Storage (LocalVariables|GetItemName))) _result))
      (Utilities|Map|Add Storage (LocalVariables|GetItemName) _structout))))

(fn RemoveSingleItem
  (params (Key :type String%20%28by%20ref%29) (input :type Map%20of%20Strings%20to%20Structs) (IsTranfer :type Boolean))
  (bind (_value _returnvalue) (Utilities|Map|Find input Key))
  (bind _amount (Utilities|Struct|BreakS_ItemData _value))
  (if _returnvalue
    (if (> _amount 1)
      (bind _structout (Utilities|Struct|SetmembersinS_ItemData _value (- _amount 1)))
      (Utilities|Map|Add input Key _structout)
      ;[1 1 1] check if transfer
      (if IsTranfer
        (return false _structout)
        (else
          (return false _structout)))
      (else
        (LocalVariables|SetDeletedItem _value)
        (Utilities|Map|Remove input Key)
        (if IsTranfer
          (return true "")
          (else
            (return true "")))))))

(fn TracefromAbove
  (bind _connectedactor (Variables|Default|GetConnectedActor))
  (bind _groundcamera (Variables|/Game/Blueprints/Characters/Player/BP_PigeonCharacter_AB.BP_PigeonCharacter_AB_C|GetGroundCamera _connectedactor))
  (bind (_outhit _returnvalue) (Collision|SphereTraceByChannel (Transformation|GetActorLocation (Game|Player|GetPlayerPawn 0)) (+ (+ (Transformation|GetWorldLocation _groundcamera) (* (Math|Vector|GetForwardVector _groundcamera) (+ (Variables|/Script/Engine.SpringArmComponent|GetTargetArmLength (Variables|/Game/Blueprints/Characters/Player/BP_PigeonCharacter_AB.BP_PigeonCharacter_AB_C|GetGroundSpringArm _connectedactor)) 1.5e+02))) "0.000000,0.000000,25.000000") 5.0 "TraceTypeQuery1" false 0 "None"))
  (if _returnvalue
    (return (.ImpactPoint (Collision|BreakHitResult _outhit)))
    (else
      (return (.TraceEnd (Collision|BreakHitResult _outhit))))))

(fn SpawnItem
  (params (Class :type Actor%20Class%20Reference) (Position :type Vector))
  (Game|SpawnActorfromClass Class (Math|Transform|MakeTransform (+ Position "0.000000,0.000000,50.000000")) "Undefined" "MultiplyWithRoot" 0 0))

(fn TraceAroundPlayer
  (bind (_start _end) (CallFunction|GetStartEndTrace (* (Transformation|GetActorForwardVector (Variables|Default|GetConnectedActor)) 1e+02)))
  (bind (_outhit _returnvalue) (Collision|SphereTraceByChannel (- _start "0.000000,0.000000,50.000000") (- _end "0.000000,0.000000,50.000000") 1e+01 "TraceTypeQuery1" false 0 "ForDuration"))
  (if _returnvalue
    (bind (_start_2 _end_2) (CallFunction|GetStartEndTrace (* (Transformation|GetActorRightVector (Variables|Default|GetConnectedActor)) 1e+02)))
    (bind (_outhit_2 _returnvalue_2) (Collision|SphereTraceByChannel (- _start_2 "0.000000,0.000000,50.000000") (- _end_2 "0.000000,0.000000,50.000000") 1e+01 "TraceTypeQuery1" false 0 "ForDuration"))
    (if _returnvalue_2
      (bind (_start_3 _end_3) (CallFunction|GetStartEndTrace (* (Transformation|GetActorRightVector (Variables|Default|GetConnectedActor)) -1e+02)))
      (bind (_outhit_3 _returnvalue_3) (Collision|SphereTraceByChannel (- _start_3 "0.000000,0.000000,50.000000") (- _end_3 "0.000000,0.000000,50.000000") 1e+01 "TraceTypeQuery1" false 0 "ForDuration"))
      (if _returnvalue_3
        (bind (_start_4 _end_4) (CallFunction|GetStartEndTrace (* (Transformation|GetActorForwardVector (Variables|Default|GetConnectedActor)) -1e+02)))
        (bind (_outhit_4 _returnvalue_4) (Collision|SphereTraceByChannel (- _start_4 "0.000000,0.000000,50.000000") (- _end_4 "0.000000,0.000000,50.000000") 1e+01 "TraceTypeQuery1" false 0 "ForDuration"))
        (if _returnvalue_4
          (return (.ImpactPoint (Collision|BreakHitResult _outhit_4)))
          (else
            (return (.TraceEnd (Collision|BreakHitResult _outhit_4)))))
        (else
          (return (.TraceEnd (Collision|BreakHitResult _outhit_3)))))
      (else
        (return (.TraceEnd (Collision|BreakHitResult _outhit_2)))))
    (else
      (return (.TraceEnd (Collision|BreakHitResult _outhit))))))

(fn RemoveItemAll
  (params (ItemName :type String))
  (bind _inventory (Variables|Default|GetInventory))
  (bind (_value _returnvalue) (Utilities|Map|Find _inventory ItemName))
  (bind _amount (Utilities|Struct|BreakS_ItemData _value))
  (if _returnvalue
    (LocalVariables|SetDeletedItem _value)
    (bind _output_get (LocalVariables|SetDropAmount _amount))
    (for _index (range 1 _output_get)
      (bind _structout (Utilities|Struct|SetmembersinS_ItemData (LocalVariables|GetDeletedItem) (- _amount 1)))
      (Utilities|Map|Add (Variables|Default|GetInventory) ItemName _structout)
      (bind _position (CallFunction|TraceAroundPlayer))
      (CallFunction|SpawnItem (.ItemClass (Utilities|Struct|BreakS_ItemData (LocalVariables|GetDeletedItem))) _position))
    (Utilities|Map|Remove (Variables|Default|GetInventory) ItemName)
    (return)))

(fn GetStartEndTrace
  (params (VectorDirection :type Vector))
  (bind _connectedactor (Variables|Default|GetConnectedActor))
  (bind _mesh (Variables|/Script/Engine.Character|GetMesh _connectedactor))
  (bind _returnvalue (Transformation|GetWorldLocation _mesh))
  (return (+ _returnvalue "0.000000,0.000000,100.000000") (+ (+ _returnvalue VectorDirection) "0.000000,0.000000,100.000000")))

(fn RemoveItembyAmount
  (params (Item :type String) (AmountToDrop :type Integer))
  (bind _inventory (Variables|Default|GetInventory))
  (bind _inventory_2 (Variables|Default|GetInventory))
  (bind (_value _returnvalue) (Utilities|Map|Find _inventory Item))
  (bind _value_2 (Utilities|Map|Find _inventory_2 Item))
  (if _returnvalue
    (LocalVariables|SetFoundItem _value)
    (for _index (range 0 (- AmountToDrop 1))
      (bind _structout (Utilities|Struct|SetmembersinS_ItemData (LocalVariables|GetFoundItem) (- (.Amount (Utilities|Struct|BreakS_ItemData _value)) 1)))
      (Utilities|Map|Add (Variables|Default|GetInventory) Item _structout)
      (bind _position (CallFunction|TraceAroundPlayer))
      (CallFunction|SpawnItem (.ItemClass (Utilities|Struct|BreakS_ItemData (LocalVariables|GetFoundItem))) _position))
    (if (== (.Amount (Utilities|Struct|BreakS_ItemData _value_2)) 0)
      (Utilities|Map|Remove (Variables|Default|GetInventory) Item)
      (return "")
      (else
        (return _value_2)))))

(fn AddItemfromShop
  (for _array_element (Variables|Default|GetShopItemArray)
    _))

(fn GetShopItems
  (bind _returnvalue (Actor|GetActorOfClass "/Game/Blueprints/Characters/NPC/InteractWithMerchant/EdgarAllanCrow/BP_MerchantTable.BP_MerchantTable_C"))
  (Variables|Default|SetShopItemArray (Utilities|Array|MakeArray (Variables|/Game/Blueprints/Characters/NPC/InteractWithMerchant/EdgarAllanCrow/BP_MerchantTable.BP_MerchantTable_C|GetItem1 _returnvalue) (Variables|/Game/Blueprints/Characters/NPC/InteractWithMerchant/EdgarAllanCrow/BP_MerchantTable.BP_MerchantTable_C|GetItem2 _returnvalue) (Variables|/Game/Blueprints/Characters/NPC/InteractWithMerchant/EdgarAllanCrow/BP_MerchantTable.BP_MerchantTable_C|GetItem3 _returnvalue) (Variables|/Game/Blueprints/Characters/NPC/InteractWithMerchant/EdgarAllanCrow/BP_MerchantTable.BP_MerchantTable_C|GetItem4 _returnvalue))))

(fn TransferItemtoStash
  (params (Item :type S%20Item%20Data%20Structure))
  (bind (_name _description _catagory _value _stackable _amount _itemclass _icon) (Utilities|Struct|BreakS_ItemData Item))
  (bind _stash (Variables|Default|GetStash))
  (if (CallFunction|IsItemAlreadyinInventory Item (Variables|Default|GetInventory))
    (CallFunction|RemoveSingleItem _name (Variables|Default|GetInventory) true)
    (if (CallFunction|IsItemAlreadyinInventory Item _stash)
      (CallFunction|IncreaseItemAmount Item _stash)
      (else
        (CallFunction|AddItemtoInventory (Utilities|Struct|MakeS_ItemData _name _description _catagory _value _stackable 1 _itemclass _icon) _stash)))
    (else
      (Development|PrintString "NICE TRY CHEATER"))))

(fn TransferItemtoInventory
  (params (Item :type S%20Item%20Data%20Structure))
  (bind (_name _description _catagory _value _stackable _amount _itemclass) (Utilities|Struct|BreakS_ItemData Item))
  (bind _inventory (Variables|Default|GetInventory))
  (if (CallFunction|IsItemAlreadyinInventory Item (Variables|Default|GetStash))
    (CallFunction|RemoveSingleItem _name (Variables|Default|GetStash) true)
    (if (CallFunction|IsItemAlreadyinInventory Item _inventory)
      (CallFunction|IncreaseItemAmount Item _inventory)
      (else
        (CallFunction|AddItemtoInventory (Utilities|Struct|MakeS_ItemData _name _description _catagory _value _stackable 1 _itemclass 0) _inventory)))
    (else
      (Development|PrintString "NICE TRY CHEATER"))))

(fn UseInvConsumable
  (bind _inventory (Variables|Default|GetInventory))
  (bind _keys (Utilities|Map|Keys _inventory))
  (CallFunction|RemoveSingleItem (Utilities|Array|Get(acopy) _keys (Utilities|Array|FindItem _keys "BREAD")) _inventory false))