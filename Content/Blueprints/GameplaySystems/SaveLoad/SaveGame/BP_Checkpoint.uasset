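; BP_Checkpoint is a trigger-sphere checkpoint that saves the game when the pigeon player character overlaps it.
; For each active quest, it writes quest details, quest log and player position to the GameInstance's SavedData, then calls a synchronous player save.
; The save, ping sound and widget sit inside that loop, so no active quests means no save.
; Sphere collision is disabled for a cooldown after BeginPlay and saving.
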(event OnComponentBeginOverlap(Sphere)
  (params (OverlappedComponent :type Primitive%20Component%20Object%20Reference) (OtherActor :type Actor%20Object%20Reference) (OtherComp :type Primitive%20Component%20Object%20Reference) (OtherBodyIndex :type Integer) (bFromSweep :type Boolean) (SweepResult :type Hit%20Result%20Structure%20%28by%20ref%29))
  (bind _sphere (Variables|Default|GetSphere))
  (bind _asbp_game_instance (Utilities|Casting|CastToBP_GameInstance (Game|GetGameInstance)))
  (bind _saveddata (Variables|/Game/Blueprints/GameplaySystems/SaveLoad/SaveGame/BP_GameInstance.BP_GameInstance_C|GetSavedData _asbp_game_instance)
    (:then
      (bind _asbp_pigeon_character_ab (Utilities|Casting|CastToBP_PigeonCharacter_AB OtherActor))
      ;[1 1 1] Checkpoint Overlap Trigger
      (bind _ac_questlog (Variables|/Game/Blueprints/Characters/Player/BP_PigeonCharacter_AB.BP_PigeonCharacter_AB_C|GetAC_QuestLog _asbp_pigeon_character_ab)
        (:then
          (for _array_element (Variables|/Game/Blueprints/GameplaySystems/Quest/QuestSystem/AC_QuestLog.AC_QuestLog_C|GetcurrentActiveQuests _ac_questlog)
            (Default|SaveQuestDetails _saveddata _array_element)
            (Default|SaveQuestLog _saveddata _ac_questlog)
            (Default|SavePlayerPos _saveddata (Variables|Default|GetPlayerRef))
            (bind _playersave (Default|GetSaveData _asbp_pigeon_character_ab))
            (Class|BPISaveGame|SavePlayer(Message) (Game|GetGameInstance) _playersave false)
            (Audio|PlaySound2D "/Engine/EngineSounds/1kSineTonePing.1kSineTonePing" 1.0 1.0 0.0 0 0)
            (bind _returnvalue (UserInterface|CreateWidget "/Game/Blueprints/GameplaySystems/SaveLoad/SaveGame/W_SaveGameWidget.W_SaveGameWidget_C"))
            (UserInterface|Viewport|AddtoViewport _returnvalue 0)
            (Collision|SetCollisionEnabled _sphere "NoCollision")
            (Utilities|FlowControl|Delay 1e+01)
            (Collision|SetCollisionEnabled _sphere "QueryAndProbe")))
        (:else)))
    (:else)))

(event EventBeginPlay
  (bind _sphere (Variables|Default|GetSphere))
  (Collision|SetCollisionEnabled _sphere "NoCollision")
  (Utilities|FlowControl|Delay 1e+01)
  (Collision|SetCollisionEnabled _sphere "QueryAndProbe"))

(event Collision|EventActorBeginOverlap
  (params (OtherActor :type Actor%20Object%20Reference))
  ;[1 1 1] Checkpoint Overlap Trigger
)

(fn ConstructionScript)