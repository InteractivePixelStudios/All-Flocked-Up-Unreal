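; Save game Blueprint that stores and restores the player's state and quest progress.
; SavePlayerPos packs transform, rotation, health, level, XP, tracked stats and inventory into a player save struct, which LoadPlayerPos applies back through PlayerReference.
; SaveQuestLog copies active and completed quest lists, while SaveQuestDetails maps each quest ID to its stage and objective progress.
; LoadQuests re-adds active quests to the given log and restores their progress from that map.
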(fn SaveQuestDetails
  (params (Quest :type BP%20Quests%20Base%20Object%20Reference))
  (Utilities|Map|Add (Variables|Default|GetquestProgress) (Variables|/Game/Blueprints/GameplaySystems/Quest/QuestSystem/BP_QuestsBase.BP_QuestsBase_C|GetquestID Quest) (Utilities|Struct|MakeS_PlayerSave "0.000000,0.000000,0.000000|0.000000,0.000000,0.000000|1.000000,1.000000,1.000000" 0.0 "0.000000,0.000000,0.000000" (Variables|/Game/Blueprints/GameplaySystems/Quest/QuestSystem/BP_QuestsBase.BP_QuestsBase_C|GetcurrentObjectiveProgress Quest) (Variables|/Game/Blueprints/GameplaySystems/Quest/QuestSystem/BP_QuestsBase.BP_QuestsBase_C|GetcurrentStage Quest))))

(fn LoadQuests
  (params (Quest%20Log%20Component :type AC%20Quest%20Log%20Object%20Reference))
  (for _array_element (Variables|Default|GetcurrentActiveQuests)
    (bind _returnvalue (Default|AddNewQuest Quest%20Log%20Component _array_element))
    (Variables|/Game/Blueprints/GameplaySystems/Quest/QuestSystem/BP_QuestsBase.BP_QuestsBase_C|SetcurrentStage _returnvalue (.CurrentQuestStage (Utilities|Struct|BreakS_PlayerSave (.Value (Utilities|Map|Find (Variables|Default|GetquestProgress) _array_element)))))
    (Variables|/Game/Blueprints/GameplaySystems/Quest/QuestSystem/BP_QuestsBase.BP_QuestsBase_C|SetcurrentObjectiveProgress _returnvalue (.QuestProgress (Utilities|Struct|BreakS_PlayerSave (.Value (Utilities|Map|Find (Variables|Default|GetquestProgress) _array_element)))))))

(fn SaveQuestLog
  (params (QuestLog :type AC%20Quest%20Log%20Object%20Reference))
  (Variables|Default|SetcurrentActiveQuests (Variables|/Game/Blueprints/GameplaySystems/Quest/QuestSystem/AC_QuestLog.AC_QuestLog_C|GetcurrentActiveQuest QuestLog))
  (Variables|Default|SetcompletedQuests (Variables|/Game/Blueprints/GameplaySystems/Quest/QuestSystem/AC_QuestLog.AC_QuestLog_C|GetcompletedQuests QuestLog)))

(fn LoadPlayerPos
  (params (NewParam :type S%20Player%20Save%20Structure))
  (bind (_transform _health _controlrotation _questprogress _currentqueststage _keyvalues _level _xp _playerstatstracked _playerinventory) (Utilities|Struct|BreakS_PlayerSave NewParam))
  (bind _playerreference (Variables|Default|GetPlayerReference))
  (bind _bp_xpmanager_js (Variables|/Game/Blueprints/Characters/Player/BP_PigeonCharacter_AB.BP_PigeonCharacter_AB_C|GetBP_XPManager_JS _playerreference))
  (Transformation|SetActorTransform _playerreference _transform)
  (Transformation|SetActorRotation _playerreference _controlrotation)
  (Variables|/Game/Blueprints/Characters/Player/ActorComponents/BP_HealthSystem_WK.BP_HealthSystem_WK_C|SetHealthCurrent (Variables|/Game/Blueprints/Characters/Player/BP_PigeonCharacter_AB.BP_PigeonCharacter_AB_C|GetBP_HealthSystem_WK _playerreference) (Math|Float|Truncate _health))
  (Variables|/Game/Blueprints/Characters/Player/BP_XPManager_JS.BP_XPManager_JS_C|SetPlayerLevel _bp_xpmanager_js _level)
  (Variables|/Game/Blueprints/Characters/Player/BP_XPManager_JS.BP_XPManager_JS_C|SetCurrentXP _bp_xpmanager_js (Math|Conversions|ToFloat(Integer) _xp))
  (Default|SetLoadedStats (Variables|/Game/Blueprints/Characters/Player/BP_PigeonCharacter_AB.BP_PigeonCharacter_AB_C|GetAC_PlayerStatTracker _playerreference) _playerstatstracked)
  (Variables|/Game/Blueprints/GameplaySystems/Inventory/AC_Inventory.AC_Inventory_C|SetInventory (Variables|/Game/Blueprints/Characters/Player/BP_PigeonCharacter_AB.BP_PigeonCharacter_AB_C|GetAC_Inventory _playerreference) _playerinventory))

(fn SavePlayerPos
  (params (Player%20Ref :type BP%20Pigeon%20Character%20AB%20Object%20Reference))
  (bind _bp_xpmanager_js (Variables|/Game/Blueprints/Characters/Player/BP_PigeonCharacter_AB.BP_PigeonCharacter_AB_C|GetBP_XPManager_JS Player%20Ref))
  (bind _questbaseref (Variables|Default|GetQuestBaseRef))
  (Utilities|IsValid Player%20Ref
    (:Is%20Valid
      (bind _playerstats (Default|GetAllStats (Variables|/Game/Blueprints/Characters/Player/BP_PigeonCharacter_AB.BP_PigeonCharacter_AB_C|GetAC_PlayerStatTracker Player%20Ref)))
      (bind _output_get (Variables|Default|SetplayerSave (Utilities|Struct|MakeS_PlayerSave (Transformation|GetActorTransform Player%20Ref) (Math|Conversions|ToFloat(Integer) (Variables|/Game/Blueprints/Characters/Player/ActorComponents/BP_HealthSystem_WK.BP_HealthSystem_WK_C|GetHealthCurrent (Variables|/Game/Blueprints/Characters/Player/BP_PigeonCharacter_AB.BP_PigeonCharacter_AB_C|GetBP_HealthSystem_WK Player%20Ref))) (Transformation|GetActorRotation Player%20Ref) (Variables|/Game/Blueprints/GameplaySystems/Quest/QuestSystem/BP_QuestsBase.BP_QuestsBase_C|GetcurrentObjectiveProgress _questbaseref) (Variables|/Game/Blueprints/GameplaySystems/Quest/QuestSystem/BP_QuestsBase.BP_QuestsBase_C|GetcurrentStage _questbaseref) 0 (Variables|/Game/Blueprints/Characters/Player/BP_XPManager_JS.BP_XPManager_JS_C|GetPlayerLevel _bp_xpmanager_js) (Math|Float|Truncate (Variables|/Game/Blueprints/Characters/Player/BP_XPManager_JS.BP_XPManager_JS_C|GetCurrentXP _bp_xpmanager_js)) _playerstats (Variables|/Game/Blueprints/GameplaySystems/Inventory/AC_Inventory.AC_Inventory_C|GetInventory (Variables|/Game/Blueprints/Characters/Player/BP_PigeonCharacter_AB.BP_PigeonCharacter_AB_C|GetAC_Inventory Player%20Ref)))))
      (return _output_get))))