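; Three-way (North, East, South) traffic intersection that queues cars and routes them along splines.
; GetCarDirection reads entry from box tags, picks a random other exit and returns whether the car can proceed.
; Tick releases stopped queued cars on NorthSouthIsGreen, as its East selector is all false, assigning a spline, travel direction and start distance.
; The built-in light-switching timer is unconnected.
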(event EventBeginPlay
  ;[1 1 1] BeginPlay
  ;;[1 1 1] For each exitSpline in array
  (for (_array_element _array_index) (Variables|Default|GetDirectional%20Exit%20Spline%20Objects)
    ;;[1 1 1] Insert Spline ref into ExitSpline array index
    (Utilities|Array|Insert (Variables|Default|GetDirectional%20Exit%20Splines) (Actor|GetComponentbyClass _array_element "/Script/Engine.SplineComponent") _array_index)))

(event EventTick
  (params (DeltaSeconds :type Float%20%28single-precision%29))
  (bind _car_priority_list (Variables|Default|GetCar%20Priority%20List))
  ;[1 1 1] EventTick
  ;;[1 1 1] For each car in prio list
  (for _array_element _car_priority_list
    ;;[1 1 1] Check if car stopped
    (if (Variables|/Game/Blueprints/GameplaySystems/TrafficSystem/BP_Car_WK.BP_Car_WK_C|GetIs%20Stopped _array_element)
      ;;[1 1 1] Check if return true/false
      (if (Utilities|Select :Index (Variables|/Game/Blueprints/GameplaySystems/TrafficSystem/BP_Car_WK.BP_Car_WK_C|GetEnter%20Direction _array_element) :Option%200 false :Option%201 false :Option%202 false)
        ;;[1 1 1] Check if East is Green
        (if (Variables|Default|GetEast%20is%20Green)
          ;;[1 1 1] Get new spline
          (bind (_out_spline _direction_is_reversed) (CallFunction|GetTravelSpline (Variables|/Game/Blueprints/GameplaySystems/TrafficSystem/BP_Car_WK.BP_Car_WK_C|GetEnter%20Direction _array_element) (Variables|/Game/Blueprints/GameplaySystems/TrafficSystem/BP_Car_WK.BP_Car_WK_C|GetExit%20Direction _array_element) :!label _label))
          ;;[1 1 1] Set spline ref and isReverse
          (Variables|/Game/Blueprints/GameplaySystems/TrafficSystem/BP_Car_WK.BP_Car_WK_C|SetSpline%20Refrence _array_element _out_spline)
          (Variables|/Game/Blueprints/GameplaySystems/TrafficSystem/BP_Car_WK.BP_Car_WK_C|SetIs%20Reverse%20Direction _array_element _direction_is_reversed)
          ;;[1 1 1] Check if start or end of spline and set distance along spline
          (Variables|/Game/Blueprints/GameplaySystems/TrafficSystem/BP_Car_WK.BP_Car_WK_C|SetCar%20Distance%20Along%20Spline _array_element (select _direction_is_reversed (Spline|GetSplineLength _out_spline) 0.0))
          ;;[1 1 1] Set WK_Car IsStopped = False
          (Variables|/Game/Blueprints/GameplaySystems/TrafficSystem/BP_Car_WK.BP_Car_WK_C|SetIs%20Stopped _array_element false)
          ;;[1 1 1] Remove car form prio list
          (Utilities|Array|RemoveItem _car_priority_list _array_element))
        (else
          ;;[1 1 1] Check if N/S is Green
          (if (Variables|Default|GetNorthSouth%20is%20Green)
            (goto _label)))))))

(fn ConstructionScript)

(fn AddtoPriorityList
  (params (Car%20In%20Question :type BP%20Car%20WK%20Object%20Reference))
  (bind _returnvalue (Utilities|Array|Add (Variables|Default|GetCar%20Priority%20List) Car%20In%20Question))
  (Variables|/Game/Blueprints/GameplaySystems/TrafficSystem/BP_Car_WK.BP_Car_WK_C|SetIntersection%20Priority Car%20In%20Question _returnvalue))

(fn GetCarDirection
  (params (Contacted%20Box :type Box%20Component%20Object%20Reference))
  (bind _componenttags (Variables|/Script/Engine.ActorComponent|GetComponentTags Contacted%20Box))
  (Variables|Default|SetGood%20To%20Go false)
  (bind (_result _opposite_result) (Utilities|Elseif (Utilities|Array|ContainsItem _componenttags "North") 0 (Utilities|Array|ContainsItem _componenttags "East") 1 (Utilities|Array|ContainsItem _componenttags "South") 2)
    (:%20%20
      (bind _exit_direction (CallFunction|GetNewRandomDirection _result))
      (if (!= _exit_direction _opposite_result)
        (Variables|Default|SetGood%20To%20Go false)
        (elif (select (Utilities|Select :Index _exit_direction :Option%200 false :Option%201 true :Option%202 false) (Variables|Default|GetEast%20is%20Green) (Variables|Default|GetNorthSouth%20is%20Green))
          (for _array_element (Variables|Default|GetCar%20Priority%20List)
            (Variables|Default|SetGood%20To%20Go (!= (Variables|/Game/Blueprints/GameplaySystems/TrafficSystem/BP_Car_WK.BP_Car_WK_C|GetExit%20Direction _array_element) _exit_direction)))))
      (return _exit_direction (Variables|Default|GetGood%20To%20Go) _result))))

(fn GetNewRandomDirection
  (params (Entering%20Direction :type Integer))
  (Utilities|Array|Clear (Variables|Default|GetRan%20Direction%20Array))
  (for (_array_element _array_index) (LocalVariables|GetRan%20Direction%20Array%20REF)
    (Utilities|Array|Insert (Variables|Default|GetRan%20Direction%20Array) _array_element _array_index))
  (Utilities|Array|RemoveIndex (Variables|Default|GetRan%20Direction%20Array) Entering%20Direction)
  (return (Utilities|Array|Get(acopy) (Variables|Default|GetRan%20Direction%20Array) (Math|Random|RandomInteger 2))))

(fn GetExitSpline
  (params (Spline%20to%20Switch%20too :type Integer) (Reveresed%20Direction :type Boolean))
  (return (Utilities|Array|Get(acopy) (Variables|Default|GetDirectional%20Exit%20Splines) Spline%20to%20Switch%20too) Reveresed%20Direction))

(fn GetTravelSpline
  (params (Entry :type Integer) (Exit :type Integer))
  (bind _southeast (Variables|Default|GetSouthEast))
  (bind _northeast (Variables|Default|GetNorthEast))
  (bind _northsouth (Variables|Default|GetNorthSouth))
  (switch int Entry
    (:0
      (switch int Exit
        (:1
          (return _northeast true))
        (:2
          (return _northsouth true))))
    (:1
      (switch int Exit
        (:0
          (return _northeast false))
        (:2
          (return _southeast true))))
    (:2
      (switch int Exit
        (:0
          (return _northsouth false))
        (:1
          (return _southeast false))))))