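; AI traffic car that follows splines in either direction with a lane offset, accelerating to a speed limit and lerping its position each tick.
; Box overlaps halt it for stopped cars outside intersections or for enemies, resuming after a delay once overlap ends.
; At BP_CarTrafficPath_WK and T-path junctions it stops, joins their priority list, takes a travel spline if clear, then switches to the exit spline at the matching direction-tagged box.
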(event OnComponentBeginOverlap(Box)
  (params (OverlappedComponent :type Primitive%20Component%20Object%20Reference) (OtherActor :type Actor%20Object%20Reference) (OtherComp :type Primitive%20Component%20Object%20Reference) (OtherBodyIndex :type Integer) (bFromSweep :type Boolean) (SweepResult :type Hit%20Result%20Structure%20%28by%20ref%29))
  ;[1 1 1] BeginOverlap
  ;;[1 1 1] cast to car and check if self. if not continue
  (bind _asbp_car_wk (Utilities|Casting|CastToBP_Car_WK OtherActor)
    (:then
      (if (not (== _asbp_car_wk self))
        ;;[1 1 1] Check if stopped
        (if (Variables|BP_Car_WK_C|GetIs%20Stopped _asbp_car_wk)
          ;;[1 1 1] check if at intersection; if NOT stop car
          (if (not (Variables|Default|GetIn%20Intersection))
            ;;[1 1 1] Stops car if overlapping self or BaseEnemy
            (CallFunction|StopCar true :!label _label)))))
    (:CastFailed
      ;;[1 1 1] fail= cast to BaseEnemy?
      (Utilities|Casting|CastToBP_BaseEnemy OtherActor
        (:then
          (goto _label))
        (:CastFailed
          ;;[1 1 1] Fail=Cast to TrafficPath?
          (bind _asbp_car_traffic_path_wk (Utilities|Casting|CastToBP_CarTrafficPath_WK OtherActor)
            (:then
              ;;[1 1 1] checks if at intersection
              (if (Variables|Default|GetIn%20Intersection)
                ;;[1 1 1] Cast to BoxComp and checks for N,S,E,W tag
                (bind _asbox_collision (Utilities|Casting|CastToBoxComponent OtherComp))
                ;;[1 1 1] sets int and checks if result=ExitDirection
                (bind _result (Utilities|Elseif (Utilities|Array|ContainsItem (Variables|/Script/Engine.ActorComponent|GetComponentTags _asbox_collision) "North") 0 (Utilities|Array|ContainsItem (Variables|/Script/Engine.ActorComponent|GetComponentTags _asbox_collision) "East") 1 (Utilities|Array|ContainsItem (Variables|/Script/Engine.ActorComponent|GetComponentTags _asbox_collision) "South") 2 (Utilities|Array|ContainsItem (Variables|/Script/Engine.ActorComponent|GetComponentTags _asbox_collision) "West") 3)
                  (:%20%20
                    (if (== _result (Variables|Default|GetExit%20Direction))
                      ;;[1 1 1] Set InIntersection = False
                      (Variables|Default|SetIn%20Intersection false)
                      ;;[1 1 1] GetExitSplinesArray and get the ExitDirection int value member; Set as Spline Ref
                      (Variables|Default|SetIs%20Reverse%20Direction (Utilities|Array|Get(acopy) (Variables|/Game/Blueprints/GameplaySystems/TrafficSystem/BP_CarTrafficPath_WK.BP_CarTrafficPath_WK_C|GetExit%20Direction%20is%20Reversed _asbp_car_traffic_path_wk) (Variables|Default|GetExit%20Direction)))
                      (Variables|Default|SetSpline%20Refrence (Utilities|Array|Get(acopy) (Variables|/Game/Blueprints/GameplaySystems/TrafficSystem/BP_CarTrafficPath_WK.BP_CarTrafficPath_WK_C|GetDirectional%20Exit%20Splines _asbp_car_traffic_path_wk) (Variables|Default|GetExit%20Direction)))
                      ;;[1 1 1] Set output and CarDistanceAlongSpline and set IsStopped=False
                      (Variables|Default|SetCar%20Distance%20Along%20Spline (select (stale _output_get_3) (Spline|GetSplineLength (stale _output_get_4)) 0.0) :!label _label_2)
                      (Variables|Default|SetIs%20Stopped false))))
                (else
                  ;;[1 1 1] Sets InIntersection = True and calls StopCar
                  (Variables|Default|SetIn%20Intersection true)
                  (CallFunction|StopCar false)
                  ;;[1 1 1] Cast to BoxComp
                  (bind _asbox_collision_2 (Utilities|Casting|CastToBoxComponent OtherComp))
                  ;;[1 1 1] Call GetCarDirection
                  (bind (_output_exit_direction _good_to_go_through _output_enter_direction) (Default|GetCarDirection _asbp_car_traffic_path_wk _asbox_collision_2))
                  ;;[1 1 1] Sets Output as Exit & Enter Direction
                  (bind _output_get (Variables|Default|SetExit%20Direction _output_exit_direction))
                  (bind _output_get_2 (Variables|Default|SetEnter%20Direction _output_enter_direction))
                  ;;[1 1 1] Add to Prio List
                  (Default|AddtoPriorityList _asbp_car_traffic_path_wk self)
                  ;;[1 1 1] Checks IfGoodToGo
                  (if _good_to_go_through
                    ;;[1 1 1] Get Next Spline
                    (bind (_out_spline _direction_is_reversed) (Default|GetTravelSpline _asbp_car_traffic_path_wk _output_get_2 _output_get))
                    ;;[1 1 1] Set if reverse direction and new spline ref
                    (bind _output_get_3 (Variables|Default|SetIs%20Reverse%20Direction _direction_is_reversed))
                    (bind _output_get_4 (Variables|Default|SetSpline%20Refrence _out_spline))
                    (goto _label_2)))))
            (:CastFailed
              ;;[1 1 1] Fail = cast to TrafficTPath?
              (bind _asbp_car_traffic_tpath_wk (Utilities|Casting|CastToBP_CarTrafficTPath_WK OtherActor))
              ;;[1 1 1] Checks if InIntersection
              (if (Variables|Default|GetIn%20Intersection)
                ;;[1 1 1] Cast to BoxComp and check for N,E,S tags
                (bind _asbox_collision_3 (Utilities|Casting|CastToBoxComponent OtherComp))
                ;;[1 1 1] Set as int and checks if result = ExitDirection
                (bind _result_2 (Utilities|Elseif (Utilities|Array|ContainsItem (Variables|/Script/Engine.ActorComponent|GetComponentTags _asbox_collision_3) "North") 0 (Utilities|Array|ContainsItem (Variables|/Script/Engine.ActorComponent|GetComponentTags _asbox_collision_3) "East") 1 (Utilities|Array|ContainsItem (Variables|/Script/Engine.ActorComponent|GetComponentTags _asbox_collision_3) "South") 2 false)
                  (:%20%20
                    ;;[1 1 1] if true set InIntersection=False
                    (if (== _result_2 (Variables|Default|GetExit%20Direction))
                      (Variables|Default|SetIn%20Intersection false)
                      ;;[1 1 1] I Think this might be the problem
                      ;;;[1 1 1] Checks if Int index is reversed
                      (Variables|Default|SetIs%20Reverse%20Direction (Utilities|Array|Get(acopy) (Variables|/Game/Blueprints/GameplaySystems/TrafficSystem/BP_CarTrafficTPath_WK.BP_CarTrafficTPath_WK_C|GetExit%20Direction%20is%20Reversed _asbp_car_traffic_tpath_wk) (Variables|Default|GetExit%20Direction)))
                      (Variables|Default|SetSpline%20Refrence (Utilities|Array|Get(acopy) (Variables|/Game/Blueprints/GameplaySystems/TrafficSystem/BP_CarTrafficTPath_WK.BP_CarTrafficTPath_WK_C|GetDirectional%20Exit%20Splines _asbp_car_traffic_tpath_wk) (Variables|Default|GetExit%20Direction)))
                      ;;[1 1 1] Set output as CarDistanceAlongSpline & IsStopped =False
                      (Variables|Default|SetCar%20Distance%20Along%20Spline (select (stale _output_get_7) (Spline|GetSplineLength (stale _output_get_8)) 0.0) :!label _label_3)
                      (Variables|Default|SetIs%20Stopped false))))
                (else
                  ;;[1 1 1] Sets InIntersection=True
                  (Variables|Default|SetIn%20Intersection true)
                  ;;[1 1 1] Call StopCar
                  (CallFunction|StopCar false)
                  ;;[1 1 1] Cast to BoxComp
                  (bind _asbox_collision_4 (Utilities|Casting|CastToBoxComponent OtherComp))
                  ;;[1 1 1] Call GetCarDirection
                  (bind (_output_exit_direction_2 _good_to_go_through_2 _output_enter_direction_2) (Default|GetCarDirection _asbp_car_traffic_tpath_wk _asbox_collision_4))
                  ;;[1 1 1] Sets output as Exit & Enter Direction
                  (bind _output_get_5 (Variables|Default|SetExit%20Direction _output_exit_direction_2))
                  (bind _output_get_6 (Variables|Default|SetEnter%20Direction _output_enter_direction_2))
                  ;;[1 1 1] Add to Prio List
                  (Default|AddtoPriorityList _asbp_car_traffic_tpath_wk self)
                  ;;[1 1 1] Check IfGoodToGo
                  (if _good_to_go_through_2
                    ;;[1 1 1] Get Next Spline
                    (bind (_out_spline_2 _direction_is_reversed_2) (Default|GetTravelSpline _asbp_car_traffic_tpath_wk _output_get_6 _output_get_5))
                    ;;[1 1 1] set IsReverse and SplineRef
                    (bind _output_get_7 (Variables|Default|SetIs%20Reverse%20Direction _direction_is_reversed_2))
                    (bind _output_get_8 (Variables|Default|SetSpline%20Refrence _out_spline_2))
                    (goto _label_3)))))))))))

(event OnComponentEndOverlap(Box)
  (params (OverlappedComponent :type Primitive%20Component%20Object%20Reference) (OtherActor :type Actor%20Object%20Reference) (OtherComp :type Primitive%20Component%20Object%20Reference) (OtherBodyIndex :type Integer))
  ;[1 1 1] BeginOverlap
  ;;[1 1 1] EndOverlap
  ;;;[1 1 1] Box not overlapping self?
  (bind _asbp_car_wk (Utilities|Casting|CastToBP_Car_WK OtherActor)
    (:then
      (if (not (== _asbp_car_wk self))
        ;;;[1 1 1] Delay and set IsStopped= False
        (Utilities|FlowControl|Delay 1.0 :!label _label)
        (Variables|Default|SetIs%20Stopped false)))
    (:CastFailed
      ;;;[1 1 1] Check if not overlapping BaseEnemy
      (Utilities|Casting|CastToBP_BaseEnemy OtherActor)
      (goto _label))))

(event EventBeginPlay
  (bind _object_with_spline_to_start_on (Variables|Default|GetObject%20with%20spline%20to%20start%20on))
  (bind _car_distance_along_spline (Variables|Default|GetCar%20Distance%20Along%20Spline))
  (bind _lane_offset (Variables|Default|GetLane%20Offset))
  (bind _is_reverse_direction (Variables|Default|GetIs%20Reverse%20Direction))
  (bind _returnvalue (Actor|GetComponentbyClass _object_with_spline_to_start_on "/Script/Engine.SplineComponent"))
  ;[1 1 1] BeginPlay
  ;;[1 1 1] Get car ref
  (Variables|/Game/Audio/Audio/Blueprints/Audio_Profiles/AudioPrfiles(v2)/BP_AP_Car2.BP_AP_Car2_C|SetCarRef (Variables|Default|GetBP_AP_Car2) self)
  (Utilities|IsValid (Variables|Default|GetSpline%20Refrence) :!label _label
    (:Is%20Valid
      ;;[1 1 1] Set Loc &Rot
      (Transformation|SetActorLocationAndRotation (+ (Spline|GetLocationatDistanceAlongSpline (Variables|Default|GetSpline%20Refrence) _car_distance_along_spline "World") (* (Class|SplineComponent|GetRightVectoratDistanceAlongSpline (Variables|Default|GetSpline%20Refrence) _car_distance_along_spline "World") (Math|Float|SelectFloat (* _lane_offset -1.0) _lane_offset _is_reverse_direction))) (Math|Rotator|MakeRotator (.roll (Spline|GetRotationatDistanceAlongSpline (Variables|Default|GetSpline%20Refrence) _car_distance_along_spline "World")) (.pitch (Spline|GetRotationatDistanceAlongSpline (Variables|Default|GetSpline%20Refrence) _car_distance_along_spline "World")) (Math|Float|SelectFloat (+ (.yaw (Spline|GetRotationatDistanceAlongSpline (Variables|Default|GetSpline%20Refrence) _car_distance_along_spline "World")) 1.8e+02) (.yaw (Spline|GetRotationatDistanceAlongSpline (Variables|Default|GetSpline%20Refrence) _car_distance_along_spline "World")) _is_reverse_direction)) false true))
    (:Is%20Not%20Valid
      ;;[1 1 1] Gets obj with spline to start and sets spline ref if not already set
      (Utilities|IsValid _returnvalue
        (:Is%20Valid
          (Variables|Default|SetSpline%20Refrence _returnvalue)
          (goto _label))))))

(event EventTick
  (params (DeltaSeconds :type Float%20%28single-precision%29))
  (bind _current_speed (Variables|Default|GetCurrent%20Speed))
  (bind _returnvalue (* _current_speed DeltaSeconds))
  ;[1 1 1] EventTick
  ;;[1 1 1] Check if stopped
  (if (Variables|Default|GetIs%20Stopped)
    (CallFunction|StopCar false)
    (else
      ;;[1 1 1] Checks if spline ref is valid
      (Utilities|IsValid (Variables|Default|GetSpline%20Refrence)
        (:Is%20Valid
          ;;[1 1 1] Set car distance along spline
          (Variables|Default|SetCar%20Distance%20Along%20Spline (Math|Float|SelectFloat (- (Variables|Default|GetCar%20Distance%20Along%20Spline) _returnvalue) (+ (Variables|Default|GetCar%20Distance%20Along%20Spline) _returnvalue) (Variables|Default|GetIs%20Reverse%20Direction)))
          (CallFunction|MoveCar))))))

(fn ConstructionScript)

(fn MoveCar
  (bind _spline_refrence (Variables|Default|GetSpline%20Refrence))
  (bind _car_distance_along_spline (Variables|Default|GetCar%20Distance%20Along%20Spline))
  (bind _lane_offset (Variables|Default|GetLane%20Offset))
  (bind _is_reverse_direction (Variables|Default|GetIs%20Reverse%20Direction))
  (bind _returnvalue (Spline|GetRotationatDistanceAlongSpline _spline_refrence _car_distance_along_spline "World"))
  ;[1 1 1] Check currentspeed less than speedlimit
  (if (< (Variables|Default|GetCurrent%20Speed) (Variables|Default|GetSpeed%20Limit))
    ;[1 1 1] if curSpd less than limit; add 2.5 and set CurrentSpeed
    (Variables|Default|SetCurrent%20Speed (+ (Variables|Default|GetCurrent%20Speed) 2.5)))
  ;[1 1 1] if curSpd greater than limit; Set Actor Loc&Rot
  (Transformation|SetActorLocationAndRotation (Math|Vector|Lerp(Vector) (Transformation|GetActorLocation) (+ (Spline|GetLocationatDistanceAlongSpline _spline_refrence _car_distance_along_spline "World") (* (Class|SplineComponent|GetRightVectoratDistanceAlongSpline _spline_refrence _car_distance_along_spline "World") (Math|Float|SelectFloat (* _lane_offset -1.0) _lane_offset _is_reverse_direction))) 0.1) (Math|Rotator|MakeRotator (.roll _returnvalue) (.pitch _returnvalue) (Math|Float|SelectFloat (+ (.yaw _returnvalue) 1.8e+02) (.yaw _returnvalue) _is_reverse_direction)) false true))

(fn StopCar
  (params (Is%20Stop%20Hard :type Boolean))
  ;[1 1 1] while currentSpeed greater than 0
  (while (> (Variables|Default|GetCurrent%20Speed) 0.0)
    ;[1 1 1] Set output as CurrentSpeed
    (Variables|Default|SetCurrent%20Speed (- (Variables|Default|GetCurrent%20Speed) (select Is%20Stop%20Hard 2.0 1.0))))
  ;[1 1 1] Set CurrentSpeed to 0 and IsStopped = true
  (Variables|Default|SetCurrent%20Speed 0.0)
  (Variables|Default|SetIs%20Stopped true)
  (return))

(fn ResetDistanceAlongSpline
  ;[1 1 1] unused
  (return))