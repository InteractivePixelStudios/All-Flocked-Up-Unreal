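; Traffic manager that cycles traffic lights and intersection right-of-way between north-south and east-west.
; A timeline started at BeginPlay fires yellow, red and green events that recolor light group A or B, with red flipping the active direction.
; Red clears and green sets the direction flags on four-way and T-path intersections.
; A separate SpawnNewCar function, not called here, spawns a randomly directed car along a straight road's spline.
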(event EventBeginPlay
  ;[1 1 1] BeginPlay
  ;;[1 1 1] Starts timeline
  (Timeline|Traffic%20Timeline Play
    (:Change%20Yellow
      ;;[1 0.8504 0.2327] YellowLight
      ;;;[1 1 1] For each light in group
      (for _array_element (select (Variables|Default|GetSwitching%20NorthSouth) (Variables|Default|GetTrafficLight%20Group%20B) (Variables|Default|GetTraffic%20Light%20Group%20A))
        ;;;[1 1 1] Casts to either traffic light
        (bind _asbp_traffic_light_straight_right (Utilities|Casting|CastToBP_TrafficLightStraightRight _array_element)
          (:then
            ;;;[1 1 1] Set straightLightColor
            (Default|SetTrafficLightColor _asbp_traffic_light_straight_right "NewEnumerator1"))
          (:CastFailed
            (bind _asbp_traffic_light_curved_right (Utilities|Casting|CastToBP_TrafficLightCurvedRight _array_element))
            ;;;[1 1 1] Set curvedLightColor
            (Default|SetTrafficLightColor _asbp_traffic_light_curved_right "NewEnumerator1")))))
    (:Change%20Red
      ;;[1 0.03417 0.2963] Red Light
      ;;;[1 1 1] For each light in group
      (for _array_element_2 (select (Variables|Default|GetSwitching%20NorthSouth) (Variables|Default|GetTrafficLight%20Group%20B) (Variables|Default|GetTraffic%20Light%20Group%20A))
        ;;;[1 1 1] Casts to either trafficLight
        (bind _asbp_traffic_light_straight_right_2 (Utilities|Casting|CastToBP_TrafficLightStraightRight _array_element_2)
          (:then
            ;;;[1 1 1] Set Straight Light Color
            (Default|SetTrafficLightColor _asbp_traffic_light_straight_right_2 "NewEnumerator2"))
          (:CastFailed
            (bind _asbp_traffic_light_curved_right_2 (Utilities|Casting|CastToBP_TrafficLightCurvedRight _array_element_2))
            ;;;[1 1 1] Set CurvedLightColor
            (Default|SetTrafficLightColor _asbp_traffic_light_curved_right_2 "NewEnumerator2"))))
      ;;;[1 1 1] for each intersections in array
      (for _array_element_3 (Variables|Default|GetIntersections)
        ;;;[1 1 1] Cast to Either TrafficPath
        (bind _asbp_car_traffic_path_wk (Utilities|Casting|CastToBP_CarTrafficPath_WK _array_element_3)
          (:then
            ;;;[1 1 1] if TrafficPath
            (Variables|/Game/Blueprints/GameplaySystems/TrafficSystem/BP_CarTrafficPath_WK.BP_CarTrafficPath_WK_C|SetNorthSouth%20is%20Green _asbp_car_traffic_path_wk false)
            (Variables|/Game/Blueprints/GameplaySystems/TrafficSystem/BP_CarTrafficPath_WK.BP_CarTrafficPath_WK_C|SetEastWest%20is%20Green _asbp_car_traffic_path_wk false))
          (:CastFailed
            (bind _asbp_car_traffic_tpath_wk (Utilities|Casting|CastToBP_CarTrafficTPath_WK _array_element_3))
            ;;;[1 1 1] if TrafficTPath
            (Variables|/Game/Blueprints/GameplaySystems/TrafficSystem/BP_CarTrafficTPath_WK.BP_CarTrafficTPath_WK_C|SetNorthSouth%20is%20Green _asbp_car_traffic_tpath_wk false)
            (Variables|/Game/Blueprints/GameplaySystems/TrafficSystem/BP_CarTrafficTPath_WK.BP_CarTrafficTPath_WK_C|SetEast%20is%20Green _asbp_car_traffic_tpath_wk false))))
      (Variables|Default|SetSwitching%20NorthSouth (select (Variables|Default|GetSwitching%20NorthSouth) false true)))
    (:Change%20Green
      ;;[0.2517 1 0.3612] GreenLight
      ;;;[1 1 1] For each light in group
      (for _array_element_4 (select (Variables|Default|GetSwitching%20NorthSouth) (Variables|Default|GetTrafficLight%20Group%20B) (Variables|Default|GetTraffic%20Light%20Group%20A))
        ;;;[1 1 1] Cast to either traffic light
        (bind _asbp_traffic_light_straight_right_3 (Utilities|Casting|CastToBP_TrafficLightStraightRight _array_element_4)
          (:then
            ;;;[1 1 1] Set Straight light color
            (Default|SetTrafficLightColor _asbp_traffic_light_straight_right_3 "NewEnumerator0"))
          (:CastFailed
            (bind _asbp_traffic_light_curved_right_3 (Utilities|Casting|CastToBP_TrafficLightCurvedRight _array_element_4))
            ;;;[1 1 1] Set Curved Light Color
            (Default|SetTrafficLightColor _asbp_traffic_light_curved_right_3 "NewEnumerator0"))))
      ;;;[1 1 1] For each intersection in array
      (for _array_element_5 (Variables|Default|GetIntersections)
        ;;;[1 1 1] Cast to Traffic Path
        (bind _asbp_car_traffic_path_wk_2 (Utilities|Casting|CastToBP_CarTrafficPath_WK _array_element_5)
          (:then
            ;;;[1 1 1] Check if Switching N/S
            (if (select (Variables|Default|GetSwitching%20NorthSouth) true false)
              (Variables|/Game/Blueprints/GameplaySystems/TrafficSystem/BP_CarTrafficPath_WK.BP_CarTrafficPath_WK_C|SetNorthSouth%20is%20Green _asbp_car_traffic_path_wk_2 true)
              (else
                (Variables|/Game/Blueprints/GameplaySystems/TrafficSystem/BP_CarTrafficPath_WK.BP_CarTrafficPath_WK_C|SetEastWest%20is%20Green _asbp_car_traffic_path_wk_2 true))))
          (:CastFailed
            ;;;[1 1 1] Cast to T Path
            (bind _asbp_car_traffic_tpath_wk_2 (Utilities|Casting|CastToBP_CarTrafficTPath_WK _array_element_5))
            ;;;[1 1 1] Check if Switching N/S
            (if (select (Variables|Default|GetSwitching%20NorthSouth) true false)
              (Variables|/Game/Blueprints/GameplaySystems/TrafficSystem/BP_CarTrafficTPath_WK.BP_CarTrafficTPath_WK_C|SetNorthSouth%20is%20Green _asbp_car_traffic_tpath_wk_2 true)
              (else
                (Variables|/Game/Blueprints/GameplaySystems/TrafficSystem/BP_CarTrafficTPath_WK.BP_CarTrafficTPath_WK_C|SetEast%20is%20Green _asbp_car_traffic_tpath_wk_2 true)))))))))

(fn ConstructionScript)

(fn SpawnNewCar
  ;[1 1 1] Get StraightRoad Actor and sets SplineRef
  (bind _returnvalue (Actor|GetActorOfClass "/Game/Blueprints/GameplaySystems/TrafficSystem/BP_StraightRoad_WK.BP_StraightRoad_WK_C"))
  ;[1 1 1] Spawns Car
  (bind _returnvalue_2 (Game|SpawnActorfromClass "/Game/Blueprints/GameplaySystems/TrafficSystem/BP_Car_WK.BP_Car_WK_C" (Spline|GetTransformatDistanceAlongSpline (Variables|/Game/Blueprints/GameplaySystems/TrafficSystem/BP_StraightRoad_WK.BP_StraightRoad_WK_C|GetSpline _returnvalue) (Math|Random|RandomFloatinRange 1e+02 3e+02) "World" false) "Undefined" "MultiplyWithRoot" 0 0))
  ;[1 1 1] Randomly Sets IsReversing in WK_Car
  (Variables|/Game/Blueprints/GameplaySystems/TrafficSystem/BP_Car_WK.BP_Car_WK_C|SetIs%20Reverse%20Direction _returnvalue_2 (Math|Random|RandomBool))
  ;[1 1 1] Sets SplineRef in WK_Car
  (Variables|/Game/Blueprints/GameplaySystems/TrafficSystem/BP_Car_WK.BP_Car_WK_C|SetSpline%20Refrence _returnvalue_2 (Variables|/Game/Blueprints/GameplaySystems/TrafficSystem/BP_StraightRoad_WK.BP_StraightRoad_WK_C|GetSpline _returnvalue)))