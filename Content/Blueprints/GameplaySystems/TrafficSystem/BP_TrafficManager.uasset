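; BP_TrafficManager drives timeline-based car movement along traffic path splines.
; On actor overlap, it finds tagged BP_TrafficPath actors, storing each as the default spline and calling MoveCar, so the last one found remains active.
; MoveCar scales timeline play rate by completion time and samples world location and rotation along the path's NorthWest spline.
; StopMoveCar halts the timeline.
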(event Custom|MoveCar
  (bind _defaultspline (Variables|Default|GetDefaultSpline))
  (bind _northwest (Variables|/Game/Blueprints/GameplaySystems/TrafficSystem/BP_TrafficPath.BP_TrafficPath_C|GetNorthWest _defaultspline))
  (Components|Timeline|SetPlayRate (Variables|Default|GetMoveObjectT) (/ 1.0 (Variables|Default|GetTime%20to%20Complete)))
  (bind _movetrack (Timeline|Timeline Play)
    (:Update
      (Variables|Default|SetNewLocation (Spline|GetLocationatDistanceAlongSpline _northwest (Math|Float|Lerp 0.0 (Spline|GetSplineLength (Variables|/Game/Blueprints/GameplaySystems/TrafficSystem/BP_TrafficPath.BP_TrafficPath_C|GetNorthWest (Variables|Default|GetDefaultSpline))) _movetrack) "World"))
      (Variables|Default|SetNewRotation (Spline|GetRotationatDistanceAlongSpline _northwest (Math|Float|Lerp 0.0 (Spline|GetSplineLength (Variables|/Game/Blueprints/GameplaySystems/TrafficSystem/BP_TrafficPath.BP_TrafficPath_C|GetNorthWest (Variables|Default|GetDefaultSpline))) _movetrack) "World")))))

(event Custom|StopMoveCar
  (bind _defaultspline (Variables|Default|GetDefaultSpline))
  (bind _northwest (Variables|/Game/Blueprints/GameplaySystems/TrafficSystem/BP_TrafficPath.BP_TrafficPath_C|GetNorthWest _defaultspline))
  (bind _movetrack (Timeline|Timeline Stop)
    (:Update
      (Variables|Default|SetNewLocation (Spline|GetLocationatDistanceAlongSpline _northwest (Math|Float|Lerp 0.0 (Spline|GetSplineLength (Variables|/Game/Blueprints/GameplaySystems/TrafficSystem/BP_TrafficPath.BP_TrafficPath_C|GetNorthWest (Variables|Default|GetDefaultSpline))) _movetrack) "World"))
      (Variables|Default|SetNewRotation (Spline|GetRotationatDistanceAlongSpline _northwest (Math|Float|Lerp 0.0 (Spline|GetSplineLength (Variables|/Game/Blueprints/GameplaySystems/TrafficSystem/BP_TrafficPath.BP_TrafficPath_C|GetNorthWest (Variables|Default|GetDefaultSpline))) _movetrack) "World")))))

(event Collision|EventActorBeginOverlap
  (params (OtherActor :type Actor%20Object%20Reference))
  (bind _outactors (Actor|GetAllActorsOfClasswithTag "/Game/Blueprints/GameplaySystems/TrafficSystem/BP_TrafficPath.BP_TrafficPath_C" (Variables|Default|GetTag)))
  (for _array_element _outactors
    (bind _asbp_traffic_path (Utilities|Casting|CastToBP_TrafficPath _array_element))
    (Variables|Default|SetDefaultSpline _asbp_traffic_path)
    (CallFunction|MoveCar)))

(event EventTick
  (params (DeltaSeconds :type Float%20%28single-precision%29)))

(fn ConstructionScript)