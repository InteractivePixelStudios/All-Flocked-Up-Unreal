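; AI controller for traffic system cars that runs the BT_aiCar behavior tree on BeginPlay.
; Perception updates feed sight and touch handlers that write the traffic light to the TargetActor blackboard key.
; Losing sight of the light also records its last known location.
; GetPath derives a normalized steering value from the yaw difference between a spline tangent-based look-at and the controller's rotation.
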(event OnPerceptionUpdated(AIPerception)
  (params (UpdatedActors :type Array%20of%20Actor%20Object%20References)))

(event OnTargetPerceptionUpdated(AIPerception)
  (params (Actor :type Actor%20Object%20Reference) (Stimulus :type AI%20Stimulus%20Structure))
  (CallFunction|HandleSightSense Actor Stimulus)
  (CallFunction|HandleTouchEvent Actor Stimulus))

(event EventBeginPlay
  (AI|RunBehaviorTree "/Game/Blueprints/GameplaySystems/TrafficSystem/BT_aiCar.BT_aiCar"))

(event Collision|EventActorBeginOverlap
  (params (OtherActor :type Actor%20Object%20Reference)))

(event EventTick
  (params (DeltaSeconds :type Float%20%28single-precision%29)))

(fn ConstructionScript)

(fn GetPath
  (bind _activepath (Variables|Default|GetActivePath))
  (bind _returnvalue (Transformation|GetActorLocation _activepath))
  (bind _spline (Variables|/Game/Blueprints/GameplaySystems/TrafficSystem/BP_TrafficPath.BP_TrafficPath_C|GetSpline _activepath))
  (return (Math|Float|MapRangeClamped (.yaw (Math|Rotator|Delta(Rotator) (Math|Rotator|FindLookatRotation _returnvalue (Spline|FindLocationClosesttoWorldLocation _spline (+ (* (Math|Vector|Normalize (Class|SplineComponent|FindTangentClosesttoWorldLocation _spline _returnvalue "World")) 2e+02) "") "World")) (Transformation|GetActorRotation))) -9e+01 9e+01 -1.0 1.0)))

(fn HandleSightSense
  (params (Actor :type Actor%20Object%20Reference) (Stimulus :type AI%20Stimulus%20Structure))
  (bind _returnvalue (Class|AIPerceptionSystem|GetSenseClassforStimulus Stimulus))
  (if (== _returnvalue "/Script/AIModule.AISense_Sight")
    (if (== Actor "/Game/Blueprints/GameplaySystems/TrafficSystem/TrafficLight/BP_TrafficLight_OLD.BP_TrafficLight_OLD")
      (AI|Components|Blackboard|SetValueasObject (Variables|Default|GetBlackboard) (Utilities|Name|MakeLiteralName "TargetActor") (Utilities|SelectObject "/Game/Blueprints/GameplaySystems/TrafficSystem/TrafficLight/BP_TrafficLight_OLD.BP_TrafficLight_OLD" 0 (.bsuccessfullysensed Stimulus)))
      (if (not (.bsuccessfullysensed Stimulus))
        (AI|Components|Blackboard|SetValueasVector (Variables|Default|GetBlackboard) (Utilities|Name|MakeLiteralName "Last Known Location") (.stimuluslocation Stimulus)))
      (else
        (return)))
    (else
      (return))))

(fn HandleTouchEvent
  (params (Actor :type Actor%20Object%20Reference) (Stimulus :type AI%20Stimulus%20Structure))
  (bind _returnvalue (Class|AIPerceptionSystem|GetSenseClassforStimulus Stimulus))
  (if (== _returnvalue "/Script/AIModule.AISense_Touch")
    (for _array_element (Collision|GetOverlappingActors Actor "/Script/Engine.Actor" :!class /Script/Engine.Actor)
      (if (== Actor _array_element)
        (AI|Components|Blackboard|SetValueasObject (Variables|Default|GetBlackboard) (Utilities|Name|MakeLiteralName "TargetActor") (Utilities|SelectObject "/Game/Blueprints/GameplaySystems/TrafficSystem/TrafficLight/BP_TrafficLight_OLD.BP_TrafficLight_OLD" 0 (.bsuccessfullysensed Stimulus)))
        (else
          (return))))
    (else
      (return))))