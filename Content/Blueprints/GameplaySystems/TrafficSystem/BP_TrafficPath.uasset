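; BP_TrafficPath is a traffic system path Blueprint that exposes points along a spline as world-space locations.
; A Pathing event increments the current PathPoint index and resets it to zero on reaching the spline's point count, forming a repeating loop.
; GetLocationofSlinePoint returns the current point's world location and is also called from the construction script, where its result is unused.
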(event Custom|Pathing
  ;[1 1 1] Adds 1 to current PathPoint and Sets
  (bind _output_get (Variables|Default|SetPathPoint (+ (Variables|Default|GetPathPoint) 1)))
  (if (== _output_get (Spline|GetNumberOfSplinePoints (Variables|Default|GetSpline)))
    ;[1 1 1] Reset PathPoint to 0
    (Variables|Default|SetPathPoint 0)))

(fn ConstructionScript
  (CallFunction|GetLocationofSlinePoint))

(fn GetLocationofSlinePoint
  (return (Spline|GetLocationatSplinePoint (Variables|Default|GetSpline) (Variables|Default|GetPathPoint) "World")))