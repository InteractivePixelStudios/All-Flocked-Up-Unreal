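; AI enemy car for the traffic system that rides along the spline of a BP_TrafficPath actor.
; BeginPlay gets one path actor and, if its tag matches, starts a timeline scaled by TimeToComplete.
; The timeline sets the car's location and rotation by distance along the spline; StopMoveCar halts it.
; Nearest-spline search, steering calculation and speed-based movement helpers exist but are not used by the live event flow.
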(event Custom|MoveCar
  (bind _defaultspline (Variables|Default|GetDefaultSpline))
  (bind _spline (Variables|/Game/Blueprints/GameplaySystems/TrafficSystem/BP_TrafficPath.BP_TrafficPath_C|GetSpline _defaultspline))
  (Components|Timeline|SetPlayRate (Variables|Default|GetMoveObjectT) (/ 1.0 (Variables|Default|GetTimeToComplete)))
  (bind _movetrack (Timeline|MoveObjectT Play)
    (:Update
      (Transformation|SetActorTransform (Math|Transform|MakeTransform (Spline|GetLocationatDistanceAlongSpline _spline (Math|Float|Lerp 0.0 (Spline|GetSplineLength (Variables|/Game/Blueprints/GameplaySystems/TrafficSystem/BP_TrafficPath.BP_TrafficPath_C|GetSpline (Variables|Default|GetDefaultSpline))) _movetrack) "World") (Spline|GetRotationatDistanceAlongSpline _spline (Math|Float|Lerp 0.0 (Spline|GetSplineLength (Variables|/Game/Blueprints/GameplaySystems/TrafficSystem/BP_TrafficPath.BP_TrafficPath_C|GetSpline (Variables|Default|GetDefaultSpline))) _movetrack) "World") "1.000000,1.000000,1.000000")))))

(event Custom|StopMoveCar
  (bind _defaultspline (Variables|Default|GetDefaultSpline))
  (bind _spline (Variables|/Game/Blueprints/GameplaySystems/TrafficSystem/BP_TrafficPath.BP_TrafficPath_C|GetSpline _defaultspline))
  (bind _movetrack (Timeline|MoveObjectT Stop)
    (:Update
      (Transformation|SetActorTransform (Math|Transform|MakeTransform (Spline|GetLocationatDistanceAlongSpline _spline (Math|Float|Lerp 0.0 (Spline|GetSplineLength (Variables|/Game/Blueprints/GameplaySystems/TrafficSystem/BP_TrafficPath.BP_TrafficPath_C|GetSpline (Variables|Default|GetDefaultSpline))) _movetrack) "World") (Spline|GetRotationatDistanceAlongSpline _spline (Math|Float|Lerp 0.0 (Spline|GetSplineLength (Variables|/Game/Blueprints/GameplaySystems/TrafficSystem/BP_TrafficPath.BP_TrafficPath_C|GetSpline (Variables|Default|GetDefaultSpline))) _movetrack) "World") "1.000000,1.000000,1.000000")))))

(event EventBeginPlay
  (bind _returnvalue (Actor|GetActorOfClass "/Game/Blueprints/GameplaySystems/TrafficSystem/BP_TrafficPath.BP_TrafficPath_C"))
  (if (Actor|ActorHasTag _returnvalue (Variables|Default|GetTag))
    (Variables|Default|SetDefaultSpline _returnvalue)
    (CallFunction|MoveCar)))

(event Collision|EventHit
  (params (MyComp :type Primitive%20Component%20Object%20Reference) (Other :type Actor%20Object%20Reference) (OtherComp :type Primitive%20Component%20Object%20Reference) (bSelfMoved :type Boolean) (HitLocation :type Vector :default "0, 0, 0") (HitNormal :type Vector :default "0, 0, 0") (NormalImpulse :type Vector :default "0, 0, 0") (Hit :type Hit%20Result%20Structure%20%28by%20ref%29)))

(event EventTick
  (params (DeltaSeconds :type Float%20%28single-precision%29)))

(fn ConstructionScript)

(fn FindNearestSpline
  (params (SplineActors :type Array%20of%20BP%20Traffic%20Path%20Object%20References))
  (bind _returnvalue (Transformation|GetActorLocation))
  (LocalVariables|SetDistance 0.0)
  (for (_array_element _array_index) SplineActors
    (if (== _array_index 0)
      (LocalVariables|SetDistance (Math|Vector|Distance(Vector) (Spline|FindLocationClosesttoWorldLocation (Variables|/Game/Blueprints/GameplaySystems/TrafficSystem/BP_TrafficPath.BP_TrafficPath_C|GetSpline _array_element) _returnvalue "World") _returnvalue) :!label _label)
      (bind _output_get (LocalVariables|SetNearestSpline _array_element))
      (elif (< (Math|Vector|Distance(Vector) (Spline|FindLocationClosesttoWorldLocation (Variables|/Game/Blueprints/GameplaySystems/TrafficSystem/BP_TrafficPath.BP_TrafficPath_C|GetSpline _array_element) _returnvalue "World") _returnvalue) (LocalVariables|GetDistance))
        (goto _label))))
  (return (LocalVariables|GetNearestSpline)))

(fn CalculateSteeringInput
  (params (Spline :type BP%20Traffic%20Path%20Object%20Reference))
  (bind _returnvalue (Transformation|GetActorLocation))
  (bind _returnvalue_2 (Transformation|GetActorLocation))
  (bind _returnvalue_3 (Transformation|GetActorRotation))
  (bind _returnvalue_4 (+ _returnvalue ""))
  (bind _returnvalue_5 (Spline|FindLocationClosesttoWorldLocation (Variables|/Game/Blueprints/GameplaySystems/TrafficSystem/BP_TrafficPath.BP_TrafficPath_C|GetSpline Spline) _returnvalue_4 "Local"))
  (bind _returnvalue_6 (Math|Rotator|FindLookatRotation _returnvalue_2 _returnvalue_5))
  (bind _returnvalue_7 (Math|Rotator|Delta(Rotator) _returnvalue_6 _returnvalue_3))
  (bind _output_get (Variables|Default|SetOffsetTangentLocation _returnvalue_5))
  (if (Variables|Default|GetDebugSteering)
    (Rendering|Debug|DrawDebugSphere _output_get 25.0 12 "(R=1.000000,G=0.015401,B=0.000000,A=1.000000)" 0.0 1.0)
    (Rendering|Debug|DrawDebugArrow _returnvalue_2 _output_get 1.0 "(R=1.000000,G=0.000000,B=0.015653,A=1.000000)" 0.0 1e+01)
    (Variables|Default|SetYawDelta (.yaw _returnvalue_7))
    (return (Math|Float|MapRangeClamped (.yaw _returnvalue_7) -15.0 15.0 -1.0 1.0))))

(fn MoveAlongSpline
  (Variables|Default|SetLocationOnSpline (+ (* (Variables|Default|GetDelta%20Seconds) (Variables|Default|GetMaxSpeed)) (Variables|Default|GetLocationOnSpline))))

(fn SetSplinePointtoMove)