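; Straight/right traffic light actor that shows one of green, yellow or red by toggling the visibility of three components.
; SetTrafficLightColor stores the color enum and switches on it to drive the per-color toggle functions, starting with StartingColor on BeginPlay.
; BeginPlay also registers the light with BP_TrafficManager_WK, in Group A if starting red, otherwise Group B.
; It caches a separate BP_TrafficManager reference, unused within this Blueprint.
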(event Custom|SetTrafficLightColor
  (params (TrafficLightColor :type E_TrafficLightColorEnum%20Enum :default "NewEnumerator0"))
  ;[1 1 1] SetTrafficLightColor Event
  ;;[1 1 1] Gets Light Color Enum State and sets ref
  (bind _output_get (Variables|Default|SettrafficLightColors TrafficLightColor))
  ;;[1 1 1] Switch on ENUM
  (switch Utilities|FlowControl|Switch|SwitchonE_TrafficLightColorEnum _output_get
    (:NewEnumerator0
      ;;[1 1 1] IF GREEN LIGHT
      (CallFunction|ToggleGreenLight true)
      (CallFunction|ToggleYellowLight false)
      (CallFunction|ToggleRedLight false))
    (:NewEnumerator1
      ;;[1 1 1] IF YELLOW LIGHT
      (CallFunction|ToggleGreenLight false)
      (CallFunction|ToggleYellowLight true)
      (CallFunction|ToggleRedLight false))
    (:NewEnumerator2
      ;;[1 1 1] IF RED LIGHT
      (CallFunction|ToggleGreenLight false)
      (CallFunction|ToggleYellowLight false)
      (CallFunction|ToggleRedLight true))))

(event EventBeginPlay
  (bind _self self)
  (bind _startingcolor (Variables|Default|GetStartingColor))
  ;[1 1 1] BeginPlay
  ;;[1 1 1] Set Start Color
  (CallFunction|SetTrafficLightColor _startingcolor)
  ;;[1 1 1] Get Traffic Mgr and set Ref
  (bind _returnvalue (Actor|GetActorOfClass "/Game/Blueprints/GameplaySystems/TrafficSystem/BP_TrafficManager.BP_TrafficManager_C"))
  (Variables|Default|SetTrafficManagerRef _returnvalue)
  ;;[1 1 1] Checks if Light is RED
  (if (Utilities|Enum|Equal(Enum) _startingcolor "NewEnumerator2")
    ;;[1 1 1] IF RED; Set to Group A
    (bind _returnvalue_2 (Actor|GetActorOfClass "/Game/Blueprints/GameplaySystems/TrafficSystem/BP_TrafficManager_WK.BP_TrafficManager_WK_C"))
    (Utilities|Array|Add (Variables|/Game/Blueprints/GameplaySystems/TrafficSystem/BP_TrafficManager_WK.BP_TrafficManager_WK_C|GetTraffic%20Light%20Group%20A _returnvalue_2) _self)
    (else
      ;;[1 1 1] IF NOT RED; Set to Group B
      (bind _returnvalue_3 (Actor|GetActorOfClass "/Game/Blueprints/GameplaySystems/TrafficSystem/BP_TrafficManager_WK.BP_TrafficManager_WK_C"))
      (Utilities|Array|Add (Variables|/Game/Blueprints/GameplaySystems/TrafficSystem/BP_TrafficManager_WK.BP_TrafficManager_WK_C|GetTrafficLight%20Group%20B _returnvalue_3) _self))))

(fn ConstructionScript)

(fn ToggleGreenLight
  (params (ToggleOn :type Boolean))
  (Rendering|SetVisibility (Variables|Default|Getgreen) ToggleOn false))

(fn ToggleYellowLight
  (params (ToggleOn :type Boolean))
  (Rendering|SetVisibility (Variables|Default|Getyellow) ToggleOn false))

(fn ToggleRedLight
  (params (ToggleOn :type Boolean))
  (Rendering|SetVisibility (Variables|Default|Getred) ToggleOn false))