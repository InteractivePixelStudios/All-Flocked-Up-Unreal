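; Controller actor for a timed checkpoint race, with win and lose screens.
; On BeginPlay it reveals the active checkpoints, enables their collision, sets the timer from the current race and adds the HUD.
; Tick counts down to a loss, while RemoveCheckpoint_Event removes checkpoints the player overlaps and declares a win when none remain.
; Either outcome shows the cursor, switches to game-and-UI input and destroys the controller.
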(event Custom|RemoveCheckpoint_Event
  (CallFunction|PlayerPassedCheckpoint))

(event Custom|CountdownEvent
  (bind _returnvalue (Game|GetPlayerController 0))
  (bind _output_get (Variables|Default|SetRaceTimer (Math|Float|Clamp(Float) (- (Variables|Default|GetRaceTimer) (Utilities|Time|GetWorldDeltaSeconds)) 0.0 (Variables|Default|GetRaceTimer))))
  (if (<= _output_get 0.0)
    (bind _returnvalue_2 (UserInterface|CreateWidget "/Game/Blueprints/GameplaySystems/Races/Races/WBP_RaceLose.WBP_RaceLose_C" _returnvalue 0.0 0 "None" 0))
    (UserInterface|Viewport|AddtoViewport _returnvalue_2 0)
    (Variables|/Script/Engine.PlayerController|SetbShowMouseCursor _returnvalue true)
    (Input|SetInputModeGameandUI _returnvalue 0 "DoNotLock" false false)
    (Actor|DestroyActor)
    (bind _racehudref (Variables|Default|GetRaceHudRef)
      (:then
        (Widget|RemovefromParent _racehudref))
      (:else))))

(event EventBeginPlay
  (CallFunction|SpawnCheckpoints)
  (CallFunction|SetTimer)
  (bind _returnvalue (UserInterface|CreateWidget "/Game/Blueprints/GameplaySystems/Races/Races/WBP_RaceHUD.WBP_RaceHUD_C" (Game|GetPlayerController 0)))
  (UserInterface|Viewport|AddtoViewport _returnvalue 0))

(event Collision|EventActorBeginOverlap
  (params (OtherActor :type Actor%20Object%20Reference)))

(event EventDestroyed
  (bind _racehudref (Variables|Default|GetRaceHudRef)
    (:then
      (Widget|RemovefromParent _racehudref))
    (:else)))

(event EventTick
  (params (DeltaSeconds :type Float%20%28single-precision%29))
  (CallFunction|CountdownEvent))

(fn ConstructionScript)

(fn PlayerPassedCheckpoint
  (bind _returnvalue (Game|GetPlayerController 0))
  (bind _activecheckpoints (Variables|Default|GetActiveCheckpoints))
  (for _array_element (Variables|Default|GetActiveCheckpoints)
    (if (Collision|IsOverlappingActor (Variables|/Game/Blueprints/GameplaySystems/Races/Races/Checkpoint/BP_RaceCheckpoint.BP_RaceCheckpoint_C|GetSphereCollision _array_element) (Game|GetPlayerCharacter 0) :!class /Script/Engine.PrimitiveComponent)
      (Actor|DestroyActor _array_element)
      (Development|PrintString "overlapped")
      (bind _returnvalue_2 (Utilities|Array|RemoveItem _activecheckpoints _array_element))
      (if _returnvalue_2
        (Math|Integer|CompareInt (Utilities|Array|Length _activecheckpoints)
          (:==
            (bind _returnvalue_3 (UserInterface|CreateWidget "/Game/Blueprints/GameplaySystems/Races/Races/WBP_RaceWin.WBP_RaceWin_C" _returnvalue 0.0 0 "None" 0))
            (UserInterface|Viewport|AddtoViewport _returnvalue_3 0)
            (Input|SetInputModeGameandUI _returnvalue _returnvalue_3 "DoNotLock" false false)
            (Variables|/Script/Engine.PlayerController|SetbShowMouseCursor _returnvalue true)
            (Actor|DestroyActor))))
      (else
        (Development|PrintString "failed overlap")))))

(fn GetRaceDetails
  (Variables|Default|SetActiveCheckpoints (Variables|/Game/Blueprints/GameplaySystems/Races/Races/BP_RaceGiverActor.BP_RaceGiverActor_C|GetTotalCheckpoints (Variables|Default|GetRaceGiverReference))))

(fn SpawnCheckpoints
  (for _array_element (Variables|Default|GetActiveCheckpoints)
    (Rendering|SetActorHiddenInGame _array_element false)
    (Collision|SetCollisionEnabled (Variables|/Game/Blueprints/GameplaySystems/Races/Races/Checkpoint/BP_RaceCheckpoint.BP_RaceCheckpoint_C|GetSphereCollision _array_element) "QueryAndPhysics")))

(fn SetTimer
  (bind _output_get (Variables|Default|SetRaceTimer (.TimeInSeconds (Utilities|Struct|BreakS_RaceDetails (Variables|Default|GetCurrentRace)))))
  (bind _racehudref (Variables|Default|GetRaceHudRef)
    (:then
      (Variables|/Game/Blueprints/GameplaySystems/Races/Races/WBP_RaceHUD.WBP_RaceHUD_C|SetWidgetTimer _racehudref _output_get))
    (:else)))

(fn UpdateCheckpointArray
  (Variables|Default|SetActiveCheckpoints (Variables|Default|GetActiveCheckpoints)))