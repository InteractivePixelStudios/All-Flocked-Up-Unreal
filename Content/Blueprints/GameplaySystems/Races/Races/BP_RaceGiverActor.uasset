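; BP_RaceGiverActor is a race giver that offers a race to the pigeon player character.
; On BeginPlay it loads its race's name, time and trinket reward from DT_Races and broadcasts them.
; Box overlap gates the Pickup event, which opens WBP_RaceWidget with those details and a reference back to the giver.
; SpawnController_Event spawns a BP_RaceController at the giver's transform, passing the race row, checkpoints and tag.
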(event OnComponentBeginOverlap(Box)
  (params (OverlappedComponent :type Primitive%20Component%20Object%20Reference) (OtherActor :type Actor%20Object%20Reference) (OtherComp :type Primitive%20Component%20Object%20Reference) (OtherBodyIndex :type Integer) (bFromSweep :type Boolean) (SweepResult :type Hit%20Result%20Structure%20%28by%20ref%29))
  (Utilities|Casting|CastToBP_PigeonCharacter_AB OtherActor)
  (Variables|Default|SetbCanInteract true) ; Sets interactivity to true
)

(event OnComponentEndOverlap(Box)
  (params (OverlappedComponent :type Primitive%20Component%20Object%20Reference) (OtherActor :type Actor%20Object%20Reference) (OtherComp :type Primitive%20Component%20Object%20Reference) (OtherBodyIndex :type Integer))
  (Utilities|Casting|CastToBP_PigeonCharacter_AB OtherActor)
  (Variables|Default|SetbCanInteract false))

(event Custom|SendRaceDetails_Event
  (params (RaceDetails :type S%20Race%20Details%20Structure)))

(event Custom|SpawnController_Event
  (CallFunction|SpawnRaceController))

(event EventBeginPlay
  (CallFunction|GetRaceDetails))

(event Collision|EventActorBeginOverlap
  (params (OtherActor :type Actor%20Object%20Reference)))

(event EventTick
  (params (DeltaSeconds :type Float%20%28single-precision%29)))

(event EventPickup
  (bind _returnvalue (Game|GetPlayerController 0))
  (bind _racedetails (Variables|Default|GetRaceDetails))
  (Input|EnableInput _returnvalue)
  (if (Variables|Default|GetbCanInteract)
    (bind _returnvalue_2 (UserInterface|CreateWidget "/Game/Blueprints/GameplaySystems/Races/Races/WBP_RaceWidget.WBP_RaceWidget_C" _returnvalue (.timeinseconds _racedetails) (.trinketreward _racedetails) (.racename _racedetails)))
    (UserInterface|Viewport|AddtoViewport _returnvalue_2 0)
    (Variables|/Game/Blueprints/GameplaySystems/Races/Races/WBP_RaceWidget.WBP_RaceWidget_C|SetRaceGiverReference _returnvalue_2 self)))

(fn ConstructionScript)

(fn GetRaceDetails
  (bind _returnvalue (Utilities|GetDataTableRow "/Game/Blueprints/GameplaySystems/Races/Races/DT_Races.DT_Races" (Variables|Default|GetRaceName))
    (:then
      (bind _output_get (Variables|Default|SetOut%20Row _returnvalue))
      (bind _output_get_2 (Variables|Default|SetRaceDetails (Utilities|Struct|MakeS_RaceDetails (.timeinseconds _output_get) (.racename _output_get) (.trinketreward _output_get))))
      (Default|CallSendRaceDetails (Utilities|Struct|MakeS_RaceDetails (.timeinseconds _output_get_2) (.racename _output_get_2) (.trinketreward _output_get_2))))))

(fn SpawnRaceController
  (bind _returnvalue (Game|SpawnActorfromClass "/Game/Blueprints/GameplaySystems/Races/Races/BP_RaceController.BP_RaceController_C" (Transformation|GetActorTransform) "Undefined" "MultiplyWithRoot" 0 (Variables|Default|GetOut%20Row) (Variables|Default|GetTotalCheckpoints) self (Variables|Default|GetTag) false 0))
  (bind _output_get (Variables|Default|SetRaceControllerRef _returnvalue))
  (Variables|/Game/Blueprints/GameplaySystems/Races/Races/BP_RaceController.BP_RaceController_C|SetRaceGiverReference _output_get self)
  (return _output_get))