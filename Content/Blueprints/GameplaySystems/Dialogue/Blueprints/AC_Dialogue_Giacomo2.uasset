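; Dialogue component, apparently for Giacomo, whose Dialogue override only calls the parent with a None row, ignoring its DialogueRow input.
; An unconnected example branch tree, which never runs, chains DDT_Test_JS row lookups into AddDialogue calls and branches on the chosen option.
; That tree repeats row 1.1.1.1.1 across several steps and ends by clearing dialogue progress and closing the conversation.
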(event EventBeginPlay)

(event EventTick
  (params (DeltaSeconds :type Float%20%28single-precision%29)))

(fn Dialogue
  (params (DialogueRow :type Name :default "None"))
  (|CallParentFunction "None"))