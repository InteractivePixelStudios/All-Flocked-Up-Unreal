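; Base NPC for the dialogue and quest system, with a camera-facing name label and a quest billboard.
; BeginPlay hides tagged quest and next-NPC actors; interacting reveals the quest actors, opens ACDialogueBase's conversation and uses a timeline to turn NPC, player and camera into a side-offset framing.
; Closing the conversation notifies ACQuestGiver and hides the billboard.
; Tick mirrors dialogue state, and MoveToLocation walks the NPC to tagged location markers.
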(event Custom|MoveToLocation
  (params (Index :type Integer))
  (bind _locationref (Variables|Default|GetLocationRef))
  (bind _output (Utilities|Array|Get(acopy) _locationref Index))
  (Utilities|FlowControl|Delay 1.0)
  (Variables|Default|SetMoveComplete false)
  (AI|AIMoveTo (Variables|Character|GetCharacterMovement) self (Transformation|GetActorLocation _output) _output 1.0 true
    (:OnSuccess
      (Variables|Default|SetMoveComplete true)
      (Variables|/Game/Blueprints/GameplaySystems/Dialogue/Blueprints/AC_Dialogue_Base.AC_Dialogue_Base_C|SetIsMoving (Variables|Default|GetAC_Dialogue_Base) false)
      (Variables|Default|SetIsMoving false))))

(event Custom|ChangeSoundEvent
  (CallFunction|ChangeSound))

(event Custom|DestroyQuestActors
  (CallFunction|DestroyActors))

(event EventInteract
  (params (Instigator :type Actor%20Object%20Reference))
  (Variables|Default|SetInteractInstigator Instigator)
  (if (not (Variables|Default|GetConvoComplete))
    (CallFunction|SpawnQuestActors)
    (Default|OpenConversation (Variables|Default|GetAC_Dialogue_Base) (Variables|Default|GetConversationStartRow))
    (Variables|Default|SetInConvo? true)
    (Variables|Default|SetPlayerStartRotation (Transformation|GetActorRotation (Game|Player|GetPlayerPawn 0)))
    (Variables|Default|SetPlayerCameraRotation (Pawn|GetControlRotation (Game|GetPlayerController 0) :!class /Script/Engine.Controller))
    (bind _turnalpha (Timeline|TurnTimeline Play)
      (:Update
        (CallFunction|NPCLookatPlayer _turnalpha)
        (CallFunction|PlayerLookatNPC _turnalpha))
      (:Finished
        (CallFunction|NPCLookatPlayer 1.0)
        (CallFunction|PlayerLookatNPC 1.0)))))

(event EventConversationClosed
  (Default|InteractwithNPC (Variables|Default|GetAC_QuestGiver))
  (Development|SetHiddeninGame (Variables|Default|GetBillboard) true false)
  (Variables|Default|SetInConvo? false))

(event EventBeginPlay
  (bind _billboard (Variables|Default|GetBillboard))
  (Variables|Default|SetOriginalRotation (Transformation|GetActorRotation))
  (CallFunction|GetQuestActors)
  (CallFunction|HideQuestActors)
  (CallFunction|GetNextNPC)
  (CallFunction|HideNextNPC)
  (Variables|/Game/Blueprints/GameplaySystems/Dialogue/Blueprints/AC_Dialogue_Base.AC_Dialogue_Base_C|SetHasQuest (Variables|Default|GetAC_Dialogue_Base) (Variables|Default|GetHasQuest))
  (bind _outactors (Actor|GetAllActorsOfClasswithTag "/Game/Blueprints/GameplaySystems/Quest/QuestSystem/QuestBuilders/BP_QuestLocationMarker.BP_QuestLocationMarker_C" (Variables|Default|GetLocationTag)))
  (Variables|Default|SetLocationRef _outactors)
  (if (Variables|Default|GetHasQuest)
    (Development|SetHiddeninGame _billboard false false)
    (else
      (Development|SetHiddeninGame _billboard true false)))
  (Variables|Default|SetQuestComplete false))

(event EventTick
  (params (DeltaSeconds :type Float%20%28single-precision%29))
  (CallFunction|RotateName)
  (bind _ac_dialogue_base (Variables|Default|GetAC_Dialogue_Base)
    (:then
      (Variables|Default|SetIsMoving (Variables|/Game/Blueprints/GameplaySystems/Dialogue/Blueprints/AC_Dialogue_Base.AC_Dialogue_Base_C|GetIsMoving _ac_dialogue_base))
      (Variables|Default|SetConvoComplete (Variables|/Game/Blueprints/GameplaySystems/Dialogue/Blueprints/AC_Dialogue_Base.AC_Dialogue_Base_C|GetConvoComplete _ac_dialogue_base))
      (Variables|Default|SetDialogueIndex (Variables|/Game/Blueprints/GameplaySystems/Dialogue/Blueprints/AC_Dialogue_Base.AC_Dialogue_Base_C|GetDialogueRow _ac_dialogue_base)))
    (:else)))

(event EventSetInteractableState
  (params (CanShowInteract :type Boolean))
  ;[1 1 1] Sets character name visibility when nearby
  (if CanShowInteract
    (Rendering|SetVisibility (Variables|Default|GetTXT_CharacterName) true false)
    (else
      (Rendering|SetVisibility (Variables|Default|GetTXT_CharacterName) false false))))

(fn ConstructionScript
  ;[1 1 1] Update Character Name
  (Rendering|Components|TextRender|SetText (Variables|Default|GetTXT_CharacterName) (Variables|Default|GetCharacterName)))

(fn NPCLookatPlayer
  (params (TurnAlpha :type Float%20%28double-precision%29))
  (Transformation|SetActorRotation (Math|Rotator|MakeRotator 0.0 0.0 (Math|Float|Lerp (.yaw (Variables|Default|GetOriginalRotation)) (.yaw (Math|Rotator|FindLookatRotation (Transformation|GetActorLocation) (Transformation|GetActorLocation (Game|Player|GetPlayerPawn 0)))) TurnAlpha))))

(fn PlayerLookatNPC
  (params (Turn%20Alpha :type Float%20%28double-precision%29))
  (bind _returnvalue (Game|Player|GetPlayerPawn 0))
  (bind _returnvalue_2 (Transformation|GetActorLocation))
  (bind _playerstartrotation (Variables|Default|GetPlayerStartRotation))
  (bind _returnvalue_3 (Transformation|GetActorLocation _returnvalue))
  (bind _returnvalue_4 (Math|Rotator|FindLookatRotation _returnvalue_3 _returnvalue_2))
  (bind _returnvalue_5 (Math|Float|Lerp (.yaw _playerstartrotation) (.yaw _returnvalue_4) Turn%20Alpha))
  (Transformation|SetActorRotation (Game|Player|GetPlayerPawn 0) (Math|Rotator|MakeRotator 0.0 0.0 _returnvalue_5))
  (CallFunction|AdjustPlayerCamera _returnvalue_5))

(fn AdjustPlayerCamera
  (params (Z-Rotation :type Float%20%28double-precision%29))
  (bind _playercamerarotation (Variables|Default|GetPlayerCameraRotation))
  (if (and (<= (.yaw _playercamerarotation) 2.7e+02) (>= (.yaw _playercamerarotation) 9e+01))
    ;[0.2623 0.552 1] Set Camera to right side of player
    (Pawn|SetControlRotation (Game|GetPlayerController 0) (Math|Rotator|MakeRotator (.roll (Variables|Default|GetPlayerCameraRotation)) (Variables|Default|GetCameraPitchAngle) (- Z-Rotation (Variables|Default|GetCameraYawAngle))))
    (else
      ;[0.2623 0.552 1] Set Camera to left side of player
      (Pawn|SetControlRotation (Game|GetPlayerController 0) (Math|Rotator|MakeRotator (.roll (Variables|Default|GetPlayerCameraRotation)) (Variables|Default|GetCameraPitchAngle) (+ Z-Rotation (Variables|Default|GetCameraYawAngle)))))))

(fn GetQuestActors
  (bind _outactors (Actor|GetAllActorswithTag (Variables|Default|GetQuestActorTag)))
  (Variables|Default|SetQuestActorArray _outactors))

(fn SpawnQuestActors
  (for _array_element (Variables|Default|GetQuestActorArray)
    (Rendering|SetActorHiddenInGame _array_element false)
    (Actor|Tick|SetActorTickEnabled _array_element true)))

(fn HideQuestActors
  (for _array_element (Variables|Default|GetQuestActorArray)
    (Rendering|SetActorHiddenInGame _array_element true)
    (Actor|Tick|SetActorTickEnabled _array_element)))

(fn ShowNextQuestActor
  (for _array_element (Variables|Default|GetNextActorArray)
    (Rendering|SetActorHiddenInGame _array_element false)
    (Components|Activation|SetActive (Variables|/Script/Engine.Actor|GetRootComponent _array_element) true true)
    (Collision|SetActorEnableCollision _array_element true)))

(fn GetNextNPC
  (bind _outactors (Actor|GetAllActorswithTag (Variables|Default|GetNextActorTag)))
  (Variables|Default|SetNextActorArray _outactors))

(fn HideNextNPC
  (for _array_element (Variables|Default|GetNextActorArray)
    (Rendering|SetActorHiddenInGame _array_element true)
    (Components|Activation|SetActive (Variables|/Script/Engine.Actor|GetRootComponent _array_element) false false)
    (Collision|SetActorEnableCollision _array_element false)))

(fn ChangeSound
  (Audio|Components|Audio|SetSound (Variables|Default|GetAudioComponent) (Utilities|Array|Get(acopy) (Variables|Default|GetSoundArray) (Math|Random|RandomInteger 24))))

(fn RotateName
  (Transformation|SetWorldRotation (Variables|Default|GetTXT_CharacterName) (Math|Conversions|RotationFromXVector (Math|Vector|RotateVector (Math|Vector|Normalize (* (- (Camera|GetCameraLocation (Game|GetPlayerCameraManager 0)) (Transformation|GetWorldLocation (Variables|Default|GetTXT_CharacterName))) "1.000000,1.000000,0.000000")) "0, 0, 0")) false false))

(fn DestroyActors
  (for _array_element (Variables|Default|GetActorsToDestroy)
    (Actor|DestroyActor _array_element)))