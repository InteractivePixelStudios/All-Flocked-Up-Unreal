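; AC_VoiceModulator is a component that turns narrative dialogue text into sound.
; On BeginPlay it reads the DialogueText and SpeakerName of the RowToVoice row in the ExcelImportNarrativeTest data table.
; Every Tick, it loops through all characters of the stored line and plays a 2D pop sound for each one containing LetterToCheck, with no pacing between characters.
; SpeakerName is stored but does not affect the sound.
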(event EventBeginPlay
  (CallFunction|GetNarrativeInfo))

(event EventTick
  (params (DeltaSeconds :type Float%20%28single-precision%29))
  (CallFunction|TexttoSound))

(fn GetNarrativeInfo
  (bind _returnvalue (Utilities|GetDataTableRow "/Game/Blueprints/GameplaySystems/Dialogue/Blueprints/DataTableTest/ExcelImportNarrativeTest.ExcelImportNarrativeTest" (Variables|Default|GetRowToVoice))
    (:then
      (Variables|Default|SetDialogueLine (.DialogueText (Utilities|Struct|BreakDialogueDataStruct_JS _returnvalue)))
      (Variables|Default|SetSpeakerName (.SpeakerName (Utilities|Struct|BreakDialogueDataStruct_JS _returnvalue))))))

(fn TexttoSound
  (for _array_element (Utilities|String|GetCharacterArrayfromString (Utilities|String|ToString(Text) (Variables|Default|GetDialogueLine)))
    (if (Utilities|String|Contains _array_element (Variables|Default|GetLetterToCheck))
      (Audio|PlaySound2D "/Game/Blueprints/GameplaySystems/Dialogue/NarrativeAudioModulator/pop-268648.pop-268648" 1.0 1.0 0.0 0 0))))