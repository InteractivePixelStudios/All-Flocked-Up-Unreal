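; BP_AudioComponentWrapper is a helper actor that watches one physics-collision audio component until playback ends.
; A 0.01-second looping timer polls AudioRef, then re-enables CanPlayAudio on PCAPBase when the sound stops.
; It then destroys the audio component and, after a short delay, itself.
; If either reference is invalid at BeginPlay, it skips polling, sets the flag and destroys itself immediately.
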(event Custom|AudioLoop
  (Utilities|Time|SetTimerbyFunctionName 0 "AudioLoop" 0.01 true)
  (if (not (Audio|Components|Audio|IsPlaying (Variables|Default|GetAudioRef)))
    (Utilities|Time|ClearTimerbyFunctionName 0 "AudioLoop")
    (Variables|/Game/Audio/Audio/Blueprints/PhysicsCollision_Profiles/PC_AP_Base.PC_AP_Base_C|SetCanPlayAudio (Variables|Default|GetPC_AP_Base) true)
    (CallFunction|Destroy)))

(event Custom|Destroy
  (Components|DestroyComponent (Variables|Default|GetAudioRef))
  (Utilities|FlowControl|Delay 0.1)
  (Actor|DestroyActor))

(event EventBeginPlay
  (if (Utilities|IsValid (Variables|Default|GetPC_AP_Base))
    (if (Utilities|IsValid (Variables|Default|GetAudioRef))
      (CallFunction|AudioLoop)
      (else
        (Variables|/Game/Audio/Audio/Blueprints/PhysicsCollision_Profiles/PC_AP_Base.PC_AP_Base_C|SetCanPlayAudio (Variables|Default|GetPC_AP_Base) true :!label _label)
        (Actor|DestroyActor)))
    (else
      (goto _label))))

(fn ConstructionScript)