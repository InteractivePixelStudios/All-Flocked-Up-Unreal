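; Test physics collision audio Blueprint that plays material-specific impact sounds for the component it is attached to.
; The hit handler switches on the attach parent's first component tag: Metal, Glass, Wood, Clay, Trash or Plastic.
; A macro then plays a random sound from that material's array at the impact point.
; The physics check and hit binding are disconnected, so BeginPlay only delays and nothing here binds the handler.
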(event Custom|CustomOnHitEvent
  (params (HitComponent :type Primitive%20Component%20Object%20Reference) (OtherActor :type Actor%20Object%20Reference) (OtherComp :type Primitive%20Component%20Object%20Reference) (NormalImpulse :type Vector) (Hit :type Hit%20Result%20Structure%20%28by%20ref%29))
  (bind _impactpoint (Collision|BreakHitResult Hit))
  (switch name (Utilities|Array|Get(acopy) (Variables|/Script/Engine.ActorComponent|GetComponentTags (Transformation|GetAttachParent (Variables|Default|GetDefaultSceneRoot))))
    (:Metal
      (Utilities|NewMacro _impactpoint _impactpoint _impactpoint _impactpoint _impactpoint _impactpoint :!label _label))
    (:Glass
      (goto _label Glass))
    (:Wood
      (goto _label Wood))
    (:Clay
      (goto _label Clay))
    (:Trash
      (goto _label Trash))
    (:Plastic
      (goto _label Plastic))))

(event EventBeginPlay
  (Utilities|FlowControl|Delay 0.5))

(fn ConstructionScript)