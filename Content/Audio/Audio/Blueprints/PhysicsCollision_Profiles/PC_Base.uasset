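; PC_Base is a physics collision audio Blueprint, apparently an unfinished base for impact sound profiles.
; Its macro plays a random sound from Metal, Glass, Wood, Clay, Trash or Plastic arrays, each at a supplied location.
; The hit handler's switch has no visible cases, and the physics check, hit binding and macro call are disconnected, so no sound plays from this graph.
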(event Custom|CustomOnHitEvent
  (params (HitComponent :type Primitive%20Component%20Object%20Reference) (OtherActor :type Actor%20Object%20Reference) (OtherComp :type Primitive%20Component%20Object%20Reference) (NormalImpulse :type Vector) (Hit :type Hit%20Result%20Structure%20%28by%20ref%29))
  (switch name "None"))

(event Custom|CustomEvent
  (Utilities|FlowControl|Delay 0.5))