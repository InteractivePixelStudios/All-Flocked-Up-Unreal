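; Base physics collision audio component that plays impact sounds for physics-simulated static meshes on its owning actor.
; On hit, the mesh's first component tag selects a material sound array for a random attached sound.
; Velocity sampled every 0.1 seconds gates playback and scales volume; untagged meshes make the component destroy itself.
; Each sound gets a BP_AudioComponentWrapper actor, and a polling timer re-enables playback after TimerTarget.
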(event Custom|CustomOnHitEvent
  (params (HitComponent :type Primitive%20Component%20Object%20Reference) (OtherActor :type Actor%20Object%20Reference) (OtherComp :type Primitive%20Component%20Object%20Reference) (NormalImpulse :type Vector) (Hit :type Hit%20Result%20Structure%20%28by%20ref%29))
  (bind _staticmeshref (Variables|Default|GetStaticMeshRef))
  (bind _lastvelocity (Variables|Default|GetLastVelocity))
  (if (Variables|Default|GetCanPlayAudio)
    (if (> _lastvelocity 1e+01)
      (if (not (<= _lastvelocity 0.0))
        (Variables|Default|SetCanPlayAudio false)
        (Variables|Default|SetHitLocation (Transformation|GetWorldLocation _staticmeshref))
        (if (> (Utilities|Array|Length (Variables|/Script/Engine.ActorComponent|GetComponentTags (Variables|Default|GetStaticMeshRef))) 0)
          (switch name (Utilities|Array|Get(acopy) (Variables|/Script/Engine.ActorComponent|GetComponentTags _staticmeshref))
            (:Metal
              (Utilities|NewMacro0 :!label _label))
            (:Glass
              (goto _label Glass))
            (:Wood
              (goto _label Wood))
            (:Clay
              (goto _label Clay))
            (:Trash
              (goto _label Trash))
            (:Plastic
              (goto _label Plastic))
            (:Can
              (goto _label Can))
            (:Cardboard
              (goto _label Cardboard))
            (:Garbage
              (goto _label Garbage))
            (:Fork
              (goto _label Fork))
            (:Ceramic
              (goto _label Ceramic))
            (:PaperCup
              (goto _label PaperCup))))))))

(event Custom|GetVel
  (Utilities|Time|SetTimerbyFunctionName 0 "GetVel" 0.1)
  (if (Utilities|IsValid (Variables|Default|GetStaticMeshRef))
    (Variables|Default|SetLastVelocity (Math|Vector|VectorLength (Transformation|GetComponentVelocity (Variables|Default|GetStaticMeshRef))))
    (Variables|Default|SetVolumeBoost (/ (Variables|Default|GetLastVelocity) 5e+02))))

(event Custom|CheckIfValid
  (Utilities|FlowControl|Delay 0.3)
  (if (not (> (Utilities|Array|Length (Variables|/Script/Engine.ActorComponent|GetComponentTags (Variables|Default|GetStaticMeshRef))) 0))
    (Components|DestroyComponent)))

(event Custom|ForceAllowAudio
  (Variables|Default|SetCanPlayAudio true))

(event Custom|AudioTimer
  (Utilities|Time|SetTimerbyFunctionName 0 "AudioTimer" 0.01 true)
  (if (>= (- (Utilities|Time|GetGameTimeinSeconds) (Variables|Default|GetLastGameTime)) (Variables|Default|GetTimerTarget))
    (Utilities|Time|ClearTimerbyFunctionName 0 "AudioTimer")
    (CallFunction|ForceAllowAudio)))

(event EventTick
  (params (DeltaSeconds :type Float%20%28single-precision%29)))

(event EventBeginPlay
  (Utilities|FlowControl|Delay 0.1)
  (for _array_element (Actor|GetComponentsByClass (Components|GetOwner (Transformation|GetAttachParent)) "/Script/Engine.StaticMeshComponent")
    (if (Physics|IsSimulatingPhysics _array_element "None")
      (Variables|Default|SetStaticMeshRef _array_element)
      (CallFunction|CheckifValid)
      (Class|PrimitiveComponent|SetNotifyRigidBodyCollision _array_element true)
      (Collision|BindEventtoOnComponentHit (Variables|Default|GetStaticMeshRef) (delegate Custom|CustomOnHitEvent))
      (CallFunction|GetVel))))