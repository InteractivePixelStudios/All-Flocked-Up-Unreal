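; BP_AP_Human is the human audio profile, which plays surface-dependent footstep sounds through the MSHuman MetaSound.
; Each Footstep event traces 100 units straight down from HumanReference and reads the physical surface type of the hit.
; Stone, grass, metal and wood each pass their sound array to the MetaSound before firing its Footstep trigger.
; The default footstep array is left unconnected, so other surfaces and trace misses trigger no sound.
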(event Custom|Footstep
  (bind _humanreference (Variables|Default|GetHumanReference))
  (bind _returnvalue (Transformation|GetActorLocation _humanreference))
  (bind (_outhit _returnvalue_2) (Collision|LineTraceByChannel _returnvalue (- _returnvalue "0.000000,0.000000,100.000000") "TraceTypeQuery1" false (Utilities|Array|MakeArray _humanreference) "None" true "(R=1.000000,G=0.000000,B=0.829904,A=1.000000)"))
  (if _returnvalue_2
    (switch Utilities|FlowControl|Switch|SwitchonEPhysicalSurface (Collision|GetSurfaceType _outhit)
      (:SurfaceType1
        (Audio|Parameter|SetObjectArrayParameter (Variables|Default|GetMS_Human) "FootstepArray" (Variables|Default|GetFootstepsStone)))
      (:SurfaceType2
        (Audio|Parameter|SetObjectArrayParameter (Variables|Default|GetMS_Human) "FootstepArray" (Variables|Default|GetFootstepsGrass)))
      (:SurfaceType3
        (Audio|Parameter|SetObjectArrayParameter (Variables|Default|GetMS_Human) "FootstepArray" (Variables|Default|GetFootstepsMetal)))
      (:SurfaceType4
        (Audio|Parameter|SetObjectArrayParameter (Variables|Default|GetMS_Human) "FootstepArray" (Variables|Default|GetFootstepsWood))))
    (Class|AudioParameterControllerInterface|SetTriggerParameter (Variables|Default|GetMS_Human) "Footstep")))