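; Player audio profile that plays splat, dooky, wing flap, damage and footstep sounds through MetaSound triggers on MSPlayer.
; External events fire the triggers, while damage binds to the player's any-damage delegate after a short BeginPlay delay.
; Footsteps use a temporary velocity check, then a downward trace picks the sound array by physical surface; the default array is unwired.
; Separate events push the stealth sound mix and clear all mix modifiers.
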(event Custom|TriggerDookySound
  (Class|AudioParameterControllerInterface|SetTriggerParameter (Variables|Default|GetMS_Player) "Dooky"))

(event Custom|TriggerWingFlapSound
  (Class|AudioParameterControllerInterface|SetTriggerParameter (Variables|Default|GetMS_Player) "Flap"))

(event Custom|TriggerSplat
  (Class|AudioParameterControllerInterface|SetTriggerParameter (Variables|Default|GetMS_Player) "Splat"))

(event Custom|TriggerFootstepSound
  (bind _playerreference (Variables|Default|GetPlayerReference))
  (bind _returnvalue (Transformation|GetActorLocation _playerreference))
  ;[1 0 0] TEMP FIX UNTIL THE MAIN ISSUE IS LOCATED
  (if (> (Math|Vector|VectorLength (Transformation|GetComponentVelocity (Variables|/Script/Engine.Actor|GetRootComponent (Variables|Default|GetPlayerReference)))) 1.0)
    (bind (_outhit _returnvalue_2) (Collision|LineTraceByChannel _returnvalue (- _returnvalue "0.000000,0.000000,25.000000") "TraceTypeQuery1" false (Utilities|Array|MakeArray _playerreference) "None" true "(R=1.000000,G=0.000000,B=0.829904,A=1.000000)"))
    (if _returnvalue_2
      (switch Utilities|FlowControl|Switch|SwitchonEPhysicalSurface (Collision|GetSurfaceType _outhit)
        (:SurfaceType1
          (Audio|Parameter|SetObjectArrayParameter (Variables|Default|GetMS_Player) "FootstepArray" (Variables|Default|GetFootstepsStone)))
        (:SurfaceType2
          (Audio|Parameter|SetObjectArrayParameter (Variables|Default|GetMS_Player) "FootstepArray" (Variables|Default|GetFootstepsGrass)))
        (:SurfaceType3
          (Audio|Parameter|SetObjectArrayParameter (Variables|Default|GetMS_Player) "FootstepArray" (Variables|Default|GetFootstepsMetal)))
        (:SurfaceType4
          (Audio|Parameter|SetObjectArrayParameter (Variables|Default|GetMS_Player) "FootstepArray" (Variables|Default|GetFootstepsWood))))
      (Class|AudioParameterControllerInterface|SetTriggerParameter (Variables|Default|GetMS_Player) "Footstep"))))

(event Custom|OnTakeAnyDamage_Event
  (params (DamagedActor :type Actor%20Object%20Reference) (Damage :type Float%20%28single-precision%29) (DamageType :type Damage%20Type%20Object%20Reference) (InstigatedBy :type Controller%20Object%20Reference) (DamageCauser :type Actor%20Object%20Reference))
  (Class|AudioParameterControllerInterface|SetTriggerParameter (Variables|Default|GetMS_Player) "TakeDamage"))

(event Custom|ClearMixer
  (Class|GameplayStatics|ClearSoundMixModifiers))

(event Custom|SwapMixer
  (Audio|PushSoundMixModifier "/Game/Audio/Audio/Volume/SM_StealthMixer.SM_StealthMixer"))

(event EventBeginPlay
  (Utilities|FlowControl|Delay 1.0)
  (EventDispatchers|AssignOnTakeAnyDamage (Variables|Default|GetPlayerReference) (delegate Custom|OnTakeAnyDamage_Event)))