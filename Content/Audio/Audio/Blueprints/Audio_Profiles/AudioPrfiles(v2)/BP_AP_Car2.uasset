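; Car audio profile Blueprint that starts the MSCar sound on its referenced car shortly after BeginPlay.
; A delayed, self-calling loop checks that the audio component is valid, plays it if silent, and retries while it is missing.
; The TryNumberOfTimes counter caps the attempts.
; An unconnected draft for driving EnginePitch from parent velocity is saved for later, and CheckIfPlaying is empty.
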(event Custom|StartAudioLoop
  (bind _carref (Variables|Default|GetCarRef))
  (bind _ms_car (Variables|/Game/Blueprints/GameplaySystems/TrafficSystem/BP_Car_WK.BP_Car_WK_C|GetMS_Car _carref))
  (Utilities|FlowControl|Delay 1.0)
  (if (Utilities|IsValid _ms_car)
    (if (not (Audio|Components|Audio|IsPlaying _ms_car))
      (Utilities|TryNumberOfTimes 20)
      (Utilities|FlowControl|Delay 0.2)
      (Audio|Components|Audio|Play _ms_car 0.0)
      (CallFunction|StartAudioLoop))
    (else
      (Utilities|TryNumberOfTimes 20)
      (Utilities|FlowControl|Delay 0.2)
      (CallFunction|StartAudioLoop))))

(event EventBeginPlay
  (Utilities|FlowControl|Delay 1.0)
  (CallFunction|StartAudioLoop))

(fn CheckifPlaying)