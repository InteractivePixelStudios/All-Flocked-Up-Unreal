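; BP_AP_Trees is an audio profile actor that plays random bird sounds from trees inside its box.
; On BeginPlay, after a short delay, it gathers overlapping static mesh actors tagged "Tree", marks each with a debug box, or destroys itself if none exist.
; A delayed cycle moves one audio source above a random tree and plays a random clip with a fade-out.
; Tick restarts the cycle whenever the source is silent.
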(event Custom|StartBirdCycle
  (bind _birdaudioarray (Variables|Default|GetBirdAudioArray))
  (bind _audiosource (Variables|Default|GetAudioSource))
  (bind _outitem (Utilities|Array|Random _birdaudioarray))
  (if (Variables|Default|GetIsEnabled)
    (Utilities|FlowControl|Delay 5.0)
    (Transformation|SetWorldLocation (Variables|Default|GetAudioSource) (+ (Transformation|GetActorLocation (.OutItem (Utilities|Array|Random (Variables|Default|GetTreeArray)))) "0.000000,0.000000,400.000000") false true)
    (Audio|Components|Audio|SetSound (Variables|Default|GetAudioSource) _outitem)
    (Audio|Components|Audio|Play _audiosource 0.0)
    (Audio|Components|Audio|FadeOut _audiosource (Variables|/Script/Engine.SoundBase|GetDuration _outitem) 0.0 "Linear" :!class /Script/Engine.AudioComponent)))

(event EventBeginPlay
  (bind _treearray (Variables|Default|GetTreeArray))
  (Collision|SetCollisionEnabled (Variables|Default|GetBox) "QueryOnly")
  (Utilities|FlowControl|Delay 1.0)
  (Variables|Default|SetIsEnabled true)
  (for _array_element (Collision|GetOverlappingActors (Variables|Default|GetBox) "/Script/Engine.StaticMeshActor" :!class /Script/Engine.PrimitiveComponent)
    (if (== (Utilities|Array|Get(acopy) (Variables|/Script/Engine.Actor|GetTags _array_element)) "Tree")
      (Utilities|Array|Add _treearray _array_element)))
  (if (> (Utilities|Array|Length _treearray) 0)
    (for _array_element_2 (Variables|Default|GetTreeArray)
      (Rendering|Debug|DrawDebugBox (+ (Transformation|GetActorLocation _array_element_2) "0.000000,0.000000,400.000000") "0.000000,0.000000,25.000000" "(R=0.362684,G=0.360786,B=0.364583,A=0.000000)" "0, 0, 0" 1e+04 1e+01)
      (CallFunction|StartBirdCycle))
    (else
      (Actor|DestroyActor))))

(event EventTick
  (params (DeltaSeconds :type Float%20%28single-precision%29))
  (if (Variables|Default|GetIsEnabled)
    (if (not (Audio|Components|Audio|IsPlaying (Variables|Default|GetAudioSource)))
      (Utilities|FlowControl|Delay 5.0)
      (CallFunction|StartBirdCycle))))

(fn ConstructionScript)