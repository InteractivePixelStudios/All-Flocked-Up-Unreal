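; BP_AP_Car is a car audio profile actor that plays engine sound driven by the movement of whatever it is attached to.
; On BeginPlay it caches the AudioWizard, creates an attenuated audio component and feeds it the engine wave from a data asset.
; Each tick it restarts stopped audio, applies the wizard's car and master volumes, and sets engine pitch from the attach parent's speed.
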(event Custom|AdjustVolume
  (bind _audiowizard (Variables|Default|GetAudioWizard))
  (Audio|Components|Audio|SetVolumeMultiplier (Variables|Default|GetAudioComp) (* (Variables|/Game/Audio/Audio/Blueprints/AudioWizard.AudioWizard_C|GetCarVolume _audiowizard) (Variables|/Game/Audio/Audio/Blueprints/AudioWizard.AudioWizard_C|GetMasterVolume _audiowizard)) :!class /Script/Engine.AudioComponent))

(event Custom|CheckIfPlaying
  (if (not (Audio|Components|Audio|IsPlaying (Variables|Default|GetAudioComp)))
    (Audio|Components|Audio|Play (stale EventBeginPlay _output_get) 0.0)))

(event EventBeginPlay
  (bind _outactors (Actor|GetAllActorsOfClass "/Game/Audio/Audio/Blueprints/AudioWizard.AudioWizard_C"))
  (bind _asaudio_wizard (Utilities|Casting|CastToAudioWizard (Utilities|Array|Get(acopy) _outactors)))
  (Variables|Default|SetAudioWizard _asaudio_wizard)
  (bind _returnvalue (AddComponent|AddAudioComponent false))
  (Variables|/Script/Engine.AudioComponent|SetAttenuationSettings _returnvalue "/Game/Audio/Audio/Attenuation/CarAttenuation.CarAttenuation")
  (bind _output_get (Variables|Default|SetAudioComp _returnvalue))
  (Class|AudioComponent|SetWaveParameter _output_get "Engine" (Variables|/Game/Audio/Audio/Blueprints/BP_DA/BP_VA_Car.BP_VA_Car_C|GetCarEngine (Variables|Default|GetDataAsset)))
  (Audio|Components|Audio|Play _output_get 0.0))

(event EventTick
  (params (DeltaSeconds :type Float%20%28single-precision%29))
  (CallFunction|CheckifPlaying)
  (CallFunction|AdjustVolume)
  (Audio|Parameter|SetFloatParameter (Variables|Default|GetAudioComp) "EnginePitch" (/ (Math|Vector|VectorLength (Transformation|GetComponentVelocity (Transformation|GetAttachParent (Variables|Default|GetDefaultSceneRoot)))) 1e+02) :!class /Script/AudioExtensions.AudioParameterControllerInterface))

(fn ConstructionScript)