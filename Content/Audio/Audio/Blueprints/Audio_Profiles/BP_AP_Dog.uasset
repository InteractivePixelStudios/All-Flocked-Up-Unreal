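; Audio profile Blueprint for the dog, with events for idle, attack and footstep sounds.
; The footstep event line-traces a short way below the actor and switches on the hit surface type.
; Nodes that would set a footstep sound array parameter and fire the Footstep trigger are disconnected from that switch, so no footstep plays.
; The idle and attack events are empty stubs.
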(event Custom|IdleSound)

(event Custom|TriggerFootstepSound
  (bind _returnvalue (Transformation|GetActorLocation))
  (bind (_outhit _returnvalue_2) (Collision|LineTraceByChannel _returnvalue (- _returnvalue "0.000000,0.000000,25.000000") "TraceTypeQuery1" false (Utilities|Array|MakeArray 0) "None" true "(R=1.000000,G=0.000000,B=0.829904,A=1.000000)"))
  (if _returnvalue_2
    (switch Utilities|FlowControl|Switch|SwitchonEPhysicalSurface (Collision|GetSurfaceType _outhit))))

(event Custom|AttackSound)

(fn ConstructionScript)