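; BP_AP_Manhole is an audio actor for a manhole, built around an MSManhole audio component.
; It starts the sound on BeginPlay and checks every Tick, restarting it whenever it is not playing.
; When BP_PigeonCharacter_AB overlaps the actor, it fires the "Push" trigger parameter on the sound and prints a debug string.
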(event Custom|CheckIfPlaying
  (bind _ms_manhole (Variables|Default|GetMS_Manhole))
  (if (not (Audio|Components|Audio|IsPlaying _ms_manhole))
    (Audio|Components|Audio|Play _ms_manhole 0.0)))

(event EventBeginPlay
  (Audio|Components|Audio|Play (Variables|Default|GetMS_Manhole) 0.0))

(event Collision|EventActorBeginOverlap
  (params (OtherActor :type Actor%20Object%20Reference))
  (Utilities|Casting|CastToBP_PigeonCharacter_AB OtherActor)
  (Class|AudioParameterControllerInterface|SetTriggerParameter (Variables|Default|GetMS_Manhole) "Push")
  (Development|PrintString "Push Sound Maybe?"))

(event EventTick
  (params (DeltaSeconds :type Float%20%28single-precision%29))
  (CallFunction|CheckifPlaying))

(fn ConstructionScript)