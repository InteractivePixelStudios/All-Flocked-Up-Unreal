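; BP_AP_Player is the player audio profile that fires wing flap, footstep and dooky sounds for the pigeon character.
; It finds the pigeon character on BeginPlay, and each sound event sets a named trigger parameter on MSPlayer.
; Footsteps play only when a short downward trace from the pigeon's location hits.
; The surface type is only printed, and the trace draws persistent debug lines.
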(event Custom|TriggerDookySound
  (Class|AudioParameterControllerInterface|SetTriggerParameter (Variables|Default|GetMS_Player) "Dooky"))

(event Custom|TriggerWingFlapSound
  (Class|AudioParameterControllerInterface|SetTriggerParameter (Variables|Default|GetMS_Player) "Flap"))

(event Custom|TriggerFootstepSound
  (bind _playerreference (Variables|Default|GetPlayerReference))
  (bind _returnvalue (Transformation|GetActorLocation _playerreference))
  (bind (_outhit _returnvalue_2) (Collision|LineTraceByChannel _returnvalue (- _returnvalue "0.000000,0.000000,25.000000") "TraceTypeQuery1" false (Utilities|Array|MakeArray _playerreference) "Persistent" true "(R=1.000000,G=0.000000,B=0.829904,A=1.000000)"))
  (if _returnvalue_2
    (Development|PrintString (Utilities|String|EnumtoString (Collision|GetSurfaceType _outhit)))
    (Class|AudioParameterControllerInterface|SetTriggerParameter (Variables|Default|GetMS_Player) "Footstep")))

(event EventBeginPlay
  (bind _outactors (Actor|GetAllActorsOfClass "/Game/Blueprints/Characters/Player/BP_PigeonCharacter_AB.BP_PigeonCharacter_AB_C"))
  (Variables|Default|SetPlayerReference (Utilities|Array|Get(acopy) _outactors)))

(fn ConstructionScript)