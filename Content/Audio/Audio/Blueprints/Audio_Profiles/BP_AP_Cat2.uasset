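; Audio profile for a cat that drives its MetaSound (MSCat) with meow, hiss, attack and footstep triggers.
; Hiss and attack follow events bound on CatRef, while a self-recalling delay loop meows at random intervals, re-rolling the threshold on each poll.
; Footstep traces down to pick a surface-specific sound array, gated by a startup delay.
; Tick fires meows while ForceStart is set, until BeginPlay clears it.
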(event Custom|Footstep
  (bind _catref (Variables|Default|GetCatRef))
  (bind _returnvalue (Transformation|GetActorLocation _catref))
  (if (Variables|Default|GetCanPlayAudio)
    (bind (_outhit _returnvalue_2) (Collision|LineTraceByChannel _returnvalue (- _returnvalue "0.000000,0.000000,100.000000") "TraceTypeQuery1" false (Utilities|Array|MakeArray _catref) "None" true "(R=1.000000,G=0.000000,B=0.829904,A=1.000000)"))
    (if _returnvalue_2
      (switch Utilities|FlowControl|Switch|SwitchonEPhysicalSurface (Collision|GetSurfaceType _outhit)
        (:SurfaceType_Default
          (Audio|Parameter|SetObjectArrayParameter (Variables|Default|GetMS_Cat) "FootstepArray" (Variables|Default|GetFootstepsGrass)))
        (:SurfaceType1
          (Audio|Parameter|SetObjectArrayParameter (Variables|Default|GetMS_Cat) "FootstepArray" (Variables|Default|GetFootstepsStone)))
        (:SurfaceType2
          (Audio|Parameter|SetObjectArrayParameter (Variables|Default|GetMS_Cat) "FootstepArray" (Variables|Default|GetFootstepsGrass)))
        (:SurfaceType3
          (Audio|Parameter|SetObjectArrayParameter (Variables|Default|GetMS_Cat) "FootstepArray" (Variables|Default|GetFootstepsMetal)))
        (:SurfaceType4
          (Audio|Parameter|SetObjectArrayParameter (Variables|Default|GetMS_Cat) "FootstepArray" (Variables|Default|GetFootstepsWood))))
      (Class|AudioParameterControllerInterface|SetTriggerParameter (Variables|Default|GetMS_Cat) "Footstep"))))

(event Custom|Hiss
  (Class|AudioParameterControllerInterface|SetTriggerParameter (Variables|Default|GetMS_Cat) "Hiss"))

(event Custom|Attack
  (Class|AudioParameterControllerInterface|SetTriggerParameter (Variables|Default|GetMS_Cat) "Attack"))

(event Custom|MeowCycle
  (Variables|Default|SetTimerTarget (Math|Random|RandomFloatinRange 4.0 8.0))
  (if (>= (- (Utilities|Time|GetGameTimeinSeconds) (Variables|Default|GetLastGameTime)) (Variables|Default|GetTimerTarget))
    (Class|AudioParameterControllerInterface|SetTriggerParameter (Variables|Default|GetMS_Cat) "Meow")
    (Utilities|FlowControl|Delay 1.0)
    (Variables|Default|SetLastGameTime (Utilities|Time|GetGameTimeinSeconds))
    (CallFunction|MeowCycle)
    (else
      (Utilities|FlowControl|Delay 0.2)
      (CallFunction|MeowCycle))))

(event Custom|AttenuationHack)

(event EventTick
  (params (DeltaSeconds :type Float%20%28single-precision%29))
  (Utilities|FlowControl|Delay 0.2)
  (if (Variables|Default|GetForceStart)
    (Class|AudioParameterControllerInterface|SetTriggerParameter (Variables|Default|GetMS_Cat) "Meow")))

(event EventBeginPlay
  (bind _catref (Variables|Default|GetCatRef))
  (Utilities|FlowControl|Sequence
    (:then_0
      (Utilities|FlowControl|Delay 1.5)
      (Variables|Default|SetLastGameTime (Utilities|Time|GetGameTimeinSeconds))
      (EventDispatchers|BindEventtoHiss _catref (delegate Custom|Hiss))
      (EventDispatchers|BindEventtoAttack _catref (delegate Custom|Attack))
      (CallFunction|MeowCycle))
    (:then_1
      (Utilities|FlowControl|Delay 2.0)
      (Variables|Default|SetForceStart false)
      (Variables|Default|SetCanPlayAudio true))))