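; AudioWizard is the audio manager that starts ambience and world music and handles master, music and SFX volume.
; On BeginPlay it finds manholes and trash pickups to attach spawned audio-profile actors, and adds audio components to environment objects.
; A separate event does the same for the pigeon player, while car audio is unwired.
; Volume events apply scaled SM_MasterMix class overrides, with master also overwriting SFX.
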(event Custom|SpawnManholeAudioProfile
  (bind _outactors (Actor|GetAllActorsOfClass "/Game/Blueprints/GameplaySystems/BP_ManholeCover.BP_ManholeCover_C"))
  (for _array_element _outactors
    (bind _returnvalue (Game|SpawnActorfromClass "/Game/Audio/Audio/Blueprints/Audio_Profiles/BP_AP_Manhole.BP_AP_Manhole_C" (Transformation|GetActorTransform _array_element) "Undefined" "MultiplyWithRoot" 0 0))
    (Transformation|AttachActorToActor _returnvalue _array_element "None" "SnapToTarget" "SnapToTarget" "SnapToTarget" true)))

(event Custom|SpawnPlayerAudio
  (bind _outactors (Actor|GetAllActorsOfClass "/Game/Blueprints/Characters/Player/BP_PigeonCharacter_AB.BP_PigeonCharacter_AB_C"))
  (bind _returnvalue (Game|SpawnActorfromClass "/Game/Audio/Audio/Blueprints/Audio_Profiles/BP_AP_Player.BP_AP_Player_C" (Transformation|GetActorTransform (Utilities|Array|Get(acopy) _outactors)) "Undefined" "MultiplyWithRoot" 0 0 0))
  (Transformation|AttachActorToActor _returnvalue (Utilities|Array|Get(acopy) _outactors) "None" "SnapToTarget" "SnapToTarget" "SnapToTarget" true))

(event Custom|AdjustSFXVolume
  (params (NewVolume :type Float%20%28double-precision%29))
  (bind _returnvalue (* NewVolume 4.0))
  ;[1 1 1] Volume Stuff
  (Audio|SetSoundMixClassOverride "/Game/Audio/Audio/Volume/SM_MasterMix.SM_MasterMix" "/Game/Audio/Audio/Volume/SoundClasses/SC_SFX.SC_SFX" _returnvalue 1.0 1.0 true)
  (Variables|Default|SetSFXVolume _returnvalue))

(event Custom|GetSettingsWidget
  (bind _foundwidgets (Widget|GetAllWidgetsOfClass "/Game/Levels/MainMenu/MainMenu/Settings.Settings_C" true))
  (Variables|Default|SetSettings (Utilities|Array|Get(acopy) _foundwidgets)))

(event Custom|ENV%20Objects
  (bind _outactors (Actor|GetAllActorsOfClass "/Game/Art/Props/EnvObjectInteraction/BP_TestEnvObjectBase.BP_TestEnvObjectBase_C"))
  (for _array_element _outactors
    (Game|AddComponentbyClass _array_element "/Game/Audio/Audio/Blueprints/PhysicsCollision_Profiles/PC_AP_Base.PC_AP_Base_C" false (Transformation|GetActorTransform _array_element))))

(event Custom|Trash
  (Utilities|FlowControl|Delay 0.5)
  (bind _outactors (Actor|GetAllActorsOfClass "/Game/Blueprints/Characters/Consumables/BP_Trash_Pick-up.BP_Trash_Pick-up_C"))
  (for _array_element _outactors
    (bind _returnvalue (Game|SpawnActorfromClass "/Game/Audio/Audio/Blueprints/Audio_Profiles/BP_AP_Trash.BP_AP_Trash_C" (Transformation|GetActorTransform _array_element) "AlwaysSpawn" "MultiplyWithRoot" 0 0))
    (Transformation|AttachActorToActor _returnvalue _array_element "None" "SnapToTarget" "SnapToTarget" "SnapToTarget" true)))

(event Custom|GetAllTrees
  (bind _outactors (Actor|GetAllActorsOfClass "/Script/Engine.StaticMeshActor"))
  (for _array_element _outactors
    (if (Actor|ActorHasTag _array_element "Tree")
      (Variables|Default|Setint (+ (Variables|Default|Getint) 1)))))

(event Custom|AdjustMasterVolume
  (params (NewVolume :type Float%20%28double-precision%29))
  (bind _returnvalue (* NewVolume 2.0))
  ;[1 1 1] Volume Stuff
  (Audio|SetSoundMixClassOverride "/Game/Audio/Audio/Volume/SM_MasterMix.SM_MasterMix" "/Game/Audio/Audio/Volume/SoundClasses/SC_Master.SC_Master" _returnvalue 1.0 1.0 true)
  (Variables|Default|SetMasterVolume _returnvalue)
  (Audio|SetSoundMixClassOverride "/Game/Audio/Audio/Volume/SM_MasterMix.SM_MasterMix" "/Game/Audio/Audio/Volume/SoundClasses/SC_SFX.SC_SFX" _returnvalue 1.0 1.0 true)
  (Variables|Default|SetSFXVolume _returnvalue))

(event Custom|AdjustMusicVolume
  (params (NewVolume :type Float%20%28double-precision%29))
  (bind _returnvalue (* NewVolume 4.0))
  ;[1 1 1] Volume Stuff
  (Audio|SetSoundMixClassOverride "/Game/Audio/Audio/Volume/SM_MasterMix.SM_MasterMix" "/Game/Audio/Audio/Volume/SoundClasses/SC_Music.SC_Music" _returnvalue 1.0 1.0 true)
  (Variables|Default|SetMusicVolume _returnvalue))

(event EventBeginPlay
  (bind _output_get (Variables|Default|SetMasterVolume 0.5))
  (Audio|SetSoundMixClassOverride "/Game/Audio/Audio/Volume/SM_MasterMix.SM_MasterMix" "/Game/Audio/Audio/Volume/SoundClasses/SC_Master.SC_Master" (* _output_get 2.0) 1.0 1.0 true)
  (Utilities|FlowControl|Delay 0.1)
  (Audio|Components|Audio|Play (Variables|Default|GetMS_Ambience) 0.0)
  (Audio|Components|Audio|Play (Variables|Default|GetMS_WorldMusic) 0.0)
  (CallFunction|Trash)
  (CallFunction|ENVObjects)
  (CallFunction|GetSettingsWidget)
  (CallFunction|SpawnManholeAudioProfile))

(fn ConstructionScript)