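; Base interactable wearable that the pigeon character puts on its head as a stealth disguise.
; Overlapping its box briefly shows a pickup prompt.
; Pickup attaches the mesh to the head socket, sets crouch and hiding states, resizes the stealth radius, raises stealth, slows walking and shows post-processing.
; RemoveItem reverts those player changes, then destroys and respawns the item above the player with a physics pop, feathers and dust.
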(event OnComponentBeginOverlap(Box)
  (params (OverlappedComponent :type Primitive%20Component%20Object%20Reference) (OtherActor :type Actor%20Object%20Reference) (OtherComp :type Primitive%20Component%20Object%20Reference) (OtherBodyIndex :type Integer) (bFromSweep :type Boolean) (SweepResult :type Hit%20Result%20Structure%20%28by%20ref%29))
  ;[1 1 1] Attach Item
  (bind _asbp_pigeon_character_ab (Utilities|Casting|CastToBP_PigeonCharacter_AB OtherActor))
  (Variables|Default|SetAs%20BP%20Pigeon%20Character%20AB _asbp_pigeon_character_ab)
  (bind _returnvalue (UserInterface|CreateWidget "/Game/Art/Props/EnvObjectInteraction/Wearables/WBP_PickupPrompt.WBP_PickupPrompt_C"))
  (UserInterface|Viewport|AddtoViewport _returnvalue 0)
  (Utilities|FlowControl|Delay 2.0)
  (Widget|RemovefromParent _returnvalue))

(event OnComponentEndOverlap(Box)
  (params (OverlappedComponent :type Primitive%20Component%20Object%20Reference) (OtherActor :type Actor%20Object%20Reference) (OtherComp :type Primitive%20Component%20Object%20Reference) (OtherBodyIndex :type Integer))
  (bind _asbp_pigeon_character_ab (Utilities|Casting|CastToBP_PigeonCharacter_AB OtherActor))
  (Variables|/Game/Blueprints/Characters/Player/BP_PigeonCharacter_AB.BP_PigeonCharacter_AB_C|SetisCrouching _asbp_pigeon_character_ab false))

(event Custom|CallVFX
  (bind _returnvalue (Transformation|GetActorLocation))
  (Niagara|SpawnSystematLocation "/Game/Art/VFX/Player/FeatherPoof/VFX_Feathers.VFX_Feathers" _returnvalue "0, 0, 0" "3.000000,3.000000,3.000000" true true "None" false)
  (Niagara|SpawnSystematLocation "/Game/DevTestMaps/Personal-Folders/Armaan/NS_FootStepDust.NS_FootStepDust" _returnvalue "0, 0, 0" "3.000000,3.000000,3.000000" true true "None" false))

(event Custom|RemoveItem
  (params (Actor :type BP%20Interactable%20Item%20Base%20Object%20Reference))
  (bind _as_bp_pigeon_character_ab (Variables|Default|GetAs%20BP%20Pigeon%20Character%20AB))
  (bind _returnvalue (Transformation|GetActorTransform _as_bp_pigeon_character_ab))
  ;[1 1 1] Detach Item
  (Variables|/Game/Blueprints/Characters/Player/BP_PigeonCharacter_AB.BP_PigeonCharacter_AB_C|SetisEnvHiding _as_bp_pigeon_character_ab false)
  (Actor|DestroyActor Actor)
  (Variables|Default|SetisHiding false)
  (Variables|/Game/Blueprints/Characters/Player/BP_PigeonCharacter_AB.BP_PigeonCharacter_AB_C|SetbaseStealthStat _as_bp_pigeon_character_ab (- (Variables|/Game/Blueprints/Characters/Player/BP_PigeonCharacter_AB.BP_PigeonCharacter_AB_C|GetbaseStealthStat _as_bp_pigeon_character_ab) 1e+01))
  (Variables|/Script/Engine.CharacterMovementComponent|SetMaxWalkSpeed (Variables|/Script/Engine.Character|GetCharacterMovement _as_bp_pigeon_character_ab) (Variables|/Game/Blueprints/Characters/Player/BP_PigeonCharacter_AB.BP_PigeonCharacter_AB_C|GetWalkSpeed _as_bp_pigeon_character_ab))
  (Variables|/Game/Blueprints/Characters/Player/BP_PigeonCharacter_AB.BP_PigeonCharacter_AB_C|SetisCrouching _as_bp_pigeon_character_ab false)
  (Default|ResizeRadius (Variables|/Game/Blueprints/Characters/Player/BP_PigeonCharacter_AB.BP_PigeonCharacter_AB_C|GetAC_StealthUser _as_bp_pigeon_character_ab) (Variables|/Game/Blueprints/Characters/Player/BP_PigeonCharacter_AB.BP_PigeonCharacter_AB_C|GetWalkingStealthRadius _as_bp_pigeon_character_ab))
  (Audio|PlaySound2D "/Game/Blueprints/GameplaySystems/Dialogue/NarrativeAudioModulator/pop-268648.pop-268648" 1.0 1.0 0.0 0 0)
  (Rendering|SetVisibility (Variables|/Game/Blueprints/Characters/Player/BP_PigeonCharacter_AB.BP_PigeonCharacter_AB_C|GetPostProcess _as_bp_pigeon_character_ab) false false)
  (bind _returnvalue_2 (Game|SpawnActorfromClass (Utilities|GetClass Actor) (Math|Transform|MakeTransform (+ (.location _returnvalue) "0.000000,0.000000,55.000000") (.rotation _returnvalue) (.scale _returnvalue)) "Undefined" "MultiplyWithRoot" Actor 0))
  (CallFunction|CallVFX _returnvalue_2)
  (Physics|SetSimulatePhysics (Variables|BP_InteractableItemBase_C|GetCube _returnvalue_2) true)
  (Class|PrimitiveComponent|AddForceatLocation (Variables|BP_InteractableItemBase_C|GetCube _returnvalue_2) "0.000000,0.000000,20000.000000" "0.000000,0.000000,-10.000000" "None")
  (Utilities|FlowControl|Delay 3.0)
  (Physics|SetSimulatePhysics (Variables|BP_InteractableItemBase_C|GetCube _returnvalue_2) false))

(event EventBeginPlay
  (bind _asbp_pigeon_character_ab (Utilities|Casting|CastToBP_PigeonCharacter_AB (Game|GetPlayerCharacter 0)))
  (Variables|Default|SetAs%20BP%20Pigeon%20Character%20AB _asbp_pigeon_character_ab))

(event EventTick
  (params (DeltaSeconds :type Float%20%28single-precision%29))
  (Variables|Default|SetOrigTransform (Transformation|GetActorTransform)))

(event EventPickup
  (bind _returnvalue (Transformation|GetActorLocation))
  (bind _returnvalue_2 (Transformation|GetActorRotation))
  (bind _returnvalue_3 (Transformation|GetActorLocation))
  (bind _returnvalue_4 (Game|GetPlayerCharacter 0))
  (bind _returnvalue_5 (Transformation|GetActorLocation))
  (bind _returnvalue_6 (Transformation|GetActorRotation))
  (bind _as_bp_pigeon_character_ab (Variables|Default|GetAs%20BP%20Pigeon%20Character%20AB))
  (bind _as_bp_pigeon_character_ab_2 (Variables|Default|GetAs%20BP%20Pigeon%20Character%20AB))
  (bind _returnvalue_7 (Transformation|GetActorLocation _returnvalue_4))
  (bind _charactermovement (Variables|/Script/Engine.Character|GetCharacterMovement _as_bp_pigeon_character_ab_2))
  (bind _returnvalue_8 (Math|Rotator|FindLookatRotation _returnvalue_3 _returnvalue_7))
  ;[1 1 1] Comment
  (Variables|/Game/Blueprints/Characters/Player/BP_PigeonCharacter_AB.BP_PigeonCharacter_AB_C|SetisCrouching _as_bp_pigeon_character_ab true)
  (Variables|/Game/Blueprints/Characters/Player/BP_PigeonCharacter_AB.BP_PigeonCharacter_AB_C|SetisEnvHiding _as_bp_pigeon_character_ab true)
  (Default|ResizeRadius (Variables|/Game/Blueprints/Characters/Player/BP_PigeonCharacter_AB.BP_PigeonCharacter_AB_C|GetAC_StealthUser _as_bp_pigeon_character_ab) (Variables|/Game/Blueprints/Characters/Player/BP_PigeonCharacter_AB.BP_PigeonCharacter_AB_C|GetCrouchingStealthRadius _as_bp_pigeon_character_ab))
  (Rendering|SetVisibility (Variables|/Game/Blueprints/Characters/Player/BP_PigeonCharacter_AB.BP_PigeonCharacter_AB_C|GetPostProcess _as_bp_pigeon_character_ab) true false)
  (Variables|/Game/Blueprints/Characters/Player/BP_PigeonCharacter_AB.BP_PigeonCharacter_AB_C|SetHeldItem _as_bp_pigeon_character_ab self)
  (Variables|Default|SetisHiding true)
  (Transformation|SetActorTransform (Math|Transform|MakeTransform (Math|Vector|MakeVector (.x _returnvalue) (.y _returnvalue) (+ (.z _returnvalue) 15.0)) (Math|Rotator|MakeRotator (.roll _returnvalue_2) (.pitch _returnvalue_2) (.yaw _returnvalue_2)) "1.000000,1.000000,1.000000"))
  (Utilities|FlowControl|Delay 0.5)
  (Transformation|SetActorTransform (Math|Transform|MakeTransform (Math|Vector|MakeVector (.x _returnvalue_5) (.y _returnvalue_5) (+ (.z _returnvalue_5) 13.0)) (Math|Rotator|MakeRotator (- (.roll _returnvalue_6) 1e+01) (.pitch _returnvalue_6) (.yaw _returnvalue_6)) "1.000000,1.000000,1.000000"))
  (Transformation|SetActorRotation (Math|Rotator|MakeRotator (.roll _returnvalue_8) (.pitch (Transformation|GetActorRotation _returnvalue_4)) (.yaw _returnvalue_8)))
  (Collision|SetCollisionEnabled (Variables|Default|GetCube) "NoCollision")
  (Transformation|AttachComponentToComponent (Variables|Default|GetStaticMesh) (Variables|/Script/Engine.Character|GetMesh _as_bp_pigeon_character_ab_2) "Center_HeadTip_JNT" "KeepRelative" "KeepWorld" "KeepWorld" false)
  (Variables|/Game/Blueprints/Characters/Player/BP_PigeonCharacter_AB.BP_PigeonCharacter_AB_C|SetbaseStealthStat _as_bp_pigeon_character_ab_2 (+ (Variables|/Game/Blueprints/Characters/Player/BP_PigeonCharacter_AB.BP_PigeonCharacter_AB_C|GetbaseStealthStat _as_bp_pigeon_character_ab_2) 1e+01))
  (Variables|/Script/Engine.CharacterMovementComponent|SetMaxWalkSpeed _charactermovement (/ (Variables|/Script/Engine.CharacterMovementComponent|GetMaxWalkSpeed _charactermovement) (Variables|Default|GetSpeedModifier)))
  (Audio|PlaySound2D "/Game/Blueprints/GameplaySystems/Dialogue/NarrativeAudioModulator/pop-268648.pop-268648" 1.0 1.0 0.0 0 0))

(fn ConstructionScript)