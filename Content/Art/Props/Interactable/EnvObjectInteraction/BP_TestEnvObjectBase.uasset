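; Test base actor for an interactable environment prop that can be disposed of in a BP_Trash_Pick-up.
; Cube hits emit short-range noise instigated by the player pawn, using the normal impulse vector as the noise location.
; On overlapping the trash actor, it passes its class as ItemClass and prints it.
; If inside GarbageHole, it plays a flap sound, deactivates GarbageSpawnPoint, spawns scaled BP_GarbageSpawn there and destroys itself.
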(event OnComponentHit(Cube)
  (params (HitComponent :type Primitive%20Component%20Object%20Reference) (OtherActor :type Actor%20Object%20Reference) (OtherComp :type Primitive%20Component%20Object%20Reference) (NormalImpulse :type Vector :default "0, 0, 0") (Hit :type Hit%20Result%20Structure%20%28by%20ref%29))
  (Class|Actor|MakeNoise 1.0 (Game|Player|GetPlayerPawn 0) NormalImpulse 1e+01 "None"))

(event OnComponentBeginOverlap(Cube)
  (params (OverlappedComponent :type Primitive%20Component%20Object%20Reference) (OtherActor :type Actor%20Object%20Reference) (OtherComp :type Primitive%20Component%20Object%20Reference) (OtherBodyIndex :type Integer) (bFromSweep :type Boolean) (SweepResult :type Hit%20Result%20Structure%20%28by%20ref%29))
  (bind _asbp_trash_pick_up (Utilities|Casting|CastToBP_Trash_Pick-up OtherActor))
  (bind _output_get (Variables|/Game/Blueprints/Characters/Consumables/BP_Trash_Pick-up.BP_Trash_Pick-up_C|SetItemClass _asbp_trash_pick_up (Utilities|GetClass self)))
  (Development|PrintString (Utilities|GetClassDisplayName _output_get))
  (if (Class|PrimitiveComponent|IsOverlappingComponent (Variables|Default|GetCube) (Variables|/Game/Blueprints/Characters/Consumables/BP_Trash_Pick-up.BP_Trash_Pick-up_C|GetGarbageHole _asbp_trash_pick_up))
    (Audio|PlaySound2D "/Game/Audio/Audio/SFX/Waves/Player/Flaps/Flap2.Flap2" 1.0 1.0 0.0 0 0)
    (Components|Activation|Deactivate (Variables|/Game/Blueprints/Characters/Consumables/BP_Trash_Pick-up.BP_Trash_Pick-up_C|GetGarbageSpawnPoint _asbp_trash_pick_up))
    (Game|SpawnActorfromClass "/Game/Art/Props/Interactable/EnvObjectInteraction/BP_GarbageSpawn.BP_GarbageSpawn_C" (Math|Transform|MakeTransform (.location (Transformation|GetSocketTransform (Variables|/Game/Blueprints/Characters/Consumables/BP_Trash_Pick-up.BP_Trash_Pick-up_C|GetGarbageSpawnPoint _asbp_trash_pick_up) "None" "RTS_World")) (.rotation (Transformation|GetSocketTransform (Variables|/Game/Blueprints/Characters/Consumables/BP_Trash_Pick-up.BP_Trash_Pick-up_C|GetGarbageSpawnPoint _asbp_trash_pick_up) "None" "RTS_World")) "2.000000,2.000000,2.000000") "AlwaysSpawn" "MultiplyWithRoot" 0 0)
    (Actor|DestroyActor)))

(event EventBeginPlay)

(event Collision|EventActorBeginOverlap
  (params (OtherActor :type Actor%20Object%20Reference)))

(event EventTick
  (params (DeltaSeconds :type Float%20%28single-precision%29)))

(fn ConstructionScript)